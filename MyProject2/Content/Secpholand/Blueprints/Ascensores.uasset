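; Pair of elevators that travel endlessly in opposite directions between zero and a configurable height, Altura.
; On BeginPlay, the Ascensores timeline's play rate is set from SegundosDeViaje, and its track drives both components' relative Z, one mirroring the other.
; A FlipFlop alternates forward and reverse playback, re-triggered after a SegundosEntreViajes pause.
; The construction script places Ascensor2 at the top, at a different X offset than the runtime updates use.
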(event EventBeginPlay
  (bind _altura (Variables|Default|GetAltura))
  (Components|Timeline|SetPlayRate (Variables|Default|Getascensores) (/ 1.0 (Variables|Default|GetsegundosDeViaje)))
  (Utilities|FlowControl|FlipFlop :!label _label
    (:A
      (bind _newtrack_0 (Timeline|ascensores PlayFromStart)
        (:Update
          (Transformation|SetRelativeLocation (Variables|Default|Getascensor1) (Math|Vector|MakeVector -1e+02 0.0 (* _newtrack_0 _altura)) false false)
          (Transformation|SetRelativeLocation (Variables|Default|Getascensor2) (Math|Vector|MakeVector 1e+02 0.0 (- _altura (* _newtrack_0 _altura))) false false))
        (:Finished
          (Utilities|FlowControl|Delay (Variables|Default|GetsegundosEntreViajes))
          (goto _label))))
    (:B
      (Timeline|ascensores ReverseFromEnd))))

(fn ConstructionScript
  (Transformation|SetRelativeLocation (Variables|Default|Getascensor2) (Math|Vector|MakeVector 1.6e+02 0.0 (Variables|Default|GetAltura)) false false))