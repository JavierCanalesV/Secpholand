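; Vehicle manager that sends Vehiculo actors on their runs one at a time, cycling through the Vehicles array.
; The array is optionally filled from all Vehiculo actors at BeginPlay.
; RunNextVehicle resets the current vehicle's Alfa, advances the wrapping index, waits a random delay, then sets the next vehicle's Go flag.
; Tick polls that flag and starts the next cycle once it clears.
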(event Custom|RunNextVehicle
  (Variables|Default|SetvehicleRunning false)
  (Variables|/Game/Secpholand/Blueprints/Vehiculo.Vehiculo_C|Setalfa (Utilities|Array|Get(acopy) (Variables|Default|Getvehicles) (Variables|Default|Geti)) 0.0)
  (bind _result (Math|Integer|IncrementInt (Variables|Default|Geti))
    (:%20%20
      (if (>= _result (Utilities|Array|Length (Variables|Default|Getvehicles)))
        (Variables|Default|Seti 0))
      (Utilities|FlowControl|Delay (Math|Random|RandomFloatinRange 8.0 2e+01))
      (Variables|/Game/Secpholand/Blueprints/Vehiculo.Vehiculo_C|Setgo (Utilities|Array|Get(acopy) (Variables|Default|Getvehicles) (Variables|Default|Geti)) true)
      (Variables|Default|SetvehicleRunning true))))

(event EventBeginPlay
  (if (Variables|Default|GetgetAllActors)
    (bind _outactors (Actor|GetAllActorsOfClass "/Game/Secpholand/Blueprints/Vehiculo.Vehiculo_C"))
    (Variables|Default|Setvehicles _outactors))
  (CallFunction|RunNextVehicle))

(event EventTick
  (params (DeltaSeconds :type Float%20%28single-precision%29))
  (if (Variables|Default|GetvehicleRunning)
    (if (not (Variables|/Game/Secpholand/Blueprints/Vehiculo.Vehiculo_C|Getgo (Utilities|Array|Get(acopy) (Variables|Default|Getvehicles) (Variables|Default|Geti))))
      (CallFunction|RunNextVehicle))))

(fn ConstructionScript)