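; Clickable arrow actor that switches the camera view in the investment forum (Foro Inversion).
; Its Action selects left, right or return-to-original, which a click forwards to the ForoInversionController.
; A click also hides the arrow and its paired arrow, then after a one-second delay reveals the opposite set from OtherFlechas: return after left/right, left/right after return.
; Return arrows start with collision disabled.
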(event Custom|handleCamerasVisibles
  (bind _otherflechatohide (Variables|Default|GetotherFlechaToHide))
  (bind _action (Variables|Default|Getaction))
  (Rendering|SetActorHiddenInGame true)
  (Collision|SetActorEnableCollision false)
  (Utilities|IsValid _otherflechatohide
    (:Is%20Valid
      (Rendering|SetActorHiddenInGame _otherflechatohide true)
      (Collision|SetActorEnableCollision _otherflechatohide false))
    (:Is%20Not%20Valid
      _))
  (Utilities|FlowControl|Delay 1.0)
  (for _array_element (Variables|Default|GetotherFlechas)
    (if (or (== _action 0) (== _action 1))
      (if (== (Variables|CambiarCamaraForoInversion_C|Getaction _array_element) 2)
        (Rendering|SetActorHiddenInGame _array_element false)
        (Collision|SetActorEnableCollision _array_element true))
      (elif (or (== (Variables|CambiarCamaraForoInversion_C|Getaction _array_element) 1) (== (Variables|CambiarCamaraForoInversion_C|Getaction _array_element) 0))
        (Rendering|SetActorHiddenInGame _array_element false)
        (Collision|SetActorEnableCollision _array_element true)))))

(event EventBeginPlay
  (if (== (Variables|Default|Getaction) 2)
    (Collision|SetActorEnableCollision false)))

(event EventClick
  (params (controller :type Client%20Side%20Controller%20Object%20Reference))
  (|CallParentFunction controller)
  (CallFunction|HandleCamerasVisibles)
  (bind _asforo_inversion_controller (Utilities|Casting|CastToForoInversionController controller))
  (switch int (Variables|Default|Getaction)
    (:Default
      (Default|GotoLeftView _asforo_inversion_controller :!label _label))
    (:0
      (goto _label))
    (:1
      (Default|GotoRightView _asforo_inversion_controller))
    (:2
      (Default|ReturntoOriginalView _asforo_inversion_controller))))

(fn ConstructionScript
  (|CallParentFunction))