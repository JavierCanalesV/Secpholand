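; AscensorB2B is a clickable elevator that teleports the local player behind a camera fade.
; Clicks from a MenuLobbyController trigger Arrived immediately, while other controllers defer to the parent Click.
; Arrived fades out player 0's ClientSide_Controller camera, then teleports and rotates the player through that controller before fading back in.
; The destination is LocationTeleport, converted from actor-relative to world space.
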(event EventArrived
  (bind _returnvalue (Transformation|GetActorTransform))
  (bind _locationteleport (Variables|Default|GetlocationTeleport))
  (bind (_location _rotation) (Math|Transform|BreakTransform _locationteleport))
  (bind _asclient_side_controller (Utilities|Casting|CastToClientSide_Controller (Game|GetPlayerController 0)))
  (CameraFades|StartCameraFade :self (Variables|/Script/Engine.PlayerController|GetPlayerCameraManager _asclient_side_controller) :ToAlpha 1.0 :Duration 0.6 :bHoldWhenFinished true)
  (Utilities|FlowControl|Delay 0.6)
  (Default|TeleportPlayer:Client _asclient_side_controller (Math|Transform|TransformLocation _returnvalue _location))
  (Default|RotatePlayer:Client _asclient_side_controller (Math|Transform|TransformRotation _returnvalue _rotation))
  (CameraFades|StartCameraFade :self (Variables|/Script/Engine.PlayerController|GetPlayerCameraManager _asclient_side_controller) :FromAlpha 1.0 :ToAlpha 0.0 :Duration 0.6 :bHoldWhenFinished true))

(event Collision|EventActorBeginOverlap
  (params (OtherActor :type Actor%20Object%20Reference)))

(event EventClick
  (params (controller :type Client%20Side%20Controller%20Object%20Reference))
  (Utilities|Casting|CastToMenuLobbyController controller
    (:then
      (CallFunction|Arrived))
    (:CastFailed
      (|CallParentFunction controller))))

(event EventBeginPlay)

(event EventTick
  (params (DeltaSeconds :type Float%20%28single-precision%29)))

(fn ConstructionScript
  (|CallParentFunction))