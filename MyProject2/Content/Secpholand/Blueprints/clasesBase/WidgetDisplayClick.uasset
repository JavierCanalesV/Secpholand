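; Base class for a clickable mesh object that displays a UI widget when clicked.
; On click it runs the parent handler, then creates a widget of a configurable class and adds it to the viewport.
; If StopClicks is set, it also calls SetControllsConstraints on the clicking controller and ResetClick.
; The construction script runs the parent's, then applies the configured mesh and per-slot materials.
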(event EventClick
  (params (controller :type Client%20Side%20Controller%20Object%20Reference))
  (|CallParentFunction controller)
  (bind _returnvalue (UserInterface|CreateWidget (Variables|Default|GetNewVar_0_0)))
  (UserInterface|Viewport|AddtoViewport _returnvalue 0)
  (if (Variables|Default|GetStopClicks)
    (Default|SetControllsConstraints controller false false false false)
    (CallFunction|ResetClick)))

(fn ConstructionScript
  (|CallParentFunction)
  (Components|StaticMesh|SetStaticMesh (Variables|Default|GetStaticMesh) (Variables|Default|GetMesh))
  (for (_array_element _array_index) (Variables|Default|Getmaterials)
    (Rendering|Material|SetMaterial (Variables|Default|GetStaticMesh) _array_index _array_element)))