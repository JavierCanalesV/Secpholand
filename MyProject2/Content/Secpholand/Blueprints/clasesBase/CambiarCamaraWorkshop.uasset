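; Clickable arrow for the workshop that switches the camera view through the WorkshopController.
; On click it runs the parent Click, updates arrow visibility, then uses Action to choose the left, right or original view.
; An arrow with a valid OtherFlecha reveals that arrow and enables its collision after a short delay.
; An arrow without one starts with collision off, and hides itself and disables collision when clicked.
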(event Custom|handleCamerasVisibles
  (bind _otherflecha (Variables|Default|GetotherFlecha))
  (Utilities|IsValid (Variables|Default|GetotherFlecha)
    (:Is%20Valid
      (Utilities|FlowControl|Delay 1.0)
      (Rendering|SetActorHiddenInGame _otherflecha false)
      (Collision|SetActorEnableCollision _otherflecha true))
    (:Is%20Not%20Valid
      (Rendering|SetActorHiddenInGame true)
      (Collision|SetActorEnableCollision false))))

(event EventBeginPlay
  (Utilities|IsValid (Variables|Default|GetotherFlecha)
    (:Is%20Not%20Valid
      (Collision|SetActorEnableCollision false))))

(event EventClick
  (params (controller :type Client%20Side%20Controller%20Object%20Reference))
  (|CallParentFunction controller)
  (CallFunction|HandleCamerasVisibles)
  (bind _asworkshop_controller (Utilities|Casting|CastToWorkshopController controller))
  (switch int (Variables|Default|Getaction)
    (:Default
      (Default|GotoLeftView _asworkshop_controller :!label _label))
    (:0
      (goto _label))
    (:1
      (Default|GotoRightView _asworkshop_controller))
    (:2
      (Default|ReturntoOriginalView _asworkshop_controller))))

(fn ConstructionScript
  (|CallParentFunction))