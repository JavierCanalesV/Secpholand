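; Base clickable that zooms the player's view onto itself, triggered directly under an InteriorController or through the parent's click and arrival flow otherwise.
; Arrived restricts controls, blends the view with distance-scaled time and sound volume, then shows an exit widget.
; Collision toggles swap which nested clickables respond while zoomed.
; Exiting restores view, controls and HUD; empty FinishedZoomIn/Out events serve as hooks.
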(event Custom|ShowClicables
  ;[1 1 1] Show/unshow clicables
  (Collision|SetActorEnableCollision false)
  (for _array_element (Variables|Default|Getclicables)
    (Collision|SetActorEnableCollision _array_element true))
  (for _array_element_2 (Variables|Default|GetClicablesToHideOnZoom)
    (Collision|SetActorEnableCollision _array_element_2 false)))

(event Custom|UnshowClicables
  ;[1 1 1] Show/unshow clicables
  (Collision|SetActorEnableCollision true)
  (for _array_element (Variables|Default|Getclicables)
    (Collision|SetActorEnableCollision _array_element false))
  (for _array_element_2 (Variables|Default|GetClicablesToHideOnZoom)
    (Collision|SetActorEnableCollision _array_element_2 true)))

(event Custom|SalirModoZoom
  (bind _clientsidepawn (Variables|Default|GetclientsidePawn))
  (bind _clientsidepawn_2 (Variables|Default|GetclientsidePawn))
  (bind _clientsidecontrollerref (Variables|/Game/Secpholand/Blueprints/ControllersYModes/baseClasses/ClientSide_Pawn.ClientSide_Pawn_C|GetClientSideControllerRef _clientsidepawn))
  (bind _clientsidecontrollerref_2 (Variables|/Game/Secpholand/Blueprints/ControllersYModes/baseClasses/ClientSide_Pawn.ClientSide_Pawn_C|GetClientSideControllerRef _clientsidepawn_2))
  ;[1 1 1] Arrive. EVENT ZOOM
  (CallFunction|PlayAirTransitionSound)
  (Default|SetControllsAlowChange _clientsidecontrollerref true true true true)
  (Default|SetControllsConstraints _clientsidecontrollerref true true true true)
  (CallFunction|UnshowClicables)
  (Game|Player|SetViewTargetwithBlend _clientsidecontrollerref_2 (Variables|Default|GetOriginalView) (Variables|Default|GetzoomTime) "VTBlend_Linear" 0.0 true)
  (Utilities|FlowControl|Delay (Variables|Default|GetzoomTime))
  (Variables|/Game/Secpholand/Blueprints/ControllersYModes/baseClasses/ClientSide_Pawn.ClientSide_Pawn_C|SetZoomed (Variables|Default|GetclientsidePawn) false)
  (Widget|SetVisibility (Variables|/Game/Secpholand/UI/Widgets/HUDYChat/HUD.HUD_C|GetHudArribaizquierda (Variables|/Game/Secpholand/Blueprints/ControllersYModes/baseClasses/ClientSide_Controller.ClientSide_Controller_C|GetHUD _clientsidecontrollerref_2)) "SelfHitTestInvisible")
  (CallFunction|FinishedZoomOut)
  (bind _asinterior_controller (Utilities|Casting|CastToInteriorController (Variables|/Game/Secpholand/Blueprints/ControllersYModes/baseClasses/ClientSide_Pawn.ClientSide_Pawn_C|GetClientSideControllerRef (Variables|Default|GetclientsidePawn))))
  (UserInterface|Viewport|AddtoViewport (Variables|/Game/Secpholand/Blueprints/ControllersYModes/InteriorController.InteriorController_C|GetWidgetSalir _asinterior_controller) 0))

(event Custom|PlayAirTransitionSound
  ;[1 1 1] PlayAirTransition
  (Audio|PlaySound2D "/Game/Secpholand/audio/transition.transition" (Math|Float|Lerp 0.2 0.5 (Math|Float|Clamp(Float) (/ (Math|Vector|Distance(Vector) (Transformation|GetWorldLocation (Variables|/Script/Engine.Actor|GetRootComponent (Pawn|GetViewTarget (Variables|/Game/Secpholand/Blueprints/ControllersYModes/baseClasses/ClientSide_Pawn.ClientSide_Pawn_C|GetClientSideControllerRef (Variables|Default|GetclientsidePawn))))) (Transformation|GetWorldLocation (Variables|Default|GetCamera))) 1.5e+03))) 1.0 0.0 0 0))

(event Custom|SetZoomTimeByDistance
  ;[1 1 1] Set traveling time
  (Variables|Default|SetzoomTime (Math|Float|Lerp 0.7 1.4 (Math|Float|Clamp(Float) (/ (Math|Vector|Distance(Vector) (Transformation|GetWorldLocation (Variables|/Script/Engine.Actor|GetRootComponent (Pawn|GetViewTarget (Variables|/Game/Secpholand/Blueprints/ControllersYModes/baseClasses/ClientSide_Pawn.ClientSide_Pawn_C|GetClientSideControllerRef (Variables|Default|GetclientsidePawn))))) (Transformation|GetWorldLocation (Variables|Default|GetCamera))) 2.5e+03)))))

(event Custom|FinishedZoomOut)

(event Custom|FinishedZoomIn)

(event EventBeginPlay
  (|CallParentFunction)
  (CallFunction|UnshowClicables))

(event EventArrived
  ;[1 1 1] Arrive. EVENT ZOOM
  (bind _asclient_side_pawn (Utilities|Casting|CastToClientSide_Pawn (Game|Player|GetPlayerPawn 0)))
  (Variables|Default|SetclientsidePawn _asclient_side_pawn)
  (CallFunction|PlayAirTransitionSound)
  (CallFunction|ResetClick)
  (Default|StopMovement:Client (Variables|/Game/Secpholand/Blueprints/ControllersYModes/baseClasses/ClientSide_Pawn.ClientSide_Pawn_C|GetClientSideControllerRef (Variables|Default|GetclientsidePawn)))
  (Default|SetControllsConstraints (Variables|/Game/Secpholand/Blueprints/ControllersYModes/baseClasses/ClientSide_Pawn.ClientSide_Pawn_C|GetClientSideControllerRef (Variables|Default|GetclientsidePawn)) false false false true)
  (Default|SetControllsAlowChange (Variables|/Game/Secpholand/Blueprints/ControllersYModes/baseClasses/ClientSide_Pawn.ClientSide_Pawn_C|GetClientSideControllerRef (Variables|Default|GetclientsidePawn)) false false false true)
  (Default|StopOutliningActor (Variables|/Game/Secpholand/Blueprints/ControllersYModes/baseClasses/ClientSide_Pawn.ClientSide_Pawn_C|GetClientSideControllerRef (Variables|Default|GetclientsidePawn)) self)
  (bind _asclient_side_controller (Utilities|Casting|CastToClientSide_Controller (Game|GetPlayerController 0)))
  (Variables|Default|SetOriginalView (Pawn|GetViewTarget _asclient_side_controller))
  (CallFunction|SetZoomTimebyDistance)
  (Game|Player|SetViewTargetwithBlend _asclient_side_controller self (Variables|Default|GetzoomTime) "VTBlend_Linear" 0.0 false)
  (Utilities|FlowControl|Delay (Variables|Default|GetzoomTime))
  (bind _returnvalue (UserInterface|CreateWidget "/Game/Secpholand/UI/Widgets/SalirEdificioZoom.SalirEdificioZoom_C"))
  (EventDispatchers|BindEventtoSalirClicked _returnvalue (delegate Custom|SalirModoZoom))
  (Widget|Panel|AddChild (Variables|/Game/Secpholand/UI/Widgets/HUDYChat/HUD.HUD_C|GetHudAbajoizquierda (Variables|/Game/Secpholand/Blueprints/ControllersYModes/baseClasses/ClientSide_Controller.ClientSide_Controller_C|GetHUD _asclient_side_controller)) _returnvalue)
  (CallFunction|ShowClicables)
  (Variables|/Game/Secpholand/Blueprints/ControllersYModes/baseClasses/ClientSide_Pawn.ClientSide_Pawn_C|SetZoomed (Variables|Default|GetclientsidePawn) true)
  (Widget|SetVisibility (Variables|/Game/Secpholand/UI/Widgets/HUDYChat/HUD.HUD_C|GetHudArribaizquierda (Variables|/Game/Secpholand/Blueprints/ControllersYModes/baseClasses/ClientSide_Controller.ClientSide_Controller_C|GetHUD _asclient_side_controller)) "Hidden")
  (CallFunction|FinishedZoomin)
  (bind _asinterior_controller (Utilities|Casting|CastToInteriorController (Variables|/Game/Secpholand/Blueprints/ControllersYModes/baseClasses/ClientSide_Pawn.ClientSide_Pawn_C|GetClientSideControllerRef (Variables|Default|GetclientsidePawn))))
  (Widget|RemovefromParent (Variables|/Game/Secpholand/Blueprints/ControllersYModes/InteriorController.InteriorController_C|GetWidgetSalir _asinterior_controller)))

(event EventClick
  (params (controller :type Client%20Side%20Controller%20Object%20Reference))
  (Utilities|Casting|CastToInteriorController controller
    (:then
      (CallFunction|Arrived))
    (:CastFailed
      (|CallParentFunction controller))))

(fn ConstructionScript
  (|CallParentFunction))