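; SittingSlot is a seat slot that sits the local player's character when it enters the GotoBox trigger.
; Overlap events maintain the Ocupada (occupied) flag, with a short delayed recount on exit.
; If Active, the local character's entry makes Parent's meshes ignore Visibility traces, then calls SitPlayerClient with the slot's yaw offset by 90 degrees.
; Blocking returns when that character leaves the slot empty; construction positions SittingOverlap from GotoBoxPos.
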(event OnComponentBeginOverlap(gotoBox)
  (params (OverlappedComponent :type Primitive%20Component%20Object%20Reference) (OtherActor :type Actor%20Object%20Reference) (OtherComp :type Primitive%20Component%20Object%20Reference) (OtherBodyIndex :type Integer) (bFromSweep :type Boolean) (SweepResult :type Hit%20Result%20Structure%20%28by%20ref%29))
  (if (== "/Script/Engine.CapsuleComponent" (Utilities|GetClass OtherComp))
    (Variables|Default|Setocupada true)
    (if (Variables|Default|Getactive)
      (bind _asserver_side_character (Utilities|Casting|CastToServerSide_Character OtherActor))
      (bind _asclient_side_controller (Utilities|Casting|CastToClientSide_Controller (Game|GetPlayerController 0)))
      (if (== _asserver_side_character (Variables|/Game/Secpholand/Blueprints/ControllersYModes/ClientSide_Controller.ClientSide_Controller_C|GetServerSideCharacterRef _asclient_side_controller))
        (Collision|SetCollisionResponsetoChannel (Variables|/Game/Secpholand/Blueprints/SillaClickable.SillaClickable_C|Getcylinder (Variables|Default|Getparent)) "ECC_Visibility" "ECR_Ignore")
        (Utilities|FlowControl|Delay 0.5)
        (Default|SitPlayer:Client _asclient_side_controller (Variables|Default|Getrotation))))))

(event OnComponentEndOverlap(gotoBox)
  (params (OverlappedComponent :type Primitive%20Component%20Object%20Reference) (OtherActor :type Actor%20Object%20Reference) (OtherComp :type Primitive%20Component%20Object%20Reference) (OtherBodyIndex :type Integer))
  (bind _asserver_side_character (Utilities|Casting|CastToServerSide_Character OtherActor))
  (Utilities|FlowControl|Delay 0.2)
  (if (> (Utilities|Array|Length (Collision|GetOverlappingActors (Variables|Default|GetgotoBox) "/Game/Secpholand/Blueprints/ControllersYModes/ServerSide_Character.ServerSide_Character_C" :!class /Script/Engine.PrimitiveComponent)) 0)
    (Variables|Default|Setocupada true)
    (else
      (Variables|Default|Setocupada false)
      (bind _asclient_side_controller (Utilities|Casting|CastToClientSide_Controller (Game|GetPlayerController 0)))
      (if (== _asserver_side_character (Variables|/Game/Secpholand/Blueprints/ControllersYModes/ClientSide_Controller.ClientSide_Controller_C|GetServerSideCharacterRef _asclient_side_controller))
        (Collision|SetCollisionResponsetoChannel (Variables|/Game/Secpholand/Blueprints/SillaClickable.SillaClickable_C|Getcylinder (Variables|Default|Getparent)) "ECC_Visibility" "ECR_Block")))))

(event EventBeginPlay
  (Variables|Default|Setrotation (+ (.yaw (Transformation|GetWorldRotation (Variables|Default|GetDefaultSceneRoot))) 9e+01)))

(fn ConstructionScript
  (Transformation|SetRelativeLocation (Variables|Default|GetsittingOverlap) (Variables|Default|GetgotoBoxPos) false false))