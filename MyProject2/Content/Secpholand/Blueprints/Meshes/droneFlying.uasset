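; Ambient drone actor that flies a mesh along the Camino spline in a repeating loop.
; Tick advances a normalized time scaled by Divider, setting the mesh's position and rotation from the spline.
; At the end it waits a random few seconds, then restarts with a randomly chosen individual or family drone mesh.
; A random body-color material setup exists but is disconnected.
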(event Custom|startVehicleWithDelay
  ;[1 1 1] StartVehicles
  (Utilities|FlowControl|Delay (Math|Random|RandomFloatinRange 2.0 12.0))
  (Components|StaticMesh|SetStaticMesh (Variables|Default|GetCar_01) (Utilities|Select :Index (Math|Random|RandomInteger 2) :Option%200 "/Game/Secpholand/Assets/meshes/PropsTransportes/SM_Dron_Individual.SM_Dron_Individual" :Option%201 "/Game/Secpholand/Assets/meshes/PropsTransportes/SM_Dron_Familiar.SM_Dron_Familiar" :Option%202 0))
  (Variables|Default|Setgo1 true)
  (Variables|Default|Setalfa 0.0))

(event Custom|setPosAlfa
  (params (alfa :type Float%20%28single-precision%29))
  (bind _camino (Variables|Default|Getcamino))
  (bind _car_01 (Variables|Default|GetCar_01))
  (bind _returnvalue (Class|SplineComponent|GetRotationatTime _camino alfa "Local" false))
  ;[1 1 1] Tick
  (Transformation|SetWorldLocation _car_01 (Spline|GetLocationatTime _camino alfa "World" false) false false)
  (Transformation|SetRelativeRotation _car_01 (Math|Rotator|MakeRotator (.roll _returnvalue) (.pitch _returnvalue) (.yaw _returnvalue)) false false))

(event Custom|StartVehicles
  ;[1 1 1] StartVehicles
  (Components|StaticMesh|SetStaticMesh (Variables|Default|GetCar_01) (Utilities|Select :Index (Math|Random|RandomInteger 2) :Option%200 "/Game/Secpholand/Assets/meshes/PropsTransportes/SM_Dron_Individual.SM_Dron_Individual" :Option%201 "/Game/Secpholand/Assets/meshes/PropsTransportes/SM_Dron_Familiar.SM_Dron_Familiar" :Option%202 0))
  (Variables|Default|Setgo1 true)
  (Variables|Default|Setalfa 0.0))

(event EventBeginPlay
  (CallFunction|StartVehicles))

(event EventTick
  (params (DeltaSeconds :type Float%20%28single-precision%29))
  ;[1 1 1] Tick
  (if (Variables|Default|Getgo1)
    (if (< (Variables|Default|Getalfa) 1.0)
      (bind _output_get (Variables|Default|Setalfa (+ (Variables|Default|Getalfa) (/ DeltaSeconds (Variables|Default|Getdivider)))))
      (CallFunction|SetPosAlfa _output_get)
      (else
        (CallFunction|StartVehiclewithDelay)
        (Variables|Default|Setgo1 false)))))

(fn ConstructionScript)

(fn GetXLength
  (params (Mesured%20mesh :type Static%20Mesh%20Object%20Reference))
  (return (* (.X (Math|Vector|BreakVector (.Max (Utilities|Struct|BreakBox (StaticMesh|GetBoundingBox Mesured%20mesh))))) 2.0)))