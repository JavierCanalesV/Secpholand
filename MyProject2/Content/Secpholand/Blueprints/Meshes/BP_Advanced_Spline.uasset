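; Spline road actor that tiles a mesh along Camino and runs simple two-way traffic on it.
; The construction script spawns collision-free spline meshes, stretching tile spacing to fit the spline length.
; ActivateTrafic toggles Tick and, when enabling, launches two cars after random delays.
; Tick moves them in opposite directions at fixed world-Y offsets, restarting each after a random delay with a randomly selected mesh, currently always a cube.
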(event Custom|startVehicleWithDelay
  ;[1 1 1] StartVehicles
  (Utilities|FlowControl|Delay (Math|Random|RandomFloatinRange 2.0 12.0))
  (Components|StaticMesh|SetStaticMesh (Variables|Default|GetCar_01) (Utilities|Select :Index (Math|Random|RandomInteger 3) :Option%200 "/Game/StarterContent/Geometry/Meshes/1M_Cube.1M_Cube" :Option%201 "/Game/StarterContent/Geometry/Meshes/1M_Cube.1M_Cube" :Option%202 "/Game/StarterContent/Geometry/Meshes/1M_Cube.1M_Cube"))
  (Variables|Default|Setgo1 true)
  (Variables|Default|Setalfa 0.0))

(event Custom|SetPosAlfa2
  (params (alfa :type Float%20%28single-precision%29))
  (bind _returnvalue (- 1.0 alfa))
  (bind _camino (Variables|Default|Getcamino))
  ;[1 1 1] Tick
  (Transformation|SetWorldLocationAndRotation (Variables|Default|Getcar_02) (+ (Spline|GetLocationatTime _camino _returnvalue "World" false) "0,-275.000000,65.000000") (Class|SplineComponent|GetRotationatTime _camino _returnvalue "World" false) false false))

(event Custom|setPosAlfa
  (params (alfa :type Float%20%28single-precision%29))
  (bind _camino (Variables|Default|Getcamino))
  ;[1 1 1] Tick
  (Transformation|SetWorldLocationAndRotation (Variables|Default|GetCar_01) (+ (Spline|GetLocationatTime _camino alfa "World" false) "0,275.000000,65.000000") (Class|SplineComponent|GetRotationatTime _camino alfa "World" false) false false))

(event Custom|startVehicle2WithDelay
  ;[1 1 1] StartVehicles
  (Utilities|FlowControl|Delay (Math|Random|RandomFloatinRange 2.0 5.0))
  (Components|StaticMesh|SetStaticMesh (Variables|Default|Getcar_02) (Utilities|Select :Index (Math|Random|RandomInteger 3) :Option%200 "/Game/StarterContent/Geometry/Meshes/1M_Cube.1M_Cube" :Option%201 "/Game/StarterContent/Geometry/Meshes/1M_Cube.1M_Cube" :Option%202 "/Game/StarterContent/Geometry/Meshes/1M_Cube.1M_Cube"))
  (Variables|Default|Setgo2 true)
  (Variables|Default|Setalfa2 0.0))

(event Custom|ActivateTrafic
  (params (activate :type Boolean))
  ;[1 1 1] ActivateTrafic
  (Actor|Tick|SetActorTickEnabled activate)
  (if activate
    (CallFunction|StartVehicles)))

(event Custom|StartVehicles
  (bind _returnvalue (Math|Random|RandomInteger 2))
  (bind _returnvalue_2 (== _returnvalue 1))
  ;[1 1 1] StartVehicles
  (Utilities|FlowControl|Sequence
    (:then_0
      (Utilities|FlowControl|Delay (select _returnvalue_2 0.0 (Math|Random|RandomFloatinRange 2.0 5.0)))
      (Components|StaticMesh|SetStaticMesh (Variables|Default|GetCar_01) (Utilities|Select :Index (Math|Random|RandomInteger 3) :Option%200 "/Game/StarterContent/Geometry/Meshes/1M_Cube.1M_Cube" :Option%201 "/Game/StarterContent/Geometry/Meshes/1M_Cube.1M_Cube" :Option%202 "/Game/StarterContent/Geometry/Meshes/1M_Cube.1M_Cube"))
      (Variables|Default|Setgo1 true)
      (Variables|Default|Setalfa 0.0))
    (:then_1
      (Utilities|FlowControl|Delay (select _returnvalue_2 (Math|Random|RandomFloatinRange 2.0 5.0) 0.0))
      (Components|StaticMesh|SetStaticMesh (Variables|Default|Getcar_02) (Utilities|Select :Index (Math|Random|RandomInteger 3) :Option%200 "/Game/StarterContent/Geometry/Meshes/1M_Cube.1M_Cube" :Option%201 "/Game/StarterContent/Geometry/Meshes/1M_Cube.1M_Cube" :Option%202 "/Game/StarterContent/Geometry/Meshes/1M_Cube.1M_Cube"))
      (Variables|Default|Setgo2 true)
      (Variables|Default|Setalfa2 0.0))))

(event EventTick
  (params (DeltaSeconds :type Float%20%28single-precision%29))
  ;[1 1 1] Tick
  (Utilities|FlowControl|Sequence
    (:then_0
      (if (Variables|Default|Getgo1)
        (if (< (Variables|Default|Getalfa) 1.0)
          (bind _output_get (Variables|Default|Setalfa (+ (Variables|Default|Getalfa) (/ DeltaSeconds (Variables|Default|Getdivider)))))
          (CallFunction|SetPosAlfa _output_get)
          (else
            (CallFunction|StartVehiclewithDelay)
            (Variables|Default|Setgo1 false)))))
    (:then_1
      (if (Variables|Default|Getgo2)
        (if (< (Variables|Default|Getalfa2) 1.0)
          (bind _output_get_2 (Variables|Default|Setalfa2 (+ (Variables|Default|Getalfa2) (/ DeltaSeconds (Variables|Default|Getdivider)))))
          (CallFunction|SetPosAlfa2 _output_get_2)
          (else
            (CallFunction|StartVehicle2withDelay)
            (Variables|Default|Setgo2 false)))))))

(fn ConstructionScript
  (bind _camino (Variables|Default|Getcamino))
  (bind _camino_2 (Variables|Default|Getcamino))
  (bind _returnvalue (Spline|GetSplineLength _camino))
  (Utilities|FlowControl|Sequence
    (:then_0
      ;[1 1 1] Get Mesh X distance before scaling
      (bind _x (CallFunction|GetXLength (Variables|Default|GetTiling%20mesh)))
      (bind _output_get (LocalVariables|SetTile%20Amount (Math|Float|Truncate (/ _returnvalue _x))))
      (LocalVariables|SetRelative%20Scale (/ (- _returnvalue (* (Math|Float|Truncate (/ _returnvalue _x)) _x)) (Math|Conversions|ToFloat(Integer) (Math|Float|Truncate (/ _returnvalue _x)))))
      (Variables|Default|SetTemp _output_get))
    (:then_1
      ;[1 1 1] Get mesh length only calculate once
      (bind _x_2 (CallFunction|GetXLength (Variables|Default|GetTiling%20mesh)))
      (LocalVariables|SetTile%20Distance (+ _x_2 (LocalVariables|GetRelative%20Scale))))
    (:then_2
      (for _index (range 0 (- (LocalVariables|GetTile%20Amount) -1))
        (bind _returnvalue_2 (AddComponent|AddSplineMeshComponent false))
        (Components|StaticMesh|SetStaticMesh _returnvalue_2 (Variables|Default|GetTiling%20mesh))
        (SplineMesh|SetStartandEnd _returnvalue_2 (Spline|GetLocationatDistanceAlongSpline _camino_2 (* _index (LocalVariables|GetTile%20Distance)) "Local") (* (Math|Vector|Normalize (Spline|GetTangentatDistanceAlongSpline _camino_2 (* _index (LocalVariables|GetTile%20Distance)) "Local")) (LocalVariables|GetTile%20Distance)) (Spline|GetLocationatDistanceAlongSpline _camino_2 (* (+ _index 1) (LocalVariables|GetTile%20Distance)) "Local") (* (Math|Vector|Normalize (Spline|GetTangentatDistanceAlongSpline _camino_2 (* (+ _index 1) (LocalVariables|GetTile%20Distance)) "Local")) (LocalVariables|GetTile%20Distance)) true :!class /Script/Engine.SplineMeshComponent)
        (Collision|SetCollisionEnabled _returnvalue_2 "NoCollision")
        (Transformation|SetMobility (Variables|Default|Getcamino) "Static")))))

(fn GetXLength
  (params (Mesured%20mesh :type Static%20Mesh%20Object%20Reference))
  (return (* (.X (Math|Vector|BreakVector (.Max (Utilities|Struct|BreakBox (StaticMesh|GetBoundingBox Mesured%20mesh))))) 2.0)))