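; Clickable seating object for a meeting table that sends the clicking player to a free seat slot.
; A click picks the first unoccupied slot, spawns a decal, moves the player there and marks it active, or shows a blocked hover message when full.
; In bird's-eye view, it instead turns the camera toward the mesh, triggers the minimap's street view and waits a distance-scaled delay before the move step, skipping the slot search.
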(event EventClick
  (params (controller :type Client%20Side%20Controller%20Object%20Reference))
  (bind _staticmesh (Variables|Default|GetStaticMesh))
  (bind _clientsidepawnref (Variables|/Game/Secpholand/Blueprints/ControllersYModes/ClientSide_Controller.ClientSide_Controller_C|GetClientSidePawnRef controller))
  (bind _hoveruserwidget (Variables|Default|GethoverUserWidget))
  (bind _clientsidepawnref_2 (Variables|/Game/Secpholand/Blueprints/ControllersYModes/ClientSide_Controller.ClientSide_Controller_C|GetClientSidePawnRef controller))
  (bind _returnvalue (Transformation|GetWorldLocation _staticmesh))
  (bind _returnvalue_2 (Transformation|GetActorLocation _clientsidepawnref_2))
  (bind _springarm (Variables|/Game/Secpholand/Blueprints/ControllersYModes/ClientSide_Pawn.ClientSide_Pawn_C|GetSpringArm _clientsidepawnref_2))
  (|CallParentFunction controller)
  (if (Variables|/Game/Secpholand/Blueprints/ControllersYModes/ClientSide_Pawn.ClientSide_Pawn_C|Getb_VistaPajaro _clientsidepawnref)
    (Transformation|SetWorldRotation _springarm (Math|Rotator|MakeRotator 0.0 (.pitch (Transformation|GetWorldRotation _springarm)) (.yaw (Math|Rotator|FindLookatRotation _returnvalue_2 _returnvalue))) false false)
    (bind _foundwidgets (Widget|GetAllWidgetsOfClass "/Game/Secpholand/UI/Widgets/HUDYChat/Minimapa/MinimapaHUD.MinimapaHUD_C" true))
    (Default|ClicarVistaCalle (Utilities|Array|Get(acopy) _foundwidgets))
    (Utilities|FlowControl|Delay (* (Math|Float|Clamp(Float) (- 1.0 (/ (Math|Vector|Distance(Vector) _returnvalue _returnvalue_2) (* (Class|MovementComponent|GetMaxSpeed (Variables|/Script/Engine.Character|GetCharacterMovement (Variables|/Game/Secpholand/Blueprints/ControllersYModes/ClientSide_Controller.ClientSide_Controller_C|GetServerSideCharacterRef controller))) 2.5)))) 2.5))
    (if (>= (Math|Vector|Distance(Vector) (Transformation|GetActorLocation _clientsidepawnref) (Transformation|GetActorLocation (Utilities|Array|Get(acopy) (Variables|Default|GetSittingSlotsActors) (stale _sittingindex)))) 8e+01) :!label _label
      (Default|SpawnDecalatLocation controller (Transformation|GetActorLocation (Utilities|Array|Get(acopy) (Variables|Default|GetSittingSlotsActors) (stale _sittingindex))))
      (Default|MovetoLocation controller (Transformation|GetActorLocation (Utilities|Array|Get(acopy) (Variables|Default|GetSittingSlotsActors) (stale _sittingindex))))
      (Variables|/Game/Secpholand/Blueprints/SittingSlot.SittingSlot_C|Setactive (Utilities|Array|Get(acopy) (Variables|Default|GetSittingSlotsActors) (Variables|Default|GetcurrentIndex)) true))
    (else
      (bind _sittingindex (CallFunction|GetFreeSlot))
      (bind _output_get (Variables|Default|SetcurrentIndex _sittingindex))
      (if (>= _output_get 0)
        (goto _label)
        (else
          (Audio|PlaySound2D "/Game/Secpholand/audio/UISounds/UI_close.UI_close" 1.0 0.5 0.1 0 0)
          (Default|FillHoverInfo _hoveruserwidget "Mesa de reunión" "No quedan espacios disponibles en la mesa")
          (Default|Blocked _hoveruserwidget))))))

(event EventResetClick
  (bind _currentindex (Variables|Default|GetcurrentIndex))
  (|CallParentFunction)
  (if (>= _currentindex 0)
    (Variables|/Game/Secpholand/Blueprints/SittingSlot.SittingSlot_C|Setactive (Utilities|Array|Get(acopy) (Variables|Default|GetSittingSlotsActors) _currentindex) true)))

(fn ConstructionScript
  (|CallParentFunction)
  (Utilities|Array|Resize (Variables|Default|GetSittingSlotsActors) (Variables|Default|GetsittingSlotsNum)))

(fn GetFreeSlot
  (for (_array_element _array_index) (Variables|Default|GetSittingSlotsActors)
    (if (not (Variables|/Game/Secpholand/Blueprints/SittingSlot.SittingSlot_C|Getocupada _array_element))
      (return _array_index)))
  (return -1))