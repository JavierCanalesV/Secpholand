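; Roaming AI character that wanders the navmesh on its own from the moment it begins play.
; After a short delay, it moves to a random navigable point around its current location and picks a new one whenever the move succeeds or fails, looping indefinitely.
; Disconnected leftover nodes for an authority check, disabling movement component tick and a longer delay never run.
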(event Custom|move
  (Utilities|FlowControl|Delay 1.2)
  (AI|AIMoveTo self (.RandomLocation (Class|NavigationSystemV1|GetRandomPointinNavigableRadius (Transformation|GetActorLocation) 3.5e+03 0 0)) 0 5.0 false :!label _label
    (:OnSuccess
      (goto _label))
    (:OnFail
      (goto _label))))

(event EventBeginPlay
  (|CallParentFunction)
  (CallFunction|Move))

(fn ConstructionScript
  (|CallParentFunction))