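; Player controller for Secpholand interiors such as the Meeting Center, meeting and challenge rooms, using tagged fixed cameras and clickables instead of free movement.
; The server spawns and possesses a separate character and controller, then the client builds HUD, chat and exit widgets.
; Room changes fade between cameras, gate guests from challenge rooms and join meeting calls.
; Client-to-server RPCs forward challenge, super-user moderation and presenter slide actions, checking permissions server-side.
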(event Custom|possesCamera
  (params (CameraTag :type Name))
  (bind _outactors (Actor|GetAllActorswithTag CameraTag))
  (if (> (Utilities|Array|Length _outactors) 0)
    (bind _ascamera_actor (Utilities|Casting|CastToCameraActor (Utilities|Array|Get(acopy) _outactors)))
    (Game|Player|SetViewTargetwithBlend self _ascamera_actor 0.0 "VTBlend_Linear" 0.0 false)
    (else
      (Development|PrintString (Utilities|String|Append "cant find camera: " (Utilities|String|ToString(Name) CameraTag)) true true "(R=0.000000,G=0.660000,B=1.000000,A=1.000000)" 1e+01))))

(event Custom|CreateChatWidget
  (switch Utilities|FlowControl|Switch|SwitchonInGameLocation (.IngameLocation (Utilities|Struct|BreakUserInfo_Public (Variables|Default|GetUserInfo)))
    (:NewEnumerator8
      (bind _returnvalue (UserInterface|CreateWidget "/Game/Secpholand/UI/Widgets/AuditorioChat.AuditorioChat_C"))
      (Class|VerticalBox|AddChildtoVerticalBox (Variables|/Game/Secpholand/UI/Widgets/HUDYChat/HUD.HUD_C|GetHudArribaizquierda (Variables|Default|GetHUD)) _returnvalue))))

(event Custom|ReceiveRetoAvatarsToSit:Client
  (params (AvatarsToSit :type Array%20of%20Avatar%20Structures) (Names :type Array%20of%20Names))
  ;[1 0.533 0.1939] MeetingCenter EP Deprecated
)

(event Custom|ReceiveRetoAvatarsToSit:Server
  (params (AvatarsToSit :type Array%20of%20Avatar%20Structures) (Names :type Array%20of%20Names))
  ;[1 0.533 0.1939] MeetingCenter EP Deprecated
)

(event EventBeginPlay
  (CallFunction|Client:Init)
  (Variables|Default|SetcanRotate? false)
  (Variables|Default|SetcanZoom? false))

(event EventSetControllsConstraints
  (params (CanMove? :type Boolean) (CanRotate? :type Boolean) (CanZoom? :type Boolean) (CanClick? :type Boolean))
  (Variables|Default|SetcanClick? (and CanClick? (Variables|Default|GetcanChangeClick?))))

(event EventTick
  (params (DeltaSeconds :type Float%20%28single-precision%29))
  (CallFunction|LookforClickables))

(event EventSpawnDecal
  (params (Hit :type Hit%20Result%20Structure)))

(event EventSpawnDecalatLocation
  (params (Location :type Vector :default "0, 0, 0")))

(event EventMovetoLocation
  (params (Location :type Vector :default "0, 0, 0")))

(fn ConstructionScript
  (|CallParentFunction))

(event Custom|ReceiveProjectsXenterprise:Client
  (params (List%20Projects :type Array%20of%20Proyecto%20X%20Empresa%20Structures))
  (bind _foundwidgets (Widget|GetAllWidgetsOfClass "/Game/Secpholand/UI/Widgets/HUDYChat/ProyectosDeEmpresa/Proyectos.Proyectos_C" true))
  (if (> (Utilities|Array|Length _foundwidgets) 0)
    (Default|FillPlayers (Utilities|Array|Get(acopy) _foundwidgets) List%20Projects)))

(event Custom|RetrieveProjectsXenterprise
  (CallFunction|RetrieveProjectsXenterprise:Server))

(event Custom|ReceiveProjectsXenterprise:Server
  (params (List%20Projects :type Array%20of%20Proyecto%20X%20Empresa%20Structures))
  (CallFunction|ReceiveProjectsXenterprise:Client List%20Projects))

(event Custom|RetrieveProjectsXenterprise:Server
  (bind _asnetwork_game_state (Utilities|Casting|CastToNetworkGameState (Game|GetGameState)))
  (Default|RetrieveProjectsXenterpriseList:Server _asnetwork_game_state self))

(event Custom|CambiarDeSala
  (params (IDSala :type Integer) (IngameLoc :type InGameLocation%20Enum :default "NewEnumerator12"))
  (bind _widgetsalir (Variables|Default|GetWidgetSalir))
  (Utilities|Struct|SetmembersinUserInfo_Public (Variables|Default|GetUserInfo) IngameLoc)
  (Variables|Default|SetIDSala IDSala)
  (Utilities|IsValid _widgetsalir
    (:Is%20Valid
      (Widget|RemovefromParent _widgetsalir))
    (:Is%20Not%20Valid
      _))
  (CameraFades|StartCameraFade :self (Variables|Default|GetPlayerCameraManager) :ToAlpha 1.0 :Duration 0.6 :bHoldWhenFinished true)
  (Utilities|FlowControl|Delay 0.6)
  (switch Utilities|FlowControl|Switch|SwitchonInGameLocation (.IngameLocation (Utilities|Struct|BreakUserInfo_Public (Variables|Default|GetUserInfo)))
    (:NewEnumerator8
      (bind _nametag (CallFunction|IngameLocationtoCameraTag "NewEnumerator8"))
      (CallFunction|PossesCamera _nametag)
      (CallFunction|ColgarLlamada:Client)
      (CameraFades|StartCameraFade :self (Variables|Default|GetPlayerCameraManager) :FromAlpha 1.0 :Duration 0.6 :bHoldWhenFinished true)
      (Utilities|FlowControl|Delay 0.6)
      (CallFunction|SetControllsConstraints false false false true)
      (CallFunction|AñadirSalirMapaWidget))
    (:NewEnumerator13
      (bind _nametag_2 (CallFunction|IngameLocationtoCameraTag "NewEnumerator13"))
      (bind _outactors (Actor|GetAllActorsOfClass "/Game/Secpholand/Blueprints/Clicables/ZoomClicables/AscensorRetos.AscensorRetos_C"))
      (for _array_element _outactors
        (Default|ResetRoom _array_element))
      (CallFunction|PossesCamera (Utilities|String|StringToName (Utilities|String|Append (Utilities|String|ToString(Name) _nametag_2) (Utilities|String|ToString(Integer) (Variables|Default|GetIDSala)))))
      (CameraFades|StartCameraFade :self (Variables|Default|GetPlayerCameraManager) :FromAlpha 1.0 :Duration 0.6 :bHoldWhenFinished true)
      (Utilities|FlowControl|Delay 0.6)
      (CallFunction|SetControllsConstraints false false false true)
      (CallFunction|AñadirSalirMapaWidget)
      (CallFunction|EntrarEnLlamada (Variables|Default|GetIDSala))
      (bind _returnvalue (UserInterface|CreateWidget "/Game/Secpholand/UI/Widgets/Llamada.Llamada_C"))
      (UserInterface|Viewport|AddtoViewport _returnvalue 0))
    (:NewEnumerator14
      (if (.Invitado (Utilities|Struct|BreakUserInfo_Private (Variables|Default|GetuserInfo_Private)))
        (bind _returnvalue_2 (UserInterface|CreateWidget "/Game/Secpholand/UI/Widgets/UpgradeInvitado.UpgradeInvitado_C"))
        (UserInterface|Viewport|AddtoViewport _returnvalue_2 0)
        (else
          (bind _nametag_3 (CallFunction|IngameLocationtoCameraTag "NewEnumerator14"))
          (bind _outactors_2 (Actor|GetAllActorsOfClass "/Game/Secpholand/Blueprints/Clicables/ZoomClicables/AscensorRetos.AscensorRetos_C"))
          (for _array_element_2 _outactors_2
            (Default|ResetRoom _array_element_2))
          (CallFunction|PossesCamera (Utilities|String|StringToName (Utilities|String|Append (Utilities|String|ToString(Name) _nametag_3) (Utilities|String|ToString(Integer) (Variables|Default|GetIDSala)))))
          (CameraFades|StartCameraFade :self (Variables|Default|GetPlayerCameraManager) :FromAlpha 1.0 :Duration 0.6 :bHoldWhenFinished true)
          (Utilities|FlowControl|Delay 0.6)
          (CallFunction|SetControllsConstraints false false false true)
          (CallFunction|AñadirSalirMapaWidget))))))

(event Custom|AñadirSalirMapaWidget
  (bind _userinfo (Variables|Default|GetUserInfo))
  (bind _ingamelocation (Utilities|Struct|BreakUserInfo_Public _userinfo))
  (bind _returnvalue (UserInterface|CreateWidget "/Game/Secpholand/UI/Widgets/SalirMapa.SalirMapa_C" 0 (Utilities|Select :Index _ingamelocation :NewEnumerator12 "Salir a Secpholand central" :NewEnumerator2 "" :NewEnumerator3 "" :NewEnumerator4 "" :NewEnumerator5 "" :NewEnumerator6 "" :NewEnumerator7 "" :NewEnumerator8 "Salir a Secpholand central" :NewEnumerator9 "Salir a Secpholand central" :NewEnumerator10 "Salir a Secpholand central" :NewEnumerator11 "" :NewEnumerator13 "Volver al hall" :NewEnumerator14 "Volver al hall" :NewEnumerator15 "" :NewEnumerator16 "" :NewEnumerator17 "" :NewEnumerator18 "" :NewEnumerator19 "Volver al hall" :NewEnumerator20 "" :NewEnumerator21 "") (Utilities|Select :Index _ingamelocation :NewEnumerator12 "NewEnumerator0" :NewEnumerator2 "NewEnumerator0" :NewEnumerator3 "NewEnumerator0" :NewEnumerator4 "NewEnumerator0" :NewEnumerator5 "NewEnumerator0" :NewEnumerator6 "NewEnumerator0" :NewEnumerator7 "NewEnumerator0" :NewEnumerator8 "NewEnumerator0" :NewEnumerator9 "NewEnumerator0" :NewEnumerator10 "NewEnumerator0" :NewEnumerator11 "NewEnumerator0" :NewEnumerator13 "NewEnumerator0" :NewEnumerator14 "NewEnumerator0" :NewEnumerator15 "NewEnumerator1" :NewEnumerator16 "NewEnumerator0" :NewEnumerator17 "NewEnumerator0" :NewEnumerator18 "NewEnumerator0" :NewEnumerator19 "NewEnumerator6" :NewEnumerator20 "NewEnumerator0" :NewEnumerator21 "NewEnumerator0")))
  (bind _output_get (Variables|Default|SetWidgetSalir _returnvalue))
  (UserInterface|Viewport|AddtoViewport _output_get 0))

(event Custom|SetCharacter
  (params (ServerSideCharacterRef :type Server%20Side%20Character%20Object%20Reference))
  (bind _output_get (Variables|Default|SetServerSideCharacterRef ServerSideCharacterRef))
  (Development|PrintString (Utilities|GetDisplayName _output_get)))

(event EventServerSpawnPlayer
  (params (playerStartIndex :type Player%20Start%20Object%20Reference) (UserInfo :type User%20Info%20Public%20Structure))
  (bind _clientsidepawnref (Variables|Default|GetClientSidePawnRef))
  (bind _returnvalue (Transformation|GetActorTransform _clientsidepawnref))
  (Networking|SwitchHasAuthority
    (:Authority
      (Utilities|FlowControl|DoOnce false
        (:Completed
          (Transformation|SetActorLocation _clientsidepawnref "-10000.000000,10000.000000,260.000000" false false)
          (bind _returnvalue_2 (Game|SpawnActorfromClass "/Game/Secpholand/Blueprints/ControllersYModes/baseClasses/ServerSide_Character.ServerSide_Character_C" _returnvalue "AlwaysSpawn" 0 UserInfo self 0))
          (bind _output_get (Variables|Default|SetServerSideCharacterRef _returnvalue_2))
          (CallFunction|SetCharacter _output_get)
          (Default|SetName _output_get)
          (bind _asnetwork_player_state (Utilities|Casting|CastToNetworkPlayerState (Variables|Default|GetPlayerState)))
          (Variables|/Game/Secpholand/Blueprints/ControllersYModes/baseClasses/NetworkPlayerState.NetworkPlayerState_C|SetServerSideCharacterRef _asnetwork_player_state (Variables|Default|GetServerSideCharacterRef))
          (bind _returnvalue_3 (Game|SpawnActorfromClass "/Game/Secpholand/Blueprints/ControllersYModes/baseClasses/ServerSide_Controller.ServerSide_Controller_C" _returnvalue "AdjustIfPossibleButAlwaysSpawn" 0 self 0))
          (bind _output_get_2 (Variables|Default|SetServerSideControllerRef _returnvalue_3))
          (Variables|/Game/Secpholand/Blueprints/ControllersYModes/baseClasses/ServerSide_Controller.ServerSide_Controller_C|SetServerSideCharacter _output_get_2 (Variables|Default|GetServerSideCharacterRef))
          (Pawn|Possess (Variables|Default|GetServerSideControllerRef) (Variables|Default|GetServerSideCharacterRef))
          (CallFunction|Server:RetrievePrivateInfo)
          (bind _asnetwork_game_state (Utilities|Casting|CastToNetworkGameState (Game|GetGameState)))
          ;[0 1 1] bypass
          (if (Variables|/Game/Secpholand/Blueprints/ControllersYModes/baseClasses/NetworkGameState.NetworkGameState_C|GetUsingBypasses _asnetwork_game_state)
            (CallFunction|PlayerHasBeenSpawn:Client)))))))

(event EventPlayerHasBeenSpawn:Client
  (Utilities|FlowControl|Delay 1.5)
  (bind _foundwidgets (Widget|GetAllWidgetsOfClass "/Game/Secpholand/UI/Widgets/LoadingScreen.LoadingScreen_C" true))
  (Progress|SetPercent (Variables|/Game/Secpholand/UI/Widgets/LoadingScreen.LoadingScreen_C|GetProgressBar_111 (Utilities|Array|Get(acopy) _foundwidgets)) 1.0)
  (CallFunction|PossesCamera "StartCam")
  (Utilities|FlowControl|Delay 0.5)
  (bind _returnvalue (UserInterface|CreateWidget "/Game/Secpholand/UI/Widgets/HUDYChat/HUD.HUD_C" self))
  (bind _output_get (Variables|Default|SetHUD _returnvalue))
  (UserInterface|Viewport|AddtoViewport _output_get 0)
  (bind _foundwidgets_2 (Widget|GetAllWidgetsOfClass "/Game/Secpholand/UI/Widgets/LoadingScreen.LoadingScreen_C" true))
  (Widget|RemovefromParent (Utilities|Array|Get(acopy) _foundwidgets_2))
  (CallFunction|InitVoiceCapture)
  (bind _asnetwork_game_state (Utilities|Casting|CastToNetworkGameState (Game|GetGameState)))
  ;[0 1 1] Bypass
  (if (Variables|/Game/Secpholand/Blueprints/ControllersYModes/baseClasses/NetworkGameState.NetworkGameState_C|GetUsingBypasses _asnetwork_game_state)
    (Utilities|Struct|SetmembersinUserInfo_Public (Variables|Default|GetUserInfo) "NewEnumerator8"))
  (CallFunction|AñadirSalirMapaWidget)
  (CallFunction|CreateChatWidget)
  (if (Utilities|Enum|Equal(Enum) (.IngameLocation (Utilities|Struct|BreakUserInfo_Public (Variables|Default|GetUserInfo))) "NewEnumerator19")
    (CallFunction|CompleteObjective 2)))

(event Custom|VerReto:Server
  (params (RetoID :type Integer))
  (bind _asmeeting_center_game_state (Utilities|Casting|CastToMeetingCenterGameState (Game|GetGameState)))
  (Default|VerReto _asmeeting_center_game_state RetoID self))

(event Custom|EnviarPropuesta:Client
  (params (RetoID :type Integer))
  (CallFunction|EnviarPropuesta:Server RetoID))

(event Custom|VerReto:Client
  (params (RetoID :type Integer))
  (CallFunction|VerReto:Server RetoID))

(event Custom|EnviarPropuesta:Server
  (params (RetoID :type Integer))
  (bind _asmeeting_center_game_state (Utilities|Casting|CastToMeetingCenterGameState (Game|GetGameState)))
  (Default|EnviarPropuesta _asmeeting_center_game_state RetoID self))

(event Custom|SuperUserAñadirUsuarioReunion:Client
  (params (NumReunion :type Integer) (UsernameToAdd :type String%20%28by%20ref%29) (NombreReunion :type String))
  ;[1 1 1] SuperUser: SalasReunión
  (CallFunction|SuperUserAñadirUsuarioReunion:Server NumReunion UsernameToAdd NombreReunion))

(event Custom|SuperUserResetReunion:Server
  (params (NumReunion :type Integer))
  ;[1 1 1] SuperUser: SalasReunión
  (if (.SuperUser (Utilities|Struct|BreakUserInfo_Private (Variables|Default|GetuserInfo_Private)))
    (Default|SuperUsuario:ResetSalaReunión (.AsMeeting%20Center%20Game%20State (Utilities|Casting|CastToMeetingCenterGameState (Game|GetGameState))) NumReunion)))

(event Custom|SuperUserQuitarUsuarioReunion:Server
  (params (NumReunion :type Integer) (UsernameToRemove :type String%20%28by%20ref%29))
  ;[1 1 1] SuperUser: SalasReunión
  (if (.SuperUser (Utilities|Struct|BreakUserInfo_Private (Variables|Default|GetuserInfo_Private)))
    (Default|SuperUser:RemoveUsuarioReunion (.AsMeeting%20Center%20Game%20State (Utilities|Casting|CastToMeetingCenterGameState (Game|GetGameState))) NumReunion UsernameToRemove)))

(event Custom|SuperUser:AddReto:Server
  (params (Numsala :type Integer) (NombreReto :type String%20%28by%20ref%29) (URL :type String))
  (bind _returnvalue (Game|GetGameState))
  (bind _array (Utilities|Array|MakeArray))
  (bind _asmeeting_center_game_state (Utilities|Casting|CastToMeetingCenterGameState _returnvalue))
  ;[1 1 1] SuperUser: SalasReunión
  (if (.SuperUser (Utilities|Struct|BreakUserInfo_Private (Variables|Default|GetuserInfo_Private)))
    (Utilities|Array|SetArrayElem (Variables|/Game/Secpholand/Blueprints/ControllersYModes/MeetingCenterGameState.MeetingCenterGameState_C|GetRetoInfos _asmeeting_center_game_state) Numsala (Utilities|Struct|MakeRetoInfo (+ Numsala 1) NombreReto URL (Utilities|Array|MakeArray) _array _array _array (Utilities|Array|MakeArray)))
    (Default|Activar/desactivarObjetivoReto _asmeeting_center_game_state Numsala NombreReto true)))

(event Custom|DeshabilitarSalaReto:Server
  (params (Numsala :type Integer))
  (bind _returnvalue (Game|GetGameState))
  (bind _asmeeting_center_game_state (Utilities|Casting|CastToMeetingCenterGameState _returnvalue))
  ;[1 1 1] SuperUser: SalasReunión
  (if (.SuperUser (Utilities|Struct|BreakUserInfo_Private (Variables|Default|GetuserInfo_Private)))
    (Utilities|Array|SetArrayElem :TargetArray (Variables|/Game/Secpholand/Blueprints/ControllersYModes/MeetingCenterGameState.MeetingCenterGameState_C|GetRetoInfos _asmeeting_center_game_state) :Index Numsala)
    (Default|Activar/desactivarObjetivoReto _asmeeting_center_game_state Numsala "" false)))

(event Custom|AñadirRequerimientoaReto:Server
  (params (Numsala :type Integer) (NombreReq :type String%20%28by%20ref%29))
  ;[1 1 1] SuperUser: SalasReunión
  (if (.SuperUser (Utilities|Struct|BreakUserInfo_Private (Variables|Default|GetuserInfo_Private)))
    (Utilities|Array|Add (.Requerimientos (Utilities|Struct|BreakRetoInfo (Utilities|Array|Get(acopy) (Variables|/Game/Secpholand/Blueprints/ControllersYModes/MeetingCenterGameState.MeetingCenterGameState_C|GetRetoInfos (.AsMeeting%20Center%20Game%20State (Utilities|Casting|CastToMeetingCenterGameState (Game|GetGameState)))) Numsala))) (Utilities|Struct|MakeRequerimientoReto (Utilities|Array|MakeArray) (Utilities|Array|MakeArray) NombreReq))))

(event Custom|AñadirRequerimientoaReto:Client
  (params (Numsala :type Integer) (NombreReq :type String%20%28by%20ref%29))
  ;[1 1 1] SuperUser: SalasReunión
  (CallFunction|AñadirRequerimientoaReto:Server Numsala NombreReq))

(event Custom|SuperUserAñadirUsuarioReunion:Server
  (params (NumReunion :type Integer) (UsernameToAdd :type String%20%28by%20ref%29) (NombreReunion :type String))
  ;[1 1 1] SuperUser: SalasReunión
  (if (.SuperUser (Utilities|Struct|BreakUserInfo_Private (Variables|Default|GetuserInfo_Private)))
    (Default|SuperUser:AddUsuariotoReunión (.AsMeeting%20Center%20Game%20State (Utilities|Casting|CastToMeetingCenterGameState (Game|GetGameState))) NumReunion UsernameToAdd NombreReunion)))

(event Custom|QuitarReq:Server
  (params (Numsala :type Integer) (NombreReq :type String%20%28by%20ref%29))
  (bind _returnvalue (Game|GetGameState))
  (bind _asmeeting_center_game_state (Utilities|Casting|CastToMeetingCenterGameState _returnvalue))
  (bind _retoinfos (Variables|/Game/Secpholand/Blueprints/ControllersYModes/MeetingCenterGameState.MeetingCenterGameState_C|GetRetoInfos _asmeeting_center_game_state))
  (bind _output (Utilities|Array|Get(acopy) _retoinfos Numsala))
  (bind _requerimientos (Utilities|Struct|BreakRetoInfo _output))
  ;[1 1 1] SuperUser: SalasReunión
  (if (.SuperUser (Utilities|Struct|BreakUserInfo_Private (Variables|Default|GetuserInfo_Private)))
    (for (_array_element _array_index) _requerimientos
      (if (Utilities|Enum|Equal(Enum) (.Requerimineto (Utilities|Struct|BreakRequerimientoReto _array_element)) NombreReq)
        (Utilities|Array|RemoveIndex _requerimientos _array_index)))))

(event Custom|QuitarReq:Client
  (params (Numsala :type Integer) (NombreReq :type String%20%28by%20ref%29))
  ;[1 1 1] SuperUser: SalasReunión
  (CallFunction|QuitarReq:Server Numsala NombreReq))

(event Custom|SuperUserMutearTodosRequest:Client
  (params (Mutear? :type Boolean))
  ;[1 1 1] SuperUser: SalasReunión
  (CallFunction|SuperUserMutearTodos:Server (Variables|Default|GetTalkRoomID) Mutear?))

(event Custom|SuperUserMutearTodos:Server
  (params (TalkRoomID :type Integer) (Mutear? :type Boolean))
  ;[1 1 1] SuperUser: SalasReunión
  (if (.SuperUser (Utilities|Struct|BreakUserInfo_Private (Variables|Default|GetuserInfo_Private)))
    (Default|SuperUser:MutearUsuariosEnSala (.AsMeeting%20Center%20Game%20State (Utilities|Casting|CastToMeetingCenterGameState (Game|GetGameState))) TalkRoomID Mutear?)))

(event Custom|DeshabilitarSalaReto:Client
  (params (Numsala :type Integer))
  ;[1 1 1] SuperUser: SalasReunión
  (CallFunction|DeshabilitarSalaReto:Server Numsala))

(event Custom|SuperUserResetReunion:client
  (params (NumReunion :type Integer))
  ;[1 1 1] SuperUser: SalasReunión
  (CallFunction|SuperUserResetReunion:Server NumReunion))

(event Custom|SuperUser:AddReto:Client
  (params (Numsala :type Integer) (NombreReto :type String%20%28by%20ref%29) (URL :type String))
  ;[1 1 1] SuperUser: SalasReunión
  (CallFunction|SuperUser:AddReto:Server Numsala NombreReto URL))

(event Custom|SuperUserQuitarUsuarioReunion:Client
  (params (NumReunion :type Integer) (UsernameToRemove :type String%20%28by%20ref%29))
  ;[1 1 1] SuperUser: SalasReunión
  (CallFunction|SuperUserQuitarUsuarioReunion:Server NumReunion UsernameToRemove))

(event Custom|SuperUserQuitarRolPresentador:Server
  (params (UserName :type String))
  ;[1 1 1] Dar Rol presentador
  (if (.SuperUser (Utilities|Struct|BreakUserInfo_Private (Variables|Default|GetuserInfo_Private))) ; Solo le permitimos cambiar el rol de presentador si es un superUser
    (Default|QuitarRolPresentador (.AsMeeting%20Center%20Game%20State (Utilities|Casting|CastToMeetingCenterGameState (Game|GetGameState))) UserName)))

(event Custom|Server:Asignar%20Rol%20Presentador
  (params (UserName :type String) (NombreSala/Pantalla :type String) (PresentacionACargar :type String) (NumSlides :type Integer))
  ;[1 1 1] Dar Rol presentador
  (if (.SuperUser (Utilities|Struct|BreakUserInfo_Private (Variables|Default|GetuserInfo_Private))) ; Solo le permitimos cambiar el rol de presentador si es un superUser
    (Default|DarRolPresentador (.AsMeeting%20Center%20Game%20State (Utilities|Casting|CastToMeetingCenterGameState (Game|GetGameState))) UserName NombreSala/Pantalla PresentacionACargar NumSlides)))

(event Custom|Event:%20Next%20Slider
  (params (Pantalla :type Pantalla%20Presentación%20Object%20Reference))
  ;[1 1 1] PasarSlides
  (CallFunction|Server:NextSlide Pantalla))

(event Custom|Event:Previous%20Slider
  (params (pantalla :type Pantalla%20Presentación%20Object%20Reference))
  ;[1 1 1] PasarSlides
  (CallFunction|Server:PreviousSlide pantalla))

(event Custom|RecibirQuitarRolPresentador:client
  (bind _ref_widgetcontrol (Variables|Default|GetRef_WidgetControl))
  ;[1 1 1] Permission for Screen TV
  (Utilities|IsValid _ref_widgetcontrol
    (:Is%20Valid
      (Default|RemoveScreenWB _ref_widgetcontrol))))

(event Custom|Recibir%20rol%20presentador:%20Client
  (params (PantallaEnLaQuePresento :type String))
  ;[1 1 1] Permission for Screen TV
  (bind _outactors (Actor|GetAllActorsOfClasswithTag "/Game/Secpholand/Blueprints/OtherBP/PantallaPresentación.PantallaPresentación_C" (Utilities|String|StringToName PantallaEnLaQuePresento)))
  (Utilities|IsValid (Variables|Default|GetRef_WidgetControl)
    (:Is%20Valid
      _)
    (:Is%20Not%20Valid
      (bind _returnvalue (UserInterface|CreateWidget "/Game/Secpholand/UI/Widgets/ScreenHall_WB.ScreenHall_WB_C" 0 (.AsPantalla%20Presentación (Utilities|Casting|CastToPantallaPresentación (Utilities|Array|Get(acopy) _outactors)))))
      (bind _output_get (Variables|Default|SetRef_WidgetControl _returnvalue))))
  (UserInterface|Viewport|AddtoViewport _output_get 0))

(event Custom|Server:Previous%20Slide
  (params (Pantalla :type Pantalla%20Presentación%20Object%20Reference))
  ;[1 1 1] PasarSlides
  (if (Variables|Default|GetIsPresenter?)
    (Default|Multicast:PreviousSlide Pantalla)))

(event Custom|Server:Next%20Slide
  (params (Pantalla :type Pantalla%20Presentación%20Object%20Reference))
  ;[1 1 1] PasarSlides
  (if (Variables|Default|GetIsPresenter?)
    (Default|Multicast:NextSlide Pantalla)))

(event Custom|Client:Asignar%20Rol%20Presentador
  (params (UserName :type String) (NombreSala/Pantalla :type String) (PresentacionACargar :type String) (NumSlides :type Integer))
  ;[1 1 1] Dar Rol presentador
  (CallFunction|Server:AsignarRolPresentador UserName NombreSala/Pantalla PresentacionACargar NumSlides))

(event Custom|RecibirQuitarRolPresentador:Server
  ;[1 1 1] Permission for Screen TV
  (Variables|Default|SetIsPresenter? false)
  (CallFunction|RecibirQuitarRolPresentador:client))

(event Custom|SuperUserQuitarRolPresentador:Client
  (params (UserName :type String))
  ;[1 1 1] Dar Rol presentador
  (CallFunction|SuperUserQuitarRolPresentador:Server UserName))

(event Custom|Recibir%20rol%20presentador:%20Server
  (params (NombreSala/Pantalla :type String) (PresentacionACargar :type String) (NumSlides :type Integer))
  ;[1 1 1] Permission for Screen TV
  (Variables|Default|SetIsPresenter? true)
  (bind _output_get (Variables|Default|SetRoomName NombreSala/Pantalla))
  (bind _outactors (Actor|GetAllActorsOfClasswithTag "/Game/Secpholand/Blueprints/OtherBP/PantallaPresentación.PantallaPresentación_C" (Utilities|String|StringToName _output_get)))
  (Default|Multicast:BuildTextures (.AsPantalla%20Presentación (Utilities|Casting|CastToPantallaPresentación (Utilities|Array|Get(acopy) _outactors))) PresentacionACargar NumSlides)
  (CallFunction|RecibirRolPresentador:Client (Variables|Default|GetRoomName))
  (CallFunction|ActualizarPresentador:Server (Variables|Default|GetUserInfo)))

(event Custom|ActualizarPresentador:Server
  (params (UserInfo :type User%20Info%20Public%20Structure))
  (bind _outactors (Actor|GetAllActorswithTag "Presentador"))
  (for _array_element _outactors
    (bind _asserver_side_character_presentador (Utilities|Casting|CastToServerSide_Character_Presentador _array_element))
    (Default|ActualizarPresentador _asserver_side_character_presentador UserInfo true)))

(event Input|KeyboardEvents|X
  (params (Key :type Key%20Structure :default "None"))
  ;[0 0.82 1] By Pass Changue Name Client
  (:Pressed
    (CallFunction|InputX)
    (Variables|Default|SetUserInfo (Utilities|Struct|MakeUserInfo_Public 0 "User X" "None" "NewEnumerator0" false 0 "NewEnumerator8" "(Male?_1_4F059EB24111B7F69951FC908F407398=True,HairType_25_93A342E84CFD69BCE081C399812BF9B1=0,HairColor_26_BCFD46B448819E473AF0AE9151135E2D=0,SkinColor_27_FD344504414841F55D90FC9ED782E0E5=0,Class_15_24DA666548B155AFC0FE1FBFD4B0167C=NewEnumerator0,beardType_28_1C7EFC02400FF0BC88F39297521A0ECD=0,Glasses_29_7F7EE8F9437364B6FD7ED19916E9D8D4=0,Complemento_30_AED5EEC44EEA6509825E26B9E1F0D000=0)" (Utilities|Array|MakeArray "") (Utilities|Array|MakeArray "") "(ID_2_652DDBC544094EA3A624DA870A6FB6A6=0,Name_6_26B28C3349E7825E6BD0BB860DD767F0=\"Secpho\",Descripcion_51_33EDF47445C30234D32CE291439AA909=\"\",URL_52_9726AC9548205C7C5F9742818CBAB7B9=\"\",TipodeEntidad_53_7AAAC82E4A3747E701CFD7B5B2F1AB40=\"\",Actividad_54_B7A1D4FE48E9E3D6DFC9F1BA41BB7552=\"\",Direccion_55_CEACA9F34628C0C0F3E6B6A8C5D31091=\"\",Contacto_56_8E0470B046B6E584D5B3F396C3466041=\"\",Tecnologias_67_95B60E92403361EA765E5E8BCDA64C5E=,Sectores_69_E9FA7B954648B724724030A41C5C0C6B=,Cadenadevalor_59_84A3F0DA4B490A670E3F248BD981B590=\"\",Empleados-Cargo_60_A87BE6844050D6BA2DA46AA7ADA917D6=(\"\"),LogoURL_63_F6D503C34F06B2E7A5CE4EB4FBA8F83F=\"https://www.accio.gencat.cat/web/.content/01_Serveis/clusters/Troba-el-teu-cluster/clusters/img/secpho.png_941384905.png\",Level_66_519114264E08F71AE32BEA9D20DA16B5=1)"))
    (Development|PrintString (.Username (Utilities|Struct|BreakUserInfo_Public (Variables|Default|GetUserInfo))) true false "(R=0.000000,G=0.030967,B=1.000000,A=1.000000)" 1e+03)))

(event Input|KeyboardEvents|U
  (params (Key :type Key%20Structure :default "None"))
  ;[0 0.82 1] By Pass Changue Name Client
  (:Pressed
    (CallFunction|InputU)
    (Variables|Default|SetUserInfo (Utilities|Struct|MakeUserInfo_Public 0 "User U" "None" "NewEnumerator0" false 0 "NewEnumerator8" "(Male?_1_4F059EB24111B7F69951FC908F407398=True,HairType_25_93A342E84CFD69BCE081C399812BF9B1=0,HairColor_26_BCFD46B448819E473AF0AE9151135E2D=0,SkinColor_27_FD344504414841F55D90FC9ED782E0E5=0,Class_15_24DA666548B155AFC0FE1FBFD4B0167C=NewEnumerator0,beardType_28_1C7EFC02400FF0BC88F39297521A0ECD=0,Glasses_29_7F7EE8F9437364B6FD7ED19916E9D8D4=0,Complemento_30_AED5EEC44EEA6509825E26B9E1F0D000=0)" (Utilities|Array|MakeArray "") (Utilities|Array|MakeArray "") "(ID_2_652DDBC544094EA3A624DA870A6FB6A6=0,Name_6_26B28C3349E7825E6BD0BB860DD767F0=\"Secpho\",Descripcion_51_33EDF47445C30234D32CE291439AA909=\"\",URL_52_9726AC9548205C7C5F9742818CBAB7B9=\"\",TipodeEntidad_53_7AAAC82E4A3747E701CFD7B5B2F1AB40=\"\",Actividad_54_B7A1D4FE48E9E3D6DFC9F1BA41BB7552=\"\",Direccion_55_CEACA9F34628C0C0F3E6B6A8C5D31091=\"\",Contacto_56_8E0470B046B6E584D5B3F396C3466041=\"\",Tecnologias_67_95B60E92403361EA765E5E8BCDA64C5E=,Sectores_69_E9FA7B954648B724724030A41C5C0C6B=,Cadenadevalor_59_84A3F0DA4B490A670E3F248BD981B590=\"\",Empleados-Cargo_60_A87BE6844050D6BA2DA46AA7ADA917D6=(\"\"),LogoURL_63_F6D503C34F06B2E7A5CE4EB4FBA8F83F=\"https://www.accio.gencat.cat/web/.content/01_Serveis/clusters/Troba-el-teu-cluster/clusters/img/secpho.png_941384905.png\",Level_66_519114264E08F71AE32BEA9D20DA16B5=1)"))
    (Development|PrintString (.Username (Utilities|Struct|BreakUserInfo_Public (Variables|Default|GetUserInfo))) true false "(R=0.000000,G=0.030967,B=1.000000,A=1.000000)" 1e+03)))

(event Input|KeyboardEvents|Y
  (params (Key :type Key%20Structure :default "None"))
  ;[0 0.82 1] By Pass Changue Name Client
  (:Pressed
    (CallFunction|InputY)
    (Variables|Default|SetUserInfo (Utilities|Struct|MakeUserInfo_Public 0 "User Y" "None" "NewEnumerator0" false 0 "NewEnumerator8" "(Male?_1_4F059EB24111B7F69951FC908F407398=True,HairType_25_93A342E84CFD69BCE081C399812BF9B1=0,HairColor_26_BCFD46B448819E473AF0AE9151135E2D=0,SkinColor_27_FD344504414841F55D90FC9ED782E0E5=0,Class_15_24DA666548B155AFC0FE1FBFD4B0167C=NewEnumerator0,beardType_28_1C7EFC02400FF0BC88F39297521A0ECD=0,Glasses_29_7F7EE8F9437364B6FD7ED19916E9D8D4=0,Complemento_30_AED5EEC44EEA6509825E26B9E1F0D000=0)" (Utilities|Array|MakeArray "") (Utilities|Array|MakeArray "") "(ID_2_652DDBC544094EA3A624DA870A6FB6A6=0,Name_6_26B28C3349E7825E6BD0BB860DD767F0=\"Secpho\",Descripcion_51_33EDF47445C30234D32CE291439AA909=\"\",URL_52_9726AC9548205C7C5F9742818CBAB7B9=\"\",TipodeEntidad_53_7AAAC82E4A3747E701CFD7B5B2F1AB40=\"\",Actividad_54_B7A1D4FE48E9E3D6DFC9F1BA41BB7552=\"\",Direccion_55_CEACA9F34628C0C0F3E6B6A8C5D31091=\"\",Contacto_56_8E0470B046B6E584D5B3F396C3466041=\"\",Tecnologias_67_95B60E92403361EA765E5E8BCDA64C5E=,Sectores_69_E9FA7B954648B724724030A41C5C0C6B=,Cadenadevalor_59_84A3F0DA4B490A670E3F248BD981B590=\"\",Empleados-Cargo_60_A87BE6844050D6BA2DA46AA7ADA917D6=(\"\"),LogoURL_63_F6D503C34F06B2E7A5CE4EB4FBA8F83F=\"https://www.accio.gencat.cat/web/.content/01_Serveis/clusters/Troba-el-teu-cluster/clusters/img/secpho.png_941384905.png\",Level_66_519114264E08F71AE32BEA9D20DA16B5=1)"))
    (Development|PrintString (.Username (Utilities|Struct|BreakUserInfo_Public (Variables|Default|GetUserInfo))) true false "(R=0.000000,G=0.030967,B=1.000000,A=1.000000)" 1e+03)))