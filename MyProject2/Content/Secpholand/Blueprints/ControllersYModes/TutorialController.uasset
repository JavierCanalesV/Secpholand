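; Player controller for the tutorial level: point-and-click movement with an orbit and zoom camera.
; Client init creates the HUD, fetches personal info from NetworkGameState, places the tutorial character at a PlayerStart and plays a faded, train-sound intro cutscene with input disabled.
; Left-click traces route to clickable actors, other characters' menus or navmesh movement.
; Hold-to-move gates, input re-enabling and TutorialManager spawning sit in unconnected, never-run chains.
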(event Custom|RetrievePersonalInformation
  (bind _asnetwork_game_state (Utilities|Casting|CastToNetworkGameState (Game|GetGameState)))
  (Default|RetrievePersonalInfo _asnetwork_game_state (Variables|Default|GetuniqueID) self))

(event EventBeginPlay
  (CallFunction|Client:Init))

(event EventClient:Init
  (CallFunction|SetControllsConstraints false false false false)
  (Variables|Default|SetbShowMouseCursor true)
  (bind _returnvalue (UserInterface|CreateWidget "/Game/Secpholand/UI/Widgets/HUDYChat/HUD.HUD_C" self))
  (Variables|Default|SetHUD _returnvalue)
  (Variables|Default|SetbShowMouseCursor true)
  (CallFunction|RetrievePersonalInformation)
  (bind _asserver_side_character_tutorial (Utilities|Casting|CastToServerSide_CharacterTUTORIAL (Game|GetPlayerCharacter 0)))
  (Variables|Default|SettutorialCharRef _asserver_side_character_tutorial)
  (Variables|/Game/Secpholand/Blueprints/ControllersYModes/ServerSide_CharacterTUTORIAL.ServerSide_CharacterTUTORIAL_C|SetclientSideControllerRef _asserver_side_character_tutorial self)
  (bind _outactors (Actor|GetAllActorsOfClass "/Script/Engine.PlayerStart"))
  (Transformation|SetActorLocation _asserver_side_character_tutorial (Transformation|GetActorLocation (Utilities|Array|Get(acopy) _outactors 1)) false false)
  (CameraFades|StartCameraFade :self (Variables|Default|GetPlayerCameraManager) :FromAlpha 1.0 :ToAlpha 1.0 :Duration 0.6 :bHoldWhenFinished true)
  (Audio|PlaySound2D "/Game/Secpholand/audio/train.train" 1.0 1.0 0.0 0 0)
  (Utilities|FlowControl|Delay 3.0)
  (CameraFades|StartCameraFade :self (Variables|Default|GetPlayerCameraManager) :FromAlpha 1.0 :Duration 0.6 :bHoldWhenFinished true)
  (Utilities|FlowControl|Delay 1.0)
  (CallFunction|MovetoLocation "0,5964.903320,277.300964")
  (bind _returnvalue_2 (Sequencer|Player|CreateLevelSequencePlayer "/Game/Secpholand/Assets/Cinematics/NewLevelSequence.NewLevelSequence"))
  (bind _output_get (Variables|Default|SetintroCutscene _returnvalue_2))
  (Input|DisableInput (Variables|Default|GettutorialCharRef) self)
  (Sequencer|Player|Play _output_get :!class /Script/MovieScene.MovieSceneSequencePlayer)
  (Utilities|FlowControl|Delay 8.0))

(event EventMovetoLocation
  (params (Location :type Vector :default "0, 0, 0"))
  (AI|Navigation|SimpleMovetoLocation self Location))

(event EventCameraRotation
  (bind _canrotate_ (Variables|Default|GetcanRotate?))
  (bind _tutorialcharref (Variables|Default|GettutorialCharRef))
  (bind _rotateleft (Variables|Default|GetrotateLeft))
  (bind _springarm (Variables|/Game/Secpholand/Blueprints/ControllersYModes/ServerSide_CharacterTUTORIAL.ServerSide_CharacterTUTORIAL_C|GetSpringArm _tutorialcharref))
  (if (and (Variables|Default|GetRMpressed) _canrotate_)
    (Utilities|IsValid _tutorialcharref
      (:Is%20Valid
        (Transformation|AddRelativeRotation _springarm (Math|Rotator|MakeRotator 0.0 0.0 (* (Class|Actor|GetInputAxisKeyValue) 4.0)) false false)))
    (elif _canrotate_
      (if (or (Variables|Default|GetrotateRight) _rotateleft)
        (Transformation|AddRelativeRotation _springarm (Math|Rotator|MakeRotator 0.0 0.0 (select _rotateleft -3.0 3.0)) false false)))))

(event EventZoomCamera
  (params (ZoomAmount :type Float%20%28single-precision%29))
  (bind _tutorialcharref (Variables|Default|GettutorialCharRef))
  (bind _springarm (Variables|/Game/Secpholand/Blueprints/ControllersYModes/ServerSide_CharacterTUTORIAL.ServerSide_CharacterTUTORIAL_C|GetSpringArm _tutorialcharref))
  (bind _returnvalue (Transformation|GetWorldRotation _springarm))
  (if (and (> (+ ZoomAmount (Variables|Default|Getzoom)) 0.0) (< (+ ZoomAmount (Variables|Default|Getzoom)) 0.8))
    (bind _output_get (Variables|Default|Setzoom (+ ZoomAmount (Variables|Default|Getzoom))))
    (Utilities|IsValid _tutorialcharref
      (:Is%20Valid
        (Variables|/Script/Engine.SpringArmComponent|SetTargetArmLength _springarm (Math|Float|Lerp 6e+02 3.1e+03 _output_get))
        (Transformation|SetWorldRotation _springarm (Math|Rotator|MakeRotator (.roll _returnvalue) (Math|Interpolation|Ease "EaseOut" _output_get -15.0 -38.0 6.0) (.yaw _returnvalue)) false false)
        (Transformation|SetRelativeRotation (Variables|/Game/Secpholand/Blueprints/ControllersYModes/ServerSide_CharacterTUTORIAL.ServerSide_CharacterTUTORIAL_C|GetCameraOrighinalPos (Variables|Default|GettutorialCharRef)) (Math|Rotator|MakeRotator 0.0 (Math|Float|Lerp 2e+01 0.0 _output_get) 0.0) false false)
        (CallFunction|HandleNamePlates)
        (Development|ExecuteConsoleCommand (Utilities|String|Append "r.setNearClipPlane 1" "") 0)
        (Rendering|Material|SetScalarParameterValue "/Game/Secpholand/Assets/Materials/oclusionMPC.oclusionMPC" "Distance" (- (Math|Float|Lerp 6e+02 3.1e+03 0.0) 85.0) :!class /Script/Engine.KismetMaterialLibrary)
        (Rendering|Material|SetScalarParameterValue "/Game/Secpholand/Assets/Materials/oclusionMPC.oclusionMPC" "subtr" (Math|Float|Lerp -1.3e+02 -1e+02 0.0) :!class /Script/Engine.KismetMaterialLibrary)))))

(event EventTick
  (params (DeltaSeconds :type Float%20%28single-precision%29))
  (|CallParentFunction DeltaSeconds))

(event Input|ActionEvents|InputActionSetDestination
  (params (Key :type Key%20Structure :default "None"))
  (:Pressed
    (Utilities|FlowControl|Gate true) ; enters at Open
  )
  (:Released
    (Utilities|FlowControl|Gate true) ; enters at Close
  ))

(event Input|MouseEvents|LeftMouseButton
  (params (Key :type Key%20Structure :default "None"))
  (bind (_hitresult _returnvalue) (Game|Player|GetHitResultUnderCursorbyChannel "TraceTypeQuery1" true))
  (bind _hitactor (Collision|BreakHitResult _hitresult))
  (:Pressed
    (if (and (Variables|Default|GetcanClick?) _returnvalue)
      (Utilities|IsValid (Variables|Default|GetClickableClicked)
        (:Is%20Valid
          (if (!= (Variables|Default|GetClickableClicked) _hitactor)
            (Default|ResetClick (Variables|Default|GetClickableClicked))
            (Variables|Default|SetClickableClicked 0)
            (bind _asclickable_actor (Utilities|Casting|CastToClickableActor _hitactor :!label _label)
              (:then
                (bind _output_get (Variables|Default|SetClickableClicked _asclickable_actor))
                (Default|Click _output_get self))
              (:CastFailed
                (bind _asserver_side_character (Utilities|Casting|CastToServerSide_Character _hitactor)
                  (:then
                    (if (!= _asserver_side_character (Variables|Default|GetServerSideCharacterRef))
                      (CallFunction|OpenDesplegableMenuPlayer)
                      (Variables|Default|SetclickedCharacter _asserver_side_character)))
                  (:CastFailed
                    (Utilities|IsValid (Variables|Default|GettutorialCharRef)
                      (:Is%20Valid
                        (if (Variables|Default|GetcanMove?)
                          (CallFunction|SpawnDecal)
                          (CallFunction|CloseDesplegableMenuPlayer)
                          (CallFunction|MovetoLocation (Variables|Default|GetMouseLocation)))))))))))
        (:Is%20Not%20Valid
          (goto _label)))
      (else
        (Development|PrintString "CANT CLICK")))))

(event Input|KeyboardEvents|B
  (params (Key :type Key%20Structure :default "None"))
  (:Pressed
    (Game|OpenLevel(byName) "01SecpholandIvanTutorial")))

(event Input|TouchEvents|InputTouch
  (params (Location :type Vector) (FingerIndex :type ETouchIndex%20Enum))
  (bind _returnvalue (Utilities|Enum|Equal(Enum) FingerIndex "Touch1"))
  (:Pressed
    (if _returnvalue
      (Utilities|FlowControl|Gate true) ; enters at Open
    ))
  (:Released
    (if _returnvalue
      (Utilities|FlowControl|Gate true) ; enters at Close
    )))

(fn ConstructionScript
  (|CallParentFunction))

(fn MovetoHitLocation
  (params (NewParam :type Hit%20Result%20Structure))
  (bind _location (Collision|BreakHitResult NewParam))
  (if (>= (Math|Vector|VectorLength (- (Transformation|GetActorLocation (Pawn|GetControlledPawn)) _location)) 0.1) ; Don't move if player clicks too close to pawn
    (AI|Navigation|SimpleMovetoLocation self _location)))