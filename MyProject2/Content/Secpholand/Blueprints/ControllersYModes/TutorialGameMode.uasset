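; Game mode for Secpholand that bridges client controllers and a backend, apparently a database, over a local TCP socket.
; It spawns and connects the socket on BeginPlay, and SendMessage writes through it.
; Received messages dispatch on a protocol byte to NetworkGameState handlers for account, friend and chat features, with pendingMessages re-entering that dispatch.
; PostLogin stamps each controller's IP and unique ID, while logout removes the user and cleans up.
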(event Custom|SetIPAndUniqueID
  (params (ip :type String) (uniqueID :type String) (player :type Client%20Side%20Controller%20Object%20Reference))
  (Variables|/Game/Secpholand/Blueprints/ControllersYModes/ClientSide_Controller.ClientSide_Controller_C|Setip player ip)
  (Variables|/Game/Secpholand/Blueprints/ControllersYModes/ClientSide_Controller.ClientSide_Controller_C|SetuniqueID player uniqueID))

(event Custom|pendingMessages
  (params (message :type Array%20of%20Bytes))
  (bind _returnvalue (Game|GetGameState))
  (if (> (Math|Conversions|ToByte(Integer) (Utilities|Array|Length message)) 0)
    (Variables|Default|SetpendingMessage true)
    (bind _returnvalue_2 (Class|TcpSocketConnection|MessageReadByte (select (Variables|Default|GetpendingMessage) message (stale Custom|OnMessageReceivedEvent Message))))
    (switch Utilities|FlowControl|Switch|SwitchonTCPProtocol (Utilities|Enum|ByteToEnumTCPProtocol _returnvalue_2)
      (:NewEnumerator1
        (bind _asnetwork_game_state (Utilities|Casting|CastToNetworkGameState _returnvalue))
        (Default|LoginRetrievenInformation _asnetwork_game_state (select (Variables|Default|GetpendingMessage) message (stale Custom|OnMessageReceivedEvent Message))))
      (:NewEnumerator2
        (bind _asnetwork_game_state_2 (Utilities|Casting|CastToNetworkGameState _returnvalue))
        (Default|ConfirmPasswordChange _asnetwork_game_state_2 (select (Variables|Default|GetpendingMessage) message (stale Custom|OnMessageReceivedEvent Message))))
      (:NewEnumerator3
        (bind _asnetwork_game_state_3 (Utilities|Casting|CastToNetworkGameState _returnvalue))
        (Default|ConfirmInfoChanged _asnetwork_game_state_3 (select (Variables|Default|GetpendingMessage) message (stale Custom|OnMessageReceivedEvent Message))))
      (:NewEnumerator5
        (bind _asnetwork_game_state_4 (Utilities|Casting|CastToNetworkGameState _returnvalue))
        (Default|ReceiveFriendList _asnetwork_game_state_4 (select (Variables|Default|GetpendingMessage) message (stale Custom|OnMessageReceivedEvent Message))))
      (:NewEnumerator6
        (bind _asnetwork_game_state_5 (Utilities|Casting|CastToNetworkGameState _returnvalue))
        (Default|ReceiveFriendStates _asnetwork_game_state_5 (select (Variables|Default|GetpendingMessage) message (stale Custom|OnMessageReceivedEvent Message))))
      (:NewEnumerator8
        (bind _asnetwork_game_state_6 (Utilities|Casting|CastToNetworkGameState _returnvalue))
        (Default|ReceiveFriendRequest _asnetwork_game_state_6 (select (Variables|Default|GetpendingMessage) message (stale Custom|OnMessageReceivedEvent Message))))
      (:NewEnumerator7
        (bind _asnetwork_game_state_7 (Utilities|Casting|CastToNetworkGameState _returnvalue))
        (Default|ReceiveNewFriend _asnetwork_game_state_7 (select (Variables|Default|GetpendingMessage) message (stale Custom|OnMessageReceivedEvent Message))))
      (:NewEnumerator9
        (bind _asnetwork_game_state_8 (Utilities|Casting|CastToNetworkGameState _returnvalue))
        (Default|ReceiveRemovedFriend _asnetwork_game_state_8 (select (Variables|Default|GetpendingMessage) message (stale Custom|OnMessageReceivedEvent Message))))
      (:NewEnumerator11
        (bind _asnetwork_game_state_9 (Utilities|Casting|CastToNetworkGameState _returnvalue))
        (Default|ReceiveMessage _asnetwork_game_state_9 (select (Variables|Default|GetpendingMessage) message (stale Custom|OnMessageReceivedEvent Message))))
      (:NewEnumerator12
        (bind _asnetwork_game_state_10 (Utilities|Casting|CastToNetworkGameState _returnvalue))
        (Default|ReceiveChatHistory _asnetwork_game_state_10 (select (Variables|Default|GetpendingMessage) message (stale Custom|OnMessageReceivedEvent Message))))
      (:NewEnumerator13
        (bind _asnetwork_game_state_11 (Utilities|Casting|CastToNetworkGameState _returnvalue))
        (Default|ReceiveFilteredUsersbyName _asnetwork_game_state_11 (select (Variables|Default|GetpendingMessage) message (stale Custom|OnMessageReceivedEvent Message))))
      (:NewEnumerator14
        (bind _asnetwork_game_state_12 (Utilities|Casting|CastToNetworkGameState _returnvalue))
        (Default|ReceiveFriendNewState _asnetwork_game_state_12 (select (Variables|Default|GetpendingMessage) message (stale Custom|OnMessageReceivedEvent Message)))))))

(event Custom|ConnectedEvent
  (params (ConnectionId :type Integer))
  (Development|PrintString "connected!"))

(event Custom|DisconnectedEvent
  (params (ConnectionId :type Integer))
  (Development|PrintString "Disconnected!"))

(event Custom|OnMessageReceivedEvent
  (params (ConnectionId :type Integer) (Message :type Array%20of%20Bytes))
  (bind _returnvalue (Game|GetGameState))
  (Variables|Default|SetpendingMessage false)
  (bind _returnvalue_2 (Class|TcpSocketConnection|MessageReadByte (select (Variables|Default|GetpendingMessage) (stale Custom|pendingMessages message) Message)))
  (switch Utilities|FlowControl|Switch|SwitchonTCPProtocol (Utilities|Enum|ByteToEnumTCPProtocol _returnvalue_2)
    (:NewEnumerator1
      (bind _asnetwork_game_state (Utilities|Casting|CastToNetworkGameState _returnvalue))
      (Default|LoginRetrievenInformation _asnetwork_game_state (select (Variables|Default|GetpendingMessage) (stale Custom|pendingMessages message) Message)))
    (:NewEnumerator2
      (bind _asnetwork_game_state_2 (Utilities|Casting|CastToNetworkGameState _returnvalue))
      (Default|ConfirmPasswordChange _asnetwork_game_state_2 (select (Variables|Default|GetpendingMessage) (stale Custom|pendingMessages message) Message)))
    (:NewEnumerator3
      (bind _asnetwork_game_state_3 (Utilities|Casting|CastToNetworkGameState _returnvalue))
      (Default|ConfirmInfoChanged _asnetwork_game_state_3 (select (Variables|Default|GetpendingMessage) (stale Custom|pendingMessages message) Message)))
    (:NewEnumerator5
      (bind _asnetwork_game_state_4 (Utilities|Casting|CastToNetworkGameState _returnvalue))
      (Default|ReceiveFriendList _asnetwork_game_state_4 (select (Variables|Default|GetpendingMessage) (stale Custom|pendingMessages message) Message)))
    (:NewEnumerator6
      (bind _asnetwork_game_state_5 (Utilities|Casting|CastToNetworkGameState _returnvalue))
      (Default|ReceiveFriendStates _asnetwork_game_state_5 (select (Variables|Default|GetpendingMessage) (stale Custom|pendingMessages message) Message)))
    (:NewEnumerator8
      (bind _asnetwork_game_state_6 (Utilities|Casting|CastToNetworkGameState _returnvalue))
      (Default|ReceiveFriendRequest _asnetwork_game_state_6 (select (Variables|Default|GetpendingMessage) (stale Custom|pendingMessages message) Message)))
    (:NewEnumerator7
      (bind _asnetwork_game_state_7 (Utilities|Casting|CastToNetworkGameState _returnvalue))
      (Default|ReceiveNewFriend _asnetwork_game_state_7 (select (Variables|Default|GetpendingMessage) (stale Custom|pendingMessages message) Message)))
    (:NewEnumerator9
      (bind _asnetwork_game_state_8 (Utilities|Casting|CastToNetworkGameState _returnvalue))
      (Default|ReceiveRemovedFriend _asnetwork_game_state_8 (select (Variables|Default|GetpendingMessage) (stale Custom|pendingMessages message) Message)))
    (:NewEnumerator11
      (bind _asnetwork_game_state_9 (Utilities|Casting|CastToNetworkGameState _returnvalue))
      (Default|ReceiveMessage _asnetwork_game_state_9 (select (Variables|Default|GetpendingMessage) (stale Custom|pendingMessages message) Message)))
    (:NewEnumerator12
      (bind _asnetwork_game_state_10 (Utilities|Casting|CastToNetworkGameState _returnvalue))
      (Default|ReceiveChatHistory _asnetwork_game_state_10 (select (Variables|Default|GetpendingMessage) (stale Custom|pendingMessages message) Message)))
    (:NewEnumerator13
      (bind _asnetwork_game_state_11 (Utilities|Casting|CastToNetworkGameState _returnvalue))
      (Default|ReceiveFilteredUsersbyName _asnetwork_game_state_11 (select (Variables|Default|GetpendingMessage) (stale Custom|pendingMessages message) Message)))
    (:NewEnumerator14
      (bind _asnetwork_game_state_12 (Utilities|Casting|CastToNetworkGameState _returnvalue))
      (Default|ReceiveFriendNewState _asnetwork_game_state_12 (select (Variables|Default|GetpendingMessage) (stale Custom|pendingMessages message) Message)))))

(event Custom|SendMessage
  (params (messageToSend :type Array%20of%20Bytes))
  (bind _sockettodb (Variables|Default|GetsocketToDB))
  (Utilities|IsValid _sockettodb
    (:Is%20Valid
      (bind _returnvalue (Class|TcpSocketConnection|SendData _sockettodb (Variables|Default|GetconnectionID) messageToSend))
      (if _returnvalue
        (Development|PrintString "Message sent")
        (else
          (Development|PrintString "Error: Not connected to the server"))))
    (:Is%20Not%20Valid
      (Development|PrintString "Error: Socket not initialized"))))

(event EventBeginPlay
  (bind _returnvalue (Game|SpawnActorfromClass "/Script/TcpSocketPlugin.TcpSocketConnection" (Transformation|GetWorldTransform (Variables|Default|GetDefaultSceneRoot)) "Undefined" 0 0))
  (Variables|Default|SetsocketToDB _returnvalue)
  (bind _connectionid (Class|TcpSocketConnection|Connect (Variables|Default|GetsocketToDB) "127.0.0.1" (Variables|Default|Getport) (delegate Custom|DisconnectedEvent) (delegate Custom|ConnectedEvent) (delegate Custom|OnMessageReceivedEvent)))
  (Variables|Default|SetconnectionID _connectionid))

(event EventTick
  (params (DeltaSeconds :type Float%20%28single-precision%29)))

(event EventOnLogout
  (params (ExitingController :type Controller%20Object%20Reference))
  (bind _asclient_side_controller (Utilities|Casting|CastToClientSide_Controller ExitingController))
  (bind _asnetwork_game_state (Utilities|Casting|CastToNetworkGameState (Game|GetGameState)))
  (Default|RemoveUser _asnetwork_game_state 0 "" "" _asclient_side_controller "NewEnumerator2")
  (Default|DestroyAll _asclient_side_controller))

(event EventPostLogin
  (params (NewPlayer :type Player%20Controller%20Object%20Reference))
  (bind _asclient_side_controller (Utilities|Casting|CastToClientSide_Controller NewPlayer))
  (CallFunction|SetIPandUniqueID (Class|NetworkGameModeOverrided|GetPlayerIP) (Class|NetworkGameModeOverrided|GetPlayerUniqueID) _asclient_side_controller))

(fn ConstructionScript)