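; LogginPawn is a pawn that switches the player's view to a fixed bird's-eye camera once it is possessed.
; After a one-second delay it finds the first actor tagged "VistaDePajaro" and casts it to a CameraActor.
; Player controller 0 then sets that camera as its view target with the outgoing view locked.
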(event EventPossessed
  (params (NewController :type Controller%20Object%20Reference))
  (Utilities|FlowControl|Delay 1.0)
  (bind _outactors (Actor|GetAllActorswithTag "VistaDePajaro"))
  (if (> (Utilities|Array|Length _outactors) 0)
    (bind _ascamera_actor (Utilities|Casting|CastToCameraActor (Utilities|Array|Get(acopy) _outactors)))
    (Game|Player|SetViewTargetwithBlend (Game|GetPlayerController 0) _ascamera_actor 0.0 "VTBlend_Linear" 0.0 true)))

(fn ConstructionScript
  (|CallParentFunction))