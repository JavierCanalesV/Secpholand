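; Tutorial player controller that spawns a player's server-side avatar into the tutorial level and releases the loading screen.
; On authority, it runs once: teleports the client-side pawn to the start, then spawns a separate server-side character and controller, linking and possessing them.
; ShowPlayer retries until the character is valid, reveals it and spawns an actor for disabling other players' collisions.
; A client event then clears the loading screen and enables movement.
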(event Custom|ShowPlayer
  (bind _serversidecharacterref (Variables|Default|GetServerSideCharacterRef))
  (Utilities|IsValid _serversidecharacterref :!label _label
    (:Is%20Valid
      (Rendering|SetVisibility (Variables|/Script/Engine.Character|GetMesh _serversidecharacterref) true true)
      (CallFunction|SetMovementUpdateTime)
      (Game|SpawnActorfromClass "/Game/Secpholand/Blueprints/OtherBP/DisableOtherPlayersCollisions.DisableOtherPlayersCollisions_C" (Math|Transform|MakeTransform "-1261.671265,1833.884766, 0") "Undefined" 0 0))
    (:Is%20Not%20Valid
      (Utilities|FlowControl|Delay 0.2)
      (goto _label))))

(event EventPlayerHasBeenSpawn:Client
  (bind _foundwidgets (Widget|GetAllWidgetsOfClass "/Game/Secpholand/UI/Widgets/LoadingScreen.LoadingScreen_C" true))
  (Progress|SetPercent (Variables|/Game/Secpholand/UI/Widgets/LoadingScreen.LoadingScreen_C|GetProgressBar_111 (Utilities|Array|Get(acopy) _foundwidgets)) 1.0)
  (Utilities|FlowControl|Delay 0.5)
  (Widget|RemovefromParent (Utilities|Array|Get(acopy) _foundwidgets))
  (CallFunction|SetControllsConstraints true false false false))

(event EventServerSpawnPlayer
  (params (playerStartIndex :type Player%20Start%20Object%20Reference) (UserInfo :type User%20Info%20Public%20Structure))
  (bind _self self)
  (bind _clientsidepawnref (Variables|Default|GetClientSidePawnRef))
  (Networking|SwitchHasAuthority
    (:Authority
      (Utilities|FlowControl|DoOnce false
        (:Completed
          (Transformation|SetActorLocation _clientsidepawnref (Transformation|GetActorLocation playerStartIndex) false true)
          (bind _returnvalue (Game|SpawnActorfromClass "/Game/Secpholand/Blueprints/ControllersYModes/baseClasses/ServerSide_Character.ServerSide_Character_C" (Transformation|GetActorTransform _clientsidepawnref) "AdjustIfPossibleButAlwaysSpawn" _self UserInfo _self 0))
          (bind _output_get (Variables|Default|SetServerSideCharacterRef _returnvalue))
          (Default|SetName _output_get)
          (bind _asnetwork_player_state (Utilities|Casting|CastToNetworkPlayerState (Variables|Default|GetPlayerState)))
          (Variables|/Game/Secpholand/Blueprints/ControllersYModes/baseClasses/NetworkPlayerState.NetworkPlayerState_C|SetServerSideCharacterRef _asnetwork_player_state (Variables|Default|GetServerSideCharacterRef))
          (bind _returnvalue_2 (Game|SpawnActorfromClass "/Game/Secpholand/Blueprints/ControllersYModes/baseClasses/ServerSide_Controller.ServerSide_Controller_C" (Transformation|GetActorTransform (Variables|Default|GetClientSidePawnRef)) "AdjustIfPossibleButAlwaysSpawn" 0 self 0))
          (bind _output_get_2 (Variables|Default|SetServerSideControllerRef _returnvalue_2))
          (Variables|/Game/Secpholand/Blueprints/ControllersYModes/baseClasses/ServerSide_Controller.ServerSide_Controller_C|SetServerSideCharacter _output_get_2 (Variables|Default|GetServerSideCharacterRef))
          (Pawn|Possess (Variables|Default|GetServerSideControllerRef) (Variables|Default|GetServerSideCharacterRef))
          (CallFunction|Server:RetrievePrivateInfo)
          (Rendering|SetVisibility (Variables|/Script/Engine.Character|GetMesh (Variables|Default|GetServerSideCharacterRef)) false true)
          (Default|HideNamePlate (Variables|Default|GetServerSideCharacterRef) true)
          (CallFunction|ShowPlayer)
          ;[0 1 1] bypass
          (CallFunction|PlayerHasBeenSpawn:Client))))))

(fn ConstructionScript
  (|CallParentFunction))