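; Server-side character Blueprint that shows a nameplate with the user's name and company.
; On BeginPlay, setName casts the NamePlate component's widget to NombrePlayer and fills its Nombre and Empresa texts from UserInfo, joining name and surname.
; A hideNamePlate event toggles the nameplate's visibility, propagating to its children.
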(event Custom|setName
  (bind _userinfo (Variables|Default|GetUserInfo))
  (bind (_id _username _name _surname _empresa) (Utilities|Struct|BreakUserInfo_Public _userinfo))
  (bind _asnombre_player (Utilities|Casting|CastToNombrePlayer (UserInterface|GetUserWidgetObject (Variables|Default|GetnamePlate))))
  (Rendering|Components|TextRender|SetText (Variables|/Game/Secpholand/UI/Widgets/NombrePlayer.NombrePlayer_C|GetNombre _asnombre_player) (Utilities|Text|ToText(String) (Utilities|String|Append (Utilities|String|ToString(Name) _name) " " (Utilities|String|ToString(Name) _surname))))
  (Rendering|Components|TextRender|SetText (Variables|/Game/Secpholand/UI/Widgets/NombrePlayer.NombrePlayer_C|GetEmpresa _asnombre_player) (Utilities|Text|ToText(Name) (.Name (Utilities|Struct|BreakEmpresa _empresa)))))

(event Custom|hideNamePlate
  (params (hide? :type Boolean))
  (Development|SetHiddeninGame (Variables|Default|GetnamePlate) hide? true))

(event EventBeginPlay
  (CallFunction|SetName))

(fn ConstructionScript)