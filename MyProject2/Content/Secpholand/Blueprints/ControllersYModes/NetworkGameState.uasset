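; Server-side game state that tracks connected users and relays chat, player names and challenge lists (retos) to their player controllers.
; Login, password and avatar updates go through NetworkGameMode as length-prefixed, protocol-tagged byte messages, the updates carrying raw concatenated SQL.
; Replies are parsed and routed by username to the matching controller.
; Friend and user-filter events return placeholder data, and public user info is empty.
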(event Custom|AddNewPlayerController
  (params (name :type String) (controller :type Client%20Side%20Controller%20Object%20Reference))
  (bind _userarray (Variables|Default|GetUserArray))
  (bind _found_ (CallFunction|GetUser "NewEnumerator1" 0 name))
  (if (not _found_)
    (Utilities|Array|Add _userarray (Utilities|Struct|MakeUser (Utilities|Array|Length _userarray) name controller))))

(event Custom|SendMessage
  (params (everyone? :type Boolean) (SenderName :type Name) (ReceiverName :type Name) (message :type Text) (timeStamp :type Date%20Time%20Compressed%20Structure))
  (if everyone?
    (for _array_element (Variables|Default|GetUserArray)
      (if (Utilities|Enum|NotEqual(Enum) (.username _array_element) (Utilities|String|ToString(Name) SenderName))
        (Default|ReceiveMessageServer (.playercontroller _array_element) SenderName message timeStamp)))
    (else
      (bind (_found_ _user) (CallFunction|GetUser "NewEnumerator1" 0 (Utilities|String|ToString(Name) ReceiverName)))
      (if _found_
        (Default|ReceiveMessageServer (.playercontroller _user) SenderName message timeStamp)))))

(event Custom|ConfirmPasswordChange
  (params (message :type Array%20of%20Bytes))
  (bind _returnvalue (Class|TcpSocketConnection|MessageReadInt message))
  (bind _returnvalue_2 (Class|TcpSocketConnection|MessageReadString message _returnvalue))
  (bind (_found_ _user) (CallFunction|GetUser "NewEnumerator1" 0 _returnvalue_2))
  (if _found_
    (Default|PWChangedSuccesfullServer (.PlayerController (Utilities|Struct|BreakUser _user)))))

(event Custom|ConfirmInfoChanged
  (params (message :type Array%20of%20Bytes))
  (bind _returnvalue (Class|TcpSocketConnection|MessageReadInt message))
  (bind _returnvalue_2 (Class|TcpSocketConnection|MessageReadString message _returnvalue))
  (bind (_found_ _user) (CallFunction|GetUser "NewEnumerator1" 0 _returnvalue_2))
  (if _found_
    (Default|UpdateInfoSuccesfullServer (.PlayerController (Utilities|Struct|BreakUser _user)))))

(event Custom|RetrieveFriendList
  (params (user :type Client%20Side%20Controller%20Object%20Reference))
  ;[1 1 0] Hace query a base de datos para extraer todos los amigos de un jugador
  (Default|ReceiveFriendList:Server user (Utilities|Array|MakeArray "Ivan Anfruns Ortiz" "Guillermo Esteban Plazas" "Brandon Jibaja") (Utilities|Array|MakeArray "NewEnumerator0" "NewEnumerator1" "NewEnumerator2")))

(event Custom|UpdateFriendStates
  (params (User :type Client%20Side%20Controller%20Object%20Reference) (friendNames :type Array%20of%20Strings))
  ;[1 1 0] Devuelve una lista con los nombres y estados de cada amigo
  (Default|ReceiveFriendUpdates:Server User (Utilities|Array|MakeArray "NewEnumerator0")))

(event Custom|AddFriend
  (params (User :type Client%20Side%20Controller%20Object%20Reference) (Friend :type String))
  ;[1 1 0] Query a base de datos para actualizar las friendlists de los 2 jugadores y devuelve la nueva lista
  (bind _user (CallFunction|GetUser "NewEnumerator1" 0 Friend))
  (Default|ReceiveFriendList:Server User (Utilities|Array|MakeArray "") (Utilities|Array|MakeArray "NewEnumerator0")))

(event Custom|RemoveFriend
  (params (User :type Client%20Side%20Controller%20Object%20Reference) (Friend :type String))
  ;[1 1 0] Query a base de datos para actualizar las friendlists de los 2 jugadores y devuelve la nueva lista
  (bind _user (CallFunction|GetUser "NewEnumerator1" 0 Friend))
  (Default|ReceiveFriendList:Server (.PlayerController (Utilities|Struct|BreakUser _user)) (Utilities|Array|MakeArray "") (Utilities|Array|MakeArray "NewEnumerator0")))

(event Custom|RetrieveAllFilteredUsers
  (params (User :type Client%20Side%20Controller%20Object%20Reference) (filter :type String))
  ;[1 1 0] Query a base de datos para encontrar todos los usuarios con ese filtro, devuelve el array resultante
  (Default|ReceiveAllFilteredUsers:Server User (Utilities|Array|MakeArray "")))

(event Custom|RetrievePublicUserInfo
  (params (User :type Client%20Side%20Controller%20Object%20Reference) (OtherUser :type String)))

(event Custom|RetrieveRetos
  (params (clientSideController :type Client%20Side%20Controller%20Object%20Reference))
  (CallFunction|SendRetos clientSideController))

(event Custom|SendRetos
  (params (ClientSideController :type Client%20Side%20Controller%20Object%20Reference))
  (Default|ReceiveRetosServer ClientSideController (Variables|Default|GetListaDeRetos)))

(event Custom|LogginAtempt
  (params (Username :type String) (Password :type String) (playerController :type Client%20Side%20Controller%20Object%20Reference))
  (bind (_found_ _user) (CallFunction|GetUser "NewEnumerator2" 0 Username playerController))
  (if _found_
    (CallFunction|UpdateUser 0 Username playerController "NewEnumerator2" (Utilities|Struct|MakeUser (.id _user) Username playerController))
    (else
      (CallFunction|AddNewPlayerController Username playerController)))
  (bind _asnetwork_game_mode (Utilities|Casting|CastToNetworkGameMode (Game|GetGameMode)))
  (Default|SendMessage _asnetwork_game_mode (Class|TcpSocketConnection|ConcatBytesBytes (Class|TcpSocketConnection|ToBytes(Byte) (Utilities|Enum|LiteralenumTCPProtocol "NewEnumerator1")) (Class|TcpSocketConnection|ToBytes(Integer) (Utilities|String|Len Username)) (Class|TcpSocketConnection|ToBytes(String) Username) (Class|TcpSocketConnection|ToBytes(Integer) (Utilities|String|Len Password)) (Class|TcpSocketConnection|ToBytes(String) Password))))

(event Custom|SendPlayers
  (params (Client%20Side%20%20%20Controller :type Client%20Side%20Controller%20Object%20Reference%20%28by%20ref%29))
  (bind _names (CallFunction|GetPlayerNames))
  (Default|RecieveUserNamesServer Client%20Side%20%20%20Controller _names))

(event Custom|RetrivePlayers
  (params (Client%20Side%20%20%20Controller :type Client%20Side%20Controller%20Object%20Reference%20%28by%20ref%29))
  (CallFunction|SendPlayers Client%20Side%20%20%20Controller))

(event Custom|LoginRetrievenInformation
  (params (loginInfo :type Array%20of%20Bytes))
  (bind _returnvalue (Class|TcpSocketConnection|MessageReadInt loginInfo))
  (bind _returnvalue_2 (Class|TcpSocketConnection|MessageReadString loginInfo _returnvalue))
  (bind (_found_ _user) (CallFunction|GetUser "NewEnumerator1" 0 _returnvalue_2))
  (if _found_
    (bind _returnvalue_3 (Class|TcpSocketConnection|MessageReadByte loginInfo))
    (if (== _returnvalue_3 1)
      (bind _returnvalue_4 (Class|TcpSocketConnection|MessageReadByte loginInfo))
      (bind _returnvalue_5 (Class|TcpSocketConnection|MessageReadInt loginInfo))
      (bind _returnvalue_6 (Class|TcpSocketConnection|MessageReadString loginInfo _returnvalue_5))
      (bind _returnvalue_7 (Class|TcpSocketConnection|MessageReadInt loginInfo))
      (bind _returnvalue_8 (Class|TcpSocketConnection|MessageReadString loginInfo _returnvalue_7))
      (bind _returnvalue_9 (Class|TcpSocketConnection|MessageReadInt loginInfo))
      (bind _returnvalue_10 (Class|TcpSocketConnection|MessageReadString loginInfo _returnvalue_9))
      (bind _returnvalue_11 (Class|TcpSocketConnection|MessageReadInt loginInfo))
      (bind _returnvalue_12 (Class|TcpSocketConnection|MessageReadString loginInfo _returnvalue_11))
      (bind _returnvalue_13 (Class|TcpSocketConnection|MessageReadInt loginInfo))
      (bind _returnvalue_14 (Class|TcpSocketConnection|MessageReadString loginInfo _returnvalue_13))
      (if (== _returnvalue_4 1)
        (Default|ReturnLogginServer (.PlayerController (Utilities|Struct|BreakUser _user)) true (Utilities|Struct|MakeUserInfo (.ID (Utilities|Struct|BreakUser _user)) (.UserName (Utilities|Struct|BreakUser _user)) (Utilities|String|StringToName _returnvalue_6) (Utilities|String|StringToName _returnvalue_8) "(ID_2_652DDBC544094EA3A624DA870A6FB6A6=0,Name_6_26B28C3349E7825E6BD0BB860DD767F0=\"Secpho\",Descripcion_24_33EDF47445C30234D32CE291439AA909=NSLOCTEXT(\"[55938857445BF7C3D098D69A36DD9FDB]\", \"FFB856E347D41B823FE664802F3B177B\", \"Somos secpho, un cluster de innovación tecnológica formado por empresas, centros tecnológicos y grupos de investigación, expertos en tecnologías fotónicas, que creen firmemente en la colaboración.De ahí que nuestro leitmotiv sea ‘collaborate to innovate’. Porque nadie llega muy lejos yendo solo y únicamente aquellos que colaboran y conectan sus ideas son capaces de llegar adonde no ha llegado nadie.secpho está enfocado en promover la innovación tecnológica mediante la aplicación de tecnologías fotónicas, o tecnologías basadas en la luz, a todo tipo de sectores de nuestra economía. Estas tecnologías van a ser la auténtica revolución del s.XXI y las podemos englobar en los siguientes grupos:Sensores, sistemas de escaneo e imagenSistemas láserSistemas de comunicación, redes y transmisión de datosIluminación avanzadaPantallas y displaysSistemas de energía fotovoltaicasecpho está orientado principalmente a los siguientes sectores de la economía: Salud, Agroalimentación, Cosmética y Estética, Industria Química, sector Farmacéutico, Automoción, Fabricación avanzada, Energía y Medioambiente, Ferroviario, Aeroespacial, defensa y seguridad, Telecomunicaciones, Construcción, Instalaciones científicas y centros de I+D.\"),Logo_22_3072392C48D44DF2D3F47A997016BD40=None,URL_28_9726AC9548205C7C5F9742818CBAB7B9=NSLOCTEXT(\"[55938857445BF7C3D098D69A36DD9FDB]\", \"44BB53C444E1AE7E866478846CE59C0F\", \"http//:www.secpho.org\"),TipodeEntidad_48_7AAAC82E4A3747E701CFD7B5B2F1AB40=NSLOCTEXT(\"[55938857445BF7C3D098D69A36DD9FDB]\", \"AF671F1C4DD04220A3A19A8ED7937FDE\", \"Cluster de empresas\"),Actividad_33_B7A1D4FE48E9E3D6DFC9F1BA41BB7552=NSLOCTEXT(\"[55938857445BF7C3D098D69A36DD9FDB]\", \"C2E0E0E54022A226B1D645B599A705B8\", \"Secpho se dedica a agrupar empresas en el sector de la fotonica\"),Direccion_35_CEACA9F34628C0C0F3E6B6A8C5D31091=NSLOCTEXT(\"[55938857445BF7C3D098D69A36DD9FDB]\", \"48ED59B84F3B174C46FF3C9D4518188C\", \"C/ Milà i Fontanals 14-26, 1º-6ª, 08012 Barcelona\"),Contacto_50_8E0470B046B6E584D5B3F396C3466041=NSLOCTEXT(\"[55938857445BF7C3D098D69A36DD9FDB]\", \"AAC960C04B8F9D7E99D05783B10C94EB\", \"Tel. (+34) 93 783 36 64 - info@secpho.org\"),Tecnologias_46_95B60E92403361EA765E5E8BCDA64C5E=,Sectores_47_E9FA7B954648B724724030A41C5C0C6B=,Cadenadevalor_44_84A3F0DA4B490A670E3F248BD981B590=NSLOCTEXT(\"[55938857445BF7C3D098D69A36DD9FDB]\", \"C758BEB848E13DCFF6AAFCA1C4198B6E\", \"Cadena de valor\"),Empleados-Cargo_49_A87BE6844050D6BA2DA46AA7ADA917D6=(NSLOCTEXT(\"[55938857445BF7C3D098D69A36DD9FDB]\", \"A500AAB941A324E937635AB0993FAD8E\", \"Empleado 1 - Cargo\"),NSLOCTEXT(\"[55938857445BF7C3D098D69A36DD9FDB]\", \"1020B45E4890447054045194A54E614B\", \"Empleado 2 - Cargo\"),NSLOCTEXT(\"[55938857445BF7C3D098D69A36DD9FDB]\", \"4940EB5D487B801DFD9F319A01E49654\", \"Empleado 3 - Cargo\")))" (Utilities|Text|ToText(String) _returnvalue_10) "/Game/Secpholand/UI/Images/Iconos/Captura.Captura" (Utilities|Text|ToText(String) _returnvalue_14) 0 (Utilities|Text|ToText(String) _returnvalue_12) (Utilities|Array|MakeArray "") (Utilities|Array|MakeArray "")) true)
        (else
          (bind _returnvalue_15 (Class|TcpSocketConnection|MessageReadInt loginInfo))
          (bind _returnvalue_16 (Class|TcpSocketConnection|MessageReadByte loginInfo))
          (bind _returnvalue_17 (Class|TcpSocketConnection|MessageReadByte loginInfo))
          (bind _returnvalue_18 (Class|TcpSocketConnection|MessageReadByte loginInfo))
          (bind _returnvalue_19 (Class|TcpSocketConnection|MessageReadByte loginInfo))
          (bind _returnvalue_20 (Class|TcpSocketConnection|MessageReadByte loginInfo))
          (bind _returnvalue_21 (Class|TcpSocketConnection|MessageReadByte loginInfo))
          (bind _returnvalue_22 (Class|TcpSocketConnection|MessageReadByte loginInfo))
          (Default|ReturnLogginServer (.PlayerController (Utilities|Struct|BreakUser _user)) true (Utilities|Struct|MakeUserInfo (.ID (Utilities|Struct|BreakUser _user)) (.UserName (Utilities|Struct|BreakUser _user)) (Utilities|String|StringToName _returnvalue_6) (Utilities|String|StringToName _returnvalue_8) "(ID_2_652DDBC544094EA3A624DA870A6FB6A6=0,Name_6_26B28C3349E7825E6BD0BB860DD767F0=\"Secpho\",Descripcion_24_33EDF47445C30234D32CE291439AA909=NSLOCTEXT(\"[55938857445BF7C3D098D69A36DD9FDB]\", \"D2E756D3408383E523F594A413260319\", \"Somos secpho, un cluster de innovación tecnológica formado por empresas, centros tecnológicos y grupos de investigación, expertos en tecnologías fotónicas, que creen firmemente en la colaboración.De ahí que nuestro leitmotiv sea ‘collaborate to innovate’. Porque nadie llega muy lejos yendo solo y únicamente aquellos que colaboran y conectan sus ideas son capaces de llegar adonde no ha llegado nadie.secpho está enfocado en promover la innovación tecnológica mediante la aplicación de tecnologías fotónicas, o tecnologías basadas en la luz, a todo tipo de sectores de nuestra economía. Estas tecnologías van a ser la auténtica revolución del s.XXI y las podemos englobar en los siguientes grupos:Sensores, sistemas de escaneo e imagenSistemas láserSistemas de comunicación, redes y transmisión de datosIluminación avanzadaPantallas y displaysSistemas de energía fotovoltaicasecpho está orientado principalmente a los siguientes sectores de la economía: Salud, Agroalimentación, Cosmética y Estética, Industria Química, sector Farmacéutico, Automoción, Fabricación avanzada, Energía y Medioambiente, Ferroviario, Aeroespacial, defensa y seguridad, Telecomunicaciones, Construcción, Instalaciones científicas y centros de I+D.\"),Logo_22_3072392C48D44DF2D3F47A997016BD40=None,URL_28_9726AC9548205C7C5F9742818CBAB7B9=NSLOCTEXT(\"[55938857445BF7C3D098D69A36DD9FDB]\", \"B4852E034EC4BECBF326299A1B388331\", \"http//:www.secpho.org\"),TipodeEntidad_48_7AAAC82E4A3747E701CFD7B5B2F1AB40=NSLOCTEXT(\"[55938857445BF7C3D098D69A36DD9FDB]\", \"2278AB3A4428F29448DDB3B0790DDE42\", \"Cluster de empresas\"),Actividad_33_B7A1D4FE48E9E3D6DFC9F1BA41BB7552=NSLOCTEXT(\"[55938857445BF7C3D098D69A36DD9FDB]\", \"93DD5B6C4B8EEF7E823DBCAEB4B2D704\", \"Secpho se dedica a agrupar empresas en el sector de la fotonica\"),Direccion_35_CEACA9F34628C0C0F3E6B6A8C5D31091=NSLOCTEXT(\"[55938857445BF7C3D098D69A36DD9FDB]\", \"DCE62BF84DCF9435FF7DD5A97E8C284E\", \"C/ Milà i Fontanals 14-26, 1º-6ª, 08012 Barcelona\"),Contacto_50_8E0470B046B6E584D5B3F396C3466041=NSLOCTEXT(\"[55938857445BF7C3D098D69A36DD9FDB]\", \"FAB8E55C47CD1DD29C8B57BE33D21A96\", \"Tel. (+34) 93 783 36 64 - info@secpho.org\"),Tecnologias_46_95B60E92403361EA765E5E8BCDA64C5E=,Sectores_47_E9FA7B954648B724724030A41C5C0C6B=,Cadenadevalor_44_84A3F0DA4B490A670E3F248BD981B590=NSLOCTEXT(\"[55938857445BF7C3D098D69A36DD9FDB]\", \"AAA1B50A45FAFBEF43498789459F6D36\", \"Cadena de valor\"),Empleados-Cargo_49_A87BE6844050D6BA2DA46AA7ADA917D6=(NSLOCTEXT(\"[55938857445BF7C3D098D69A36DD9FDB]\", \"C858354841A7EAC4345AC290BC75F19F\", \"Empleado 1 - Cargo\"),NSLOCTEXT(\"[55938857445BF7C3D098D69A36DD9FDB]\", \"74AD115A40F7F7209B57ADBF385A88C4\", \"Empleado 2 - Cargo\"),NSLOCTEXT(\"[55938857445BF7C3D098D69A36DD9FDB]\", \"290FBCCF45E60CFAF1FA47A11E0E2B0B\", \"Empleado 3 - Cargo\")))" (Utilities|Text|ToText(String) _returnvalue_10) "/Game/Secpholand/UI/Images/Iconos/Captura.Captura" (Utilities|Text|ToText(String) _returnvalue_14) _returnvalue_15 (Utilities|Text|ToText(String) _returnvalue_12) (Utilities|Array|MakeArray "") (Utilities|Array|MakeArray "") "" "" "" "" "" "" "" "" "" (Utilities|Struct|MakeAvatar (Math|Conversions|ToBoolean(Integer) (Math|Conversions|ToInteger(Byte) _returnvalue_20)) (Math|Conversions|ToInteger(Byte) _returnvalue_18) (Math|Conversions|ToInteger(Byte) _returnvalue_19) (Math|Conversions|ToInteger(Byte) _returnvalue_17) (Utilities|Enum|ByteToEnumClasseUsuario _returnvalue_16) (Math|Conversions|ToInteger(Byte) _returnvalue_21) (Math|Conversions|ToInteger(Byte) _returnvalue_22))) false)))
      (Development|PrintString "Login successfull")
      (else
        (Default|ReturnLogginServer :self (.PlayerController (Utilities|Struct|BreakUser _user)))
        (Development|PrintString "Login failed")))
    (else
      (Development|PrintString "Error: User not in UserArray"))))

(event Custom|UpdateCharacterCreationInfo
  (params (UserInfo :type User%20Info%20Structure) (playerController :type Client%20Side%20Controller%20Object%20Reference))
  (bind _avatarinfo (Utilities|Struct|BreakUserInfo UserInfo))
  (bind (_male_ _hairtype _haircolor _skincolor _class _beardtype _glasses) (Utilities|Struct|BreakAvatar _avatarinfo))
  (bind (_found_ _user) (CallFunction|GetUser "NewEnumerator2" 0 "" playerController))
  (if _found_
    (bind _asnetwork_game_mode (Utilities|Casting|CastToNetworkGameMode (Game|GetGameMode)))
    (Default|SendMessage _asnetwork_game_mode (Class|TcpSocketConnection|ConcatBytesBytes (Class|TcpSocketConnection|ToBytes(Byte) (Utilities|Enum|LiteralenumTCPProtocol "NewEnumerator3")) (Class|TcpSocketConnection|ToBytes(Integer) (Utilities|String|Len (.UserName (Utilities|Struct|BreakUser _user)))) (Class|TcpSocketConnection|ToBytes(String) (.UserName (Utilities|Struct|BreakUser _user))) (Class|TcpSocketConnection|ToBytes(Integer) (Utilities|String|Len (Utilities|String|Append "UPDATE Users SET PrimerInicio = '0'," " GenderID = '" (Utilities|String|ToString(Integer) (Math|Conversions|ToInteger(Boolean) _male_)) "', SkinID = '" (Utilities|String|ToString(Integer) _skincolor) "', HairID = '" (Utilities|String|ToString(Integer) _hairtype) "', HairColorID = '" (Utilities|String|ToString(Integer) _haircolor) "', ClaseID = '" (Utilities|String|ToString(Integer) (Math|Conversions|ToInteger(Byte) _class)) "', BeardID = '" (Utilities|String|ToString(Integer) _beardtype) "', GlassesID = '" (Utilities|String|ToString(Integer) _glasses) (Utilities|String|MakeLiteralString "' WHERE Username = '") (.UserName (Utilities|Struct|BreakUser _user)) (Utilities|String|MakeLiteralString "'")))) (Class|TcpSocketConnection|ToBytes(String) (Utilities|String|Append "UPDATE Users SET PrimerInicio = '0'," " GenderID = '" (Utilities|String|ToString(Integer) (Math|Conversions|ToInteger(Boolean) _male_)) "', SkinID = '" (Utilities|String|ToString(Integer) _skincolor) "', HairID = '" (Utilities|String|ToString(Integer) _hairtype) "', HairColorID = '" (Utilities|String|ToString(Integer) _haircolor) "', ClaseID = '" (Utilities|String|ToString(Integer) (Math|Conversions|ToInteger(Byte) _class)) "', BeardID = '" (Utilities|String|ToString(Integer) _beardtype) "', GlassesID = '" (Utilities|String|ToString(Integer) _glasses) (Utilities|String|MakeLiteralString "' WHERE Username = '") (.UserName (Utilities|Struct|BreakUser _user)) (Utilities|String|MakeLiteralString "'")))))))

(event Custom|UpdatePassword
  (params (newPassword :type String) (playerController :type Client%20Side%20Controller%20Object%20Reference))
  (bind (_found_ _user) (CallFunction|GetUser "NewEnumerator2" 0 "" playerController))
  (if _found_
    (bind _asnetwork_game_mode (Utilities|Casting|CastToNetworkGameMode (Game|GetGameMode)))
    (Default|SendMessage _asnetwork_game_mode (Class|TcpSocketConnection|ConcatBytesBytes (Class|TcpSocketConnection|ToBytes(Byte) (Utilities|Enum|LiteralenumTCPProtocol "NewEnumerator2")) (Class|TcpSocketConnection|ToBytes(Integer) (Utilities|String|Len (.UserName (Utilities|Struct|BreakUser _user)))) (Class|TcpSocketConnection|ToBytes(String) (.UserName (Utilities|Struct|BreakUser _user))) (Class|TcpSocketConnection|ToBytes(Integer) (Utilities|String|Len (Utilities|String|Append "UPDATE Users SET Password = '" newPassword "' WHERE Username = '" (.UserName (Utilities|Struct|BreakUser _user)) "'"))) (Class|TcpSocketConnection|ToBytes(String) (Utilities|String|Append "UPDATE Users SET Password = '" newPassword "' WHERE Username = '" (.UserName (Utilities|Struct|BreakUser _user)) "'"))))))

(fn ConstructionScript)

(fn GetUser
  (params (lookBy :type UserSearchType%20Enum :default "NewEnumerator0") (ID :type Integer) (UserName :type String) (PlayerController :type Client%20Side%20Controller%20Object%20Reference))
  (bind _array_element (Utilities|Array|ForEachLoopwithBreak (Variables|Default|GetUserArray) :!label _label)
    (:LoopBody
      (switch Utilities|FlowControl|Switch|SwitchonUserSearchType lookBy
        (:NewEnumerator0
          (if (== ID (.id _array_element))
            (LocalVariables|Setfound true :!label _label_2)
            (LocalVariables|SetfoundUser (Utilities|Struct|MakeUser (.id _array_element) (.username _array_element) (.playercontroller _array_element)))
            (goto _label Break)))
        (:NewEnumerator1
          (if (Utilities|Enum|Equal(Enum) UserName (.username _array_element))
            (goto _label_2)))
        (:NewEnumerator2
          (if (== PlayerController (.playercontroller _array_element))
            (goto _label_2)))))
    (:Completed
      (return (LocalVariables|Getfound) (LocalVariables|GetfoundUser)))))

(fn GetPlayerNames
  (bind _newlocalvar_0 (LocalVariables|GetNewLocalVar_0))
  (for _array_element (Variables|Default|GetUserArray)
    (Utilities|Array|Add _newlocalvar_0 (Utilities|String|StringToName (.UserName (Utilities|Struct|BreakUser _array_element)))))
  (return _newlocalvar_0))

(fn UpdateUser
  (params (ID :type Integer) (Username :type String) (playerController :type Client%20Side%20Controller%20Object%20Reference) (SearchBy :type UserSearchType%20Enum :default "NewEnumerator0") (infoToUpdate :type User%20Structure))
  (bind _userarray (Variables|Default|GetUserArray))
  (bind (_array_element _array_index) (Utilities|Array|ForEachLoopwithBreak _userarray :!label _label)
    (:LoopBody
      (switch Utilities|FlowControl|Switch|SwitchonUserSearchType SearchBy
        (:NewEnumerator0
          (if (== ID (.ID (Utilities|Struct|BreakUser _array_element)))
            (LocalVariables|Setfound true :!label _label_2)
            (Utilities|Array|SetArrayElem _userarray _array_index infoToUpdate)
            (goto _label Break)))
        (:NewEnumerator1
          (if (Utilities|Enum|Equal(Enum) Username (.UserName (Utilities|Struct|BreakUser _array_element)))
            (goto _label_2)))
        (:NewEnumerator2
          (if (== playerController (.PlayerController (Utilities|Struct|BreakUser _array_element)))
            (goto _label_2)))))
    (:Completed
      (return (LocalVariables|Getfound)))))

(fn RemoveUser
  (params (ID :type Integer) (Username :type String) (playerController :type Client%20Side%20Controller%20Object%20Reference) (lookBy :type UserSearchType%20Enum :default "NewEnumerator0"))
  (bind _userarray (Variables|Default|GetUserArray))
  (bind (_array_element _array_index) (Utilities|Array|ForEachLoopwithBreak _userarray :!label _label)
    (:LoopBody
      (switch Utilities|FlowControl|Switch|SwitchonUserSearchType lookBy
        (:NewEnumerator0
          (if (== ID (.id _array_element))
            (Utilities|Array|RemoveIndex _userarray _array_index :!label _label_2)
            (goto _label Break)))
        (:NewEnumerator1
          (if (Utilities|Enum|Equal(Enum) Username (.username _array_element))
            (goto _label_2)))
        (:NewEnumerator2
          (if (== playerController (.playercontroller _array_element))
            (goto _label_2)))))))