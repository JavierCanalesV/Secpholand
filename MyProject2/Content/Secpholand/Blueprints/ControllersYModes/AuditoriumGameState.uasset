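; Game state for the auditorium that holds an event room entry flag and a list of allowed usernames.
; An incoming byte message is decoded as a count and string list, then appended to the allowed list.
; The entry query reports whether a username is listed but always returns CanEnter as true, leaving the combined flag-and-list check unused.
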(event Custom|SetCanEnterEventRoom
  (params (NewValue :type Boolean))
  (Variables|Default|SetCanEnterEventRoom NewValue))

(event Custom|ReceiveUsernamesAllowed
  (params (Username :type Array%20of%20Strings))
  ;[1 1 1] Receive Auditorio Usernames
  (for _array_element Username
    (Utilities|Array|Add (Variables|Default|GetUsernamesAllowed) _array_element)))

(event Custom|ReceiveAuditorioUsernames
  (params (Bytes :type Array%20of%20Bytes))
  ;[1 1 1] Receive Auditorio Usernames
  (bind _returnvalue (Class|TcpSocketConnection|MessageReadInt Bytes))
  (bind _stringlist (CallFunction|MakeStringList Bytes _returnvalue))
  (CallFunction|ReceiveUsernamesAllowed _stringlist))

(fn ConstructionScript
  (|CallParentFunction))

(fn GetCanEnterEventRoom
  (params (Username :type String))
  (return true (>= (Utilities|Array|FindItem (Variables|Default|GetUsernamesAllowed) Username) 0)))