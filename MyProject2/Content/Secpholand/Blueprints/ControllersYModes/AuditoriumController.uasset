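; Auditorium controller that handles a player joining or leaving a round table (Mesa Redonda).
; On join, the server binds the player to the presenter avatar tagged with the table ID, and the client creates or updates the call widget with the mic state.
; On leave, the server hides the avatar, and the client removes the call widget without hanging up and mutes non-superusers in certain locations such as the auditorium.
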(event Custom|ReceiveIrAMesaRedonda:Server
  (params (ID :type Integer) (Entrar :type Boolean))
  (if Entrar
    (bind _outactors (Actor|GetAllActorsOfClasswithTag "/Game/Secpholand/Blueprints/Clicables/Avatares/ClicableAvatar_Presentador.ClicableAvatar_Presentador_C" (Utilities|String|StringToName (Utilities|String|Append "MesaRedonda" (Utilities|String|ToString(Integer) ID)))))
    (if (> (Utilities|Array|Length _outactors) 0)
      (CallFunction|SetRepresentativeAvatar (Utilities|Array|Get(acopy) _outactors) false)
      (CallFunction|ReceiveIrAMesaRedonda:Client))
    (else
      (CallFunction|MakeAvatarDisappear)
      (CallFunction|ReceiveSalirMesaRedonda:Client (Utilities|Struct|BreakUserInfo_Private (Variables|Default|GetuserInfo_Private))))))

(event Custom|ReceiveIrAMesaRedonda:Client
  (bind _micactivated (Variables|Default|GetMicActivated))
  (bind (_widget _found) (CallFunction|GetWidgetLlamada))
  (if _found
    (Default|UpdateMicState _widget _micactivated false)
    (else
      (bind _returnvalue (UserInterface|CreateWidget "/Game/Secpholand/UI/Widgets/Llamada.Llamada_C")) ; Si no creamos uno
      (Default|UpdateMicState _returnvalue _micactivated false)
      (Class|VerticalBox|AddChildtoVerticalBox (Variables|/Game/Secpholand/UI/Widgets/HUDYChat/HUD.HUD_C|GetHudArribaizquierda (Variables|Default|GetHUD)) _returnvalue)
      (CallFunction|ModifyWidgetLlamadaBasedonLocation))))

(event Custom|ReceiveSalirMesaRedonda:Client
  (params (SU :type Boolean))
  (bind _serversidecharacterref (Variables|Default|GetServerSideCharacterRef))
  (bind _userinfo (Variables|/Game/Secpholand/Blueprints/ControllersYModes/baseClasses/ServerSide_Character.ServerSide_Character_C|GetUserInfo _serversidecharacterref))
  (bind _ingamelocation (Utilities|Struct|BreakUserInfo_Public _userinfo))
  (if (and (not SU) (Math|Boolean|ORBoolean (Utilities|Enum|Equal(Enum) _ingamelocation "NewEnumerator19") (Utilities|Enum|Equal(Enum) _ingamelocation "NewEnumerator10") (Utilities|Enum|Equal(Enum) _ingamelocation "NewEnumerator9")))
    (CallFunction|QuitarWidgetLlamadaSinColgar)
    (CallFunction|ToggleMic:Server false true)))

(fn ConstructionScript
  (|CallParentFunction))