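; Tutorial player character Blueprint that shows the user's name and company on a nameplate, which can be hidden, and sets up the follow camera.
; On BeginPlay, unless the controller is an InteriorController, it maps the ClientSide_Controller's Zoom to spring arm length and pitch plus camera tilt.
; The same zoom-derived distance, slightly reduced, feeds the OclusionMPC material parameter collection.
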(event Custom|setName
  (bind _userinfo (Variables|Default|GetUserInfo))
  (bind (_id _username _name _userclass _reputationsticker _level _ingamelocation _avatarinfo _tecnologíasquedomina _sectoresqueconoce _empresa) (Utilities|Struct|BreakUserInfo_Public _userinfo))
  (bind _asnombre_player (Utilities|Casting|CastToNombrePlayer (UserInterface|GetUserWidgetObject (Variables|Default|GetnamePlate))))
  (Rendering|Components|TextRender|SetText (Variables|/Game/Secpholand/UI/Widgets/NombrePlayer.NombrePlayer_C|GetNombre _asnombre_player) (Utilities|Text|ToText(String) _username))
  (Rendering|Components|TextRender|SetText (Variables|/Game/Secpholand/UI/Widgets/NombrePlayer.NombrePlayer_C|GetEmpresa _asnombre_player) (Utilities|Text|ToText(Name) (.Name (Utilities|Struct|BreakEmpresa _empresa)))))

(event Custom|hideNamePlate
  (params (hide? :type Boolean))
  (Development|SetHiddeninGame (Variables|Default|GetnamePlate) hide? true))

(event EventBeginPlay
  (bind _returnvalue (Pawn|GetController))
  (bind _springarm (Variables|Default|GetSpringArm))
  (bind _returnvalue_2 (Transformation|GetWorldRotation _springarm))
  (CallFunction|SetName)
  (bind _asclient_side_controller (Utilities|Casting|CastToClientSide_Controller _returnvalue))
  (Utilities|Casting|CastToInteriorController _returnvalue
    (:CastFailed
      (Variables|/Script/Engine.SpringArmComponent|SetTargetArmLength _springarm (Math|Float|Lerp 6e+02 3.1e+03 (Variables|/Game/Secpholand/Blueprints/ControllersYModes/baseClasses/ClientSide_Controller.ClientSide_Controller_C|Getzoom _asclient_side_controller)))
      (Transformation|SetWorldRotation _springarm (Math|Rotator|MakeRotator (.roll _returnvalue_2) (Math|Interpolation|Ease "EaseOut" (Variables|/Game/Secpholand/Blueprints/ControllersYModes/baseClasses/ClientSide_Controller.ClientSide_Controller_C|Getzoom _asclient_side_controller) -15.0 -38.0 6.0) (.yaw _returnvalue_2)) false false)
      (Transformation|SetRelativeRotation (Variables|Default|GetCamera) (Math|Rotator|MakeRotator 0.0 (Math|Float|Lerp 13.0 0.0 (Variables|/Game/Secpholand/Blueprints/ControllersYModes/baseClasses/ClientSide_Controller.ClientSide_Controller_C|Getzoom _asclient_side_controller)) 0.0) false false)
      (Rendering|Material|SetScalarParameterValue "/Game/Secpholand/Assets/Materials/oclusionMPC.oclusionMPC" "Distance" (- (Math|Float|Lerp 6e+02 3.1e+03 (Variables|/Game/Secpholand/Blueprints/ControllersYModes/baseClasses/ClientSide_Controller.ClientSide_Controller_C|Getzoom _asclient_side_controller)) 85.0) :!class /Script/Engine.KismetMaterialLibrary))))

(fn ConstructionScript)