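; Game state for the Secpholand central world that relays shop purchases, kiosk news, job offers, market ads and deprecated office events to a TCP backend.
; Server events pack protocol opcodes and payloads, mostly length-prefixed strings, into bytes sent through NetworkGameMode; news is requested on connect.
; Receive handlers parse replies, update all kiosk, job-offer and market actors or the requesting controller, then return leftover bytes to PendingMessages.
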(event Custom|ReceiveNoticias:Server
  (params (Arrays :type Array%20of%20Bytes))
  ;[1 1 1] Retrieve Noticias
  (bind (_noticiaskiosco _pending) (CallFunction|MakeListNotice Arrays))
  (bind _outactors (Actor|GetAllActorsOfClass "/Game/Secpholand/Blueprints/Clicables/ZoomClicables/KioscoHolograma.KioscoHolograma_C"))
  (for _array_element _outactors
    (Variables|/Game/Secpholand/Blueprints/Clicables/ZoomClicables/KioscoHolograma.KioscoHolograma_C|SetNoticias _array_element _noticiaskiosco))
  (Default|PendingMessages (.AsNetwork%20Game%20Mode (Utilities|Casting|CastToNetworkGameMode (Game|GetGameMode))) _pending))

(event Custom|RetrieveNoticias:Server
  ;[1 1 1] Retrieve Noticias
  (bind _asnetwork_game_mode (Utilities|Casting|CastToNetworkGameMode (Game|GetGameMode)))
  (Default|SendMessage _asnetwork_game_mode (Class|TcpSocketConnection|ToBytes(Byte) (Utilities|Enum|LiteralenumTCPProtocol "NewEnumerator81"))))

(event Custom|ComprarObjetoTienda:Server
  (params (PlayerController :type Client%20Side%20Controller%20Object%20Reference) (Token :type String) (Tipo :type TipoObjetoComprable%20Enum :default "NewEnumerator0") (ID :type Byte) (lambas :type Integer))
  (bind _returnvalue (Class|TcpSocketConnection|ToBytes(String) Token))
  ;[1 1 1] Comprar Objeto en tienda
  (bind (_found_ _user) (CallFunction|GetUser "NewEnumerator2" 0 "" "" PlayerController))
  (if _found_
    (bind _asnetwork_game_mode (Utilities|Casting|CastToNetworkGameMode (Game|GetGameMode)))
    (Default|SendMessage _asnetwork_game_mode (Class|TcpSocketConnection|ConcatBytesBytes (Class|TcpSocketConnection|ToBytes(Byte) (Utilities|Enum|LiteralenumTCPProtocol "NewEnumerator6")) (Class|TcpSocketConnection|ToBytes(Integer) (Utilities|Array|Length (Class|TcpSocketConnection|ToBytes(String) (.username _user)))) (Class|TcpSocketConnection|ToBytes(String) (.username _user)) (Class|TcpSocketConnection|ToBytes(Integer) (Utilities|Array|Length _returnvalue)) _returnvalue (Class|TcpSocketConnection|ToBytes(Byte) Tipo) (Class|TcpSocketConnection|ToBytes(Byte) ID) (Class|TcpSocketConnection|ToBytes(Integer) lambas)))))

(event EventBeginPlay)

(event EventTick
  (params (DeltaSeconds :type Float%20%28single-precision%29)))

(event EventOnServerConnected
  ;[1 1 1] Fuction on server Connect
  (|CallParentFunction)
  (CallFunction|RetrieveNoticias:Server))

(fn ConstructionScript
  (|CallParentFunction))

(fn MakeListNotice
  (params (InputPin :type Array%20of%20Bytes))
  (bind _returnvalue (Class|TcpSocketConnection|MessageReadInt InputPin))
  (for _index (range 0 (- _returnvalue 1))
    (bind _returnvalue_2 (Class|TcpSocketConnection|MessageReadInt InputPin))
    (bind _returnvalue_3 (Class|TcpSocketConnection|MessageReadString InputPin _returnvalue_2))
    (bind _returnvalue_4 (Class|TcpSocketConnection|MessageReadInt InputPin))
    (bind _returnvalue_5 (Class|TcpSocketConnection|MessageReadString InputPin _returnvalue_4))
    (bind _returnvalue_6 (Class|TcpSocketConnection|MessageReadInt InputPin))
    (bind _returnvalue_7 (Class|TcpSocketConnection|MessageReadString InputPin _returnvalue_6))
    (bind _returnvalue_8 (Class|TcpSocketConnection|MessageReadInt InputPin))
    (bind _returnvalue_9 (Class|TcpSocketConnection|MessageReadString InputPin _returnvalue_8))
    (Utilities|Array|Add (LocalVariables|GetNoticiasAux) (Utilities|Struct|MakeNoticiaKiosco _returnvalue_3 _returnvalue_5 _returnvalue_7 _returnvalue_9)))
  (return (LocalVariables|GetNoticiasAux) InputPin))

(event Custom|ReceiveOfertasTrabajos:Server
  (params (message :type Array%20of%20Bytes))
  ;[1 1 1] Retrieve OfertasTrabajo
  (bind (_listofertastrabajo _pending) (CallFunction|MakeOfertasTrabajo message))
  (bind _outactors (Actor|GetAllActorsOfClass "/Game/Secpholand/Blueprints/Clicables/OfertaTrabajo.OfertaTrabajo_C"))
  (for _array_element _outactors
    (Variables|/Game/Secpholand/Blueprints/Clicables/OfertaTrabajo.OfertaTrabajo_C|SetOfertas%20Trabajo _array_element _listofertastrabajo))
  (Default|PendingMessages (.AsNetwork%20Game%20Mode (Utilities|Casting|CastToNetworkGameMode (Game|GetGameMode))) _pending))

(event Custom|ADD_OfertaTrabajo:Server
  (params (PlayerController :type Client%20Side%20Controller%20Object%20Reference) (Token :type String) (Oferta%20Trabajo :type Oferta%20Trabajo%20Structure))
  (bind (_titulo _descripción _empresa _duracióndelcontrato _contacto) (Utilities|Struct|BreakOfertaTrabajo Oferta%20Trabajo))
  (bind _returnvalue (Class|TcpSocketConnection|ToBytes(String) Token))
  (bind _returnvalue_2 (Utilities|String|ToString(Name) "Secpho"))
  (bind _returnvalue_3 (Class|TcpSocketConnection|ToBytes(String) _titulo))
  (bind _returnvalue_4 (Class|TcpSocketConnection|ToBytes(String) _descripción))
  (bind _returnvalue_5 (Class|TcpSocketConnection|ToBytes(String) _returnvalue_2))
  (bind _returnvalue_6 (Class|TcpSocketConnection|ToBytes(String) _duracióndelcontrato))
  (bind _returnvalue_7 (Class|TcpSocketConnection|ToBytes(String) _contacto))
  ;[1 1 1] Ofertas de Trabajo
  (bind (_found_ _user) (CallFunction|GetUser "NewEnumerator2" 0 "" "" PlayerController))
  (if _found_
    (Default|SendMessage (.AsNetwork%20Game%20Mode (Utilities|Casting|CastToNetworkGameMode (Game|GetGameMode))) (Class|TcpSocketConnection|ConcatBytesBytes (Class|TcpSocketConnection|ToBytes(Byte) (Utilities|Enum|LiteralenumTCPProtocol "NewEnumerator75")) (Class|TcpSocketConnection|ToBytes(Integer) (Utilities|Array|Length (Class|TcpSocketConnection|ToBytes(String) (Utilities|Struct|BreakUser _user)))) (Class|TcpSocketConnection|ToBytes(String) (Utilities|Struct|BreakUser _user)) (Class|TcpSocketConnection|ToBytes(Integer) (Utilities|Array|Length _returnvalue)) _returnvalue (Class|TcpSocketConnection|ToBytes(Integer) (Utilities|Array|Length _returnvalue_3)) _returnvalue_3 (Class|TcpSocketConnection|ToBytes(Integer) (Utilities|Array|Length _returnvalue_4)) _returnvalue_4 (Class|TcpSocketConnection|ToBytes(Integer) (Utilities|Array|Length _returnvalue_5)) _returnvalue_5 (Class|TcpSocketConnection|ToBytes(Integer) (Utilities|Array|Length _returnvalue_6)) _returnvalue_6 (Class|TcpSocketConnection|ToBytes(Integer) (Utilities|Array|Length _returnvalue_7)) _returnvalue_7))))

(event Custom|RetrieveOfertasMarkets:Server
  ;[1 1 1] Ofertas Market
  (Default|SendMessage (.AsNetwork%20Game%20Mode (Utilities|Casting|CastToNetworkGameMode (Game|GetGameMode))) (Class|TcpSocketConnection|ToBytes(Byte) (Utilities|Enum|LiteralenumTCPProtocol "NewEnumerator77"))))

(event Custom|ADD_Eventos_Office
  (params (PlayerController :type Client%20Side%20Controller%20Object%20Reference) (Token :type String) (Url :type String) (Img :type String))
  (bind _returnvalue (Class|TcpSocketConnection|ToBytes(String) Token))
  (bind _returnvalue_2 (Class|TcpSocketConnection|ToBytes(String) Url))
  (bind _returnvalue_3 (Class|TcpSocketConnection|ToBytes(String) Img))
  ;[1 0.8948 0] Eventos Office -DEPRECATED
  (bind (_found_ _user) (CallFunction|GetUser "NewEnumerator2" 0 "" "" PlayerController))
  (if _found_
    (Default|SendMessage (.AsNetwork%20Game%20Mode (Utilities|Casting|CastToNetworkGameMode (Game|GetGameMode))) (Class|TcpSocketConnection|ConcatBytesBytes (Class|TcpSocketConnection|ToBytes(Byte) (Utilities|Enum|LiteralenumTCPProtocol "NewEnumerator80")) (Class|TcpSocketConnection|ToBytes(Integer) (Utilities|Array|Length (Class|TcpSocketConnection|ToBytes(String) (Utilities|Struct|BreakUser _user)))) (Class|TcpSocketConnection|ToBytes(String) (Utilities|Struct|BreakUser _user)) (Class|TcpSocketConnection|ToBytes(Integer) (Utilities|Array|Length _returnvalue)) _returnvalue (Class|TcpSocketConnection|ToBytes(Integer) (Utilities|Array|Length _returnvalue_2)) _returnvalue_2 (Class|TcpSocketConnection|ToBytes(Integer) (Utilities|Array|Length _returnvalue_3)) _returnvalue_3))))

(event Custom|RetrieveEventosOffice:Server
  (params (PlayerController :type Client%20Side%20Controller%20Object%20Reference) (Token :type String))
  (bind _returnvalue (Class|TcpSocketConnection|ToBytes(String) Token))
  ;[1 0.8948 0] Eventos Office -DEPRECATED
  (bind (_found_ _user) (CallFunction|GetUser "NewEnumerator2" 0 "" "" PlayerController))
  (if _found_
    (Default|SendMessage (.AsNetwork%20Game%20Mode (Utilities|Casting|CastToNetworkGameMode (Game|GetGameMode))) (Class|TcpSocketConnection|ConcatBytesBytes (Class|TcpSocketConnection|ToBytes(Byte) (Utilities|Enum|LiteralenumTCPProtocol "NewEnumerator79")) (Class|TcpSocketConnection|ToBytes(Integer) (Utilities|Array|Length (Class|TcpSocketConnection|ToBytes(String) (Utilities|Struct|BreakUser _user)))) (Class|TcpSocketConnection|ToBytes(String) (Utilities|Struct|BreakUser _user)) (Class|TcpSocketConnection|ToBytes(Integer) (Utilities|Array|Length _returnvalue)) _returnvalue))))

(event Custom|ReceiveOfertasMarket:Server
  (params (message :type Array%20of%20Bytes))
  ;[1 1 1] Ofertas Market
  (bind (_listofertastrabajo _pending) (CallFunction|MakeOfertasMarket message))
  (bind _outactors (Actor|GetAllActorsOfClass "/Game/Secpholand/Blueprints/Clicables/Market.Market_C"))
  (for _array_element _outactors
    (Variables|/Game/Secpholand/Blueprints/Clicables/Market.Market_C|SetAnuncios _array_element _listofertastrabajo))
  (Default|PendingMessages (.AsNetwork%20Game%20Mode (Utilities|Casting|CastToNetworkGameMode (Game|GetGameMode))) _pending))

(event Custom|ADDOfertasMarket:Server
  (params (PlayerController :type Client%20Side%20Controller%20Object%20Reference) (Token :type String) (Oferta%20Trabajo :type Oferta%20Trabajo%20Structure))
  (bind (_titulo _descripción _contacto) (Utilities|Struct|BreakOfertaTrabajo Oferta%20Trabajo))
  (bind _returnvalue (Class|TcpSocketConnection|ToBytes(String) Token))
  (bind _returnvalue_2 (Class|TcpSocketConnection|ToBytes(String) _titulo))
  (bind _returnvalue_3 (Class|TcpSocketConnection|ToBytes(String) _descripción))
  (bind _returnvalue_4 (Class|TcpSocketConnection|ToBytes(String) _contacto))
  ;[1 1 1] Ofertas Market
  (bind (_found_ _user) (CallFunction|GetUser "NewEnumerator2" 0 "" "" PlayerController))
  (if _found_
    (Default|SendMessage (.AsNetwork%20Game%20Mode (Utilities|Casting|CastToNetworkGameMode (Game|GetGameMode))) (Class|TcpSocketConnection|ConcatBytesBytes (Class|TcpSocketConnection|ToBytes(Byte) (Utilities|Enum|LiteralenumTCPProtocol "NewEnumerator78")) (Class|TcpSocketConnection|ToBytes(Integer) (Utilities|Array|Length (Class|TcpSocketConnection|ToBytes(String) (Utilities|Struct|BreakUser _user)))) (Class|TcpSocketConnection|ToBytes(String) (Utilities|Struct|BreakUser _user)) (Class|TcpSocketConnection|ToBytes(Integer) (Utilities|Array|Length _returnvalue)) _returnvalue (Class|TcpSocketConnection|ToBytes(Integer) (Utilities|Array|Length _returnvalue_2)) _returnvalue_2 (Class|TcpSocketConnection|ToBytes(Integer) (Utilities|Array|Length _returnvalue_3)) _returnvalue_3 (Class|TcpSocketConnection|ToBytes(Integer) (Utilities|Array|Length _returnvalue_4)) _returnvalue_4))))

(event Custom|RetrieveOfertasTrabajos:Server
  ;[1 1 1] Retrieve OfertasTrabajo
  (Default|SendMessage (.AsNetwork%20Game%20Mode (Utilities|Casting|CastToNetworkGameMode (Game|GetGameMode))) (Class|TcpSocketConnection|ToBytes(Byte) (Utilities|Enum|LiteralenumTCPProtocol "NewEnumerator74"))))

(event Custom|ReceiveEventosOffice:Server
  (params (message :type Array%20of%20Bytes))
  ;[1 0.8948 0] Eventos Office -DEPRECATED
  (bind _returnvalue (Class|TcpSocketConnection|MessageReadInt message))
  (bind _returnvalue_2 (Class|TcpSocketConnection|MessageReadString message _returnvalue))
  (bind (_found_ _user) (CallFunction|GetUser "NewEnumerator1" 0 _returnvalue_2))
  (bind _returnvalue_3 (Class|TcpSocketConnection|MessageReadInt message))
  (bind (_stringlist _namelist _pendingbytes) (CallFunction|MakeStringList message _returnvalue_3))
  (bind (_stringlist_2 _namelist_2 _pendingbytes_2) (CallFunction|MakeStringList _pendingbytes _returnvalue_3))
  (if _found_
    (Default|ReceiveEventosOffice:Server (.AsSecpholand%20Central%20Controller (Utilities|Casting|CastToSecpholandCentralController (Utilities|Struct|BreakUser _user))) _stringlist _stringlist_2))
  (Default|PendingMessages (.AsNetwork%20Game%20Mode (Utilities|Casting|CastToNetworkGameMode (Game|GetGameMode))) _pendingbytes_2))