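; Expo player controller that lets users leave contact cards with messages at stand counters (mostradores) and view the cards left there.
; Adding a card routes from client to server event, which stores user and message on the counter and reports the stand interaction with the user's email.
; Viewing cards makes a server round trip that returns the counter's lists to the client, which shows them in a ContenedorDeTarjetas widget.
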(event Custom|Añadir%20tarjeta%20a%20mostrador:Server
  (params (User :type Usuario%20Tarjeta%20Structure) (Mensaje :type String) (RefMostrador :type Mostrador%20EC%20Object%20Reference))
  (Utilities|Array|Add (Variables|/Game/Secpholand/Blueprints/Clicables/MostradorEC.MostradorEC_C|GetTarjetasDejadas RefMostrador) User)
  (Utilities|Array|Add (Variables|/Game/Secpholand/Blueprints/Clicables/MostradorEC.MostradorEC_C|GetMensajes RefMostrador) Mensaje)
  (Default|InteraccionesStandFuction (Variables|Default|GetReportsEPs) (Utilities|String|ToString(Text) (Variables|/Game/Secpholand/Blueprints/clasesBase/ClickableActor.ClickableActor_C|GethoverTitle RefMostrador)) (Utilities|String|ToString(Name) (Variables|/Game/Secpholand/Blueprints/Clicables/MostradorEC.MostradorEC_C|Getempresa RefMostrador)) (Utilities|Struct|BreakUsuarioTarjeta User)))

(event Custom|Añadir%20tarjeta%20a%20mostrador:Client
  (params (User :type Usuario%20Tarjeta%20Structure) (Mensaje :type String) (RefMostrador :type Mostrador%20EC%20Object%20Reference))
  (CallFunction|AñadirTarjetaAMostrador:Server User Mensaje RefMostrador))

(event Custom|Ver%20tarjetas:%20Server
  (params (RefMostrador :type Mostrador%20EC%20Object%20Reference))
  (CallFunction|VerTarjetas:Client (Variables|/Game/Secpholand/Blueprints/Clicables/MostradorEC.MostradorEC_C|GetTarjetasDejadas RefMostrador) (Variables|/Game/Secpholand/Blueprints/Clicables/MostradorEC.MostradorEC_C|GetMensajes RefMostrador)))

(event Custom|Ver%20tarjetas
  (params (RefMostrador :type Mostrador%20EC%20Object%20Reference))
  (CallFunction|VerTarjetas:Server RefMostrador))

(event Custom|Ver%20Tarjetas:Client
  (params (Users :type Array%20of%20Usuario%20Tarjeta%20Structures) (mensajes :type Array%20of%20Strings))
  (bind _returnvalue (UserInterface|CreateWidget "/Game/Secpholand/UI/Widgets/EC/ContenedorDeTarjetas.ContenedorDeTarjetas_C"))
  (Default|FillUsers _returnvalue Users mensajes)
  (UserInterface|Viewport|AddtoViewport _returnvalue 0))

(event EventBeginPlay
  (|CallParentFunction) ; This node is disabled and will not be called.\nDrag off pins to build functionality.
)

(event EventTick
  (params (DeltaSeconds :type Float%20%28single-precision%29))
  (|CallParentFunction DeltaSeconds) ; This node is disabled and will not be called.\nDrag off pins to build functionality.
)

(fn ConstructionScript
  (|CallParentFunction))