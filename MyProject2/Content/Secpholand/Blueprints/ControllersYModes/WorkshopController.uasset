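; Player controller for the workshop mode that joins the player into a group call and lets the view switch between cameras.
; On client spawn it starts the call with HUD widgets, caches tagged left and right cameras, and creates a camera-switch widget.
; View changes blend to those cameras or the original target.
; Presentation screen zoom events hide or restore that widget, and server spawns notify WorkshopGameState of the entering avatar.
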(event Custom|GoToLeftView
  (Game|Player|SetViewTargetwithBlend (Variables|Default|GetCameraLeft) (Variables|Default|GetTiempoTransicion) "VTBlend_EaseInOut" (Variables|Default|GetExponenteTransicion) false)
  (Variables|Default|SetCurrentView 0))

(event Custom|ReturnToOriginalView
  (Game|Player|SetViewTargetwithBlend (Variables|Default|GetPlayerOriginalViewTarget) (Variables|Default|GetTiempoTransicion) "VTBlend_EaseInOut" (Variables|Default|GetExponenteTransicion) false)
  (Variables|Default|SetCurrentView 1))

(event Custom|GoToRightView
  (Game|Player|SetViewTargetwithBlend (Variables|Default|GetCameraRight) (Variables|Default|GetTiempoTransicion) "VTBlend_EaseInOut" (Variables|Default|GetExponenteTransicion) false)
  (Variables|Default|SetCurrentView 2))

(event Custom|ListenForZoomUnZoomEvents
  (bind _pantallapresentacion (Variables|Default|GetPantallaPresentacion))
  (EventDispatchers|BindEventtoHasZoomed _pantallapresentacion (delegate Custom|HideChangeCamUI))
  (EventDispatchers|BindEventtoHasUnZoomed _pantallapresentacion (delegate Custom|ShowChangeCamUI)))

(event Custom|HideChangeCamUI
  (Default|HideAll (Variables|Default|GetUIReference)))

(event Custom|ShowChangeCamUI
  (Default|UpdateHiddenState (Variables|Default|GetUIReference)))

(event Custom|CrearWidgetCambiarCamara
  (bind _returnvalue (UserInterface|CreateWidget "/Game/Secpholand/UI/Widgets/WorkshopCambiarCamara.WorkshopCambiarCamara_C" 0 self))
  (Variables|Default|SetUIReference _returnvalue)
  (Utilities|IsValid _returnvalue
    (:Is%20Valid
      (UserInterface|Viewport|AddtoViewport _returnvalue 0))))

(event Custom|GetCamerasReferences
  (bind _cameraactor (CallFunction|GetCameraActorwithTag "StartCam"))
  (Variables|Default|SetCamaraPosInicial _cameraactor)
  (bind _cameraactor_2 (CallFunction|GetCameraActorwithTag "LeftLocation"))
  (Variables|Default|SetCameraLeft _cameraactor_2)
  (bind _cameraactor_3 (CallFunction|GetCameraActorwithTag "RightLocation"))
  (Variables|Default|SetCameraRight _cameraactor_3))

(event Custom|StartCallWithEveryone
  (bind _hud (Variables|Default|GetHUD))
  (bind _hudarribaizquierda (Variables|/Game/Secpholand/UI/Widgets/HUDYChat/HUD.HUD_C|GetHudArribaizquierda _hud))
  (Utilities|FlowControl|Sequence
    (:then_0
      (CallFunction|EntrarEnLlamada)
      (bind _returnvalue (UserInterface|CreateWidget "/Game/Secpholand/UI/Widgets/Llamada.Llamada_C" 0 "Llamada" false false "0.000000,0.000000,0.000000" true))
      (bind _output_get (Variables|Default|SetLlamada _returnvalue))
      (Class|VerticalBox|AddChildtoVerticalBox _hudarribaizquierda _output_get)
      (bind _returnvalue_2 (UserInterface|CreateWidget "/Game/Secpholand/UI/Widgets/PedirTurnoChat.PedirTurnoChat_C"))
      (Class|VerticalBox|AddChildtoVerticalBox _hudarribaizquierda _returnvalue_2))
    (:then_1
      (Utilities|FlowControl|Delay 3.0)
      (CallFunction|UpdateUsuariosLLamada))))

(event EventPlayerHasBeenSpawn:Client
  (|CallParentFunction)
  (Utilities|FlowControl|Delay 3.0)
  (CallFunction|StartCallwithEveryone)
  (CallFunction|CompleteObjective 1)
  (CallFunction|CrearWidgetCambiarCamara)
  (Variables|Default|SetPlayerOriginalViewTarget (Pawn|GetViewTarget (Game|GetPlayerController 0)))
  (CallFunction|GetCamerasReferences)
  (bind _outactors (Actor|GetAllActorsOfClass "/Game/Secpholand/Blueprints/OtherBP/PantallaPresentación.PantallaPresentación_C"))
  (Variables|Default|SetPantallaPresentacion (Utilities|Array|Get(acopy) _outactors))
  (CallFunction|ListenforZoomUnZoomEvents))

(event EventServerSpawnPlayer
  (params (playerStartIndex :type Player%20Start%20Object%20Reference) (UserInfo :type User%20Info%20Public%20Structure))
  (|CallParentFunction playerStartIndex UserInfo)
  (bind _asworkshop_game_state (Utilities|Casting|CastToWorkshopGameState (Game|GetGameState)))
  (Default|AvatarHasEntered _asworkshop_game_state UserInfo))

(fn ConstructionScript
  (|CallParentFunction))

(fn GetCameraActorwithTag
  (params (Tag :type Name))
  (bind _outactors (Actor|GetAllActorsOfClasswithTag "/Script/Engine.CameraActor" Tag))
  (bind _ascamera_actor (Utilities|Casting|CastToCameraActor (Utilities|Array|Get(acopy) _outactors)))
  (return _ascamera_actor))