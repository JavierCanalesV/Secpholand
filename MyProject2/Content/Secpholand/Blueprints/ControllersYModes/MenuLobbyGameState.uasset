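; Menu lobby GameState for Secpholand that creates guest accounts and emails their credentials.
; CreateInvitedAccount queues the requesting controller by email and sends name, company, email and a random password as a length-prefixed TCP message through NetworkGameMode.
; ReturnCrearCuentaInvitado parses the reply, finds that controller, and either reports the email as taken or sends a TLS welcome email and reports whether sending succeeded.
; Handled requests are then removed from the pending list.
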(event Custom|ReturnCrearCuentaInvitado
  (params (Message :type Array%20of%20Bytes))
  ;[1 1 1] Crear cuenta de Invitado
  (bind _returnvalue (Class|TcpSocketConnection|MessageReadByte Message))
  (bind _returnvalue_2 (Class|TcpSocketConnection|MessageReadByte Message))
  (bind _returnvalue_3 (Class|TcpSocketConnection|MessageReadInt Message))
  (bind _returnvalue_4 (Class|TcpSocketConnection|MessageReadString Message _returnvalue_3))
  (bind _returnvalue_5 (Class|TcpSocketConnection|MessageReadInt Message))
  (bind _returnvalue_6 (Class|TcpSocketConnection|MessageReadString Message _returnvalue_5))
  (bind (_found_ _user) (CallFunction|GetInvitedUser _returnvalue_4))
  (if _found_
    (if (Math|Conversions|ToBoolean(Integer) (Math|Conversions|ToInteger(Byte) _returnvalue))
      (Default|EmailDeInvitadoYaEnUso:Server (.AsMenu%20Lobby%20Controller (Utilities|Casting|CastToMenuLobbyController _user)))
      (else
        (bind _outresult (Class|EmailFL|SendEmailV2 (Class|EmailFL|MakeEmailDetailsfromAsset "Secpholand" "/Game/Secpholand/Blueprints/OtherBP/emailSecpho.emailSecpho" _returnvalue_4 "Cuenta Creada de Secpholand" (Utilities|String|Append "Bienvenido a Secpholand! Ya puedes acceder al entorno virtual con los siguientes credenciales 
 
Nombre de usuario: 
" _returnvalue_4 " 
Contraseña: 
" _returnvalue_6 " 
 
Una vez realices la primera entrada deberás asignar un nombre de usuario y contraseña escogidos por ti.  
 
Si tienes cualquier problema contacta con: 
SecpholandSupport@secpho.org") (Utilities|Array|MakeArray)) "UTF8" "TLS"))
        (Default|InvitedAccSentSuccesfully:Server (.AsMenu%20Lobby%20Controller (Utilities|Casting|CastToMenuLobbyController _user)) (Utilities|Enum|Equal(Enum) _outresult "Success"))))
    (CallFunction|RemoveInvitedUser _returnvalue_4)))

(event Custom|CreateInvitedAccount
  (params (Nombre :type String) (Empresa :type String) (Mail :type String) (controller :type Client%20Side%20Controller%20Object%20Reference))
  (bind _returnvalue (Class|TcpSocketConnection|ToBytes(String) Mail))
  (bind _returnvalue_2 (Class|TcpSocketConnection|ToBytes(String) Nombre))
  (bind _returnvalue_3 (Class|TcpSocketConnection|ToBytes(String) Empresa))
  (bind _randomstring1 (CallFunction|MakeRandomString 12))
  (bind _returnvalue_4 (Class|TcpSocketConnection|ToBytes(String) _randomstring1))
  ;[1 1 1] Crear cuenta de Invitado
  (Utilities|Array|Add (Variables|Default|GetCreatingInvitedUsers) (Utilities|Struct|MakeUser 0 Mail "" controller))
  (Default|SendMessage (.AsNetwork%20Game%20Mode (Utilities|Casting|CastToNetworkGameMode (Game|GetGameMode))) (Class|TcpSocketConnection|ConcatBytesBytes (Class|TcpSocketConnection|ToBytes(Byte) (Utilities|Enum|LiteralenumTCPProtocol "NewEnumerator73")) (Class|TcpSocketConnection|ToBytes(Integer) (Utilities|Array|Length _returnvalue_2)) _returnvalue_2 (Class|TcpSocketConnection|ToBytes(Integer) (Utilities|Array|Length _returnvalue_3)) _returnvalue_3 (Class|TcpSocketConnection|ToBytes(Integer) (Utilities|Array|Length _returnvalue)) _returnvalue (Class|TcpSocketConnection|ToBytes(Integer) (Utilities|Array|Length _returnvalue_4)) _returnvalue_4)))

(fn ConstructionScript
  (|CallParentFunction))

(fn GetInvitedUser
  (params (Mail :type String))
  (for _array_element (Variables|Default|GetCreatingInvitedUsers)
    (if (Utilities|Enum|Equal(Enum) Mail (.UserName (Utilities|Struct|BreakUser _array_element)))
      (return true (.PlayerController (Utilities|Struct|BreakUser _array_element)))))
  (return false 0))

(fn RemoveInvitedUser
  (params (Mail :type String))
  (for (_array_element _array_index) (Variables|Default|GetCreatingInvitedUsers)
    (if (Utilities|Enum|Equal(Enum) Mail (.UserName (Utilities|Struct|BreakUser _array_element)))
      (Utilities|Array|RemoveIndex (Variables|Default|GetCreatingInvitedUsers) _array_index)
      (return))))