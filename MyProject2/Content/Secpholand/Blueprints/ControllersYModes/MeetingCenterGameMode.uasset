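; MeetingCenterGameMode is a game mode for the meeting center that sends requests for a user's personal information over the network.
; RetrievePersonalInformation packs a TCP protocol opcode with length-prefixed username, password, and the player controller's unique ID and IP into one byte array.
; It casts the current game mode to NetworkGameMode and passes the packet to SendMessage; no reply is handled here.
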(event Custom|RetrievePersonalInformation
  (params (Username :type String) (Password :type String) (playerController :type Client%20Side%20Controller%20Object%20Reference))
  (bind _ip (Variables|/Game/Secpholand/Blueprints/ControllersYModes/ClientSide_Controller.ClientSide_Controller_C|Getip playerController))
  (bind _uniqueid (Variables|/Game/Secpholand/Blueprints/ControllersYModes/ClientSide_Controller.ClientSide_Controller_C|GetuniqueID playerController))
  (bind _asnetwork_game_mode (Utilities|Casting|CastToNetworkGameMode (Game|GetGameMode)))
  (Default|SendMessage _asnetwork_game_mode (Class|TcpSocketConnection|ConcatBytesBytes (Class|TcpSocketConnection|ToBytes(Byte) (Utilities|Enum|LiteralenumTCPProtocol "NewEnumerator1")) (Class|TcpSocketConnection|ToBytes(Integer) (Utilities|String|Len Username)) (Class|TcpSocketConnection|ToBytes(String) Username) (Class|TcpSocketConnection|ToBytes(Integer) (Utilities|String|Len Password)) (Class|TcpSocketConnection|ToBytes(String) Password) (Class|TcpSocketConnection|ToBytes(Integer) (Utilities|String|Len _uniqueid)) (Class|TcpSocketConnection|ToBytes(String) _uniqueid) (Class|TcpSocketConnection|ToBytes(Integer) (Utilities|String|Len _ip)) (Class|TcpSocketConnection|ToBytes(String) _ip))))

(event EventBeginPlay
  (|CallParentFunction) ; This node is disabled and will not be called.\nDrag off pins to build functionality.
)

(event EventTick
  (params (DeltaSeconds :type Float%20%28single-precision%29))
  (|CallParentFunction DeltaSeconds) ; This node is disabled and will not be called.\nDrag off pins to build functionality.
)

(fn ConstructionScript
  (|CallParentFunction))