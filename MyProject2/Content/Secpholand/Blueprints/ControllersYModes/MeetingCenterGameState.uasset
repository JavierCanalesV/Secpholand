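; Game state for the Secpholand meeting center, holding challenge ("reto") data and seated-avatar info, plus superuser control of meeting rooms.
; Sends TCP protocol requests through NetworkGameMode to fetch retos, view them or submit proposals.
; Receive events parse byte replies into the RetoInfos and RetoAvatars arrays, returning leftover bytes to PendingMessages.
; Other events edit meeting attendees, grant or revoke the presenter role and mute call participants by room.
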(event Custom|RetrieveRetoInfo
  (params (RetoID :type Integer))
  ;[1 1 1] Reto Info
  (bind _asnetwork_game_mode (Utilities|Casting|CastToNetworkGameMode (Game|GetGameMode)))
  (Default|SendMessage _asnetwork_game_mode (Class|TcpSocketConnection|ConcatBytesBytes (Class|TcpSocketConnection|ToBytes(Byte) (Utilities|Enum|LiteralenumTCPProtocol "NewEnumerator26")) (Class|TcpSocketConnection|ToBytes(Integer) RetoID))))

(event Custom|ReceiveRetoInfo
  (params (bytes :type Array%20of%20Bytes))
  (bind _retoinfos (Variables|Default|GetRetoInfos))
  ;[1 1 1] Reto Info
  (bind (_reto _pendingbytes) (CallFunction|MakeRetoInfo bytes))
  (bind (_found _index) (CallFunction|GetRetoInfo (.SalaDeRetoID (Utilities|Struct|BreakRetoInfo _reto))))
  (if _found
    (Utilities|Array|SetArrayElem _retoinfos _index _reto)
    (else
      (Utilities|Array|Add _retoinfos _reto)))
  (bind _asnetwork_game_mode (Utilities|Casting|CastToNetworkGameMode (Game|GetGameMode)))
  (Default|PendingMessages _asnetwork_game_mode _pendingbytes))

(event Custom|SuperUser:RemoveUsuarioReunion
  (params (NumReunion :type Integer) (UsernameToRemove :type String%20%28by%20ref%29))
  ;[1 1 1] SuperUser:SalasReunion
  (Utilities|Array|RemoveItem (.AsistentesUsernames (Utilities|Struct|BreakreunionMC (Utilities|Array|Get(acopy) (Variables|Default|GetUsernamesEnReuniones) NumReunion))) UsernameToRemove))

(event Custom|SuperUser:AddUsuarioToReunión
  (params (NumReunion :type Integer) (UsernameToAdd :type String%20%28by%20ref%29) (NombreReunion :type String))
  (bind _usernamesenreuniones (Variables|Default|GetUsernamesEnReuniones))
  (bind _output (Utilities|Array|Get(acopy) _usernamesenreuniones NumReunion))
  ;[1 1 1] SuperUser:SalasReunion
  (if (Utilities|Enum|Equal(Enum) NombreReunion "")
    _
    (else
      (Utilities|Struct|SetmembersinreunionMC _output NombreReunion)))
  (Utilities|Array|Add (.AsistentesUsernames (Utilities|Struct|BreakreunionMC _output)) UsernameToAdd))

(event Custom|SuperUser:%20MutearUsuariosEnSala
  (params (SalaID :type Integer) (Mutear? :type Boolean))
  (Development|PrintString "Usuarios encontrados para mutear: ")
  (for _array_element (Utilities|Struct|BreakUsuarioPorLlamada (Utilities|Array|Get(acopy) (Variables|Default|GetUsuarios%20por%20Llamadas) SalaID))
    (Development|PrintString (.Nombre (Utilities|Struct|BreakUsuarioEncontrado _array_element)))
    (bind (_found_ _user) (CallFunction|GetUser "NewEnumerator0" 0 (.Nombre (Utilities|Struct|BreakUsuarioEncontrado _array_element))))
    (if _found_
      (Default|ToggleMic:Server (.PlayerController (Utilities|Struct|BreakUser _user)) (not Mutear?))
      (Default|Server:RequestActualizarWidget (.PlayerController (Utilities|Struct|BreakUser _user)))
      (else
        (Development|PrintString "User not found")))))

(event Custom|SuperUsuario:ResetSalaReunión
  (params (SalaReunion :type Integer))
  ;[1 1 1] SuperUser:SalasReunion
  (Utilities|Struct|SetmembersinreunionMC (Utilities|Array|Get(acopy) (Variables|Default|GetUsernamesEnReuniones) SalaReunion) "" (Utilities|Array|MakeArray)))

(event Custom|Dar%20rol%20presentador
  (params (UserName :type String) (NombreSala/Pantalla :type String) (PresentacionACargar :type String) (NumSlides :type Integer))
  ;[1 1 1] Dar/Quitar Rol Presentador
  (bind (_found_ _user) (CallFunction|GetUser "NewEnumerator0" 0 UserName))
  (if _found_
    (Default|RecibirRolPresentador:Server (.AsInterior%20Controller (Utilities|Casting|CastToInteriorController (.PlayerController (Utilities|Struct|BreakUser _user)))) NombreSala/Pantalla PresentacionACargar NumSlides)))

(event Custom|ReceiveAvatarsToSit
  (params (bytes :type Array%20of%20Bytes))
  (bind _retoavatars (Variables|Default|GetRetoAvatars))
  ;[1 1 1] Avatars To Sit
  (bind (_retoavatars_2 _pendingbytes) (CallFunction|MakeAvatarstoSit bytes))
  (bind (_found _index) (CallFunction|GetRetoAvatars))
  (if _found
    (Utilities|Array|SetArrayElem _retoavatars _index _retoavatars_2)
    (else
      (Utilities|Array|Add _retoavatars _retoavatars_2)))
  (bind _asnetwork_game_mode (Utilities|Casting|CastToNetworkGameMode (Game|GetGameMode)))
  (Default|PendingMessages _asnetwork_game_mode _pendingbytes))

(event Custom|VerReto
  (params (RetoID :type Integer) (User :type Client%20Side%20Controller%20Object%20Reference))
  ;[1 1 1] Ver Reto / Enviar Propuesta
  (bind (_found_ _user) (CallFunction|GetUser "NewEnumerator2" 0 "" "" User))
  (if _found_
    (bind _asnetwork_game_mode (Utilities|Casting|CastToNetworkGameMode (Game|GetGameMode)))
    (Default|SendMessage _asnetwork_game_mode (Class|TcpSocketConnection|ConcatBytesBytes (Class|TcpSocketConnection|ToBytes(Byte) (Utilities|Enum|LiteralenumTCPProtocol "NewEnumerator29")) (Class|TcpSocketConnection|ToBytes(Integer) (Utilities|String|Len (.username _user))) (Class|TcpSocketConnection|ToBytes(String) (.username _user)) (Class|TcpSocketConnection|ToBytes(Integer) RetoID)))))

(event Custom|EnviarPropuesta
  (params (RetoID :type Integer) (User :type Client%20Side%20Controller%20Object%20Reference))
  ;[1 1 1] Ver Reto / Enviar Propuesta
  (bind (_found_ _user) (CallFunction|GetUser "NewEnumerator2" 0 "" "" User))
  (if _found_
    (bind _asnetwork_game_mode (Utilities|Casting|CastToNetworkGameMode (Game|GetGameMode)))
    (Default|SendMessage _asnetwork_game_mode (Class|TcpSocketConnection|ConcatBytesBytes (Class|TcpSocketConnection|ToBytes(Byte) (Utilities|Enum|LiteralenumTCPProtocol "NewEnumerator30")) (Class|TcpSocketConnection|ToBytes(Integer) (Utilities|String|Len (.username _user))) (Class|TcpSocketConnection|ToBytes(String) (.username _user)) (Class|TcpSocketConnection|ToBytes(Integer) RetoID)))))

(event Custom|RetrieveAllRetos
  ;[1 1 1] Init Reto Infos
  (bind _asnetwork_game_mode (Utilities|Casting|CastToNetworkGameMode (Game|GetGameMode)))
  (Default|SendMessage _asnetwork_game_mode (Class|TcpSocketConnection|ConcatBytesBytes (Class|TcpSocketConnection|ToBytes(Byte) (Utilities|Enum|LiteralenumTCPProtocol "NewEnumerator31")) (Class|TcpSocketConnection|ToBytes(Integer)))))

(event Custom|ReceiveAllRetos
  (params (bytes :type Array%20of%20Bytes))
  ;[1 1 1] Init Reto Infos
  (bind _pendingbytes (CallFunction|FillAllRetos bytes))
  (bind _asnetwork_game_mode (Utilities|Casting|CastToNetworkGameMode (Game|GetGameMode)))
  (Default|PendingMessages _asnetwork_game_mode _pendingbytes))

(event Custom|RetrieveAvatarsToSit
  (params (ID :type Integer))
  ;[1 1 1] Avatars To Sit
  (bind _asnetwork_game_mode (Utilities|Casting|CastToNetworkGameMode (Game|GetGameMode)))
  (Default|SendMessage _asnetwork_game_mode (Class|TcpSocketConnection|ConcatBytesBytes (Class|TcpSocketConnection|ToBytes(Byte) (Utilities|Enum|LiteralenumTCPProtocol "NewEnumerator28")) (Class|TcpSocketConnection|ToBytes(Integer) ID))))

(event Custom|Quitar%20rol%20presentador
  (params (UserName :type String))
  ;[1 1 1] Dar/Quitar Rol Presentador
  (bind (_found_ _user) (CallFunction|GetUser "NewEnumerator0" 0 UserName))
  (if _found_
    (Default|RecibirQuitarRolPresentador:Server (.AsInterior%20Controller (Utilities|Casting|CastToInteriorController (.PlayerController (Utilities|Struct|BreakUser _user)))))))

(event EventOnServerConnected
  ;[1 1 1] Initialize Info
  (|CallParentFunction)
  (Utilities|FlowControl|Delay 1.0))

(fn ConstructionScript
  (|CallParentFunction))

(fn MakeRetoInfo
  (params (bytes :type Array%20of%20Bytes))
  (bind _returnvalue (Class|TcpSocketConnection|MessageReadInt bytes))
  (bind _returnvalue_2 (Class|TcpSocketConnection|MessageReadInt bytes))
  (bind _returnvalue_3 (Class|TcpSocketConnection|MessageReadString bytes _returnvalue_2))
  (bind _returnvalue_4 (Class|TcpSocketConnection|MessageReadInt bytes))
  (bind _returnvalue_5 (Class|TcpSocketConnection|MessageReadString bytes _returnvalue_4))
  (bind _returnvalue_6 (Class|TcpSocketConnection|MessageReadInt bytes))
  (bind (_stringlist _namelist _pendingbytes) (CallFunction|MakeStringList bytes _returnvalue_6))
  (LocalVariables|SetpendingBytesAux _pendingbytes)
  (Utilities|FlowControl|Sequence
    (:then_0
      (for _index (range 0 (- _returnvalue_6 1))
        (bind _returnvalue_7 (Class|TcpSocketConnection|MessageReadInt (LocalVariables|GetpendingBytesAux)))
        (bind (_stringlist_2 _namelist_2 _pendingbytes_2) (CallFunction|MakeStringList (LocalVariables|GetpendingBytesAux) _returnvalue_7))
        (LocalVariables|SetpendingBytesAux _pendingbytes_2)
        (Utilities|Array|Add (LocalVariables|GetEspectadoresXEmpresaAux) (Utilities|Struct|MakestringArray _stringlist_2))))
    (:then_1
      (for _index_2 (range 0 (- _returnvalue_6 1))
        (bind _returnvalue_8 (Class|TcpSocketConnection|MessageReadInt (LocalVariables|GetpendingBytesAux)))
        (bind (_stringlist_3 _namelist_3 _pendingbytes_3) (CallFunction|MakeStringList (LocalVariables|GetpendingBytesAux) _returnvalue_8))
        (LocalVariables|SetpendingBytesAux _pendingbytes_3)
        (Utilities|Array|Add (LocalVariables|GetParticipantesSinValidarXEmpresaAux) (Utilities|Struct|MakestringArray _stringlist_3))))
    (:then_2
      (for _index_3 (range 0 (- _returnvalue_6 1))
        (bind _returnvalue_9 (Class|TcpSocketConnection|MessageReadInt (LocalVariables|GetpendingBytesAux)))
        (bind (_stringlist_4 _namelist_4 _pendingbytes_4) (CallFunction|MakeStringList (LocalVariables|GetpendingBytesAux) _returnvalue_9))
        (LocalVariables|SetpendingBytesAux _pendingbytes_4)
        (Utilities|Array|Add (LocalVariables|GetParticipantesValidadosXEmpresaAux) (Utilities|Struct|MakestringArray _stringlist_4))))
    (:then_3
      (bind _returnvalue_10 (Class|TcpSocketConnection|MessageReadInt (LocalVariables|GetpendingBytesAux)))
      (for _index_4 (range 0 (- _returnvalue_10 1))
        (bind _returnvalue_11 (Class|TcpSocketConnection|MessageReadInt (LocalVariables|GetpendingBytesAux)))
        (bind (_stringlist_5 _namelist_5 _pendingbytes_5) (CallFunction|MakeStringList (LocalVariables|GetpendingBytesAux) _returnvalue_11))
        (bind _output_get (LocalVariables|SetpendingBytesAux _pendingbytes_5))
        (bind (_intlist _pendingbytes_6) (CallFunction|MakeIntList _output_get _returnvalue_11))
        (LocalVariables|SetpendingBytesAux _pendingbytes_6)
        (Utilities|Array|Add (LocalVariables|GetPorcentajesDeRequerimientosAux) (Utilities|Struct|MakeRequerimientoReto _namelist_5 _intlist "Req test"))))
    (:then_4
      (LocalVariables|SetAuxReto (Utilities|Struct|MakeRetoInfo _returnvalue _returnvalue_3 _returnvalue_5 _stringlist (LocalVariables|GetEspectadoresXEmpresaAux) (LocalVariables|GetParticipantesSinValidarXEmpresaAux) (LocalVariables|GetParticipantesValidadosXEmpresaAux) (LocalVariables|GetPorcentajesDeRequerimientosAux) 0))
      (return (LocalVariables|GetAuxReto) (LocalVariables|GetpendingBytesAux)))))

(fn MakeAvatarstoSit
  (params (bytes :type Array%20of%20Bytes))
  (bind _output_get (LocalVariables|SetPendingBytesAux bytes))
  (bind _returnvalue (Class|TcpSocketConnection|MessageReadInt _output_get))
  (bind _returnvalue_2 (Class|TcpSocketConnection|MessageReadInt _output_get))
  (Utilities|FlowControl|Sequence
    (:then_0
      (for _index (range 0 (- _returnvalue_2 1))
        (bind _returnvalue_3 (Class|TcpSocketConnection|MessageReadByte (LocalVariables|GetPendingBytesAux)))
        (bind _returnvalue_4 (Class|TcpSocketConnection|MessageReadByte (LocalVariables|GetPendingBytesAux)))
        (bind _returnvalue_5 (Class|TcpSocketConnection|MessageReadByte (LocalVariables|GetPendingBytesAux)))
        (bind _returnvalue_6 (Class|TcpSocketConnection|MessageReadByte (LocalVariables|GetPendingBytesAux)))
        (bind _returnvalue_7 (Class|TcpSocketConnection|MessageReadByte (LocalVariables|GetPendingBytesAux)))
        (bind _returnvalue_8 (Class|TcpSocketConnection|MessageReadByte (LocalVariables|GetPendingBytesAux)))
        (bind _returnvalue_9 (Class|TcpSocketConnection|MessageReadByte (LocalVariables|GetPendingBytesAux)))
        (bind _returnvalue_10 (Class|TcpSocketConnection|MessageReadByte (LocalVariables|GetPendingBytesAux)))
        (Utilities|Array|Add (LocalVariables|GetAvatarsToSitAux) (Utilities|Struct|MakeAvatar (Math|Conversions|ToBoolean(Integer) (Math|Conversions|ToInteger(Byte) _returnvalue_3)) _returnvalue_4 _returnvalue_5 _returnvalue_6 (Utilities|Enum|ByteToEnumClasseUsuario _returnvalue_7) _returnvalue_8 _returnvalue_9 _returnvalue_10))))
    (:then_1
      (bind (_stringlist _namelist _pendingbytes) (CallFunction|MakeStringList (LocalVariables|GetPendingBytesAux) (- _returnvalue_2 1)))
      (LocalVariables|SetPendingBytesAux _pendingbytes)
      (for _array_element _stringlist
        (Utilities|FlowControl|FlipFlop
          (:A
            (Utilities|Array|Add (LocalVariables|GetnameListAux) _array_element))
          (:B
            (Utilities|Array|Add (LocalVariables|GetusernameListAux) _array_element)))))
    (:then_2
      (LocalVariables|SetRetoAvatarsAux (Utilities|Struct|MakeRetoAvatars _returnvalue (LocalVariables|GetAvatarsToSitAux) (LocalVariables|GetusernameListAux) (LocalVariables|GetnameListAux)))
      (return (LocalVariables|GetRetoAvatarsAux) (LocalVariables|GetPendingBytesAux)))))

(fn GetRetoInfo
  (params (RetoID :type Integer))
  (bind (_array_element _array_index) (Utilities|Array|ForEachLoopwithBreak (Variables|Default|GetRetoInfos))
    (:LoopBody
      (if (== (.SalaDeRetoID (Utilities|Struct|BreakRetoInfo _array_element)) RetoID)
        (LocalVariables|SetauxFound true)
        (LocalVariables|SetauxReto _array_element)))
    (:Completed
      (return (LocalVariables|GetauxFound) (LocalVariables|GetauxIndex) (LocalVariables|GetauxReto)))))

(fn GetRetoAvatars
  (params (RetoID :type Integer))
  (bind (_array_element _array_index) (Utilities|Array|ForEachLoopwithBreak (Variables|Default|GetRetoAvatars) :!label _label)
    (:LoopBody
      (if (== (.RetoID (Utilities|Struct|BreakRetoAvatars _array_element)) RetoID)
        (LocalVariables|SetfoundAux true)
        (LocalVariables|SetindexAux _array_index)
        (LocalVariables|SetRetoAvatarAux _array_element)
        (goto _label Break)))
    (:Completed
      (return (LocalVariables|GetfoundAux) (LocalVariables|GetindexAux) (LocalVariables|GetRetoAvatarAux)))))

(fn FillAllRetos
  (params (bytes :type Array%20of%20Bytes))
  (bind _output_get (LocalVariables|SetauxBytes bytes))
  (bind _returnvalue (Class|TcpSocketConnection|MessageReadInt _output_get))
  (for _index (range 0 (- _returnvalue 1))
    (bind (_reto _pendingbytes) (CallFunction|MakeRetoInfo (LocalVariables|GetauxBytes)))
    (LocalVariables|SetauxBytes _pendingbytes)
    (Utilities|Array|SetArrayElem (Variables|Default|GetRetoInfos) _index _reto true)
    (bind (_retoavatars _pendingbytes_2) (CallFunction|MakeAvatarstoSit (LocalVariables|GetauxBytes)))
    (LocalVariables|SetauxBytes _pendingbytes_2)
    (Utilities|Array|SetArrayElem (Variables|Default|GetRetoAvatars) _index _retoavatars true))
  (return (LocalVariables|GetauxBytes)))

(fn ReadBytetoString
  (params (Message :type Array%20of%20Bytes))
  (bind _returnvalue (Class|TcpSocketConnection|MessageReadInt Message))
  (bind _returnvalue_2 (Class|TcpSocketConnection|MessageReadString Message _returnvalue))
  (return _returnvalue_2))