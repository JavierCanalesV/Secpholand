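; Player controller for Secpholand's central world, handling pawn swapping, shop purchases, office events, job offers and marketplace listings.
; Client calls pass a security token to server events: purchases are checked against Lambdas and level, then forwarded with job offers to SecpholandCentralGameState.
; Event and market results return by client RPC to fill their widgets, with bypass flags substituting local test data.
; Server-side event and market retrieval and market posting are empty stubs.
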(event Custom|changePawn
  (params (NewParam :type Flying%20Pawn%202%20Object%20Reference))
  (Pawn|UnPossess)
  (Pawn|Possess NewParam))

(event EventPlayerHasBeenSpawn:Client
  (|CallParentFunction)
  (if (Variables|/Game/Secpholand/Blueprints/ControllersYModes/baseClasses/NetworkGameState.NetworkGameState_C|GetUsingBypasses (.AsNetwork%20Game%20State (Utilities|Casting|CastToNetworkGameState (Game|GetGameState))))
    _))

(event Input|KeyboardEvents|X
  (params (Key :type Key%20Structure :default "None")))

(fn ConstructionScript
  (|CallParentFunction))

(event Custom|ComprarObjetoTienda:Server
  (params (TipoObjeto :type TipoObjetoComprable%20Enum :default "NewEnumerator0") (Id :type Byte) (Token :type String) (Tienda :type Goto%20Tienda%20Object%20Reference))
  (bind _userinfo_private (Variables|Default|GetuserInfo_Private))
  (bind _userinfo_private_2 (Variables|Default|GetuserInfo_Private))
  (bind (_level _lambdas) (Utilities|Struct|BreakUserInfo_Private _userinfo_private))
  (bind (_level_2 _lambdas_2 _objetosadquiridosporcategoria) (Utilities|Struct|BreakUserInfo_Private _userinfo_private_2))
  (Variables|Default|SetTienda Tienda)
  (if (and (<= (.Coste (Utilities|Struct|BreakObjetoTienda (Utilities|Array|Get(acopy) (.Objetos (Utilities|Struct|BreakObjetosDeTiendaPorCategoria (Utilities|Array|Get(acopy) (Variables|/Game/Secpholand/Blueprints/Clicables/GotoTienda.GotoTienda_C|GetObjetosDeLaTiendaPorCategorias (Variables|Default|GetTienda)) (Math|Conversions|ToInteger(Byte) TipoObjeto)))) (Math|Conversions|ToInteger(Byte) Id)))) _lambdas) (>= _level (.NivelMinimo (Utilities|Struct|BreakObjetoTienda (Utilities|Array|Get(acopy) (.Objetos (Utilities|Struct|BreakObjetosDeTiendaPorCategoria (Utilities|Array|Get(acopy) (Variables|/Game/Secpholand/Blueprints/Clicables/GotoTienda.GotoTienda_C|GetObjetosDeLaTiendaPorCategorias (Variables|Default|GetTienda)) (Math|Conversions|ToInteger(Byte) TipoObjeto)))) (Math|Conversions|ToInteger(Byte) Id))))))
    (Utilities|Struct|SetmembersinUserInfo_Private _userinfo_private_2 (- _lambdas (.Coste (Utilities|Struct|BreakObjetoTienda (Utilities|Array|Get(acopy) (.Objetos (Utilities|Struct|BreakObjetosDeTiendaPorCategoria (Utilities|Array|Get(acopy) (Variables|/Game/Secpholand/Blueprints/Clicables/GotoTienda.GotoTienda_C|GetObjetosDeLaTiendaPorCategorias (Variables|Default|GetTienda)) (Math|Conversions|ToInteger(Byte) TipoObjeto)))) (Math|Conversions|ToInteger(Byte) Id))))))
    (Utilities|Array|Add (Utilities|Struct|BreakCategoriaObjetoObtenido (Utilities|Array|Get(acopy) _objetosadquiridosporcategoria (Math|Conversions|ToInteger(Byte) TipoObjeto))) Id)
    (Default|ComprarObjetoTienda:Server (.AsSecpholand%20Central%20Game%20State (Utilities|Casting|CastToSecpholandCentralGameState (Game|GetGameState))) self Token TipoObjeto Id _lambdas_2)))

(event Custom|ComprarObjetoTienda:Client
  (params (TipoObjeto :type TipoObjetoComprable%20Enum :default "NewEnumerator0") (Id :type Byte))
  (bind _userinfo_private (Variables|Default|GetuserInfo_Private))
  (Utilities|Struct|SetmembersinUserInfo_Private _userinfo_private)
  (Utilities|Array|Add (Utilities|Struct|BreakCategoriaObjetoObtenido (Utilities|Array|Get(acopy) (.ObjetosAdquiridosPorCategoria (Utilities|Struct|BreakUserInfo_Private _userinfo_private)) (Math|Conversions|ToInteger(Byte) TipoObjeto))) Id)
  (CallFunction|ComprarObjetoTienda:Server TipoObjeto Id (Variables|/Game/Secpholand/Blueprints/ControllersYModes/baseClasses/NetworkGameInstance.NetworkGameInstance_C|GetsecurityToken (.AsNetwork%20Game%20Instance (Utilities|Casting|CastToNetworkGameInstance (Game|GetGameInstance)))) (Variables|Default|GetTienda)))

(event Custom|RetrieveEventosOffice
  (bind _returnvalue (Game|GetGameState))
  (bind (_array _array2) (|ByPassEventosOffice_2))
  (bind _asnetwork_game_state (Utilities|Casting|CastToNetworkGameState _returnvalue))
  (if (and (Variables|/Game/Secpholand/Blueprints/ControllersYModes/baseClasses/NetworkGameState.NetworkGameState_C|GetUsingBypasses _asnetwork_game_state) (not (Variables|/Game/Secpholand/Blueprints/ControllersYModes/baseClasses/NetworkGameState.NetworkGameState_C|GetUsingByPassesDani _asnetwork_game_state)))
    (CallFunction|ReceiveEventosOffice:Client _array _array2)
    (else
      (CallFunction|RetrieveEventosOffice:Server (Variables|/Game/Secpholand/Blueprints/ControllersYModes/baseClasses/NetworkGameInstance.NetworkGameInstance_C|GetsecurityToken (.AsNetwork%20Game%20Instance (Utilities|Casting|CastToNetworkGameInstance (Game|GetGameInstance))))))))

(event Custom|ReceiveEventosOffice:Server
  (params (Urls :type Array%20of%20Strings) (Imgs :type Array%20of%20Strings))
  (CallFunction|ReceiveEventosOffice:Client Urls Imgs))

(event Custom|ReceiveEventosOffice:Client
  (params (Urls :type Array%20of%20Strings) (Imgs :type Array%20of%20Strings))
  (bind _foundwidgets (Widget|GetAllWidgetsOfClass "/Game/Secpholand/UI/Widgets/OficinaInfo/AgendaEventosOfiInfo.AgendaEventosOfiInfo_C" true))
  (Utilities|IsValid (Utilities|Array|Get(acopy) _foundwidgets)
    (:Is%20Valid
      (Default|FillEventos (Utilities|Array|Get(acopy) _foundwidgets) Urls Imgs))))

(event Custom|RetrieveEventosOffice:Server
  (params (Token :type String)))

(event Custom|ADD_OfertaTrabajo
  (params (Oferta%20Trabajo :type Oferta%20Trabajo%20Structure))
  (CallFunction|ADDOfertaTrabajo:Server (Variables|/Game/Secpholand/Blueprints/ControllersYModes/baseClasses/NetworkGameInstance.NetworkGameInstance_C|GetsecurityToken (.AsNetwork%20Game%20Instance (Utilities|Casting|CastToNetworkGameInstance (Game|GetGameInstance)))) Oferta%20Trabajo))

(event Custom|ADD_OfertaTrabajo:Server
  (params (Token :type String) (Oferta%20Trabajo :type Oferta%20Trabajo%20Structure))
  (Default|ADDOfertaTrabajo:Server (.AsSecpholand%20Central%20Game%20State (Utilities|Casting|CastToSecpholandCentralGameState (Game|GetGameState))) self Token Oferta%20Trabajo))

(event Custom|RetrieveOfertaMarket
  (bind _returnvalue (Game|GetGameState))
  (bind _asnetwork_game_state (Utilities|Casting|CastToNetworkGameState _returnvalue))
  (if (and (Variables|/Game/Secpholand/Blueprints/ControllersYModes/baseClasses/NetworkGameState.NetworkGameState_C|GetUsingBypasses _asnetwork_game_state) (not (Variables|/Game/Secpholand/Blueprints/ControllersYModes/baseClasses/NetworkGameState.NetworkGameState_C|GetUsingByPassesDani _asnetwork_game_state)))
    (CallFunction|ReceiveOfertaMarket:Client (|ByPassMarket_2))
    (else
      (CallFunction|RetrieveOfertaMarket:Server (Variables|/Game/Secpholand/Blueprints/ControllersYModes/baseClasses/NetworkGameInstance.NetworkGameInstance_C|GetsecurityToken (.AsNetwork%20Game%20Instance (Utilities|Casting|CastToNetworkGameInstance (Game|GetGameInstance))))))))

(event Custom|ADD_Oferta_Market:Server
  (params (Token :type String) (Oferta%20Trabajo :type Oferta%20Trabajo%20Structure)))

(event Custom|RetrieveOfertaMarket:Server
  (params (Token :type String)))

(event Custom|ReceiveOfertaMarket:Server
  (params (Ofertas :type Array%20of%20Oferta%20Trabajo%20Structures))
  (CallFunction|ReceiveOfertaMarket:Client Ofertas))

(event Custom|ReceiveOfertaMarket:Client
  (params (Ofertas :type Array%20of%20Oferta%20Trabajo%20Structures))
  (bind _foundwidgets (Widget|GetAllWidgetsOfClass "/Game/Secpholand/UI/Widgets/OficinaInfo/Marketplace2.Marketplace2_C" true))
  (Utilities|IsValid (Utilities|Array|Get(acopy) _foundwidgets)
    (:Is%20Valid
      (Default|FillAnuncios (Utilities|Array|Get(acopy) _foundwidgets) Ofertas))))

(event Custom|ADD_Oferta_Market
  (params (Oferta%20Trabajo :type Oferta%20Trabajo%20Structure))
  (CallFunction|ADDOfertaMarket:Server (Variables|/Game/Secpholand/Blueprints/ControllersYModes/baseClasses/NetworkGameInstance.NetworkGameInstance_C|GetsecurityToken (.AsNetwork%20Game%20Instance (Utilities|Casting|CastToNetworkGameInstance (Game|GetGameInstance)))) Oferta%20Trabajo))