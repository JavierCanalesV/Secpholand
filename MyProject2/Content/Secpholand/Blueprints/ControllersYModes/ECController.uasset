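; ECController is a player controller child class that adds a default movement speed and camera zoom to the pawn.
; Server spawning runs the parent logic, then sets speed through ChangeSpeedServer.
; ZoomCamera keeps a bounded zoom alpha that drives spring arm length, eased arm pitch and camera pitch.
; Each zoom also refreshes nameplates, sets the near clip plane and updates occlusion material parameter collection values.
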(event EventServerSpawnPlayer
  (params (playerStartIndex :type Player%20Start%20Object%20Reference) (UserInfo :type User%20Info%20Public%20Structure))
  (|CallParentFunction playerStartIndex UserInfo)
  (CallFunction|ChangeSpeed:Server 6.5e+02))

(event EventZoomCamera
  (params (ZoomAmount :type Float%20%28single-precision%29))
  (bind _clientsidepawnref (Variables|Default|GetClientSidePawnRef))
  (bind _clientsidepawnref_2 (Variables|Default|GetClientSidePawnRef))
  (bind _springarm (Variables|/Game/Secpholand/Blueprints/ControllersYModes/baseClasses/ClientSide_Pawn.ClientSide_Pawn_C|GetSpringArm _clientsidepawnref_2))
  (bind _springarm_2 (Variables|/Game/Secpholand/Blueprints/ControllersYModes/baseClasses/ClientSide_Pawn.ClientSide_Pawn_C|GetSpringArm _clientsidepawnref))
  (bind _returnvalue (Transformation|GetWorldRotation _springarm))
  (if (and (> (+ ZoomAmount (Variables|Default|Getzoom)) 0.0) (< (+ ZoomAmount (Variables|Default|Getzoom)) 0.8))
    (bind _output_get (Variables|Default|Setzoom (+ ZoomAmount (Variables|Default|Getzoom))))
    (Utilities|IsValid _clientsidepawnref
      (:Is%20Valid
        (Variables|/Script/Engine.SpringArmComponent|SetTargetArmLength _springarm_2 (Math|Float|Lerp 3.5e+02 1.8e+03 _output_get))
        (Transformation|SetWorldRotation _springarm_2 (Math|Rotator|MakeRotator (.roll _returnvalue) (Math|Interpolation|Ease "EaseOut" _output_get -2e+01 -38.0 6.0) (.yaw _returnvalue)) false false)
        (Transformation|SetRelativeRotation (Variables|/Game/Secpholand/Blueprints/ControllersYModes/baseClasses/ClientSide_Pawn.ClientSide_Pawn_C|GetCamera (Variables|Default|GetClientSidePawnRef)) (Math|Rotator|MakeRotator 0.0 (Math|Float|Lerp 15.0 1e+01 _output_get) 0.0) false false)
        (CallFunction|HandleNamePlates)
        (Development|ExecuteConsoleCommand (Utilities|String|Append "r.setNearClipPlane 1" "") 0)
        (Rendering|Material|SetScalarParameterValue "/Game/Secpholand/Assets/Materials/oclusionMPC.oclusionMPC" "Distance" (- (Math|Float|Lerp 6e+02 3.1e+03 (Variables|Default|Getzoom)) 85.0) :!class /Script/Engine.KismetMaterialLibrary)
        (Rendering|Material|SetScalarParameterValue "/Game/Secpholand/Assets/Materials/oclusionMPC.oclusionMPC" "subtr" (Math|Float|Lerp -1.3e+02 -1e+02 (Variables|Default|Getzoom)) :!class /Script/Engine.KismetMaterialLibrary)))))

(fn ConstructionScript
  (|CallParentFunction))