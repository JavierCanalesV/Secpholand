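; CollisionNames is a proximity Box volume that throttles character movement ticking and toggles nameplate visibility.
; Capsule overlaps on ServerSide_Character_2 actors set a faster CharacterMovement tick interval on entry and a slower one on exit.
; AddNameplates and RemoveNameplates set ShowNameplates and show or hide nameplates on overlapping ServerSide_Character actors, a different class from the throttled one.
; Tag-based nameplate toggling logic is present but disconnected.
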(event OnComponentBeginOverlap(Box)
  (params (OverlappedComponent :type Primitive%20Component%20Object%20Reference) (OtherActor :type Actor%20Object%20Reference) (OtherComp :type Primitive%20Component%20Object%20Reference) (OtherBodyIndex :type Integer) (bFromSweep :type Boolean) (SweepResult :type Hit%20Result%20Structure%20%28by%20ref%29))
  (if (== (Utilities|GetClass OtherComp) "/Script/Engine.CapsuleComponent")
    (bind _asserver_side_character_2 (Utilities|Casting|CastToServerSide_Character_2 OtherActor))
    (Class|ActorComponent|SetComponentTickInterval (Variables|/Script/Engine.Character|GetCharacterMovement _asserver_side_character_2) 0.032)))

(event OnComponentEndOverlap(Box)
  (params (OverlappedComponent :type Primitive%20Component%20Object%20Reference) (OtherActor :type Actor%20Object%20Reference) (OtherComp :type Primitive%20Component%20Object%20Reference) (OtherBodyIndex :type Integer))
  (if (== (Utilities|GetClass OtherComp) "/Script/Engine.CapsuleComponent")
    (bind _asserver_side_character_2 (Utilities|Casting|CastToServerSide_Character_2 OtherActor))
    (Class|ActorComponent|SetComponentTickInterval (Variables|/Script/Engine.Character|GetCharacterMovement _asserver_side_character_2) 0.1)))

(event Custom|RemoveNameplates
  (Variables|Default|SetShowNameplates false)
  (for _array_element (Collision|GetOverlappingActors (Variables|Default|GetBox) "/Game/Secpholand/Blueprints/ControllersYModes/baseClasses/ServerSide_Character.ServerSide_Character_C" :!class /Script/Engine.PrimitiveComponent)
    (bind _asserver_side_character (Utilities|Casting|CastToServerSide_Character _array_element))
    (Development|SetHiddeninGame (Variables|/Game/Secpholand/Blueprints/ControllersYModes/baseClasses/ServerSide_Character.ServerSide_Character_C|GetnamePlate _asserver_side_character) true false)))

(event Custom|AddNameplates
  (Variables|Default|SetShowNameplates true)
  (for _array_element (Collision|GetOverlappingActors (Variables|Default|GetBox) "/Game/Secpholand/Blueprints/ControllersYModes/baseClasses/ServerSide_Character.ServerSide_Character_C" :!class /Script/Engine.PrimitiveComponent)
    (bind _asserver_side_character (Utilities|Casting|CastToServerSide_Character _array_element))
    (Development|SetHiddeninGame (Variables|/Game/Secpholand/Blueprints/ControllersYModes/baseClasses/ServerSide_Character.ServerSide_Character_C|GetnamePlate _asserver_side_character) false false)))

(fn ConstructionScript)