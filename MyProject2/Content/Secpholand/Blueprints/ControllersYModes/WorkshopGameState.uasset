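; Game state for the workshop that shows entering users as pre-placed clickable avatars, treated as a pool of seats.
; On BeginPlay it collects and hides the tagged avatars, tracking seat occupancy in a parallel boolean array.
; An entering user gets the first free avatar revealed with their info, while removal finds the seat by username, hides it and frees it.
; An unused test event simulates entrances and removals with delays.
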(event Custom|InitAvatars
  (Utilities|Array|Clear (Variables|Default|GetAvatars))
  (bind _outactors (Actor|GetAllActorsOfClasswithTag "/Game/Secpholand/Blueprints/Clicables/Avatares/ClicableAvatar.ClicableAvatar_C" "AvatarsWorkshop"))
  (for _array_element _outactors
    (bind _asclicable_avatar (Utilities|Casting|CastToClicableAvatar _array_element))
    (Utilities|Array|Add (Variables|Default|GetAvatars) _asclicable_avatar)
    (Default|HideActorandDisableCollision _asclicable_avatar true))
  (Utilities|Array|Resize (Variables|Default|GetAvatarState) (Utilities|Array|Length _outactors)))

(event Custom|SimulateEntrance
  (CallFunction|AvatarHasEntered (Utilities|Struct|MakeUserInfo_Public 0 "User5" "Usuario 5")))

(event Custom|AvatarHasEntered
  (params (UserInfo :type User%20Info%20Public%20Structure))
  (bind _index (CallFunction|GetFirstIndexAvailable))
  (if (!= _index -1)
    (Utilities|Array|SetArrayElem (Variables|Default|GetAvatarState) _index true)
    (Default|HideActorandDisableCollision (Utilities|Array|Get(acopy) (Variables|Default|GetAvatars) _index) false)
    (Default|SetUserInfo (Utilities|Array|Get(acopy) (Variables|Default|GetAvatars) _index) UserInfo)))

(event Custom|RemoveAvatar
  (params (UserInfo :type User%20Info%20Public%20Structure))
  (bind _index (CallFunction|FindIndexbyUserInfo UserInfo))
  (if (!= _index -1)
    (CallFunction|RemoveAvataratIndex _index)))

(event Custom|RemoveAvatarAtIndex
  (params (Index :type Integer))
  (Default|HideActorandDisableCollision (Utilities|Array|Get(acopy) (Variables|Default|GetAvatars) Index) true)
  (Utilities|Array|SetArrayElem (Variables|Default|GetAvatarState) Index false))

(event Custom|TestearFuncionalidad
  (Utilities|FlowControl|Delay 7.0)
  (CallFunction|SimulateEntrance)
  (Utilities|FlowControl|Delay 2.0)
  (CallFunction|SimulateEntrance)
  (Utilities|FlowControl|Delay 2.0)
  (CallFunction|SimulateEntrance)
  (Utilities|FlowControl|Delay 2.0)
  (CallFunction|RemoveAvatar (Utilities|Struct|MakeUserInfo_Public "TestUsername"))
  (Utilities|FlowControl|Delay 2.0)
  (CallFunction|RemoveAvatar (Utilities|Struct|MakeUserInfo_Public "TestUsername"))
  (Utilities|FlowControl|Delay 2.0)
  (CallFunction|RemoveAvatar (Utilities|Struct|MakeUserInfo_Public "User5"))
  (Utilities|FlowControl|Delay 2.0)
  (CallFunction|RemoveAvatar (Utilities|Struct|MakeUserInfo_Public "User5"))
  (Utilities|FlowControl|Delay 2.0)
  (CallFunction|SimulateEntrance)
  (Utilities|FlowControl|Delay 2.0)
  (CallFunction|SimulateEntrance))

(event EventBeginPlay
  (CallFunction|InitAvatars))

(fn ConstructionScript
  (|CallParentFunction))

(fn GetFirstIndexAvailable
  (bind (_array_element _array_index) (Utilities|Array|ForEachLoopwithBreak (Variables|Default|GetAvatarState) :!label _label)
    (:LoopBody
      (if (not _array_element)
        (Utilities|FlowControl|Sequence
          (:then_0
            (goto _label Break))
          (:then_1
            (return _array_index)))))
    (:Completed
      (return -1))))

(fn FindIndexbyUserInfo
  (params (UserInfo :type User%20Info%20Public%20Structure))
  (bind (_array_element _array_index) (Utilities|Array|ForEachLoopwithBreak (Variables|Default|GetAvatars))
    (:LoopBody
      (if (and (Utilities|Array|Get(acopy) (Variables|Default|GetAvatarState) _array_index) (Utilities|Enum|Equal(Enum) (Utilities|Struct|BreakUserInfo_Public (Variables|/Game/Secpholand/Blueprints/Clicables/Avatares/ClicableAvatar.ClicableAvatar_C|GetUserInfo _array_element)) (Utilities|Struct|BreakUserInfo_Public UserInfo)))
        (return _array_index)))
    (:Completed
      (return -1))))