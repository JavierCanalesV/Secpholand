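; Player controller for Secpholand's Meeting Center levels, handling client setup, per-level UI and reto (challenge) screens.
; On spawn it switches to the tagged fixed camera, creates the HUD, then picks exit, first-visit or tutorial UI by level name and user progress.
; It dresses and names seated ClicableAvatars from received data, destroying extras.
; Reto widgets receive hard-coded placeholder participant data, as server retrieval is stubbed or disconnected.
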(event Custom|possesCamera
  (bind _outactors (Actor|GetAllActorswithTag "MCCamera"))
  (bind _ascamera_actor (Utilities|Casting|CastToCameraActor (Utilities|Array|Get(acopy) _outactors)))
  (Game|Player|SetViewTargetwithBlend self _ascamera_actor 0.0 "VTBlend_Linear" 0.0 false)
  (Development|ExecuteConsoleCommand "r.setNearClipPlane 5" 0))

(event Custom|RetrievePersonalInformation
  (bind _asmeeting_center_game_state (Utilities|Casting|CastToMeetingCenterGameState (Game|GetGameState)))
  (Default|RetrievePersonalInfo _asmeeting_center_game_state (Variables|Default|GetuniqueID) self))

(event Custom|ReceiveRetoInfo:Client
  (params (Empresas :type Array%20of%20Names) (EspectadoresXEmpresa :type Array%20of%20String%20Array%20Structures) (ParticipantesSinValidarXEmpresa :type Array%20of%20String%20Array%20Structures) (participantesValidadosXEmpresa :type Array%20of%20String%20Array%20Structures) (PorcentajesDeRequerimientos :type Array%20of%20Porcentaje%20Requerimiento%20Reto%20Structures))
  ;[1 1 1] MeetingCenter EP
  (bind _foundwidgets (Widget|GetAllWidgetsOfClass "/Game/Secpholand/UI/Widgets/MCWidgets/RETO.RETO_C" true))
  (if (> (Utilities|Array|Length _foundwidgets) 0)
    (Default|FillParticipantesInfo (Utilities|Array|Get(acopy) _foundwidgets) Empresas EspectadoresXEmpresa ParticipantesSinValidarXEmpresa participantesValidadosXEmpresa)
    (Default|FillBarrasRequerimientos (Utilities|Array|Get(acopy) _foundwidgets) PorcentajesDeRequerimientos)))

(event Custom|RetrieveRetoInfo:Client
  (params (RetoID :type Integer))
  (bind _array (Utilities|Array|MakeArray "empleado 1 - cargo" "empleado 2 - cargo" "empleado 3 - cargo"))
  (bind _stringarray (Utilities|Struct|MakestringArray _array))
  (bind _stringarray_2 (Utilities|Struct|MakestringArray _array))
  (bind _stringarray_3 (Utilities|Struct|MakestringArray _array))
  (bind _array_2 (Utilities|Array|MakeArray _stringarray _stringarray_2 _stringarray_3))
  ;[1 1 1] MeetingCenter EP
  (CallFunction|ReceiveRetoInfo:Client (Utilities|Array|MakeArray "secpho" "empresa 2" "empresa 3") _array_2 _array_2 _array_2 (Utilities|Array|MakeArray "" "" "" "")))

(event Custom|RetrieveRetoInfo:Server
  (params (RetoID :type Integer))
  ;[1 1 1] MeetingCenter EP
)

(event Custom|ReceiveRetoInfo:Server
  (params (UsersToSit :type Array%20of%20User%20Info%20Public%20Structures) (Empresas :type Array%20of%20Names) (EspectadoresXEmpresa :type Array%20of%20String%20Array%20Structures) (ParticipantesSinValidarXEmpresa :type Array%20of%20String%20Array%20Structures) (participantesValidadosXEmpresa :type Array%20of%20String%20Array%20Structures) (PorcentajesDeRequerimientos :type Array%20of%20Porcentaje%20Requerimiento%20Reto%20Structures))
  (bind _array (Utilities|Array|MakeArray "empleado 1 - cargo" "empleado 2 - cargo" "empleado 3 - cargo"))
  (bind _stringarray (Utilities|Struct|MakestringArray _array))
  (bind _stringarray_2 (Utilities|Struct|MakestringArray _array))
  (bind _stringarray_3 (Utilities|Struct|MakestringArray _array))
  (bind _array_2 (Utilities|Array|MakeArray _stringarray _stringarray_2 _stringarray_3))
  ;[1 1 1] MeetingCenter EP
  (CallFunction|ReceiveRetoInfo:Client (Utilities|Array|MakeArray "secpho" "empresa 2" "empresa 3") _array_2 _array_2 _array_2 (Utilities|Array|MakeArray "" "" "" "")))

(event Custom|RetrieveRetoAvatarsToSit:Client
  (params (ID :type Integer))
  ;[1 1 1] MeetingCenter EP
  (CallFunction|RetrieveRetoAvatarstoSit:Server ID))

(event Custom|RetrieveRetoAvatarsToSit:Server
  (params (ID :type Integer))
  ;[1 1 1] MeetingCenter EP
)

(event Custom|ReceiveRetoAvatarsToSit
  (params (AvatarsToSit :type Array%20of%20Avatar%20Structures) (Names :type Array%20of%20Names))
  ;[1 1 1] MeetingCenter EP
  (bind _outactors (Actor|GetAllActorsOfClass "/Game/Secpholand/Blueprints/Clicables/Avatares/ClicableAvatar.ClicableAvatar_C"))
  (for (_array_element _array_index) _outactors
    (if (<= _array_index (Utilities|Array|LastIndex AvatarsToSit))
      (Default|Dress _array_element (Utilities|Array|Get(acopy) AvatarsToSit _array_index))
      (bind _asnombre_player (Utilities|Casting|CastToNombrePlayer (UserInterface|GetUserWidgetObject (Variables|/Game/Secpholand/Blueprints/Clicables/Avatares/ClicableAvatar.ClicableAvatar_C|GetNombreyEmpresa _array_element))))
      (Rendering|Components|TextRender|SetText (Variables|/Game/Secpholand/UI/Widgets/NombrePlayer.NombrePlayer_C|GetNombre _asnombre_player) (Utilities|Text|ToText(Name) (Utilities|Array|Get(acopy) Names _array_index)))
      (else
        (Actor|DestroyActor _array_element)))))

(event Custom|ManageTutorial
  (Utilities|FlowControl|Delay 1.0)
  (if (== (.Level (Utilities|Struct|BreakUserInfo_Private (Variables|Default|GetuserInfo_Private))) 0)
    (bind _returnvalue (Actor|GetActorOfClass "/Game/Secpholand/Blueprints/Clicables/Avatares/AvatarAyuda.AvatarAyuda_C"))
    (Default|Click _returnvalue self)
    (CallFunction|CheckObjectiveDone/Collected false)))

(event Custom|ReceivePersonalInformation:Server
  (params (User%20info :type User%20Info%20Public%20Structure) (user%20info%20priv :type User%20Info%20Private%20Structure))
  (Variables|Default|SetuserInfo_Private user%20info%20priv)
  (Variables|Default|SetUserInfo User%20info)
  (CallFunction|ServerInitPlayer))

(event Custom|VerReto)

(event Custom|EnviarPropuesta)

(event EventBeginPlay
  (|CallParentFunction)
  (Variables|Default|SetcanRotate? false)
  (Variables|Default|SetcanZoom? false))

(event EventSetControllsConstraints
  (params (CanMove? :type Boolean) (CanRotate? :type Boolean) (CanZoom? :type Boolean) (CanClick? :type Boolean))
  (Variables|Default|SetcanClick? CanClick?))

(event EventClient:Init
  (Variables|Default|SetbShowMouseCursor true)
  (Input|SetInputModeGameandUI self 0 "DoNotLock" false)
  (Utilities|FlowControl|Delay 0.2)
  (Input|SetInputModeGameandUI self 0 "DoNotLock" false)
  (CallFunction|ServerInitPlayer)
  (CallFunction|ReturnLogginServer :LogginSuccessfull true))

(event EventServerInitPlayer
  (bind _asclient_side_pawn (Utilities|Casting|CastToClientSide_Pawn (Pawn|GetControlledPawn)))
  (bind _output_get (Variables|Default|SetClientSidePawnRef _asclient_side_pawn))
  (Variables|/Game/Secpholand/Blueprints/ControllersYModes/baseClasses/ClientSide_Pawn.ClientSide_Pawn_C|SetClientSideControllerRef _output_get self))

(event EventPlayerHasBeenSpawn:Client
  (CallFunction|PossesCamera)
  (Utilities|FlowControl|Delay 1.0)
  (bind _returnvalue (UserInterface|CreateWidget "/Game/Secpholand/UI/Widgets/HUDYChat/HUD.HUD_C" self))
  (bind _output_get (Variables|Default|SetHUD _returnvalue))
  (UserInterface|Viewport|AddtoViewport _output_get 0)
  (if (> (.Level (Utilities|Struct|BreakUserInfo_Private (Variables|Default|GetuserInfo_Private))) 0)
    (bind _returnvalue_2 (Game|GetCurrentLevelName true))
    (switch string _returnvalue_2
      (:Hall_MC
        (if (not (Utilities|Array|Get(acopy) (.TutorialsDoneFlags (Utilities|Struct|BreakUserInfo_Private (Variables|Default|GetuserInfo_Private))) 2))
          (bind _returnvalue_3 (UserInterface|CreateWidget "/Game/Secpholand/UI/Widgets/Tutoriales/PrimeraVezEdificios/PrimeraVezEdificio.PrimeraVezEdificio_C" 0 "NewEnumerator2"))
          (UserInterface|Viewport|AddtoViewport _returnvalue_3 0)
          (bind _returnvalue_4 (UserInterface|CreateWidget "/Game/Secpholand/UI/Widgets/SalirMapa.SalirMapa_C" 0 "01Secpholand2" "Salir a Secpholand central" :!label _label))
          (UserInterface|Viewport|AddtoViewport _returnvalue_4 0)))
      (:Sala_Retos
        (bind _returnvalue_5 (UserInterface|CreateWidget "/Game/Secpholand/UI/Widgets/SalirMapa.SalirMapa_C" 0 "Hall_MC" "Volver al Hall" :!label _label_2))
        (UserInterface|Viewport|AddtoViewport _returnvalue_5 0))
      (:SmallMeetingRoom
        (goto _label_2))
      (:Auditorio
        (if (not (Utilities|Array|Get(acopy) (.TutorialsDoneFlags (Utilities|Struct|BreakUserInfo_Private (Variables|Default|GetuserInfo_Private))) 1))
          (bind _returnvalue_6 (UserInterface|CreateWidget "/Game/Secpholand/UI/Widgets/Tutoriales/PrimeraVezEdificios/PrimeraVezEdificio.PrimeraVezEdificio_C" 0 "NewEnumerator1"))
          (UserInterface|Viewport|AddtoViewport _returnvalue_6 0)
          (goto _label)))
      (:Bolsa_Inversion_Hall
        (if (not (Utilities|Array|Get(acopy) (.TutorialsDoneFlags (Utilities|Struct|BreakUserInfo_Private (Variables|Default|GetuserInfo_Private))) 3))
          (bind _returnvalue_7 (UserInterface|CreateWidget "/Game/Secpholand/UI/Widgets/Tutoriales/PrimeraVezEdificios/PrimeraVezEdificio.PrimeraVezEdificio_C" 0 "NewEnumerator3"))
          (UserInterface|Viewport|AddtoViewport _returnvalue_7 0)
          (goto _label))))
    (else
      ;[1 1 1] Tutoriales
      (bind _returnvalue_8 (Game|GetCurrentLevelName true))
      (switch string _returnvalue_8
        (:Hall_MC
          (CallFunction|Client:CompleteObjective 1)
          (bind _returnvalue_9 (Actor|GetActorOfClass "/Game/Secpholand/Blueprints/Clicables/Avatares/AvatarAyuda.AvatarAyuda_C"))
          (Variables|/Game/Secpholand/Blueprints/Clicables/Avatares/AvatarAyuda.AvatarAyuda_C|SetTextosDeAyuda _returnvalue_9 (Utilities|Array|MakeArray "Hola! bienvenido al meeting center. En este edificio podrás consultar toda la información de los últimos retos tecnológicos que ofrece Secpho. " "Además también podras realizar reuniones concertadas con Secpho.  
Ten en cuenta que a estas salas de reunión solo podras acceder si tienes permisos. " "Has completado el segundo objetivo \"Entrar al Meeting center\". Recuerda recojer tu recompensa en el menú de objetivos." "Para finalizar el tutorial haz click en el ascensor izquierdo para visitar una sala de reto."))
          (Default|UpdateTexts _returnvalue_9)
          (Default|Click _returnvalue_9 self))
        (:Sala_Retos
          (bind _returnvalue_10 (UserInterface|CreateWidget "/Game/Secpholand/UI/Widgets/Tutoriales/TutorialInteracciónRETO.TutorialInteracciónRETO_C" 0 self))
          (UserInterface|Viewport|AddtoViewport _returnvalue_10 0))))))

(fn ConstructionScript
  (|CallParentFunction))