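; Proximity volume that sets the update detail and nameplate visibility of server-side characters based on whether they overlap its Box.
; BeginPlay polls until the client controller's server-side character reference is valid, then sets that character to full-rate updates and enables overlap events.
; Overlapping characters get every-frame movement ticks without mesh update-rate optimizations; leaving restores throttling.
; Overlaps also toggle tagged nameplates while ShowNameplates is on, which Add/RemoveNameplates switch for everyone inside.
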(event OnComponentBeginOverlap(Box)
  (params (OverlappedComponent :type Primitive%20Component%20Object%20Reference) (OtherActor :type Actor%20Object%20Reference) (OtherComp :type Primitive%20Component%20Object%20Reference) (OtherBodyIndex :type Integer) (bFromSweep :type Boolean) (SweepResult :type Hit%20Result%20Structure%20%28by%20ref%29))
  (bind _asserver_side_character (Utilities|Casting|CastToServerSide_Character OtherActor)
    (:then
      (Class|ActorComponent|SetComponentTickInterval (Variables|/Script/Engine.Character|GetCharacterMovement _asserver_side_character) 0.0)
      (Variables|/Script/Engine.SkinnedMeshComponent|SetbEnableUpdateRateOptimizations (Variables|/Script/Engine.Character|GetMesh _asserver_side_character) false))
    (:CastFailed
      _))
  (if (Variables|Default|GetShowNameplates)
    (if (Actor|ActorHasTag OtherActor "NamePlate")
      (bind _asscene_component (Utilities|Casting|CastToSceneComponent (Utilities|Array|Get(acopy) (Actor|GetComponentsbyTag OtherActor "/Script/Engine.ActorComponent" "NamePlate"))))
      (Development|SetHiddeninGame _asscene_component false false))))

(event OnComponentEndOverlap(Box)
  (params (OverlappedComponent :type Primitive%20Component%20Object%20Reference) (OtherActor :type Actor%20Object%20Reference) (OtherComp :type Primitive%20Component%20Object%20Reference) (OtherBodyIndex :type Integer))
  (bind _asserver_side_character (Utilities|Casting|CastToServerSide_Character OtherActor)
    (:then
      (Class|ActorComponent|SetComponentTickInterval (Variables|/Script/Engine.Character|GetCharacterMovement _asserver_side_character) 0.2)
      (Variables|/Script/Engine.SkinnedMeshComponent|SetbEnableUpdateRateOptimizations (Variables|/Script/Engine.Character|GetMesh _asserver_side_character) true))
    (:CastFailed
      _))
  (if (Variables|Default|GetShowNameplates)
    (if (Actor|ActorHasTag OtherActor "NamePlate")
      (bind _asscene_component (Utilities|Casting|CastToSceneComponent (Utilities|Array|Get(acopy) (Actor|GetComponentsbyTag OtherActor "/Script/Engine.ActorComponent" "NamePlate"))))
      (Development|SetHiddeninGame _asscene_component true false))))

(event Custom|RemoveNameplates
  (Variables|Default|SetShowNameplates false)
  (for _array_element (Collision|GetOverlappingActors (Variables|Default|GetBox) "/Game/Secpholand/Blueprints/ControllersYModes/baseClasses/ServerSide_Character.ServerSide_Character_C" :!class /Script/Engine.PrimitiveComponent)
    (bind _asserver_side_character (Utilities|Casting|CastToServerSide_Character _array_element))
    (Development|SetHiddeninGame (Variables|/Game/Secpholand/Blueprints/ControllersYModes/baseClasses/ServerSide_Character.ServerSide_Character_C|GetnamePlate _asserver_side_character) true false)))

(event Custom|AddNameplates
  (Variables|Default|SetShowNameplates true)
  (for _array_element (Collision|GetOverlappingActors (Variables|Default|GetBox) "/Game/Secpholand/Blueprints/ControllersYModes/baseClasses/ServerSide_Character.ServerSide_Character_C" :!class /Script/Engine.PrimitiveComponent)
    (bind _asserver_side_character (Utilities|Casting|CastToServerSide_Character _array_element))
    (Development|SetHiddeninGame (Variables|/Game/Secpholand/Blueprints/ControllersYModes/baseClasses/ServerSide_Character.ServerSide_Character_C|GetnamePlate _asserver_side_character) false false)))

(event EventBeginPlay
  (bind _asclient_side_controller (Utilities|Casting|CastToClientSide_Controller (Game|GetPlayerController 0)))
  (Default|SetMovementUpdateTime _asclient_side_controller)
  (Utilities|IsValid (Variables|/Game/Secpholand/Blueprints/ControllersYModes/baseClasses/ClientSide_Controller.ClientSide_Controller_C|GetServerSideCharacterRef _asclient_side_controller) :!label _label
    (:Is%20Valid
      (Class|ActorComponent|SetComponentTickInterval (Variables|/Script/Engine.Character|GetCharacterMovement (Variables|/Game/Secpholand/Blueprints/ControllersYModes/baseClasses/ClientSide_Controller.ClientSide_Controller_C|GetServerSideCharacterRef _asclient_side_controller)) 0.0)
      (Variables|/Script/Engine.SkinnedMeshComponent|SetbEnableUpdateRateOptimizations (Variables|/Script/Engine.Character|GetMesh (Variables|/Game/Secpholand/Blueprints/ControllersYModes/baseClasses/ClientSide_Controller.ClientSide_Controller_C|GetServerSideCharacterRef _asclient_side_controller)) false)
      (Variables|/Script/Engine.PrimitiveComponent|SetbGenerateOverlapEvents (Variables|Default|GetBox) true))
    (:Is%20Not%20Valid
      (Utilities|FlowControl|Delay 0.2)
      (goto _label))))

(fn ConstructionScript)