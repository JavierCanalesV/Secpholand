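; Main menu player controller that handles player login between client and server.
; On client init it shows the cursor and Loggin widget, then calls ServerInitPlayer to cross-link the controller with its ClientSide_Pawn.
; Login attempts are forwarded to NetworkGameState with the controller as reply target.
; ReturnLogginServer relays the result, user info and character-creation flag through ReturnLogginClient.
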(event EventReturnLogginServer
  (params (LogginSuccessfull :type Boolean) (User%20Info :type User%20Info%20Public%20Structure) (CreateCharactter :type Boolean))
  (CallFunction|ReturnLogginClient LogginSuccessfull User%20Info CreateCharactter))

(event EventClient:Init
  (Variables|Default|SetbShowMouseCursor true)
  (Input|SetInputModeGameandUI self 0 "DoNotLock" false)
  (bind _returnvalue (UserInterface|CreateWidget "/Game/Secpholand/UI/Widgets/OnlineWidgets/Loggin.Loggin_C"))
  (bind _output_get (Variables|Default|SetlogginScreen _returnvalue))
  (UserInterface|Viewport|AddtoViewport _output_get 0)
  (CallFunction|ServerInitPlayer))

(event EventServerInitPlayer
  (bind _asclient_side_pawn (Utilities|Casting|CastToClientSide_Pawn (Pawn|GetControlledPawn)))
  (bind _output_get (Variables|Default|SetClientSidePawnRef _asclient_side_pawn))
  (Variables|/Game/Secpholand/Blueprints/ControllersYModes/baseClasses/ClientSide_Pawn.ClientSide_Pawn_C|SetClientSideControllerRef _output_get self))

(event EventLogginAtemptServer
  (params (Username :type String) (Password :type String))
  (bind _asnetwork_game_state (Utilities|Casting|CastToNetworkGameState (Game|GetGameState)))
  (Default|LogginAtempt _asnetwork_game_state Username Password self))

(fn ConstructionScript
  (|CallParentFunction))