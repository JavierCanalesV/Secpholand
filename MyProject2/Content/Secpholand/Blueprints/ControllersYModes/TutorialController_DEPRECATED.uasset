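; Deprecated player controller for the Secpholand tutorial, linking itself to the tutorial character and handling HUD creation, mouse input and camera rotation.
; Left-click cursor traces either activate a ClickableActor, open a menu for another character, or spawn a decal and navigate to the point.
; Camera input yaws the character's spring arm.
; Zoom, intro cinematic, tutorial manager spawning and hold-to-move gate triggers remain as disconnected, never-executed logic.
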(event EventBeginPlay
  (CallFunction|Client:Init))

(event EventClient:Init
  (CallFunction|SetControllsConstraints false false false false)
  (Variables|Default|SetbShowMouseCursor true)
  (Input|SetInputModeGameandUI self 0 "DoNotLock" false)
  (CallFunction|ServerInitPlayer))

(event EventMovetoLocation
  (params (Location :type Vector :default "0, 0, 0"))
  (AI|Navigation|SimpleMovetoLocation self Location))

(event EventPlayerHasBeenSpawn:Client
  (bind _returnvalue (UserInterface|CreateWidget "/Game/Secpholand/UI/Widgets/HUDYChat/HUD.HUD_C" self))
  (Variables|Default|SetHUD _returnvalue)
  (bind _asserver_side_character_tutorial (Utilities|Casting|CastToServerSide_CharacterTUTORIAL (Game|GetPlayerCharacter 0)))
  (Variables|Default|SettutorialCharRef _asserver_side_character_tutorial)
  (Variables|/Game/Secpholand/Blueprints/ControllersYModes/ServerSide_CharacterTUTORIAL.ServerSide_CharacterTUTORIAL_C|SetclientSideControllerRef _asserver_side_character_tutorial self))

(event EventServerInitPlayer
  (bind _asserver_side_character_tutorial (Utilities|Casting|CastToServerSide_CharacterTUTORIAL (Pawn|GetControlledPawn)))
  (Variables|Default|SettutorialCharRef _asserver_side_character_tutorial)
  (Variables|/Game/Secpholand/Blueprints/ControllersYModes/ServerSide_CharacterTUTORIAL.ServerSide_CharacterTUTORIAL_C|SetclientSideControllerRef (Variables|Default|GettutorialCharRef) self)
  (CallFunction|Server:RetrievePersonalInfo))

(event EventCameraRotation
  (params (deltaT :type Float%20%28single-precision%29))
  (bind _canrotate_ (Variables|Default|GetcanRotate?))
  (bind _tutorialcharref (Variables|Default|GettutorialCharRef))
  (bind _rotateleft (Variables|Default|GetrotateLeft))
  (bind _springarm (Variables|/Game/Secpholand/Blueprints/ControllersYModes/ServerSide_CharacterTUTORIAL.ServerSide_CharacterTUTORIAL_C|GetSpringArm _tutorialcharref))
  (if (and (Variables|Default|GetRMpressed) _canrotate_)
    (Utilities|IsValid _tutorialcharref
      (:Is%20Valid
        (Transformation|AddRelativeRotation _springarm (Math|Rotator|MakeRotator 0.0 0.0 (* (Class|Actor|GetInputAxisKeyValue) 4.0)) false false)))
    (elif _canrotate_
      (if (or (Variables|Default|GetrotateRight) _rotateleft)
        (Transformation|AddRelativeRotation _springarm (Math|Rotator|MakeRotator 0.0 0.0 (select _rotateleft -3.0 3.0)) false false)))))

(event EventTick
  (params (DeltaSeconds :type Float%20%28single-precision%29))
  (|CallParentFunction DeltaSeconds))

(event Input|ActionEvents|InputActionSetDestination
  (params (Key :type Key%20Structure :default "None"))
  (:Pressed
    (Utilities|FlowControl|Gate true) ; enters at Open
  )
  (:Released
    (Utilities|FlowControl|Gate true) ; enters at Close
  ))

(event Input|MouseEvents|LeftMouseButton
  (params (Key :type Key%20Structure :default "None"))
  (bind (_hitresult _returnvalue) (Game|Player|GetHitResultUnderCursorbyChannel "TraceTypeQuery1" true))
  (bind (_bblockinghit _binitialoverlap _time _distance _location _impactpoint _normal _impactnormal _physmat _hitactor) (Collision|BreakHitResult _hitresult))
  (:Pressed
    (if (and (Variables|Default|GetcanClick?) _returnvalue)
      (Utilities|IsValid (Variables|Default|GetClickableClicked)
        (:Is%20Valid
          (if (!= (Variables|Default|GetClickableClicked) _hitactor)
            (Default|ResetClick (Variables|Default|GetClickableClicked))
            (Variables|Default|SetClickableClicked 0)
            (bind _asclickable_actor (Utilities|Casting|CastToClickableActor _hitactor :!label _label)
              (:then
                (bind _output_get (Variables|Default|SetClickableClicked _asclickable_actor))
                (Default|Click _output_get self))
              (:CastFailed
                (bind _asserver_side_character (Utilities|Casting|CastToServerSide_Character _hitactor)
                  (:then
                    (if (!= _asserver_side_character (Variables|Default|GetServerSideCharacterRef))
                      (CallFunction|OpenDesplegableMenuPlayer)
                      (Variables|Default|SetclickedCharacter _asserver_side_character)))
                  (:CastFailed
                    (Utilities|IsValid (Variables|Default|GettutorialCharRef)
                      (:Is%20Valid
                        (if (Variables|Default|GetcanMove?)
                          (CallFunction|SpawnDecal)
                          (CallFunction|CloseDesplegableMenuPlayer)
                          (CallFunction|MovetoLocation _location))))))))))
        (:Is%20Not%20Valid
          (goto _label)))
      (else
        (Development|PrintString "CANT CLICK")))))

(event Input|TouchEvents|InputTouch
  (params (Location :type Vector) (FingerIndex :type ETouchIndex%20Enum))
  (bind _returnvalue (Utilities|Enum|Equal(Enum) FingerIndex "Touch1"))
  (:Pressed
    (if _returnvalue
      (Utilities|FlowControl|Gate true) ; enters at Open
    ))
  (:Released
    (if _returnvalue
      (Utilities|FlowControl|Gate true) ; enters at Close
    )))

(fn ConstructionScript
  (|CallParentFunction))

(fn MovetoHitLocation
  (params (NewParam :type Hit%20Result%20Structure))
  (bind _location (Collision|BreakHitResult NewParam))
  (if (>= (Math|Vector|VectorLength (- (Transformation|GetActorLocation (Pawn|GetControlledPawn)) _location)) 0.1) ; Don't move if player clicks too close to pawn
    (AI|Navigation|SimpleMovetoLocation self _location)))