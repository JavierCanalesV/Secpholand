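; Client-side camera pawn with a spring-arm view and a switchable bird's-eye view.
; On BeginPlay, unless possessed by a MeetingCenterController, the ClientSide_Controller's Zoom sets arm length, pitch, near clip plane and occlusion MPC distance.
; VistaDePajaro plays a timeline blending the camera from its original transform to a fixed overhead one while brightening the outline MPC's emissive.
; vistaDeCalle reverses that timeline to return to street view.
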(event Custom|VistaDePajaro
  (Variables|Default|Setb_VistaPajaro true)
  (bind _newtrack_0 (Timeline|VistaPajaro Play)
    (:Update
      (Transformation|SetWorldLocationAndRotation (Variables|Default|GetCamera) (.location (Math|Transform|Lerp(Transform) (Transformation|GetWorldTransform (Variables|Default|GetCameraOrighinalPos)) (Math|Transform|MakeTransform "0, 0,12000.000000" "-90.000000, 0, 0") _newtrack_0)) (.rotation (Math|Transform|Lerp(Transform) (Transformation|GetWorldTransform (Variables|Default|GetCameraOrighinalPos)) (Math|Transform|MakeTransform "0, 0,12000.000000" "-90.000000, 0, 0") _newtrack_0)) false false)
      (Rendering|Material|SetVectorParameterValue "/Game/ImportedContent/OutLineMaterals/OutlineParameters.OutlineParameters" "EmissiveOutline" (Utilities|Struct|MakeLinearColor (+ (* _newtrack_0 5e+01) 12.0) (+ (* _newtrack_0 5e+01) 12.0) (+ (* _newtrack_0 5e+01) 12.0) (+ (* _newtrack_0 5e+01) 12.0)) :!class /Script/Engine.KismetMaterialLibrary))
    (:Finished
      (if (Variables|Default|Getb_VistaPajaro)
        _))))

(event Custom|vistaDeCalle
  (Variables|Default|Setb_VistaPajaro false)
  (bind _newtrack_0 (Timeline|VistaPajaro Reverse)
    (:Update
      (Transformation|SetWorldLocationAndRotation (Variables|Default|GetCamera) (.location (Math|Transform|Lerp(Transform) (Transformation|GetWorldTransform (Variables|Default|GetCameraOrighinalPos)) (Math|Transform|MakeTransform "0, 0,12000.000000" "-90.000000, 0, 0") _newtrack_0)) (.rotation (Math|Transform|Lerp(Transform) (Transformation|GetWorldTransform (Variables|Default|GetCameraOrighinalPos)) (Math|Transform|MakeTransform "0, 0,12000.000000" "-90.000000, 0, 0") _newtrack_0)) false false)
      (Rendering|Material|SetVectorParameterValue "/Game/ImportedContent/OutLineMaterals/OutlineParameters.OutlineParameters" "EmissiveOutline" (Utilities|Struct|MakeLinearColor (+ (* _newtrack_0 5e+01) 12.0) (+ (* _newtrack_0 5e+01) 12.0) (+ (* _newtrack_0 5e+01) 12.0) (+ (* _newtrack_0 5e+01) 12.0)) :!class /Script/Engine.KismetMaterialLibrary))
    (:Finished
      (if (Variables|Default|Getb_VistaPajaro)
        _))))

(event EventBeginPlay
  (bind _returnvalue (Pawn|GetController))
  (bind _springarm (Variables|Default|GetSpringArm))
  (bind _returnvalue_2 (Transformation|GetWorldRotation _springarm))
  (Components|Timeline|SetPlayRate (Variables|Default|GetVistaPajaro) 0.4)
  (bind _asclient_side_controller (Utilities|Casting|CastToClientSide_Controller _returnvalue))
  (Utilities|Casting|CastToMeetingCenterController _returnvalue
    (:CastFailed
      (Variables|/Script/Engine.SpringArmComponent|SetTargetArmLength _springarm (Math|Float|Lerp 6e+02 3.1e+03 (Variables|/Game/Secpholand/Blueprints/ControllersYModes/ClientSide_Controller.ClientSide_Controller_C|Getzoom _asclient_side_controller)))
      (Transformation|SetWorldRotation _springarm (Math|Rotator|MakeRotator (.roll _returnvalue_2) (Math|Interpolation|Ease "EaseOut" (Variables|/Game/Secpholand/Blueprints/ControllersYModes/ClientSide_Controller.ClientSide_Controller_C|Getzoom _asclient_side_controller) -15.0 -38.0 6.0) (.yaw _returnvalue_2)) false false)
      (Transformation|SetRelativeRotation (Variables|Default|GetCamera) (Math|Rotator|MakeRotator 0.0 (Math|Float|Lerp 13.0 0.0 (Variables|/Game/Secpholand/Blueprints/ControllersYModes/ClientSide_Controller.ClientSide_Controller_C|Getzoom _asclient_side_controller)) 0.0) false false)
      (Development|ExecuteConsoleCommand (Utilities|String|Append "r.setNearClipPlane " (Utilities|String|ToString(Float) (Math|Float|Lerp 4.3e+02 8e+02 (Variables|/Game/Secpholand/Blueprints/ControllersYModes/ClientSide_Controller.ClientSide_Controller_C|Getzoom _asclient_side_controller)))) 0)
      (Rendering|Material|SetScalarParameterValue "/Game/Secpholand/Assets/Materials/oclusionMPC.oclusionMPC" "Distance" (- (Math|Float|Lerp 6e+02 3.1e+03 (Variables|/Game/Secpholand/Blueprints/ControllersYModes/ClientSide_Controller.ClientSide_Controller_C|Getzoom _asclient_side_controller)) 85.0) :!class /Script/Engine.KismetMaterialLibrary))))

(fn ConstructionScript)