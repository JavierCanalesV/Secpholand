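; AvatarModel is an avatar Blueprint with adjustable hair and skin colors and animated zoom positions.
; The construction script creates the skin dynamic material, and color events set its Color parameter or the hair material's.
; Two reversible timelines lerp the skeletal mesh between offsets from InitialLoc for two zoom stages, moving the model itself.
; BeginPlay is empty; setup of the hair/beard material and InitialLoc sits in unconnected nodes that never run.
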(event Custom|updatePielColor
  (params (NewParam :type Linear%20Color%20Structure))
  (Rendering|Material|SetVectorParameterValue (Variables|Default|GetskinColor) "Color" NewParam :!class /Script/Engine.MaterialInstanceDynamic))

(event Custom|ZoomIn
  (bind _initialloc (Variables|Default|GetinitialLoc))
  (bind _newtrack_0 (Timeline|zoom Play)
    (:Update
      (Transformation|SetRelativeLocation (Variables|Default|GetSkeletalMesh) (Math|Vector|Lerp(Vector) _initialloc (- _initialloc "120.000000,60.000000,65.000000") _newtrack_0) false false))))

(event Custom|ChangeHairColor
  (params (NewParam :type Linear%20Color%20Structure))
  (Rendering|Material|SetVectorParameterValue (Variables|Default|GetPeloColor) "Color" NewParam :!class /Script/Engine.MaterialInstanceDynamic))

(event Custom|ZoomOut
  (bind _initialloc (Variables|Default|GetinitialLoc))
  (bind _newtrack_0 (Timeline|zoom Reverse)
    (:Update
      (Transformation|SetRelativeLocation (Variables|Default|GetSkeletalMesh) (Math|Vector|Lerp(Vector) _initialloc (- _initialloc "120.000000,60.000000,65.000000") _newtrack_0) false false))))

(event Custom|Zoom%203rd
  (bind _initialloc (Variables|Default|GetinitialLoc))
  (bind _returnvalue (- _initialloc "120.000000,60.000000,65.000000"))
  (bind _newtrack_0 (Timeline|Timeline_0 Play)
    (:Update
      (Transformation|SetRelativeLocation (Variables|Default|GetSkeletalMesh) (Math|Vector|Lerp(Vector) _returnvalue (+ _returnvalue "220.000000,190.000000,80.000000") _newtrack_0) false false))))

(event Custom|ZoomOutt3rd
  (bind _initialloc (Variables|Default|GetinitialLoc))
  (bind _returnvalue (- _initialloc "120.000000,60.000000,65.000000"))
  (bind _newtrack_0 (Timeline|Timeline_0 Reverse)
    (:Update
      (Transformation|SetRelativeLocation (Variables|Default|GetSkeletalMesh) (Math|Vector|Lerp(Vector) _returnvalue (+ _returnvalue "220.000000,190.000000,80.000000") _newtrack_0) false false))))

(event EventBeginPlay)

(fn ConstructionScript
  (bind _returnvalue (Rendering|Material|CreateDynamicMaterialInstance (Variables|Default|GetSkeletalMesh) 0 "/Game/Secpholand/Assets/Prototipo/Materiales/BaseColor_Inst.BaseColor_Inst" "None" :!class /Script/Engine.PrimitiveComponent))
  (bind _output_get (Variables|Default|SetskinColor _returnvalue))
  (Rendering|Material|SetVectorParameterValue _output_get "Color" "(R=0.976471,G=0.650980,B=0.435294,A=1.000000)" :!class /Script/Engine.MaterialInstanceDynamic))