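; Short-lived auto-tuner actor that picks a graphics quality level from measured frame time at BeginPlay.
; It averages six delta-time samples taken 0.3s apart, then moves the player controller's saved level one or two steps using millisecond thresholds.
; Changes update GraphicQuality and apply scalability, AA and screen-percentage console commands.
; It resamples after the first change and self-destroys after a second or when frame time is acceptable.
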(event Custom|AdjustSettings
  (bind _returnvalue (Game|GetPlayerController 0))
  (bind _asclient_side_controller (Utilities|Casting|CastToClientSide_Controller _returnvalue))
  (bind _settings (Variables|/Game/Secpholand/Blueprints/ControllersYModes/baseClasses/ClientSide_Controller.ClientSide_Controller_C|Getsettings _asclient_side_controller))
  (switch int (Variables|Default|GetcurrentGraphicLevel)
    (:0
      (Utilities|Struct|SetmembersinSettingValues _settings 0)
      (Development|ExecuteConsoleCommand "sg.PostProcessQuality 0" 0)
      (Development|ExecuteConsoleCommand "sg.TextureQuality 0" 0)
      (Development|ExecuteConsoleCommand "r.PostProcessAAQuality 0" 0)
      (Development|ExecuteConsoleCommand "sg.ShadowQuality 0" 0)
      (Development|ExecuteConsoleCommand "r.ScreenPercentage 75" 0))
    (:1
      (Utilities|Struct|SetmembersinSettingValues _settings 1)
      (Development|ExecuteConsoleCommand "sg.PostProcessQuality 0" 0)
      (Development|ExecuteConsoleCommand "sg.TextureQuality 0" 0)
      (Development|ExecuteConsoleCommand "r.PostProcessAAQuality 0" 0)
      (Development|ExecuteConsoleCommand "sg.ShadowQuality 0" 0)
      (Development|ExecuteConsoleCommand "r.ScreenPercentage 100" 0 :!label _label))
    (:2
      (Utilities|Struct|SetmembersinSettingValues _settings 2)
      (Development|ExecuteConsoleCommand "sg.PostProcessQuality 1" 0)
      (Development|ExecuteConsoleCommand "sg.TextureQuality 1" 0)
      (Development|ExecuteConsoleCommand "r.PostProcessAAQuality 2" 0)
      (Development|ExecuteConsoleCommand "sg.ShadowQuality 1" 0)
      (goto _label))
    (:3
      (Utilities|Struct|SetmembersinSettingValues _settings 3)
      (Development|ExecuteConsoleCommand "sg.PostProcessQuality 3" 0)
      (Development|ExecuteConsoleCommand "sg.TextureQuality 3" 0)
      (Development|ExecuteConsoleCommand "r.PostProcessAAQuality 6" 0)
      (Development|ExecuteConsoleCommand "sg.ShadowQuality 3" 0)
      (goto _label)))
  (Variables|Default|SetCounterFrames 0)
  (Variables|Default|SetAverageDeltaT 0.0)
  (if (Variables|Default|GetfirstIteration)
    (Actor|DestroyActor)
    (else
      (Variables|Default|SetfirstIteration true)
      (CallFunction|SampleDeltaT))))

(event Custom|SampleDeltaT
  (if (< (Variables|Default|GetCounterFrames) 5)
    (Variables|Default|SetAverageDeltaT (+ (Utilities|Time|GetWorldDeltaSeconds) (Variables|Default|GetAverageDeltaT)))
    (Math|Integer|IncrementInt (Variables|Default|GetCounterFrames)
      (:%20%20
        (Utilities|FlowControl|Delay 0.3)
        (CallFunction|SampleDeltaT)))
    (else
      (Variables|Default|SetAverageDeltaT (+ (Utilities|Time|GetWorldDeltaSeconds) (Variables|Default|GetAverageDeltaT)))
      (if (> (* (Variables|Default|GetAverageDeltaT) 166.667007) 6e+01)
        (Math|Integer|DecrementInt (Variables|Default|GetcurrentGraphicLevel)
          (:%20%20
            (Math|Integer|DecrementInt (Variables|Default|GetcurrentGraphicLevel)
              (:%20%20
                (Variables|Default|SetcurrentGraphicLevel (Math|Integer|Clamp(Integer) (Variables|Default|GetcurrentGraphicLevel) 0 3))
                (CallFunction|AdjustSettings)))))
        (elif (> (* (Variables|Default|GetAverageDeltaT) 166.667007) 43.0)
          (if (!= (Variables|Default|GetcurrentGraphicLevel) 0)
            (Math|Integer|DecrementInt (Variables|Default|GetcurrentGraphicLevel)
              (:%20%20
                (Variables|Default|SetcurrentGraphicLevel (Math|Integer|Clamp(Integer) (Variables|Default|GetcurrentGraphicLevel) 0 3))
                (CallFunction|AdjustSettings))))
          (elif (< (* (Variables|Default|GetAverageDeltaT) 166.667007) 17.0)
            (Math|Integer|IncrementInt (Variables|Default|GetcurrentGraphicLevel)
              (:%20%20
                (Math|Integer|IncrementInt (Variables|Default|GetcurrentGraphicLevel)
                  (:%20%20
                    (Variables|Default|SetcurrentGraphicLevel (Math|Integer|Clamp(Integer) (Variables|Default|GetcurrentGraphicLevel) 0 3))
                    (CallFunction|AdjustSettings)))))
            (elif (< (* (Variables|Default|GetAverageDeltaT) 166.667007) 2e+01)
              (Math|Integer|IncrementInt (Variables|Default|GetcurrentGraphicLevel)
                (:%20%20
                  (Variables|Default|SetcurrentGraphicLevel (Math|Integer|Clamp(Integer) (Variables|Default|GetcurrentGraphicLevel) 0 3))
                  (CallFunction|AdjustSettings)))
              (else
                (Actor|DestroyActor)))))))))

(event EventBeginPlay
  (Variables|Default|SetcurrentGraphicLevel (Math|Conversions|ToInteger(Byte) (.GraphicQuality (Utilities|Struct|BreakSettingValues (Variables|/Game/Secpholand/Blueprints/ControllersYModes/baseClasses/ClientSide_Controller.ClientSide_Controller_C|Getsettings (.AsClient%20Side%20Controller (Utilities|Casting|CastToClientSide_Controller (Game|GetPlayerController 0))))))))
  (CallFunction|SampleDeltaT))

(fn ConstructionScript)