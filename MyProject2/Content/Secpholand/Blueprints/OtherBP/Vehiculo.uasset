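; Vehicle actor that drives a car mesh along the Camino spline.
; While Go is true, Tick advances Alfa at a rate scaled by Divider and sets the car's world transform from the spline, with yaw flipped 180 degrees.
; StartVehicle runs on BeginPlay and at path end, picking a random height offset for the same mesh, then snapping it to the spline start.
; At path end Go clears, but Alfa is not reset here.
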(event Custom|startVehicle
  (bind _car_01 (Variables|Default|GetCar_01))
  (switch int (Math|Random|RandomInteger 3)
    (:Default
      (Components|StaticMesh|SetStaticMesh _car_01 "/Game/Secpholand/Assets/meshes/Secpholand_Island/Props/SM_Car1.SM_Car1" :!label _label)
      (Transformation|SetRelativeLocation _car_01 "0, 0,17.000000" false false))
    (:0
      (goto _label))
    (:1
      (Components|StaticMesh|SetStaticMesh _car_01 "/Game/Secpholand/Assets/meshes/Secpholand_Island/Props/SM_Car1.SM_Car1")
      (Transformation|SetRelativeLocation _car_01 "0,0.000000,44.000000" false false))
    (:2
      (Components|StaticMesh|SetStaticMesh _car_01 "/Game/Secpholand/Assets/meshes/Secpholand_Island/Props/SM_Car1.SM_Car1")
      (Transformation|SetRelativeLocation _car_01 "0, 0,84.000000" false false)))
  (CallFunction|SetPosAlfa 0.0))

(event Custom|setPosAlfa
  (params (alfa :type Float%20%28single-precision%29))
  (bind _camino (Variables|Default|Getcamino))
  (bind _returnvalue (Class|SplineComponent|GetRotationatTime _camino alfa "World" false))
  (Transformation|SetWorldLocationAndRotation (Variables|Default|GetCar_01) (Spline|GetLocationatTime _camino alfa "World" false) (Math|Rotator|MakeRotator (.roll _returnvalue) (.pitch _returnvalue) (+ (.yaw _returnvalue) 1.8e+02)) false false))

(event EventBeginPlay
  (CallFunction|StartVehicle))

(event EventTick
  (params (DeltaSeconds :type Float%20%28single-precision%29))
  (if (Variables|Default|Getgo)
    (if (< (Variables|Default|Getalfa) 1.0)
      (bind _output_get (Variables|Default|Setalfa (+ (Variables|Default|Getalfa) (/ DeltaSeconds (Variables|Default|Getdivider)))))
      (CallFunction|SetPosAlfa _output_get)
      (else
        (CallFunction|StartVehicle)
        (Variables|Default|Setgo false)))))

(fn ConstructionScript)