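; Clickable round-table seating prop (SillonesMesaRedondaAudi) with a static mesh and a hierarchical instanced static mesh.
; A RepNotify Visible flag drives both meshes' visibility and the actor's collision, and is also applied on BeginPlay.
; Click runs the parent behavior and hides the static mesh in game, leaving the instanced mesh untouched.
; FinishedZoomOut shows the static mesh again.
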(event EventBeginPlay
  (Rendering|SetVisibility (Variables|Default|GetHierarchicalInstancedStaticMesh) (Variables|Default|GetVisible) false)
  (Collision|SetActorEnableCollision (Variables|Default|GetVisible)))

(event EventClick
  (params (controller :type Client%20Side%20Controller%20Object%20Reference))
  (|CallParentFunction controller)
  (Development|SetHiddeninGame (Variables|Default|GetStaticMesh) true false))

(event EventFinishedZoomOut
  (Development|SetHiddeninGame (Variables|Default|GetStaticMesh) false false))

(fn ConstructionScript)

(fn OnRepVisible?
  (Rendering|SetVisibility (Variables|Default|GetHierarchicalInstancedStaticMesh) (Variables|Default|GetVisible) false)
  (Collision|SetActorEnableCollision (Variables|Default|GetVisible)))