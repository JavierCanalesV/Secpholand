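; Secpholand presentation screen that shows web-hosted slides and lets the player zoom the view onto it.
; Multicast or local build events download numbered JPGs sequentially into a texture array, shown through a dynamic material that slide updates re-texture.
; Clicks alternate a Timeline that lerps the view target to the screen's Scene transform and back.
; Zooming hides the exit-room widget until zoom-out, and linked screens lose collision during transitions.
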(event Custom|BuildTexturesAndInitScreen
  (params (UrlStart :type String) (NumSlides :type Integer) (NombrePantallaCached :type String) (DiapositivaInicial :type Integer))
  ;[1 1 1] Build textures for Role Presentator
  (Variables|Default|SetNombrePantallaCached NombrePantallaCached)
  (Variables|Default|SetNumSlides NumSlides)
  (Variables|Default|SetCountHelper 0)
  (Utilities|Array|Clear (Variables|Default|GetTexturasPresentacion))
  (bind _texture (|DownloadImage (Utilities|String|Append UrlStart (Utilities|String|ToString(Integer) (+ (Variables|Default|GetCountHelper) 1)) ".jpg") :!label _label)
    (:OnSuccess
      (Math|Integer|IncrementInt (Variables|Default|GetCountHelper)
        (:%20%20
          (Utilities|Array|Add (Variables|Default|GetTexturasPresentacion) _texture)
          (if (< (Variables|Default|GetCountHelper) (Variables|Default|GetNumSlides))
            (goto _label)
            (else
              (Variables|Default|SetCountHelper 0)
              (bind _returnvalue (Rendering|Material|CreateDynamicMaterialInstance (Variables|Default|GetStaticMesh) 1 "/Game/Secpholand/UI/Images/pantallas/SlideTexture.SlideTexture" "None" :!class /Script/Engine.PrimitiveComponent))
              (bind _output_get (Variables|Default|SetMaterialDynamic _returnvalue))
              (Rendering|Material|SetTextureParameterValue _output_get "Texture" (Utilities|Array|Get(acopy) (Variables|Default|GetTexturasPresentacion) DiapositivaInicial)))))))
    (:OnFail
      (Development|PrintString "FAILED BUILDING TEXTURES" true true "(R=0.000000,G=0.660000,B=1.000000,A=1.000000)" 1e+01))))

(event Custom|UpdateDiapositiva
  (params (Index :type Integer))
  ;[1 1 1] Build textures for Role Presentator
  (Rendering|Material|SetTextureParameterValue (Variables|Default|GetMaterialDynamic) "Texture" (Utilities|Array|Get(acopy) (Variables|Default|GetTexturasPresentacion) Index)))

(event Custom|Multicast:BuildTexture
  (params (UrlStart :type String) (NumSlides :type Integer) (NombrePantallaCached :type String) (DiapositivaInicial :type Integer))
  ;[1 1 1] Multicast atempt
  (Variables|Default|SetNombrePantallaCached NombrePantallaCached)
  (Variables|Default|SetNumSlides NumSlides)
  (Variables|Default|SetCountHelper 0)
  (Utilities|Array|Clear (Variables|Default|GetTexturasPresentacion))
  (bind _texture (|DownloadImage (Utilities|String|Append UrlStart (Utilities|String|ToString(Integer) (+ (Variables|Default|GetCountHelper) 1)) ".jpg") :!label _label)
    (:OnSuccess
      (Math|Integer|IncrementInt (Variables|Default|GetCountHelper)
        (:%20%20
          (Utilities|Array|Add (Variables|Default|GetTexturasPresentacion) _texture)
          (if (< (Variables|Default|GetCountHelper) (Variables|Default|GetNumSlides))
            (goto _label)
            (else
              (Variables|Default|SetCountHelper 0)
              (bind _returnvalue (Rendering|Material|CreateDynamicMaterialInstance (Variables|Default|GetStaticMesh) 1 "/Game/Secpholand/UI/Images/pantallas/SlideTexture.SlideTexture" "None" :!class /Script/Engine.PrimitiveComponent))
              (bind _output_get (Variables|Default|SetMaterialDynamic _returnvalue))
              (Rendering|Material|SetTextureParameterValue _output_get "Texture" (Utilities|Array|Get(acopy) (Variables|Default|GetTexturasPresentacion) DiapositivaInicial)))))))
    (:OnFail
      (Development|PrintString "FAILED BUILDING TEXTURES" true true "(R=0.000000,G=0.660000,B=1.000000,A=1.000000)" 1e+01))))

(event Custom|resetCamera
  (bind _originaltransform (Variables|Default|GetoriginalTransform))
  (if (Class|KismetMathLibrary|NotEqualExactlyVectorVector (.Location (Math|Transform|BreakTransform _originaltransform)) "0, 0, 0")
    (Transformation|SetActorTransform (Pawn|GetViewTarget (Game|GetPlayerController 0)) _originaltransform)))

(event Custom|CacheTransform
  (Variables|Default|SetoriginalTransform (Transformation|GetActorTransform (Pawn|GetViewTarget (Game|GetPlayerController 0)))))

(event Custom|CallBuildTextures
  ;[1 1 1] Multicast atempt
  (CallFunction|Multicast:BuildTexture "https://newsite.secpho.org/wp-content/uploads/2020/08/Edificios_de_secpholand" 4 "AuditorioCentro"))

(event Custom|DesactivarPantalla
  ;[1 1 1] Build textures for Role Presentator
  (Rendering|Material|SetMaterial (Variables|Default|GetStaticMesh) 1 "/Game/Secpholand/Assets/Materials/MaterialInstances/Tileables/Screen.Screen"))

(event Custom|ToggleScreens
  (params (TurnOnCollision? :type Boolean))
  ;[1 1 1] Zoom al pulsar y widgets de salida de sala
  (for _array_element (Variables|Default|GetScreensToInvalidate)
    (Utilities|IsValid _array_element
      (:Is%20Valid
        (Collision|SetActorEnableCollision _array_element TurnOnCollision?)))))

(event EventBeginPlay
  (Components|Timeline|SetPlayRate (Variables|Default|Getzoom) (/ 1.0 (Variables|Default|GetTravelSeconds))))

(event EventClick
  (params (controller :type Client%20Side%20Controller%20Object%20Reference))
  ;[1 1 1] Zoom al pulsar y widgets de salida de sala
  (CallFunction|ResetClick)
  (CallFunction|ToggleScreens false)
  (Utilities|FlowControl|FlipFlop
    (:A
      (Default|CallHasZoomed)
      (CallFunction|CacheTransform)
      (Variables|Default|SetHoverNormalHint "Haz click para volver a la vista general")
      (Variables|Default|Setzoomed true)
      (Utilities|IsValid (Variables|Default|GetRef_Salir%20Sala%20Pantalla)
        (:Is%20Valid
          _)
        (:Is%20Not%20Valid
          (bind _foundwidgets (Widget|GetAllWidgetsOfClass "/Game/Secpholand/UI/Widgets/SalirMapa.SalirMapa_C" true))
          (Variables|Default|SetRef_Salir%20Sala%20Pantalla (Utilities|Array|Get(acopy) _foundwidgets))))
      (Widget|RemovefromParent (Variables|Default|GetRef_Salir%20Sala%20Pantalla))
      (bind _newtrack_0 (Timeline|zoom Play)
        (:Update
          (Transformation|SetActorTransform (Pawn|GetViewTarget (Game|GetPlayerController 0)) (Math|Transform|Lerp(Transform) (Variables|Default|GetoriginalTransform) (Transformation|GetWorldTransform (Variables|Default|GetScene)) _newtrack_0)))
        (:Finished
          (if (Variables|Default|Getzoomed)
            _
            (else
              (UserInterface|Viewport|AddtoViewport (Variables|Default|GetRef_Salir%20Sala%20Pantalla) 0)))
          (CallFunction|ToggleScreens true))))
    (:B
      (Utilities|FlowControl|Sequence
        (:then_0
          (Variables|Default|SetHoverNormalHint "Haz click para hacer zoom")
          (Variables|Default|Setzoomed false)
          (Timeline|zoom Reverse))
        (:then_1
          (Utilities|FlowControl|Delay (Variables|Default|GetTravelSeconds))
          (Default|CallHasUnZoomed))))))

(fn ConstructionScript)