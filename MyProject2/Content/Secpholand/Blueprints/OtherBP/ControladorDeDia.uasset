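; Day controller that syncs the sky, sunlight and ambient audio to the system clock, with an optional hour override.
; From BeginPlay it refreshes every minute, passing the time to ChangeSun, which uses a timeline as a curve lookup: set the time, apply values, stop.
; The curves drive sky sun height, light intensity and color, and the day/night sound mix, with night and bird sounds muted when Interior is set.
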(event Custom|ChangeSun
  (params (Hora :type Float%20%28single-precision%29) (minutos :type Float%20%28single-precision%29))
  (bind _sky (Variables|Default|Getsky))
  (bind _sun (Variables|Default|Getsun))
  (bind (_direction _sunheight _sunintensity _sonidonoche _newtrack_3) (Timeline|Timeline_0 SetNewTime)
    (:Update
      (Variables|/Engine/EngineSky/BP_Sky_Sphere.BP_Sky_Sphere_C|SetSun%20height _sky _sunheight)
      (Default|RefreshMaterial _sky)
      (Rendering|Components|Light|SetIntensity (Variables|/Script/Engine.Light|GetLightComponent _sun) _sunintensity)
      (Rendering|Components|Light|SetLightColor (Variables|/Script/Engine.Light|GetLightComponent _sun) _newtrack_3 true)
      (Audio|Components|Audio|SetVolumeMultiplier (Variables|Default|GetnightAmbLoop) (select (Variables|Default|Getinterior) 0.0 _sonidonoche) :!class /Script/Engine.AudioComponent)
      (Audio|Components|Audio|SetVolumeMultiplier (Variables|Default|GetambLoop) (- 1.0 (* _sonidonoche 0.6)) :!class /Script/Engine.AudioComponent)
      (Audio|Components|Audio|AdjustVolume (Variables|Default|Getbirds2_Cue) 0.0 (select (Variables|Default|Getinterior) 0.0 (- 1.0 _sonidonoche)) "Linear" :!class /Script/Engine.AudioComponent)
      (Timeline|Timeline_0 Stop))))

(event Collision|EventActorBeginOverlap
  (params (OtherActor :type Actor%20Object%20Reference)))

(event EventBeginPlay
  (bind _returnvalue (Math|DateTime|Now))
  (bind _overridehour (Variables|Default|GetOverrideHour))
  (bind (_year _month _day _hour _minute) (Math|DateTime|BreakDateTime _returnvalue))
  (CallFunction|ChangeSun (select (!= _overridehour 0.0) _overridehour (Math|Conversions|ToFloat(Integer) _hour)) (Math|Conversions|ToFloat(Integer) _minute) :!label _label)
  (Utilities|FlowControl|Delay 6e+01)
  (goto _label))

(fn ConstructionScript)