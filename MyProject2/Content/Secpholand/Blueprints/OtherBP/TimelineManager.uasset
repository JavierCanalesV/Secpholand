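; TimelineManager is a short-lived helper actor that animates the opening and closing of UI panels for contacts, options, objectives and adding friends.
; Each event finds the first matching top-level widget and plays its timeline forward to open or in reverse to close.
; The timeline scales the overlay's canvas slot width, also fading a vertical box for options and objectives.
; The actor destroys itself when the timeline finishes.
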(event Custom|OpenAñadirPersonas
  (params (Open :type Boolean))
  (bind _foundwidgets (Widget|GetAllWidgetsOfClass "/Game/Secpholand/UI/Widgets/HUDYChat/AñadirAmigos/añadirAmigosPestañas.añadirAmigosPestañas_C" true))
  (if Open
    (bind _newtrack_0 (Timeline|Timeline_2 PlayFromStart)
      (:Update
        (Class|CanvasPanelSlot|SetSize (Class|WidgetLayoutLibrary|SlotasCanvasSlot (Variables|/Game/Secpholand/UI/Widgets/HUDYChat/AñadirAmigos/añadirAmigosPestañas.añadirAmigosPestañas_C|GetChatOverlay (Utilities|Array|Get(acopy) _foundwidgets))) (Math|Vector2D|MakeVector2D (* _newtrack_0 1.1e+03) (.y (Class|CanvasPanelSlot|GetSize (Class|WidgetLayoutLibrary|SlotasCanvasSlot (Variables|/Game/Secpholand/UI/Widgets/HUDYChat/AñadirAmigos/añadirAmigosPestañas.añadirAmigosPestañas_C|GetChatOverlay (Utilities|Array|Get(acopy) _foundwidgets))))))))
      (:Finished
        (Actor|DestroyActor)))
    (else
      (Timeline|Timeline_2 ReverseFromEnd))))

(event Custom|OpenContactList%20Event
  (params (Open :type Boolean))
  (bind _foundwidgets (Widget|GetAllWidgetsOfClass "/Game/Secpholand/UI/Widgets/HUDYChat/ChatWindow.ChatWindow_C" true))
  (if Open
    (bind _newtrack_0 (Timeline|OpenContactList PlayFromStart)
      (:Update
        (Class|CanvasPanelSlot|SetSize (Class|WidgetLayoutLibrary|SlotasCanvasSlot (Variables|/Game/Secpholand/UI/Widgets/HUDYChat/ChatWindow.ChatWindow_C|GetContactsOverlay (Utilities|Array|Get(acopy) _foundwidgets))) (Math|Vector2D|MakeVector2D (* _newtrack_0 4e+02) (.y (Class|CanvasPanelSlot|GetSize (Class|WidgetLayoutLibrary|SlotasCanvasSlot (Variables|/Game/Secpholand/UI/Widgets/HUDYChat/ChatWindow.ChatWindow_C|GetContactsOverlay (Utilities|Array|Get(acopy) _foundwidgets))))))))
      (:Finished
        (Actor|DestroyActor)))
    (else
      (Timeline|OpenContactList ReverseFromEnd))))

(event Custom|OpenOptionsEvent
  (params (Open :type Boolean))
  (bind _foundwidgets (Widget|GetAllWidgetsOfClass "/Game/Secpholand/UI/Widgets/HUDYChat/Opciones.Opciones_C" true))
  (if Open
    (bind _newtrack_0 (Timeline|Timeline_0 PlayFromStart)
      (:Update
        (Class|CanvasPanelSlot|SetSize (Class|WidgetLayoutLibrary|SlotasCanvasSlot (Variables|/Game/Secpholand/UI/Widgets/HUDYChat/Opciones.Opciones_C|GetChatOverlay (Utilities|Array|Get(acopy) _foundwidgets))) (Math|Vector2D|MakeVector2D (* _newtrack_0 6.5e+02) (.y (Class|CanvasPanelSlot|GetSize (Class|WidgetLayoutLibrary|SlotasCanvasSlot (Variables|/Game/Secpholand/UI/Widgets/HUDYChat/Opciones.Opciones_C|GetChatOverlay (Utilities|Array|Get(acopy) _foundwidgets)))))))
        (Widget|SetRenderOpacity (Variables|/Game/Secpholand/UI/Widgets/HUDYChat/Opciones.Opciones_C|GetVerticalBox_1 (Utilities|Array|Get(acopy) _foundwidgets)) _newtrack_0))
      (:Finished
        (Actor|DestroyActor)))
    (else
      (Timeline|Timeline_0 ReverseFromEnd))))

(event Custom|OpenObjectivesEvent
  (params (Open :type Boolean))
  (bind _foundwidgets (Widget|GetAllWidgetsOfClass "/Game/Secpholand/UI/Widgets/HUDYChat/NotificacionesYMisiones/NotificacionesYObjetivos.NotificacionesYObjetivos_C" true))
  (if Open
    (bind _newtrack_0 (Timeline|Timeline_1 PlayFromStart)
      (:Update
        (Class|CanvasPanelSlot|SetSize (Class|WidgetLayoutLibrary|SlotasCanvasSlot (Variables|/Game/Secpholand/UI/Widgets/HUDYChat/NotificacionesYMisiones/NotificacionesYObjetivos.NotificacionesYObjetivos_C|GetChatOverlay (Utilities|Array|Get(acopy) _foundwidgets))) (Math|Vector2D|MakeVector2D (* _newtrack_0 6.5e+02) (.y (Class|CanvasPanelSlot|GetSize (Class|WidgetLayoutLibrary|SlotasCanvasSlot (Variables|/Game/Secpholand/UI/Widgets/HUDYChat/NotificacionesYMisiones/NotificacionesYObjetivos.NotificacionesYObjetivos_C|GetChatOverlay (Utilities|Array|Get(acopy) _foundwidgets)))))))
        (Widget|SetRenderOpacity (Variables|/Game/Secpholand/UI/Widgets/HUDYChat/NotificacionesYMisiones/NotificacionesYObjetivos.NotificacionesYObjetivos_C|GetVerticalBox_2 (Utilities|Array|Get(acopy) _foundwidgets)) _newtrack_0))
      (:Finished
        (Actor|DestroyActor)))
    (else
      (Timeline|Timeline_1 ReverseFromEnd))))

(fn ConstructionScript)