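; Shared helper function library for Secpholand, a game with user profiles, technology and sector specialties, levels, objectives and daily rewards.
; Converts technology and sector enums and timestamps to display text, and compresses date and user info structs.
; UI helpers truncate strings, move scroll children to the top and keep mouse-positioned widgets on screen.
; Also marks HUD sub-objectives, looks up level experience and daily rewards, and opens levels, with the online check still a placeholder.
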(fn ByteTecnologiatoString
  (params (Tecnologia :type Tecnologias%20Enum :default "NewEnumerator0") (Byte :type Byte))
  (switch Utilities|FlowControl|Switch|SwitchonTecnologias Tecnologia
    (:NewEnumerator0
      (return (Utilities|String|EnumtoString (Utilities|Enum|ByteToEnumDTSensoresYSistemasDeEscaneoDeImagen Byte))))
    (:NewEnumerator1
      (return (Utilities|String|EnumtoString (Utilities|Enum|ByteToEnumDTSistemasLaser Byte))))
    (:NewEnumerator2
      (return (Utilities|String|EnumtoString (Utilities|Enum|ByteToEnumDTSistemasComunicacióRedesyTransmisióndeDatos Byte))))
    (:NewEnumerator3
      (return (Utilities|String|EnumtoString (Utilities|Enum|ByteToEnumDTIA Byte))))
    (:NewEnumerator4
      (return (Utilities|String|EnumtoString (Utilities|Enum|ByteToEnumDTMaterialesAvanzados Byte))))
    (:NewEnumerator5
      (return (Utilities|String|EnumtoString (Utilities|Enum|ByteToEnumDTTecnologiasCuanticas Byte))))
    (:NewEnumerator6
      (return (Utilities|String|EnumtoString (Utilities|Enum|ByteToEnumDTImpresion3D Byte))))
    (:NewEnumerator7
      (return (Utilities|String|EnumtoString (Utilities|Enum|ByteToEnumDTBiotecnologia Byte))))
    (:NewEnumerator8
      (return (Utilities|String|EnumtoString (Utilities|Enum|ByteToEnumDTNanotecnologia Byte))))
    (:NewEnumerator9
      (return (Utilities|String|EnumtoString (Utilities|Enum|ByteToEnumDTBlockChain Byte))))
    (:NewEnumerator10
      (return (Utilities|String|EnumtoString (Utilities|Enum|ByteToEnumDTRoboticaYDrones Byte))))
    (:NewEnumerator11
      (return (Utilities|String|EnumtoString (Utilities|Enum|ByteToEnumDTDesarrolloDeVideojuegosYSoftware Byte))))
    (:NewEnumerator12
      (return (Utilities|String|EnumtoString (Utilities|Enum|ByteToEnumDTSistemasDeEnergiaFotovoltaicos Byte))))
    (:NewEnumerator13
      (return (Utilities|String|EnumtoString (Utilities|Enum|ByteToEnumDTIluminacionAvanzada Byte))))
    (:NewEnumerator14
      (return (Utilities|String|EnumtoString (Utilities|Enum|ByteToEnumDTPantallasDisplaysYReprodImagen Byte))))
    (:NewEnumerator15
      (return (Utilities|String|EnumtoString (Utilities|Enum|ByteToEnumDTSistemasElectronicos Byte))))))

(fn Tecnologia+DisciplinastoTexts
  (params (NewParam :type Tecnologia+disciplinas%20Structure))
  (bind (_base _membervar_21) (Utilities|Struct|BreakTecnologia+disciplinas NewParam))
  (for _array_element _membervar_21
    (bind _newparam (CallFunction|ByteTecnologiatoString _base _array_element))
    (LocalVariables|Setstring (Utilities|String|Append (LocalVariables|Getstring) _newparam "; ")))
  (return (Utilities|Text|ToText(String) (LocalVariables|Getstring)) (Utilities|Text|ToText(String) (Utilities|String|Append (Utilities|String|EnumtoString _base) " con especialidad en:"))))

(fn ByteSectortoStttring
  (params (sector :type Sectores%20Enum :default "NewEnumerator0") (byte :type Byte))
  (switch Utilities|FlowControl|Switch|SwitchonSectores sector
    (:NewEnumerator0
      (return (Utilities|String|EnumtoString (Utilities|Enum|ByteToEnumSect_Salud byte))))
    (:NewEnumerator1
      (return (Utilities|String|EnumtoString (Utilities|Enum|ByteToEnumSect_Agroalimentacion byte))))
    (:NewEnumerator2
      (return (Utilities|String|EnumtoString (Utilities|Enum|ByteToEnumSect_CosmeticaYEstetica byte))))
    (:NewEnumerator3
      (return (Utilities|String|EnumtoString (Utilities|Enum|ByteToEnumSect_IndustriaQuimica byte))))
    (:NewEnumerator4
      (return (Utilities|String|EnumtoString (Utilities|Enum|ByteToEnumSect_Farmaceutico byte))))
    (:NewEnumerator5
      (return (Utilities|String|EnumtoString (Utilities|Enum|ByteToEnumSect_Automocion byte))))
    (:NewEnumerator6
      (return (Utilities|String|EnumtoString (Utilities|Enum|ByteToEnumSect_Ferroviario byte))))
    (:NewEnumerator7
      (return (Utilities|String|EnumtoString (Utilities|Enum|ByteToEnumSect_Aeroespacial byte))))
    (:NewEnumerator8
      (return (Utilities|String|EnumtoString (Utilities|Enum|ByteToEnumSect_FabricacionIndustrial byte))))
    (:NewEnumerator9
      (return (Utilities|String|EnumtoString (Utilities|Enum|ByteToEnumSect_MedioAmbienteYEnergia byte))))
    (:NewEnumerator10
      (return (Utilities|String|EnumtoString (Utilities|Enum|ByteToEnumSect_TelecomunicacionesYCiverseguridad byte))))
    (:NewEnumerator11
      (return (Utilities|String|EnumtoString (Utilities|Enum|ByteToEnumSect_Seguridad byte))))
    (:NewEnumerator12
      (return (Utilities|String|EnumtoString (Utilities|Enum|ByteToEnumSect_MateriasPrimas byte))))
    (:NewEnumerator13
      (return (Utilities|String|EnumtoString (Utilities|Enum|ByteToEnumSect_Construccion byte))))
    (:NewEnumerator14
      (return (Utilities|String|EnumtoString (Utilities|Enum|ByteToEnumSect_OtrosSectores byte))))))

(fn Sector+AmbientetoTexts
  (params (NewParam :type Sector+ambito%20Structure))
  (bind (_sector _ambitos) (Utilities|Struct|BreakSector+ambito NewParam))
  (for _array_element _ambitos
    (bind _newparam (CallFunction|ByteSectortoStttring _sector _array_element))
    (LocalVariables|Setstring (Utilities|String|Append (LocalVariables|Getstring) _newparam "; ")))
  (return (Utilities|Text|ToText(String) (LocalVariables|Getstring)) (Utilities|Text|ToText(String) (Utilities|String|Append (Utilities|String|EnumtoString _sector) " con ambito en:"))))

(fn TimestamptoText
  (params (timeStamp :type Date%20Time%20Compressed%20Structure))
  (bind (_day _month _hour _min) (Utilities|Struct|BreakDateTimeCompressed timeStamp))
  (bind _returnvalue (Math|DateTime|Now))
  (bind _returnvalue_2 (>= _month 10))
  (bind _day_2 (Math|DateTime|BreakDateTime _returnvalue))
  (bind _returnvalue_3 (>= _min 10))
  (bind _result (Utilities|Text|FormatText "{0}/{1}" _day _month))
  (bind _result_2 (Utilities|Text|FormatText "{0}:{1}" _hour _min))
  (bind _result_3 (Utilities|Text|FormatText "{0}:0{1}" _hour _min))
  (bind _result_4 (Utilities|Text|FormatText "{0}/0{1}" _day _month))
  (bind _returnvalue_4 (Math|Conversions|ToByte(Integer) _day_2))
  (bind _returnvalue_5 (select _returnvalue_2 _result _result_4))
  (bind _returnvalue_6 (select _returnvalue_3 _result_2 _result_3))
  (bind _returnvalue_7 (== _day _returnvalue_4))
  (bind _returnvalue_8 (select _returnvalue_7 _returnvalue_6 _returnvalue_5))
  (return (select (Utilities|Enum|Equal(Enum) (Utilities|Text|MakeLiteralText "0/00") _returnvalue_8) "" _returnvalue_8)))

(fn CompressDateTime
  (params (dateTime :type Date%20Time%20Structure))
  (bind (_year _month _day _hour _minute) (Math|DateTime|BreakDateTime dateTime))
  (return (Utilities|Struct|MakeDateTimeCompressed (Math|Conversions|ToByte(Integer) _day) (Math|Conversions|ToByte(Integer) _month) (Math|Conversions|ToByte(Integer) _hour) (Math|Conversions|ToByte(Integer) _minute))))

(fn PutWidgetChildonTop
  (params (scroll :type Scroll%20Box%20Object%20Reference) (WidgetPOos :type Integer))
  (LocalVariables|SetwidgetToSwap (Class|PanelWidget|GetChildat scroll WidgetPOos))
  (Class|PanelWidget|RemoveChildat scroll WidgetPOos)
  (LocalVariables|SettempChildenWidgetsToRestore (Class|PanelWidget|GetAllChildren scroll))
  (Widget|Panel|ClearChildren scroll)
  (Widget|Panel|AddChild scroll (LocalVariables|GetwidgetToSwap))
  (for _array_element (LocalVariables|GettempChildenWidgetsToRestore)
    (Widget|Panel|AddChild scroll _array_element)))

(fn GetLvlExpNeeded
  (params (level :type Integer))
  (return (Utilities|Array|Get(acopy) (LocalVariables|GetlvlExperiences) (Math|Integer|Clamp(Integer) level 0 9))))

(fn CompressUserInfo
  (params (UserInfo%20Uncompressed :type User%20Info%20Public%20Structure))
  (bind (_id _username _name _surname _empresa _cargo _profileimageurl _ubicacion _lambdas _formacion _tecnologíasquedomina _sectoresqueconoce _hobbies _invierteen _ticketmediodeinversion _tipodestartupsquebusca _numerodeoperacionesalaño _añodecreación _tamañodeinversiónbuscada _tipodeinversorpreferente _idiomas _avatarinfo _userclass _level) (Utilities|Struct|BreakUserInfo_Public UserInfo%20Uncompressed))
  (return (Utilities|Struct|MakeUserInfoCompressed _username _name _surname (.Name (Utilities|Struct|BreakEmpresa _empresa)) _cargo _ubicacion _formacion _userclass _level)))

(fn CutOutString
  (params (source :type String) (desired%20len :type Integer))
  (return (select (> (Utilities|String|Len source) desired%20len) (Utilities|String|Append (Utilities|String|Left source desired%20len) "...") source)))

(fn ClampWidgedPostoScreen
  (params (NewParam :type Float%20%28single-precision%29) (NewParam1 :type Float%20%28single-precision%29))
  (bind _returnvalue (Class|WidgetLayoutLibrary|GetViewportScale))
  (bind _returnvalue_2 (Class|WidgetLayoutLibrary|GetViewportScale))
  (bind _returnvalue_3 (Class|WidgetLayoutLibrary|GetMousePositiononViewport))
  (return (select (> (+ (* _returnvalue_2 (.x _returnvalue_3)) (* NewParam _returnvalue_2)) (.x (Viewport|GetViewportSize))) (- (.x _returnvalue_3) NewParam) (.x _returnvalue_3)) (select (> (+ (* _returnvalue (.y _returnvalue_3)) (* NewParam1 _returnvalue)) (.y (Viewport|GetViewportSize))) (- (.y _returnvalue_3) NewParam1) (.y _returnvalue_3)) (> (+ (* _returnvalue_2 (.x _returnvalue_3)) (* NewParam _returnvalue_2)) (.x (Viewport|GetViewportSize))) (> (+ (* _returnvalue (.y _returnvalue_3)) (* NewParam1 _returnvalue)) (.y (Viewport|GetViewportSize)))))

(fn ClampWidgedPostoScreenMiddle
  (params (NewParam :type Float%20%28single-precision%29) (NewParam1 :type Float%20%28single-precision%29))
  (bind _returnvalue (/ NewParam 2.0))
  (bind _returnvalue_2 (Class|WidgetLayoutLibrary|GetViewportScale))
  (bind _returnvalue_3 (Class|WidgetLayoutLibrary|GetViewportScale))
  (bind _returnvalue_4 (* _returnvalue _returnvalue_3))
  (bind _returnvalue_5 (Class|WidgetLayoutLibrary|GetMousePositiononViewport))
  (return (select (< (- (* _returnvalue_3 (.x _returnvalue_5)) _returnvalue_4) 0.0) (+ (.x _returnvalue_5) _returnvalue) (select (> (+ (* _returnvalue_3 (.x _returnvalue_5)) _returnvalue_4) (.x (Viewport|GetViewportSize))) (- (.x _returnvalue_5) _returnvalue) (.x _returnvalue_5))) (select (> (+ (* _returnvalue_2 (.y _returnvalue_5)) (* NewParam1 _returnvalue_2)) (.y (Viewport|GetViewportSize))) (- (.y _returnvalue_5) NewParam1) (.y _returnvalue_5)) (or (> (+ (* _returnvalue_3 (.x _returnvalue_5)) _returnvalue_4) (.x (Viewport|GetViewportSize))) (< (- (* _returnvalue_3 (.x _returnvalue_5)) _returnvalue_4) 0.0)) (> (+ (* _returnvalue_2 (.y _returnvalue_5)) (* NewParam1 _returnvalue_2)) (.y (Viewport|GetViewportSize)))))

(fn SetObjectiveDone/Collected
  (params (ObjectiveName :type String) (Done :type Boolean) (Collected :type Boolean))
  (bind _asclient_side_controller (Utilities|Casting|CastToClientSide_Controller (Game|GetPlayerController 0)))
  (for (_array_element _array_index) (Variables|/Game/Secpholand/UI/Widgets/HUDYChat/HUD.HUD_C|Getobjectives (Variables|/Game/Secpholand/Blueprints/ControllersYModes/ClientSide_Controller.ClientSide_Controller_C|GetHUD _asclient_side_controller))
    (for (_array_element_2 _array_index_2) (.SubObjetivos (Utilities|Struct|BreakObjetivo _array_element))
      (if (Utilities|Enum|Equal(Enum) ObjectiveName (.DescripciónSubobjetivo (Utilities|Struct|BreakSubObjetivo _array_element_2)))
        (Development|PrintString 0 "Objetivo encontrado")
        (if Done
          (Utilities|Struct|SetmembersinSubObjetivo (Utilities|Array|Get(acopy) (.SubObjetivos (Utilities|Struct|BreakObjetivo (Utilities|Array|Get(acopy) (Variables|/Game/Secpholand/UI/Widgets/HUDYChat/HUD.HUD_C|Getobjectives (Variables|/Game/Secpholand/Blueprints/ControllersYModes/ClientSide_Controller.ClientSide_Controller_C|GetHUD _asclient_side_controller)) _array_index))) _array_index_2) true))
        (if Collected
          (Utilities|Struct|SetmembersinSubObjetivo (Utilities|Array|Get(acopy) (.SubObjetivos (Utilities|Struct|BreakObjetivo (Utilities|Array|Get(acopy) (Variables|/Game/Secpholand/UI/Widgets/HUDYChat/HUD.HUD_C|Getobjectives (Variables|/Game/Secpholand/Blueprints/ControllersYModes/ClientSide_Controller.ClientSide_Controller_C|GetHUD _asclient_side_controller)) _array_index))) _array_index_2) true)
          (Development|PrintString 0 "Collected"))))))

(fn GetRecompensasDaily
  (params (dia :type Integer) (Percent :type Integer))
  (bind _returnvalue (- dia 2))
  (bind _returnvalue_2 (<= Percent 49))
  (bind _returnvalue_3 (<= Percent 94))
  (bind _returnvalue_4 (<= Percent 74))
  (bind _cantidadrecompensas (LocalVariables|GetCantidadRecompensas))
  (bind _output (Utilities|Array|Get(acopy) _cantidadrecompensas _returnvalue))
  (if (>= _returnvalue 0)
    (if (not (Math|Boolean|ORBoolean (== dia 4) (== dia 6) (== 8 dia)))
      (return _output _output "NewEnumerator1")
      (else
        (switch int dia
          (:4
            (return (select (<= Percent 49) 30 (select (<= Percent 74) 80 (select (<= Percent 94) 0 100))) (select (<= Percent 49) 30 (select (<= Percent 74) 0 100)) "NewEnumerator1"))
          (:6
            _)
          (:8
            _))
        (return (select _returnvalue_2 50 (select _returnvalue_4 0 (select _returnvalue_3 150 100))) (select _returnvalue_2 50 (select _returnvalue_4 120 (select _returnvalue_3 0 100))) (select _returnvalue_3 "NewEnumerator1" "NewEnumerator0"))))
    (else
      (return 0 0 "NewEnumerator1"))))

(fn OpenLevelOnline
  (params (LevelToOpen :type Name))
  ;[1 1 1] En este if irá la comprobación de que el usuario este conectado o no. Si esta conectado haremos el cambio de mapa online con lo que implique. Si no esta conectado haremos un open level Esto es para el desarrollo mostly
  (if (not false)
    (Game|OpenLevel(byName) 0 LevelToOpen)))