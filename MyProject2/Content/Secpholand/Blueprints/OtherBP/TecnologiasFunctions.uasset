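; Function library that turns Secpholand technology and sector selections into readable text.
; Two switch helpers cast a raw byte to the sub-enum matching the given technology or sector, then return its name as a string.
; Two wrapper functions loop over a struct's byte array through these helpers, building a semicolon-separated text of specialties or scopes plus a Spanish heading naming the parent category.
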(fn ByteTecnologiatoString
  (params (Tecnologia :type Tecnologias%20Enum :default "NewEnumerator0") (Byte :type Byte))
  (switch Utilities|FlowControl|Switch|SwitchonTecnologias Tecnologia
    (:NewEnumerator0
      (return (Utilities|String|EnumtoString (Utilities|Enum|ByteToEnumDTSensoresYSistemasDeEscaneoDeImagen Byte))))
    (:NewEnumerator1
      (return (Utilities|String|EnumtoString (Utilities|Enum|ByteToEnumDTSistemasLaser Byte))))
    (:NewEnumerator2
      (return (Utilities|String|EnumtoString (Utilities|Enum|ByteToEnumDTSistemasComunicacióRedesyTransmisióndeDatos Byte))))
    (:NewEnumerator3
      (return (Utilities|String|EnumtoString (Utilities|Enum|ByteToEnumDTIA Byte))))
    (:NewEnumerator4
      (return (Utilities|String|EnumtoString (Utilities|Enum|ByteToEnumDTMaterialesAvanzados Byte))))
    (:NewEnumerator5
      (return (Utilities|String|EnumtoString (Utilities|Enum|ByteToEnumDTTecnologiasCuanticas Byte))))
    (:NewEnumerator6
      (return (Utilities|String|EnumtoString (Utilities|Enum|ByteToEnumDTImpresion3D Byte))))
    (:NewEnumerator7
      (return (Utilities|String|EnumtoString (Utilities|Enum|ByteToEnumDTBiotecnologia Byte))))
    (:NewEnumerator8
      (return (Utilities|String|EnumtoString (Utilities|Enum|ByteToEnumDTNanotecnologia Byte))))
    (:NewEnumerator9
      (return (Utilities|String|EnumtoString (Utilities|Enum|ByteToEnumDTBlockChain Byte))))
    (:NewEnumerator10
      (return (Utilities|String|EnumtoString (Utilities|Enum|ByteToEnumDTRoboticaYDrones Byte))))
    (:NewEnumerator11
      (return (Utilities|String|EnumtoString (Utilities|Enum|ByteToEnumDTDesarrolloDeVideojuegosYSoftware Byte))))
    (:NewEnumerator12
      (return (Utilities|String|EnumtoString (Utilities|Enum|ByteToEnumDTSistemasDeEnergiaFotovoltaicos Byte))))
    (:NewEnumerator13
      (return (Utilities|String|EnumtoString (Utilities|Enum|ByteToEnumDTIluminacionAvanzada Byte))))
    (:NewEnumerator14
      (return (Utilities|String|EnumtoString (Utilities|Enum|ByteToEnumDTPantallasDisplaysYReprodImagen Byte))))
    (:NewEnumerator15
      (return (Utilities|String|EnumtoString (Utilities|Enum|ByteToEnumDTSistemasElectronicos Byte))))))

(fn Tecnologia+DisciplinastoTexts
  (params (NewParam :type Tecnologia+disciplinas%20Structure))
  (bind (_base _membervar_21) (Utilities|Struct|BreakTecnologia+disciplinas NewParam))
  (for _array_element _membervar_21
    (bind _newparam (CallFunction|ByteTecnologiatoString _base _array_element))
    (LocalVariables|Setstring (Utilities|String|Append (LocalVariables|Getstring) _newparam "; ")))
  (return (Utilities|Text|ToText(String) (LocalVariables|Getstring)) (Utilities|Text|ToText(String) (Utilities|String|Append (Utilities|String|EnumtoString _base) " con especialidad en:"))))

(fn ByteSectortoStttring
  (params (sector :type Sectores%20Enum :default "NewEnumerator0") (byte :type Byte))
  (switch Utilities|FlowControl|Switch|SwitchonSectores sector
    (:NewEnumerator0
      (return (Utilities|String|EnumtoString (Utilities|Enum|ByteToEnumSect_Salud byte))))
    (:NewEnumerator1
      (return (Utilities|String|EnumtoString (Utilities|Enum|ByteToEnumSect_Agroalimentacion byte))))
    (:NewEnumerator2
      (return (Utilities|String|EnumtoString (Utilities|Enum|ByteToEnumSect_CosmeticaYEstetica byte))))
    (:NewEnumerator3
      (return (Utilities|String|EnumtoString (Utilities|Enum|ByteToEnumSect_IndustriaQuimica byte))))
    (:NewEnumerator4
      (return (Utilities|String|EnumtoString (Utilities|Enum|ByteToEnumSect_Farmaceutico byte))))
    (:NewEnumerator5
      (return (Utilities|String|EnumtoString (Utilities|Enum|ByteToEnumSect_Automocion byte))))
    (:NewEnumerator6
      (return (Utilities|String|EnumtoString (Utilities|Enum|ByteToEnumSect_Ferroviario byte))))
    (:NewEnumerator7
      (return (Utilities|String|EnumtoString (Utilities|Enum|ByteToEnumSect_Aeroespacial byte))))
    (:NewEnumerator8
      (return (Utilities|String|EnumtoString (Utilities|Enum|ByteToEnumSect_FabricacionIndustrial byte))))
    (:NewEnumerator9
      (return (Utilities|String|EnumtoString (Utilities|Enum|ByteToEnumSect_MedioAmbienteYEnergia byte))))
    (:NewEnumerator10
      (return (Utilities|String|EnumtoString (Utilities|Enum|ByteToEnumSect_TelecomunicacionesYCiverseguridad byte))))
    (:NewEnumerator11
      (return (Utilities|String|EnumtoString (Utilities|Enum|ByteToEnumSect_Seguridad byte))))
    (:NewEnumerator12
      (return (Utilities|String|EnumtoString (Utilities|Enum|ByteToEnumSect_MateriasPrimas byte))))
    (:NewEnumerator13
      (return (Utilities|String|EnumtoString (Utilities|Enum|ByteToEnumSect_Construccion byte))))
    (:NewEnumerator14
      (return (Utilities|String|EnumtoString (Utilities|Enum|ByteToEnumSect_OtrosSectores byte))))))

(fn Sector+AmbientetoTexts
  (params (NewParam :type Sector+ambito%20Structure))
  (bind (_sector _ambitos) (Utilities|Struct|BreakSector+ambito NewParam))
  (for _array_element _ambitos
    (bind _newparam (CallFunction|ByteSectortoStttring _sector _array_element))
    (LocalVariables|Setstring (Utilities|String|Append (LocalVariables|Getstring) _newparam "; ")))
  (return (Utilities|Text|ToText(String) (LocalVariables|Getstring)) (Utilities|Text|ToText(String) (Utilities|String|Append (Utilities|String|EnumtoString _sector) " con ambito en:"))))