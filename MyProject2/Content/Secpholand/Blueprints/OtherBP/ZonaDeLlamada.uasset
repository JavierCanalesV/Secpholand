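; Call zone actor: a rotating holographic cylinder that opens a Llamada call widget when the local player's character enters.
; Client-side overlaps on separate in and out volumes, gated by paired DoOnce nodes, trigger call start and hang-up.
; Each swaps the dynamic material between green and blue and replays a timeline animating the Fresnel exponent.
; Construction scales the cylinder, counter-scales and fills four labels, and positions GotoSalir.
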(event OnComponentBeginOverlap(inOverlap)
  (params (OverlappedComponent :type Primitive%20Component%20Object%20Reference) (OtherActor :type Actor%20Object%20Reference) (OtherComp :type Primitive%20Component%20Object%20Reference) (OtherBodyIndex :type Integer) (bFromSweep :type Boolean) (SweepResult :type Hit%20Result%20Structure%20%28by%20ref%29))
  (Networking|SwitchHasAuthority
    (:Remote
      (bind _asserver_side_character (Utilities|Casting|CastToServerSide_Character OtherActor))
      (bind _asclient_side_controller (Utilities|Casting|CastToClientSide_Controller (Game|GetPlayerController 0)))
      (if (== _asserver_side_character (Variables|/Game/Secpholand/Blueprints/ControllersYModes/ClientSide_Controller.ClientSide_Controller_C|GetServerSideCharacterRef _asclient_side_controller))
        (Utilities|FlowControl|DoOnce false
          (:Completed
            (CallFunction|Llamadaon)
            (Utilities|FlowControl|DoOnce true) ; enters at Reset
          ))))))

(event OnComponentEndOverlap(outOverlap)
  (params (OverlappedComponent :type Primitive%20Component%20Object%20Reference) (OtherActor :type Actor%20Object%20Reference) (OtherComp :type Primitive%20Component%20Object%20Reference) (OtherBodyIndex :type Integer))
  (Networking|SwitchHasAuthority
    (:Remote
      (bind _asserver_side_character (Utilities|Casting|CastToServerSide_Character OtherActor))
      (bind _asclient_side_controller (Utilities|Casting|CastToClientSide_Controller (Game|GetPlayerController 0)))
      (if (== _asserver_side_character (Variables|/Game/Secpholand/Blueprints/ControllersYModes/ClientSide_Controller.ClientSide_Controller_C|GetServerSideCharacterRef _asclient_side_controller))
        (Utilities|FlowControl|DoOnce true
          (:Completed
            (CallFunction|LlamadaOff)
            (Utilities|FlowControl|DoOnce false) ; enters at Reset
          ))))))

(event Custom|LlamadaOn
  (bind _mat (Variables|Default|Getmat))
  (bind _returnvalue (UserInterface|CreateWidget "/Game/Secpholand/UI/Widgets/Llamada.Llamada_C" 0 self (Variables|Default|GetfloatingText)))
  (bind _output_get (Variables|Default|SetwidLlamada _returnvalue))
  (UserInterface|Viewport|AddtoViewport _output_get 0)
  (Rendering|Material|SetVectorParameterValue _mat "fresnelCol" "(R=0.000000,G=100.000000,B=0.000000,A=1.000000)" :!class /Script/Engine.MaterialInstanceDynamic)
  (Rendering|Material|SetVectorParameterValue _mat "Col" "(R=0.300000,G=0.800000,B=0.200000,A=1.000000)" :!class /Script/Engine.MaterialInstanceDynamic)
  (bind _newtrack_0 (Timeline|EnterZone PlayFromStart)
    (:Update
      (Rendering|Material|SetScalarParameterValue (Variables|Default|Getmat) "exponenF" (* _newtrack_0 5.0) :!class /Script/Engine.MaterialInstanceDynamic))))

(event Custom|LlamadaOff
  (bind _mat (Variables|Default|Getmat))
  (Default|ColgarEvent (Variables|Default|GetwidLlamada))
  (Rendering|Material|SetVectorParameterValue _mat "fresnelCol" "(R=5.000000,G=5.000000,B=100.000000,A=1.000000)" :!class /Script/Engine.MaterialInstanceDynamic)
  (Rendering|Material|SetVectorParameterValue _mat "Col" "(R=1.000000,G=1.000000,B=3.000000,A=1.000000)" :!class /Script/Engine.MaterialInstanceDynamic)
  (bind _newtrack_0 (Timeline|EnterZone PlayFromStart)
    (:Update
      (Rendering|Material|SetScalarParameterValue (Variables|Default|Getmat) "exponenF" (* _newtrack_0 5.0) :!class /Script/Engine.MaterialInstanceDynamic))))

(event EventBeginPlay
  (bind _returnvalue (Rendering|Material|CreateDynamicMaterialInstance (Variables|Default|GetCylinder) 0 "/Game/Secpholand/Assets/Materials/HOLOGRAFIC_Inst2.HOLOGRAFIC_Inst2" "None" :!class /Script/Engine.PrimitiveComponent))
  (Variables|Default|Setmat _returnvalue))

(event EventTick
  (params (DeltaSeconds :type Float%20%28single-precision%29))
  (Transformation|AddRelativeRotation (Variables|Default|GetrotationParent) "0,0.250000, 0" false false))

(fn ConstructionScript
  (bind _scale (Variables|Default|Getscale))
  (Transformation|SetRelativeScale3D (Variables|Default|GetCylinder) _scale)
  (Transformation|SetRelativeScale3D (Variables|Default|GetTextRender1) (/ "1.000000,1.000000,1.000000" _scale))
  (Rendering|Components|TextRender|SetText (Variables|Default|GetTextRender) (Utilities|Text|ToText(String) (Variables|Default|GetfloatingText)))
  (Transformation|SetRelativeLocation (Variables|Default|GetGotoSalir) (Variables|Default|GetGotoSalirLlamada) false false))