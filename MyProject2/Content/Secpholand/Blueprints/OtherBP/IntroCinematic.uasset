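; Intro cinematic actor for Secpholand that plays the Intro level sequence and then hands off to the tutorial.
; startCinematic applies controller constraints and disables character input for the sequence's duration, while Tick copies the actor's transform to the character's camera.
; A timeline then lerps the camera back to its original position.
; On finish it sets walk speed, spawns TutorialManagerSecpholand and destroys itself.
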(event Custom|startCinematic
  (bind _character (Variables|Default|Getcharacter))
  (bind _asclient_side_controller (Utilities|Casting|CastToClientSide_Controller (Game|GetPlayerController 0)))
  (Default|SetControllsConstraints _asclient_side_controller false false false false)
  (Variables|Default|Setstart true)
  (bind _returnvalue (Sequencer|Player|CreateLevelSequencePlayer "/Game/Secpholand/Assets/Cinematics/Intro.Intro"))
  (bind _output_get (Variables|Default|SetintroCutscene _returnvalue))
  (Input|DisableInput (Variables|Default|Getcharacter) (Game|GetPlayerController 0))
  (Sequencer|Player|Play _output_get :!class /Script/MovieScene.MovieSceneSequencePlayer)
  (Utilities|FlowControl|Delay (Class|TimeManagementBlueprintLibrary|ToSeconds(QualifiedFrameTime) (Media|MediaPlayer|GetDuration (Variables|Default|GetintroCutscene))))
  (Input|EnableInput (Variables|Default|Getcharacter) (Game|GetPlayerController 0))
  (Variables|Default|SetinitialTransform (Transformation|GetWorldTransform (Variables|Default|GetDefaultSceneRoot)))
  (bind _newtrack_0 (Timeline|Timeline_0 Play)
    (:Update
      (Transformation|SetWorldLocationAndRotation (Variables|/Game/Secpholand/Blueprints/ControllersYModes/ServerSide_CharacterTUTORIAL.ServerSide_CharacterTUTORIAL_C|GetCamera _character) (.Location (Math|Transform|BreakTransform (Math|Transform|Lerp(Transform) (Variables|Default|GetinitialTransform) (Transformation|GetWorldTransform (Variables|/Game/Secpholand/Blueprints/ControllersYModes/ServerSide_CharacterTUTORIAL.ServerSide_CharacterTUTORIAL_C|GetCameraOrighinalPos _character)) _newtrack_0))) (.Rotation (Math|Transform|BreakTransform (Math|Transform|Lerp(Transform) (Variables|Default|GetinitialTransform) (Transformation|GetWorldTransform (Variables|/Game/Secpholand/Blueprints/ControllersYModes/ServerSide_CharacterTUTORIAL.ServerSide_CharacterTUTORIAL_C|GetCameraOrighinalPos _character)) _newtrack_0))) false false))
    (:Finished
      (Variables|/Script/Engine.CharacterMovementComponent|SetMaxWalkSpeed (Variables|/Script/Engine.Character|GetCharacterMovement (Variables|Default|Getcharacter)) 9.5e+02)
      (Game|SpawnActorfromClass "/Game/Secpholand/Blueprints/OtherBP/tutoiriales/TutorialManagerSecpholand.TutorialManagerSecpholand_C" (Math|Transform|MakeTransform "0.000000,3026.318115,-440.000366") "Undefined" 0 0)
      (Actor|DestroyActor))))

(event EventTick
  (params (DeltaSeconds :type Float%20%28single-precision%29))
  (if (Variables|Default|Getstart)
    (Transformation|SetWorldTransform (Variables|/Game/Secpholand/Blueprints/ControllersYModes/ServerSide_CharacterTUTORIAL.ServerSide_CharacterTUTORIAL_C|GetCamera (Variables|Default|Getcharacter)) (Transformation|GetActorTransform) false false)))

(fn ConstructionScript)