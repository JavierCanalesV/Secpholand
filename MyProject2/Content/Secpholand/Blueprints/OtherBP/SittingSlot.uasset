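; Seat slot for a meeting table that sits the local player and joins them to the table's call.
; On client-side overlap, a crowded slot asks the parent table for a free chair; otherwise it opens the Llamada call widget, joins the meeting, disables table collision and seats the player.
; Leaving restores collision and hover prompt, leaves the meeting and hangs up.
; Active is cleared on first use and never reset here.
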(event OnComponentBeginOverlap(gotoBox)
  (params (OverlappedComponent :type Primitive%20Component%20Object%20Reference) (OtherActor :type Actor%20Object%20Reference) (OtherComp :type Primitive%20Component%20Object%20Reference) (OtherBodyIndex :type Integer) (bFromSweep :type Boolean) (SweepResult :type Hit%20Result%20Structure%20%28by%20ref%29))
  (bind _parent (Variables|Default|Getparent))
  (Networking|SwitchHasAuthority
    (:Remote
      (bind _asclient_side_pawn (Utilities|Casting|CastToClientSide_Pawn OtherActor))
      (if (and (== (Variables|/Game/Secpholand/Blueprints/ControllersYModes/baseClasses/ClientSide_Pawn.ClientSide_Pawn_C|GetClientSideControllerRef _asclient_side_pawn) (Game|GetPlayerController 0)) (Variables|Default|Getactive))
        (Variables|Default|SetSitClient (Variables|/Game/Secpholand/Blueprints/ControllersYModes/baseClasses/ClientSide_Pawn.ClientSide_Pawn_C|GetClientSideControllerRef _asclient_side_pawn))
        (Variables|Default|Setactive false)
        (if (!= (Utilities|Array|Length (Collision|GetOverlappingActors (Variables|Default|GetgotoBox) "/Game/Secpholand/Blueprints/ControllersYModes/baseClasses/ClientSide_Pawn.ClientSide_Pawn_C" :!class /Script/Engine.PrimitiveComponent)) 1)
          (Default|SentarEnSillaLibre (Variables|Default|Getparent))
          (else
            (Collision|SetCollisionResponsetoChannel (Variables|/Game/Secpholand/Blueprints/clasesBase/ClickableActor.ClickableActor_C|GetStaticMesh (Variables|Default|Getparent)) "ECC_Visibility" "ECR_Ignore")
            (bind _returnvalue (UserInterface|CreateWidget "/Game/Secpholand/UI/Widgets/Llamada.Llamada_C" 0 (Utilities|String|Append "Llamada de la mesa: " (Utilities|String|ToString(Integer) (Variables|/Game/Secpholand/Blueprints/Clicables/MesaDeReunion.MesaDeReunion_C|GetRoomID (Variables|Default|Getparent)))) false false (+ (Variables|/Game/Secpholand/Blueprints/Clicables/MesaDeReunion.MesaDeReunion_C|GetGotoColgar _parent) (Transformation|GetActorLocation _parent))))
            (UserInterface|Viewport|AddtoViewport _returnvalue 0)
            (Default|JoinMeetingTable (Variables|Default|GetSitClient) (Variables|Default|Getparent) true)
            (Collision|SetActorEnableCollision (Variables|Default|Getparent) false)
            (Utilities|FlowControl|Delay 0.5)
            (Default|SitPlayer:Client (Variables|Default|GetSitClient) (Variables|Default|Getrotation))))))))

(event OnComponentEndOverlap(gotoBox)
  (params (OverlappedComponent :type Primitive%20Component%20Object%20Reference) (OtherActor :type Actor%20Object%20Reference) (OtherComp :type Primitive%20Component%20Object%20Reference) (OtherBodyIndex :type Integer))
  (bind _parent (Variables|Default|Getparent))
  (bind _hoveruserwidget (Variables|/Game/Secpholand/Blueprints/clasesBase/ClickableActor.ClickableActor_C|GethoverUserWidget _parent))
  (Networking|SwitchHasAuthority
    (:Remote
      (bind _asclient_side_pawn (Utilities|Casting|CastToClientSide_Pawn OtherActor))
      (if (and (== (Variables|/Game/Secpholand/Blueprints/ControllersYModes/baseClasses/ClientSide_Pawn.ClientSide_Pawn_C|GetClientSideControllerRef _asclient_side_pawn) (Game|GetPlayerController 0)) (== (Variables|/Game/Secpholand/Blueprints/ControllersYModes/baseClasses/ClientSide_Pawn.ClientSide_Pawn_C|GetClientSideControllerRef _asclient_side_pawn) (Variables|Default|GetSitClient)))
        (Variables|Default|SetSitClient 0)
        (Collision|SetActorEnableCollision (Variables|Default|Getparent) true)
        (Default|JoinMeetingTable:Client (Variables|/Game/Secpholand/Blueprints/ControllersYModes/baseClasses/ClientSide_Pawn.ClientSide_Pawn_C|GetClientSideControllerRef _asclient_side_pawn) (Variables|Default|Getparent) false)
        (Utilities|IsValid _hoveruserwidget
          (:Is%20Valid
            (Default|ChangeState _hoveruserwidget "Haz click para unirte." false))
          (:Is%20Not%20Valid
            _))
        (Collision|SetCollisionResponsetoChannel (Variables|/Game/Secpholand/Blueprints/clasesBase/ClickableActor.ClickableActor_C|GetStaticMesh _parent) "ECC_Visibility" "ECR_Block")
        (bind _foundwidgets (Widget|GetAllWidgetsOfClass "/Game/Secpholand/UI/Widgets/Llamada.Llamada_C" true))
        (if (> (Utilities|Array|Length _foundwidgets) 0)
          (Default|ColgarEvent (Utilities|Array|Get(acopy) _foundwidgets)))
        (Utilities|FlowControl|Delay 0.2)))))

(event EventBeginPlay
  (Variables|Default|Setrotation (+ (.yaw (Transformation|GetWorldRotation (Variables|Default|GetDefaultSceneRoot))) 9e+01)))

(fn ConstructionScript)