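; Voice-chat calibration Blueprint that tunes the player's mic level, silence-detection threshold and Master volume through the CalibraciónAudio widget.
; Timed capture windows measure average loudness and audible-frame ratio from the VoipAudio envelope, driving mic volume, boost and iterative refinement passes.
; A separate pass plays a test sound into the mic, repeatedly raising the threshold and adjusting Master volume.
; Finishing saves the settings to NetworkGameInstance and restores the talk room.
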(event VoiceGenerated(VoipManager)
  (params (VoiceData :type Array%20of%20Bytes) (MicLevel :type Float%20%28single-precision%29))
  (Utilities|Casting|CastToClientSide_Controller (Game|GetPlayerController 0))
  (Class|VoipAudioComponent|PlayVoiceData (Variables|Default|GetVoipAudio) VoiceData))

(event OnAudioEnvelopeValue(VoipAudio)
  (params (EnvelopeValue :type Float%20%28single-precision%29))
  (bind _returnvalue (* EnvelopeValue 5e+03))
  (if (Variables|Calibración|GetCapturando)
    (if (> _returnvalue 0.0)
      (Variables|Calibración|SetvolumenSumado (+ (Variables|Calibración|GetvolumenSumado) _returnvalue))
      (Math|Float|IncrementFloat (Variables|Calibración|GetCapturasDeVolumen)
        (:%20%20
          (Variables|Calibración|SetFrameConAudioCapturado true)))
      (else
        (Variables|Calibración|SetFrameConAudioCapturado false)))))

(event Custom|startThesholdCalibration
  (bind _returnvalue (Class|SystemMicControlBPLibrary|GetMicBoost))
  (bind _volumenmicfinal (Variables|Calibración|GetvolumenMicFinal))
  (bind _returnvalue_2 (/ _returnvalue 5.0))
  (bind _returnvalue_3 (/ _volumenmicfinal 3.0))
  (bind _returnvalue_4 (- _returnvalue_3 _returnvalue_2))
  (bind _returnvalue_5 (Math|Float|Clamp(Float) _returnvalue_4))
  (Development|ExecuteConsoleCommand (Utilities|String|Append "voice.SilenceDetectionThreshold " (Utilities|String|ToString(Float) (Variables|Calibración|GetThresholdToApply))) 0)
  (Audio|Components|Audio|SetVolumeMultiplier (Variables|Default|GetVoipAudio) 0.01 :!class /Script/AudioMixer.SynthComponent)
  (Utilities|FlowControl|Delay 0.3)
  (Audio|PlaySound2D "/Game/Secpholand/audio/pruebaThreshold.pruebaThreshold" 1.0 1.0 0.0 0 0)
  (Variables|Calibración|SetCapturando true)
  (Variables|Calibración|SetFramesWithVoice 0.0)
  (Variables|Calibración|SetFramesCapturing 0.0)
  (Variables|Calibración|SetvolumenSumado 0.0)
  (Variables|Calibración|SetCapturasDeVolumen 0.0)
  (Utilities|FlowControl|Delay 3.0)
  (Variables|Calibración|SetCapturando false)
  (Audio|Components|Audio|SetVolumeMultiplier (Variables|Default|GetVoipAudio) 0.0 :!class /Script/AudioMixer.SynthComponent)
  (Variables|Calibración|SetVolumenMedio (/ (Variables|Calibración|GetvolumenSumado) (Variables|Calibración|GetCapturasDeVolumen)))
  (Variables|Calibración|SetaudibleRatio (/ (Variables|Calibración|GetFramesWithVoice) (Variables|Calibración|GetFramesCapturing)))
  (if (or (< (Variables|Calibración|GetVolumenMedio) (Math|Float|Lerp 0.8 1.2 _returnvalue_5)) (< (Variables|Calibración|GetaudibleRatio) (Math|Float|Lerp 0.1 0.15 _returnvalue_5)))
    (Default|VolverAMic (Variables|Default|GetwidgetCalibración) :!label _label)
    (elif (>= (Variables|Default|GetthresholdCalibrations) 6)
      (goto _label)
      (else
        (Variables|Calibración|SetThresholdToApply (+ (Variables|Calibración|GetThresholdToApply) (select (> (Variables|Calibración|GetaudibleRatio) 0.75) 0.04 (select (> (Variables|Calibración|GetaudibleRatio) 0.6) 0.03 (select (< (Variables|Calibración|GetaudibleRatio) 0.3) 0.01 0.02)))))
        (bind _output_get (Variables|Default|SetmasterLvl (|GetMasterDumping)))
        (Audio|SetSoundMixClassOverride "/Game/Secpholand/audio/SouyndClasses/SecpholandMix.SecpholandMix" "/Game/Secpholand/audio/SouyndClasses/Master.Master" _output_get 1.0 1.0 true)
        (Audio|SetSoundMixClassOverride "/Game/Secpholand/audio/SouyndClasses/SecpholandMixVoice.SecpholandMixVoice" "/Game/Secpholand/audio/SouyndClasses/Master.Master" _output_get 1.0 1.0 true)
        (Utilities|FlowControl|Delay 0.6)
        (Math|Integer|IncrementInt (Variables|Default|GetthresholdCalibrations)
          (:%20%20
            (CallFunction|StartThesholdCalibration)))))))

(event Custom|StartMicInputCalibration
  (Audio|Components|Audio|SetVolumeMultiplier (Variables|Default|GetVoipAudio) 0.01 :!class /Script/AudioMixer.SynthComponent)
  (Variables|Calibración|SetFramesWithVoice 0.0)
  (Variables|Calibración|SetFramesCapturing 0.0)
  (Variables|Calibración|SetvolumenSumado 0.0)
  (Variables|Calibración|SetCapturasDeVolumen 0.0)
  (Development|ExecuteConsoleCommand (Utilities|String|Append "voice.SilenceDetectionThreshold " (Utilities|String|ToString(Float) (Variables|Calibración|GetThresholdToApply))) 0)
  (Utilities|FlowControl|Delay 0.5)
  (Variables|Calibración|SetCapturando true)
  (Utilities|FlowControl|Delay 3.5)
  (Variables|Calibración|SetCapturando false)
  (Audio|Components|Audio|SetVolumeMultiplier (Variables|Default|GetVoipAudio) 0.0 :!class /Script/AudioMixer.SynthComponent)
  (Variables|Calibración|SetVolumenMedio (/ (Variables|Calibración|GetvolumenSumado) (Variables|Calibración|GetCapturasDeVolumen)))
  (Variables|Calibración|SetaudibleRatio (/ (Variables|Calibración|GetFramesWithVoice) (Variables|Calibración|GetFramesCapturing)))
  (CallFunction|AjustarVolumenMic)
  (switch int (Variables|Default|GetcalibrationIteration)
    (:Default
      (CallFunction|PaseDeRefinamiento :!label _label))
    (:0
      ;[0.7135 0.2883 0.2267] Primer Pase
      (if (>= (Variables|Calibración|GetaudibleRatio) 0.65)
        (if (> (Variables|Calibración|GetaudibleRatio) 0.95)
          (Variables|Calibración|SetThresholdToApply (+ (Variables|Calibración|GetThresholdToApply) 0.01)))
        (Default|PasarACalibraciónAltavoces (Variables|Default|GetwidgetCalibración) :!label _label_2)
        (Variables|Default|SeterrorInputs 0)
        (Math|Integer|IncrementInt (Variables|Default|GetcalibrationIteration)
          (:%20%20
            (CallFunction|PrintSettings)))
        (elif (and (> (Variables|Calibración|GetVolumenMedio) 1.6) (>= (Variables|Calibración|GetaudibleRatio) 0.5))
          (Variables|Calibración|SetThresholdToApply (+ (Variables|Calibración|GetThresholdToApply) -0.01))
          (goto _label_2)
          (else
            (if (and (> (Variables|Calibración|GetVolumenMedio) 2.0) (>= (Variables|Calibración|GetaudibleRatio) 0.15))
              (Variables|Calibración|SetThresholdToApply (+ (Variables|Calibración|GetThresholdToApply) -0.01)))
            (Math|Integer|IncrementInt (Variables|Default|GeterrorInputs)
              (:%20%20
                (Default|NoSuficienteInput (Variables|Default|GetwidgetCalibración))))))))
    (:1
      (goto _label))
    (:2
      (goto _label))))

(event Custom|FinishCalibration
  (Development|ExecuteConsoleCommand (Utilities|String|Append "voice.SilenceDetectionThreshold " (Utilities|String|ToString(Float) (Variables|Calibración|GetThresholdToApply))) 0)
  (CallFunction|PrintSettings)
  (Default|IrAPantallaFinal (Variables|Default|GetwidgetCalibración))
  (Audio|SetSoundMixClassOverride "/Game/Secpholand/audio/SouyndClasses/SecpholandMix.SecpholandMix" "/Game/Secpholand/audio/SouyndClasses/Voice.Voice" 1.0 1.0 1.0 true)
  (Audio|SetSoundMixClassOverride "/Game/Secpholand/audio/SouyndClasses/SecpholandMixVoice.SecpholandMixVoice" "/Game/Secpholand/audio/SouyndClasses/Voice.Voice" 1.0 1.0 1.0 true)
  (bind _asnetwork_game_instance (Utilities|Casting|CastToNetworkGameInstance (Game|GetGameInstance)))
  (bind _structout (Utilities|Struct|SetmembersinSettingValues (Variables|/Game/Secpholand/Blueprints/ControllersYModes/baseClasses/NetworkGameInstance.NetworkGameInstance_C|Getsettings _asnetwork_game_instance) (Variables|Calibración|GetThresholdToApply) (Variables|Calibración|GetvolumenMicFinal) (Variables|Default|GetmasterLvl)))
  (Default|SaveDatosConfig _asnetwork_game_instance _structout)
  (Variables|/Game/Secpholand/Blueprints/ControllersYModes/baseClasses/ClientSide_Controller.ClientSide_Controller_C|SetTalkRoomID (.AsClient%20Side%20Controller (Utilities|Casting|CastToClientSide_Controller (Game|GetPlayerController 0))) (Variables|Default|GetpreviousTalkRoom))
  (Default|SaveCalibratedAudio _asnetwork_game_instance true))

(event Custom|AjustarVolumenMic
  (bind _returnvalue (Class|SystemMicControlBPLibrary|GetMicBoost))
  (bind _calibrationiteration (Variables|Default|GetcalibrationIteration))
  (bind _output_get (Variables|Calibración|SetvolumenMicFinal (Math|Interpolation|Ease "EaseOut" (/ (/ 5.0 (Math|Float|Max(Float) (Variables|Calibración|GetVolumenMedio) 2.5)) 2.0) 0.4 3.0 1.5)))
  (Default|SetMicVolume:client (.AsClient%20Side%20Controller (Utilities|Casting|CastToClientSide_Controller (Game|GetPlayerController 0))) _output_get)
  (if (Math|Boolean|ANDBoolean (< (Variables|Calibración|GetVolumenMedio) 2.0) (> (Variables|Calibración|GetaudibleRatio) (Utilities|Select :Index _calibrationiteration :Option%200 0.1 :Option%201 0.5 :Option%202 1.0)) (> _returnvalue 1e+01))
    (Class|SystemMicControlBPLibrary|SetMicBoost (+ _returnvalue (Utilities|Select :Index _calibrationiteration :Option%200 5.0 :Option%201 2.0 :Option%202 0.0)))
    (if (and (< (Variables|Calibración|GetVolumenMedio) 1.8) (== (Variables|Default|GetcalibrationIteration) 0))
      (Class|SystemMicControlBPLibrary|SetMicBoost (+ (Class|SystemMicControlBPLibrary|GetMicBoost) 3.0)))))

(event Custom|PrintSettings
  (Development|PrintString (Utilities|String|Append "Auditble Rate:  " (Utilities|String|ToString(Float) (Variables|Calibración|GetaudibleRatio)) "        " "volumen aplicado: " (Utilities|String|ToString(Float) (Variables|Calibración|GetvolumenMicFinal)) "/3.0        " "nivel de activación " (Utilities|String|ToString(Float) (Variables|Calibración|GetThresholdToApply)) "   " "Master: " (Utilities|String|ToString(Float) (Variables|Default|GetmasterLvl)) "    " "Nivel captado: " (Utilities|String|ToString(Float) (Variables|Calibración|GetVolumenMedio))) true true "(R=0.169583,G=1.000000,B=0.000000,A=1.000000)" 4e+01))

(event Custom|PaseDeRefinamiento
  (bind _audibleratio (Variables|Calibración|GetaudibleRatio))
  (bind _widgetcalibración (Variables|Default|GetwidgetCalibración))
  ;[1 1 1] Pase de refinamiento
  (if (>= _audibleratio 0.7)
    (if (> _audibleratio 0.97)
      (Variables|Calibración|SetThresholdToApply (+ (Variables|Calibración|GetThresholdToApply) 0.01)))
    (if (> (Variables|Default|GetcalibrationIteration) 1) :!label _label
      (CallFunction|FinishCalibration)
      (CallFunction|PrintSettings)
      (else
        (Default|PantallaPenultima (Variables|Default|GetwidgetCalibración))
        (Variables|Default|SeterrorInputs 0)
        (Math|Integer|IncrementInt (Variables|Default|GetcalibrationIteration)
          (:%20%20
            (CallFunction|PrintSettings)))))
    (elif (and (> (Variables|Calibración|GetVolumenMedio) 2.0) (>= (Variables|Calibración|GetaudibleRatio) (Math|Float|SelectFloat 0.5 0.55 (== (Variables|Default|GetcalibrationIteration) 1))))
      (Variables|Calibración|SetThresholdToApply (+ (Variables|Calibración|GetThresholdToApply) -0.01))
      (if (>= (Variables|Calibración|GetThresholdToApply) 0.06)
        (bind _output_get (Variables|Default|SetmasterLvl (- (Variables|Default|GetmasterLvl) (Math|Float|Lerp 0.01 0.04 (Math|Float|Clamp(Float) (* (- (Variables|Calibración|GetThresholdToApply) 0.06) 16.666666))))))
        (Audio|SetSoundMixClassOverride "/Game/Secpholand/audio/SouyndClasses/SecpholandMix.SecpholandMix" "/Game/Secpholand/audio/SouyndClasses/Master.Master" _output_get 1.0 1.0 true)
        (Audio|SetSoundMixClassOverride "/Game/Secpholand/audio/SouyndClasses/SecpholandMixVoice.SecpholandMixVoice" "/Game/Secpholand/audio/SouyndClasses/Master.Master" _output_get 1.0 1.0 true)
        (goto _label)
        (else
          (goto _label)))
      (else
        (Math|Integer|IncrementInt (Variables|Default|GeterrorInputs)
          (:%20%20
            (if (> (Variables|Default|GetcalibrationIteration) 1)
              (Default|NoInputSuficiente3 _widgetcalibración)
              (else
                (Default|NoInputSuficiente2 _widgetcalibración)))
            (CallFunction|PrintSettings)))))))

(event EventBeginPlay
  (bind _returnvalue (Game|GetPlayerController 0))
  (bind _asclient_side_controller (Utilities|Casting|CastToClientSide_Controller _returnvalue))
  (Class|VoipManagerComponent|InitVoice (Variables|Default|GetVoipManager) (Game|GetPlayerController 0))
  (Audio|Components|Audio|SetVolumeMultiplier (Variables|Default|GetVoipAudio) 0.0 :!class /Script/AudioMixer.SynthComponent)
  (Audio|SetSoundMixClassOverride "/Game/Secpholand/audio/SouyndClasses/SecpholandMix.SecpholandMix" "/Game/Secpholand/audio/SouyndClasses/Master.Master" 1.0 1.0 1.0 true)
  (Audio|SetSoundMixClassOverride "/Game/Secpholand/audio/SouyndClasses/SecpholandMixVoice.SecpholandMixVoice" "/Game/Secpholand/audio/SouyndClasses/Master.Master" 1.0 1.0 1.0 true)
  (Audio|SetSoundMixClassOverride "/Game/Secpholand/audio/SouyndClasses/SecpholandMix.SecpholandMix" "/Game/Secpholand/audio/SouyndClasses/Voice.Voice" 1.0 1.0 1.0 true)
  (Audio|SetSoundMixClassOverride "/Game/Secpholand/audio/SouyndClasses/SecpholandMixVoice.SecpholandMixVoice" "/Game/Secpholand/audio/SouyndClasses/Voice.Voice" 1.0 1.0 1.0 true)
  (bind _returnvalue_2 (UserInterface|CreateWidget "/Game/Secpholand/UI/Widgets/CalibraciónAudio.CalibraciónAudio_C" 0 self))
  (bind _output_get (Variables|Default|SetwidgetCalibración _returnvalue_2))
  (UserInterface|Viewport|AddtoViewport _output_get 0)
  (Class|SystemMicControlBPLibrary|SetMicVolume 1e+02)
  (Class|SystemMicControlBPLibrary|SetMicMute false)
  (if (!= (Variables|/Game/Secpholand/Blueprints/ControllersYModes/baseClasses/ClientSide_Controller.ClientSide_Controller_C|GetTalkRoomID _asclient_side_controller) -1)
    (Variables|Default|SetpreviousTalkRoom (Variables|/Game/Secpholand/Blueprints/ControllersYModes/baseClasses/ClientSide_Controller.ClientSide_Controller_C|GetTalkRoomID _asclient_side_controller))
    (Variables|/Game/Secpholand/Blueprints/ControllersYModes/baseClasses/ClientSide_Controller.ClientSide_Controller_C|SetTalkRoomID _asclient_side_controller -1)))

(event EventTick
  (params (DeltaSeconds :type Float%20%28single-precision%29))
  (if (Variables|Calibración|GetCapturando)
    (Math|Float|IncrementFloat (Variables|Calibración|GetFramesCapturing)
      (:%20%20
        (if (Variables|Calibración|GetFrameConAudioCapturado)
          (Math|Float|IncrementFloat (Variables|Calibración|GetFramesWithVoice)
            (:%20%20
              (Variables|Calibración|SetFrameConAudioCapturado false))))))))

(fn ConstructionScript)