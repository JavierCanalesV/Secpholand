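; KioscoArrow is a clickable arrow that scrolls a KioscoHolograma hologram kiosk up or down.
; On BeginPlay it finds and caches the KioscoHolograma actor in the level by class.
; On Click it runs the parent click logic, then calls UpToDown or DownToUp on the kiosk depending on its Up flag.
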(event EventClick
  (params (controller :type Client%20Side%20Controller%20Object%20Reference))
  (bind _kiosco (Variables|Default|Getkiosco))
  (|CallParentFunction controller)
  (if (Variables|Default|GetUp?)
    (Default|UptoDown _kiosco)
    (else
      (Default|DowntoUp _kiosco))))

(event EventBeginPlay
  (bind _returnvalue (Actor|GetActorOfClass "/Game/Secpholand/Blueprints/Clicables/ZoomClicables/KioscoHolograma.KioscoHolograma_C"))
  (Variables|Default|Setkiosco _returnvalue))

(fn ConstructionScript
  (|CallParentFunction))