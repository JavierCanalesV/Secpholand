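; Clickable meeting table that sends the player's character to a seat, warning that joining an occupied table starts a call with its occupants.
; From bird's-eye view, a click turns the camera, switches to street view and, after a distance-scaled delay, heads to the first seat without occupancy checks.
; Otherwise it blocks players already in calls, rejects full tables or asks confirmation, then picks a free seat by overlap test.
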(event Custom|SentarEnSillaLibre
  (bind _hoveruserwidget (Variables|Default|GethoverUserWidget))
  (bind _asclient_side_controller (Utilities|Casting|CastToClientSide_Controller (Game|GetPlayerController 0)))
  (if (> (Utilities|Array|Length (Variables|Default|GetSittingSlotsActors)) (Variables|Default|GetcurrentPlayers))
    (bind _sittingindex (CallFunction|GetFreeSlot))
    (Default|SpawnDecalatLocation _asclient_side_controller (Transformation|GetActorLocation (Utilities|Array|Get(acopy) (Variables|Default|GetSittingSlotsActors) _sittingindex)))
    (Default|MovetoLocation _asclient_side_controller (Transformation|GetActorLocation (Utilities|Array|Get(acopy) (Variables|Default|GetSittingSlotsActors) _sittingindex)))
    (Variables|/Game/Secpholand/Blueprints/OtherBP/SittingSlot.SittingSlot_C|Setactive (Utilities|Array|Get(acopy) (Variables|Default|GetSittingSlotsActors) _sittingindex) true)
    (else
      (Audio|PlaySound2D "/Game/Secpholand/audio/UISounds/UI_close.UI_close" 1.0 0.5 0.1 0 0)
      (Default|FillHoverInfo _hoveruserwidget "Mesa de reunión" "No quedan espacios disponibles en la mesa")
      (Default|Blocked _hoveruserwidget))))

(event Custom|ResetClickBind
  (CallFunction|ResetClick))

(event Custom|current%20client
  (params (NewParam :type Integer))
  (CallFunction|SetCurrent NewParam))

(event Custom|setCurrent
  (params (NewParam :type Integer))
  (Variables|Default|SetcurrentPlayers NewParam))

(event EventClick
  (params (controller :type Client%20Side%20Controller%20Object%20Reference))
  (bind _staticmesh (Variables|Default|GetStaticMesh))
  (bind _sittingslotsactors (Variables|Default|GetSittingSlotsActors))
  (bind _hoveruserwidget (Variables|Default|GethoverUserWidget))
  (bind _clientsidepawnref (Variables|/Game/Secpholand/Blueprints/ControllersYModes/baseClasses/ClientSide_Controller.ClientSide_Controller_C|GetClientSidePawnRef controller))
  (bind _returnvalue (Transformation|GetWorldLocation _staticmesh))
  (bind _returnvalue_2 (Transformation|GetActorLocation _clientsidepawnref))
  (bind _output (Utilities|Array|Get(acopy) _sittingslotsactors))
  (bind _springarm (Variables|/Game/Secpholand/Blueprints/ControllersYModes/baseClasses/ClientSide_Pawn.ClientSide_Pawn_C|GetSpringArm _clientsidepawnref))
  (bind _returnvalue_3 (Transformation|GetActorLocation _output))
  (|CallParentFunction controller)
  (if (Variables|/Game/Secpholand/Blueprints/ControllersYModes/baseClasses/ClientSide_Pawn.ClientSide_Pawn_C|Getb_VistaPajaro (Variables|/Game/Secpholand/Blueprints/ControllersYModes/baseClasses/ClientSide_Controller.ClientSide_Controller_C|GetClientSidePawnRef controller))
    (Transformation|SetWorldRotation _springarm (Math|Rotator|MakeRotator 0.0 (.pitch (Transformation|GetWorldRotation _springarm)) (.yaw (Math|Rotator|FindLookatRotation _returnvalue_2 _returnvalue))) false false)
    (bind _foundwidgets (Widget|GetAllWidgetsOfClass "/Game/Secpholand/UI/Widgets/HUDYChat/Minimapa/BotonVistaPajaro.BotonVistaPajaro_C" true))
    (Default|ClicarVistaCalle (Utilities|Array|Get(acopy) _foundwidgets))
    (Utilities|FlowControl|Delay (* (Math|Float|Clamp(Float) (- 1.0 (/ (Math|Vector|Distance(Vector) _returnvalue _returnvalue_2) (* (Class|MovementComponent|GetMaxSpeed (Variables|/Script/Engine.Character|GetCharacterMovement (Variables|/Game/Secpholand/Blueprints/ControllersYModes/baseClasses/ClientSide_Controller.ClientSide_Controller_C|GetServerSideCharacterRef controller))) 2.5)))) 2.5))
    (Default|SpawnDecalatLocation controller _returnvalue_3 :!label _label)
    (Default|MovetoLocation controller _returnvalue_3)
    (Variables|/Game/Secpholand/Blueprints/OtherBP/SittingSlot.SittingSlot_C|Setactive (Utilities|Array|Get(acopy) (Variables|Default|GetSittingSlotsActors) (Variables|Default|GetcurrentPlayers)) true)
    (elif (== (Variables|/Game/Secpholand/Blueprints/ControllersYModes/baseClasses/ClientSide_Controller.ClientSide_Controller_C|GetTalkRoomID controller) -1)
      (if (== (Variables|Default|GetcurrentPlayers) 0)
        (goto _label)
        (elif (> (Variables|Default|GetcurrentPlayers) (Utilities|Array|Length (Variables|Default|GetSittingSlotsActors)))
          (Audio|PlaySound2D "/Game/Secpholand/audio/UISounds/UI_close.UI_close" 1.0 0.5 0.1 0 0)
          (Default|FillHoverInfo _hoveruserwidget "Mesa de reunión" "No quedan espacios disponibles en la mesa")
          (Default|Blocked _hoveruserwidget)
          (else
            (bind _returnvalue_4 (UserInterface|CreateWidget "/Game/Secpholand/UI/Widgets/ContinueNotif.ContinueNotif_C" 0 "Mesa de reunión" "Esta mesa esta ocupada por una o más personas. Si te unes a la mesa entraras en una llamada con ellos. Estás seguro/a que quieres unirte? " "Unirme a la mesa"))
            (UserInterface|Viewport|AddtoViewport _returnvalue_4 0)
            (EventDispatchers|BindEventtoContinueButtonEvent _returnvalue_4 (delegate Custom|SentarEnSillaLibre))
            (EventDispatchers|BindEventtoCloseEvent _returnvalue_4 (delegate Custom|ResetClickBind)))))
      (else
        (bind _returnvalue_5 (UserInterface|CreateWidget "/Game/Secpholand/UI/Widgets/NotificaciónEnMedio.NotificaciónEnMedio_C" 0 "Cuelga tu llamada primero para poder sentarte"))
        (UserInterface|Viewport|AddtoViewport _returnvalue_5 0)))))

(event EventResetClick
  (bind _currentplayers (Variables|Default|GetcurrentPlayers))
  (|CallParentFunction)
  (if (>= _currentplayers 0)
    (Variables|/Game/Secpholand/Blueprints/OtherBP/SittingSlot.SittingSlot_C|Setactive (Utilities|Array|Get(acopy) (Variables|Default|GetSittingSlotsActors) _currentplayers) false)))

(fn ConstructionScript
  (|CallParentFunction)
  (Utilities|Array|Resize (Variables|Default|GetSittingSlotsActors) (Variables|Default|GetsittingSlotsNum)))

(fn GetFreeSlot
  (for (_array_element _array_index) (Variables|Default|GetSittingSlotsActors)
    (if (== (Utilities|Array|Length (Collision|GetOverlappingActors (Variables|/Game/Secpholand/Blueprints/OtherBP/SittingSlot.SittingSlot_C|GetgotoBox _array_element) "/Game/Secpholand/Blueprints/ControllersYModes/baseClasses/ClientSide_Pawn.ClientSide_Pawn_C" :!class /Script/Engine.PrimitiveComponent)) 0)
      (return _array_index)))
  (return -1))

(fn OnRepCurrentIndex)