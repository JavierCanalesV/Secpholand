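; Clickable office info avatar that shows a nameplate on hover and opens the Eventos widget when clicked.
; On BeginPlay it writes Username into the NombrePlayer widget held by the NoimbreyEmpresa component.
; Hover events call the parent logic and toggle that component's visibility, which HideNamePlate can also set directly.
; Each click runs the parent handler, adds a new Eventos widget to the viewport for the clicking controller, then calls ResetClick.
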(event Custom|HideNamePlate
  (params (NewParam :type Boolean))
  (Development|SetHiddeninGame (Variables|Default|GetNoimbreyEmpresa) NewParam true))

(event EventStopHover
  (|CallParentFunction)
  (Development|SetHiddeninGame (Variables|Default|GetNoimbreyEmpresa) true false))

(event EventClick
  (params (controller :type Client%20Side%20Controller%20Object%20Reference))
  (|CallParentFunction controller)
  (bind _returnvalue (UserInterface|CreateWidget "/Game/Secpholand/UI/Widgets/OficinaInfo/Eventos.Eventos_C" controller))
  (UserInterface|Viewport|AddtoViewport _returnvalue 0)
  (CallFunction|ResetClick))

(event EventHover
  (|CallParentFunction)
  (Development|SetHiddeninGame (Variables|Default|GetNoimbreyEmpresa) false false))

(event EventBeginPlay
  (bind _asnombre_player (Utilities|Casting|CastToNombrePlayer (UserInterface|GetUserWidgetObject (Variables|Default|GetNoimbreyEmpresa))))
  (Rendering|Components|TextRender|SetText (Variables|/Game/Secpholand/UI/Widgets/NombrePlayer.NombrePlayer_C|GetNombre _asnombre_player) (Utilities|Text|ToText(String) (Utilities|String|ToString(Name) (Variables|Default|GetUsername)))))

(fn ConstructionScript
  (|CallParentFunction))