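; EdificioEmpresa is a clickable company building in Secpholand that opens an information card for its company.
; Its Click event creates a FichaEmpresa widget owned by the clicking controller, passes in the building's Empresa value and adds it to the viewport.
; BeginPlay, overlap and Tick are disabled stubs, and the construction script only calls its parent.
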(event EventBeginPlay
  (|CallParentFunction) ; This node is disabled and will not be called.\nDrag off pins to build functionality.
)

(event Collision|EventActorBeginOverlap
  (params (OtherActor :type Actor%20Object%20Reference))
  (|CallParentFunction OtherActor) ; This node is disabled and will not be called.\nDrag off pins to build functionality.
)

(event EventTick
  (params (DeltaSeconds :type Float%20%28single-precision%29))
  (|CallParentFunction DeltaSeconds) ; This node is disabled and will not be called.\nDrag off pins to build functionality.
)

(event EventClick
  (params (hit :type Hit%20Result%20Structure) (controller :type Client%20Side%20Controller%20Object%20Reference))
  (bind _returnvalue (UserInterface|CreateWidget "/Game/Secpholand/UI/Widgets/FichaEmpresa.FichaEmpresa_C" controller (Variables|Default|Getempresa)))
  (UserInterface|Viewport|AddtoViewport _returnvalue 0))

(fn ConstructionScript
  (|CallParentFunction))