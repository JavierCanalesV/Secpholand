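; Clickable indoor meeting table that seats a player and joins them to the table's voice/call room.
; The server builds seats from child ClicableAvatar actors and tracks occupants in a Usernames array, where an empty string means free.
; Clicking rejects players already in a call, confirms before joining occupied tables, then requests the first free seat through the Controller.
; Sitting blends the camera to the table and opens a call widget, whose hang-up event triggers leaving.
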(event Custom|Mesa%20Llena
  (bind _hoveruserwidget (Variables|Default|GethoverUserWidget))
  ;[1 1 1] Mesa Llena
  (Audio|PlaySound2D "/Game/Secpholand/audio/UISounds/UI_close.UI_close" 1.0 0.5 0.1 0 0)
  (CallFunction|Hover)
  (Utilities|IsValid _hoveruserwidget
    (:Is%20Valid
      (Default|FillHoverInfo _hoveruserwidget "Mesa de reunión" "No quedan espacios disponibles en la mesa")
      (Default|Blocked _hoveruserwidget))))

(event Custom|SentarEnSillaLibre
  ;[1 1 1] Evento Click
  (CallFunction|PedirAccesoMesa (stale EventClick controller)))

(event Custom|InitAsientos
  ;[1 1 1] Inicializar Asientos
  (for _array_element (Actor|GetAllChildActors true)
    (bind _asclicable_avatar (Utilities|Casting|CastToClicableAvatar _array_element))
    (Utilities|Array|Add (Variables|Default|GetAvatars) _asclicable_avatar))
  (Utilities|Array|Resize (Variables|Default|GetUsernames) (Utilities|Array|Length (Variables|Default|GetAvatars))))

(event Custom|PedirAccesoMesa
  (params (Controller :type Client%20Side%20Controller%20Object%20Reference%20%28by%20ref%29))
  ;[1 1 1] Pedir Acceso a Mesa
  (bind _index (CallFunction|GetAsientoLibre))
  (if (!= _index -1)
    (Default|SentarseEnMesaReunionInterior Controller _index self)
    (CallFunction|SeHaSentado)
    (else
      (CallFunction|MesaLlena))))

(event Custom|ResetClickBind
  ;[1 1 1] Evento Click
  (CallFunction|ResetClick))

(event Custom|SeHaSentado
  (bind _returnvalue (Game|GetPlayerController 0))
  ;[1 1 1] Jugador Se Ha Sentado
  (Variables|Default|SetCachedViewTarget (Pawn|GetViewTarget _returnvalue))
  (Game|Player|SetViewTargetwithBlend _returnvalue self 2.0 "VTBlend_EaseInOut" 2.0 false)
  (bind _asclient_side_controller (Utilities|Casting|CastToClientSide_Controller (Game|GetPlayerController 0)))
  (Default|EntrarEnLlamada:Client _asclient_side_controller (Variables|Default|GetRoomID))
  (bind (_widget _found) (Default|GetWidgetLlamada _asclient_side_controller))
  (if _found
    (Widget|RemovefromParent _widget))
  (bind _returnvalue_2 (UserInterface|CreateWidget "/Game/Secpholand/UI/Widgets/Llamada.Llamada_C" 0 (Utilities|String|Append "Llamada de la mesa: " (Utilities|String|ToString(Integer) (Variables|Default|GetRoomID)))))
  (Class|VerticalBox|AddChildtoVerticalBox (Variables|/Game/Secpholand/UI/Widgets/HUDYChat/HUD.HUD_C|GetHudArribaizquierda (Variables|/Game/Secpholand/Blueprints/ControllersYModes/baseClasses/ClientSide_Controller.ClientSide_Controller_C|GetHUD _asclient_side_controller)) _returnvalue_2)
  (Default|QuitarParticipantesForce _returnvalue_2)
  (EventDispatchers|BindEventtoLlamadaColgada _returnvalue_2 (delegate Custom|PedirSalirDeReunion))
  (Collision|SetActorEnableCollision false))

(event Custom|PedirSalirDeReunion
  ;[1 1 1] Jugador Se Ha Sentado
  (bind _asclient_side_controller (Utilities|Casting|CastToClientSide_Controller (Game|GetPlayerController 0)))
  (bind _idx (CallFunction|GetIdxbyUsername (.Username (Utilities|Struct|BreakUserInfo_Public (Variables|/Game/Secpholand/Blueprints/ControllersYModes/baseClasses/ServerSide_Character.ServerSide_Character_C|GetUserInfo (Variables|/Game/Secpholand/Blueprints/ControllersYModes/baseClasses/ClientSide_Controller.ClientSide_Controller_C|GetServerSideCharacterRef _asclient_side_controller))))))
  (if (!= _idx -1)
    (Default|PedirSalirMesaReunion:Client _asclient_side_controller self _idx))
  (CallFunction|SalirDeReunion:Client true))

(event Custom|SetUsernameInArray
  (params (Username :type String) (Index :type Integer))
  (Networking|SwitchHasAuthority
    (:Authority
      (Utilities|Array|SetArrayElem (Variables|Default|GetUsernames) Index Username))))

(event Custom|SalirDeReunion:Client
  (params (PossessExtCamera? :type Boolean))
  ;[1 1 1] Jugador ha Salido de la Reunión
  (CallFunction|UnBindfromLlamadaColgada)
  (if PossessExtCamera?
    (Game|Player|SetViewTargetwithBlend (Game|GetPlayerController 0) (Variables|Default|GetCachedViewTarget) 2.0 "VTBlend_EaseInOut" 2.0 false))
  (CallFunction|ActivarMesaClicable)
  (bind _asinterior_controller (Utilities|Casting|CastToInteriorController (Game|GetPlayerController 0)))
  (Default|ColgarLlamada:Client _asinterior_controller))

(event Custom|ActivarMesaClicable
  ;[1 1 1] Jugador ha Salido de la Reunión
  (Collision|SetActorEnableCollision true))

(event Custom|UnBindFromLlamadaColgada
  ;[1 1 1] Jugador Se Ha Sentado
  (bind _asclient_side_controller (Utilities|Casting|CastToClientSide_Controller (Game|GetPlayerController 0)))
  (bind (_widget _found) (Default|GetWidgetLlamada _asclient_side_controller))
  (if _found
    (EventDispatchers|UnbindEventfromLlamadaColgada _widget (delegate Custom|PedirSalirDeReunion))))

(event EventBeginPlay
  (|CallParentFunction)
  (Networking|SwitchHasAuthority
    (:Authority
      (CallFunction|InitAsientos))))

(event EventClick
  (params (controller :type Client%20Side%20Controller%20Object%20Reference))
  ;[1 1 1] Evento Click
  (|CallParentFunction controller)
  (if (== (Variables|/Game/Secpholand/Blueprints/ControllersYModes/baseClasses/ClientSide_Controller.ClientSide_Controller_C|GetTalkRoomID controller) -1)
    (bind _isnotempty_ (CallFunction|IsNotEmpty))
    (if _isnotempty_
      (bind _returnvalue (UserInterface|CreateWidget "/Game/Secpholand/UI/Widgets/ContinueNotif.ContinueNotif_C" 0 "Mesa de reunión" "Esta mesa esta ocupada por una o más personas. Si te unes a la mesa entraras en una llamada con ellos. Estás seguro/a que quieres unirte? " "Unirme a la mesa"))
      (UserInterface|Viewport|AddtoViewport _returnvalue 0)
      (EventDispatchers|BindEventtoContinueButtonEvent _returnvalue (delegate Custom|SentarEnSillaLibre))
      (EventDispatchers|BindEventtoCloseEvent _returnvalue (delegate Custom|ResetClickBind))
      (else
        (CallFunction|PedirAccesoMesa controller)))
    (else
      (bind _returnvalue_2 (UserInterface|CreateWidget "/Game/Secpholand/UI/Widgets/NotificaciónEnMedio.NotificaciónEnMedio_C" 0 "Cuelga tu llamada primero para poder sentarte"))
      (UserInterface|Viewport|AddtoViewport _returnvalue_2 0)
      (CallFunction|ResetClick))))

(fn ConstructionScript
  (|CallParentFunction))

(fn GetAsientoLibre
  (for (_array_element _array_index) (Variables|Default|GetUsernames)
    (if (Utilities|Enum|Equal(Enum) _array_element "")
      (return _array_index)))
  (return -1))

(fn IsNotEmpty
  (for _array_element (Variables|Default|GetUsernames)
    (if (Utilities|Enum|NotEqual(Enum) _array_element "")
      (return true)))
  (return false))

(fn GetIdxbyUsername
  (params (Username :type String))
  (for (_array_element _array_index) (Variables|Default|GetUsernames)
    (if (Utilities|Enum|Equal(Enum) _array_element Username)
      (return _array_index)))
  (return -1))