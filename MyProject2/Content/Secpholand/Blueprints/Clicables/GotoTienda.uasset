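; A clickable in the Secpholand world that opens the shop UI when the player arrives at it.
; Arrival completes objective 19, resets the click, registers itself on the central player controller and creates the Tienda widget.
; It then fills the widget with its per-category item lists, mapping each category enum to one of three tabs and using the enum name as the section title.
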(event EventArrived
  (CallFunction|CompleteObjective 19)
  (CallFunction|ResetClick)
  (Variables|/Game/Secpholand/Blueprints/ControllersYModes/SecpholandCentralController.SecpholandCentralController_C|SetTienda (.AsSecpholand%20Central%20Controller (Utilities|Casting|CastToSecpholandCentralController (Game|GetPlayerController 0))) self)
  (bind _returnvalue (UserInterface|CreateWidget "/Game/Secpholand/UI/Widgets/Tienda/Tienda.Tienda_C"))
  (UserInterface|Viewport|AddtoViewport _returnvalue 0)
  (for _array_element (Variables|Default|GetObjetosDeLaTiendaPorCategorias)
    (Default|FillCategoriaEnTab _returnvalue (Utilities|Select :Index (.Categoria (Utilities|Struct|BreakObjetosDeTiendaPorCategoria _array_element)) :NewEnumerator0 1 :NewEnumerator1 1 :NewEnumerator2 2 :NewEnumerator3 2 :NewEnumerator4 1 :NewEnumerator5 3) (.Objetos (Utilities|Struct|BreakObjetosDeTiendaPorCategoria _array_element)) (Utilities|Text|ToText(String) (Utilities|String|EnumtoString (.Categoria (Utilities|Struct|BreakObjetosDeTiendaPorCategoria _array_element)))))))

(fn ConstructionScript
  (|CallParentFunction))