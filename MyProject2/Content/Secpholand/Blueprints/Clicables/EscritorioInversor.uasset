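; EscritorioInversor is a clickable investor desk that opens a company profile when clicked.
; On click it runs the parent behavior, then creates a FichaEmpresa widget with its NombreEmpresa value and adds it to the viewport.
; Its construction script also copies NombreEmpresa into HoverTitle, so the company name serves as the hover title.
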(event EventBeginPlay
  (|CallParentFunction))

(event EventClick
  (params (controller :type Client%20Side%20Controller%20Object%20Reference))
  (|CallParentFunction controller)
  (bind _returnvalue (UserInterface|CreateWidget "/Game/Secpholand/UI/Widgets/Perfiles/FichaEmpresa.FichaEmpresa_C" 0 (Variables|Default|GetNombreEmpresa)))
  (UserInterface|Viewport|AddtoViewport _returnvalue 0))

(fn ConstructionScript
  (|CallParentFunction)
  (Variables|Default|SethoverTitle (Utilities|Text|ToText(String) (Variables|Default|GetNombreEmpresa))))