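; Clickable auditorium elevator that requests entry to a destination room when clicked.
; On click it clears its outline and sends its destination room ID through the InteriorController.
; A blocked response shows "Access not allowed" on the hover widget, explaining either that the room is closed or that the player lacks permission, depending on list membership.
; An allowed response only resets the click state.
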(event Custom|ReceiveElevatorBlocked
  (params (IsInTheList :type Boolean))
  (bind _hoveruserwidget (Variables|Default|GethoverUserWidget))
  (if IsInTheList
    (Default|FillHoverInfo _hoveruserwidget "Access not allowed" "The room is not open at the moment")
    (Default|Blocked _hoveruserwidget)
    (else
      (Default|FillHoverInfo _hoveruserwidget "Access not allowed" "You're not allowed in this room")
      (Default|Blocked _hoveruserwidget))))

(event Custom|ReceiveCanEnterElevator
  (CallFunction|ResetClick))

(event EventBeginPlay
  (|CallParentFunction))

(event EventClick
  (params (controller :type Client%20Side%20Controller%20Object%20Reference))
  (Default|StopOutliningActor controller self)
  (bind _asinterior_controller (Utilities|Casting|CastToInteriorController controller))
  (Default|SolicitarEntrarSala:Client _asinterior_controller (Variables|Default|GetIDSalaDestinacion)))

(fn ConstructionScript
  (|CallParentFunction))