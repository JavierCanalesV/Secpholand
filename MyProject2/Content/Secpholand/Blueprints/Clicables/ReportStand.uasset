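; ReportStand is a clickable exhibition stand Blueprint that reports visitor interactions with a company's stand.
; Click and construction only call the parent logic.
; On Arrived, after the parent behavior, it casts player controller 0 to EC_expo_Controller and calls its ReportsEPs InteraccionesStandFuction, passing the hover title, the company name and an empty contact.
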(event EventBeginPlay)

(event Collision|EventActorBeginOverlap
  (params (OtherActor :type Actor%20Object%20Reference)))

(event EventTick
  (params (DeltaSeconds :type Float%20%28single-precision%29)))

(event EventArrived
  (|CallParentFunction)
  (Default|InteraccionesStandFuction (Variables|/Game/Secpholand/Blueprints/ControllersYModes/baseClasses/ClientSide_Controller.ClientSide_Controller_C|GetReportsEPs (.AsEC%20Expo%20Controller (Utilities|Casting|CastToEC_expo_Controller (Game|GetPlayerController 0)))) (Utilities|String|ToString(Text) (Variables|Default|GethoverTitle)) (Variables|Default|Getempresa)))

(event EventClick
  (params (controller :type Client%20Side%20Controller%20Object%20Reference))
  (|CallParentFunction controller))

(fn ConstructionScript
  (|CallParentFunction))