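; Clickable actor in Secpholand that opens the job offers (ofertas de trabajo) screen.
; One second after BeginPlay it asks SecpholandCentralGameState to retrieve the offers from the server.
; A click creates the OfertasDeTrabajo widget, adds it to the viewport and, after a short retriggerable delay, fills it from the OfertasTrabajo variable.
; Both BeginPlay and the click call the parent class logic first.
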(event Collision|EventActorBeginOverlap
  (params (OtherActor :type Actor%20Object%20Reference)))

(event EventTick
  (params (DeltaSeconds :type Float%20%28single-precision%29)))

(event EventClick
  (params (controller :type Client%20Side%20Controller%20Object%20Reference))
  (|CallParentFunction controller)
  (bind _returnvalue (UserInterface|CreateWidget "/Game/Secpholand/UI/Widgets/OficinaInfo/ofertasDeTrabajo.ofertasDeTrabajo_C"))
  (UserInterface|Viewport|AddtoViewport _returnvalue 0)
  (Utilities|FlowControl|RetriggerableDelay 0.3)
  (Default|FillOfertas _returnvalue (Variables|Default|GetOfertas%20Trabajo)))

(event EventBeginPlay
  (|CallParentFunction)
  (Utilities|FlowControl|Delay 1.0)
  (Default|RetrieveOfertasTrabajos:Server (.AsSecpholand%20Central%20Game%20State (Utilities|Casting|CastToSecpholandCentralGameState (Game|GetGameState)))))

(fn ConstructionScript
  (|CallParentFunction))