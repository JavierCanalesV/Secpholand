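; ClicableAvatar is a clickable user avatar with a hideable name and company plate.
; Hover spawns a TargetaUsuario2 profile card at an offset from the actor's projected screen position, unless one is already valid, and has ClientSide_Controller retrieve that Username's info into it.
; Click opens a DesplegableMenu dropdown for that Username at the mouse position.
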(event Custom|HideNamePlate
  (params (NewParam :type Boolean))
  (Development|SetHiddeninGame (Variables|Default|GetNoimbreyEmpresa) NewParam true))

(event EventClick
  (params (hit :type Hit%20Result%20Structure) (controller :type Client%20Side%20Controller%20Object%20Reference))
  (bind _returnvalue (UserInterface|CreateWidget "/Game/Secpholand/UI/Widgets/desplegableMenu.desplegableMenu_C" controller (Variables|Default|GetUsername)))
  (UserInterface|Viewport|AddtoViewport _returnvalue 0)
  (bind _returnvalue_2 (Class|WidgetLayoutLibrary|GetMousePositiononViewport))
  (Class|UserWidget|SetPositioninViewport _returnvalue (Math|Vector2D|MakeVector2D (.x _returnvalue_2) (.y _returnvalue_2)) false))

(event EventHover
  (bind _returnvalue (Transformation|GetActorLocation))
  (bind _returnvalue_2 (Game|GetPlayerController 0))
  (bind _screenposition (Class|GameplayStatics|ProjectWorldtoScreen _returnvalue_2 _returnvalue true))
  (Utilities|IsValid (Variables|Default|Getwidget)
    (:Is%20Not%20Valid
      (bind _returnvalue_3 (UserInterface|CreateWidget (Variables|Default|GetwidgetClass)))
      (bind _output_get (Variables|Default|Setwidget _returnvalue_3))
      (UserInterface|Viewport|AddtoViewport _output_get 0)
      (bind _astargeta_usuario_2 (Utilities|Casting|CastToTargetaUsuario2 (Variables|Default|Getwidget)))
      (bind _asclient_side_controller (Utilities|Casting|CastToClientSide_Controller _returnvalue_2))
      (Default|RetrieveUserInfoCompressed _asclient_side_controller (Variables|Default|GetUsername) _astargeta_usuario_2)
      (Class|UserWidget|SetPositioninViewport (Variables|Default|Getwidget) (Math|Vector2D|MakeVector2D (- (.x _screenposition) 5.8e+02) (- (.y _screenposition) 1.8e+02)) true))))

(event EventBeginPlay
  (Variables|Default|SetwidgetClass "/Game/Secpholand/UI/Widgets/TargetaUsuario2.TargetaUsuario2_C"))

(fn ConstructionScript
  (|CallParentFunction))