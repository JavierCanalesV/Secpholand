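; SergioMC is a clickable helper in the Secpho meeting center that explains, in Spanish, the tech challenge information and permission-restricted meeting rooms.
; On BeginPlay it writes its Username into the NombrePlayer name widget, then creates a BocadilloDeAyuda speech bubble with two texts for the WidgetAyuda component.
; Clicking runs the parent logic, resets the click and unhides the bubble.
; Hover events defer to the parent.
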(event EventStopHover
  (|CallParentFunction))

(event EventClick
  (params (controller :type Client%20Side%20Controller%20Object%20Reference))
  (|CallParentFunction controller)
  (CallFunction|ResetClick)
  (Development|SetHiddeninGame (Variables|Default|GetwidgetAyuda) false false))

(event EventHover
  (|CallParentFunction))

(event EventBeginPlay
  (bind _asnombre_player (Utilities|Casting|CastToNombrePlayer (UserInterface|GetUserWidgetObject (Variables|Default|GetNoimbreyEmpresa))))
  (Rendering|Components|TextRender|SetText (Variables|/Game/Secpholand/UI/Widgets/NombrePlayer.NombrePlayer_C|GetNombre _asnombre_player) (Utilities|Text|ToText(String) (Utilities|String|ToString(Name) (Variables|Default|GetUsername))))
  (bind _returnvalue (UserInterface|CreateWidget "/Game/Secpholand/UI/Widgets/Tutoriales/BocadilloDeAyuda.BocadilloDeAyuda_C"))
  (Default|SetTexts _returnvalue (Utilities|Array|MakeArray "Hola! bienvenido al meeting center. En este edificio podrás consultar toda la información de los últimos retos tecnológicos que ofrece Secpho. " "Además también podras realizar reuniones concertadas con Secpho.  
Ten en cuenta que a estas salas de reunión solo podras acceder si tienes permisos. "))
  (UserInterface|SetWidget (Variables|Default|GetwidgetAyuda) _returnvalue))

(fn ConstructionScript
  (|CallParentFunction))