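; Clickable cafeteria building whose elevator carries the player between street and upper floor.
; Click exits any bird's-eye view, shows a first-visit tutorial and walks the player to the entrance; proximity or box overlap starts the ride.
; Timed sequences animate doors and camera, then hide the teleport behind a screen fade.
; Arrival flips OnTop, hover text and floor collision, so the next click makes the return trip.
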(event OnComponentBeginOverlap(BoxBOT)
  (params (OverlappedComponent :type Primitive%20Component%20Object%20Reference) (OtherActor :type Actor%20Object%20Reference) (OtherComp :type Primitive%20Component%20Object%20Reference) (OtherBodyIndex :type Integer) (bFromSweep :type Boolean) (SweepResult :type Hit%20Result%20Structure%20%28by%20ref%29))
  (bind _playercontroller (Variables|Default|GetPlayerController))
  (bind _serversidecharacterref (Variables|/Game/Secpholand/Blueprints/ControllersYModes/baseClasses/ClientSide_Controller.ClientSide_Controller_C|GetServerSideCharacterRef _playercontroller))
  (if (Variables|Default|Getactive)
    (bind _asserver_side_character (Utilities|Casting|CastToServerSide_Character OtherActor))
    (Utilities|IsValid _playercontroller
      (:Is%20Valid
        (if (== _asserver_side_character _serversidecharacterref)
          (CallFunction|BotElevatorEvent _serversidecharacterref))))))

(event OnComponentBeginOverlap(BoxTOP)
  (params (OverlappedComponent :type Primitive%20Component%20Object%20Reference) (OtherActor :type Actor%20Object%20Reference) (OtherComp :type Primitive%20Component%20Object%20Reference) (OtherBodyIndex :type Integer) (bFromSweep :type Boolean) (SweepResult :type Hit%20Result%20Structure%20%28by%20ref%29))
  (bind _playercontroller (Variables|Default|GetPlayerController))
  (if (Variables|Default|Getactive)
    (bind _asserver_side_character (Utilities|Casting|CastToServerSide_Character OtherActor))
    (Utilities|IsValid _playercontroller
      (:Is%20Valid
        (if (== _asserver_side_character (Variables|/Game/Secpholand/Blueprints/ControllersYModes/baseClasses/ClientSide_Controller.ClientSide_Controller_C|GetServerSideCharacterRef _playercontroller))
          (CallFunction|TopElevatorEvent))))))

(event Custom|abrir/cerrar%20%20puertas
  (bind _newtrack_0 (Timeline|Timeline_0 PlayFromStart)
    (:Update
      (Transformation|SetRelativeLocation (Variables|Default|GetBotL) (Math|Vector|MakeVector (+ (* _newtrack_0 1.3e+02) 131.0) -1e+01 0.0) false false)
      (Transformation|SetRelativeLocation (Variables|Default|GetBotR) (Math|Vector|MakeVector (- (* _newtrack_0 -1.3e+02) 1.0) -12.0 0.0) false false))))

(event Custom|CameraTraveling
  (params (Forward? :type Boolean))
  (bind _playercontroller (Variables|Default|GetPlayerController))
  (bind _clientsidepawnref (Variables|/Game/Secpholand/Blueprints/ControllersYModes/baseClasses/ClientSide_Controller.ClientSide_Controller_C|GetClientSidePawnRef _playercontroller))
  (if Forward?
    (bind _newtrack_0 (Timeline|CameraTimeline PlayFromStart)
      (:Update
        (Transformation|SetWorldLocationAndRotation (Variables|/Game/Secpholand/Blueprints/ControllersYModes/baseClasses/ClientSide_Pawn.ClientSide_Pawn_C|GetCamera _clientsidepawnref) (.Location (Math|Transform|BreakTransform (Math|Transform|Lerp(Transform) (Transformation|GetWorldTransform (Variables|/Game/Secpholand/Blueprints/ControllersYModes/baseClasses/ClientSide_Pawn.ClientSide_Pawn_C|GetCameraOrighinalPos _clientsidepawnref)) (Variables|Default|GetCameraSnap) _newtrack_0))) (.Rotation (Math|Transform|BreakTransform (Math|Transform|Lerp(Transform) (Transformation|GetWorldTransform (Variables|/Game/Secpholand/Blueprints/ControllersYModes/baseClasses/ClientSide_Pawn.ClientSide_Pawn_C|GetCameraOrighinalPos _clientsidepawnref)) (Variables|Default|GetCameraSnap) _newtrack_0))) false false)))
    (else
      (Timeline|CameraTimeline ReverseFromEnd))))

(event Custom|gotoTOP%20event
  (bind _gototop (Variables|Default|GetGotoTop))
  (bind _playercontroller (Variables|Default|GetPlayerController))
  (bind _returnvalue (Transformation|GetWorldLocation _gototop))
  (if (<= (Math|Vector|Distance(Vector) (Transformation|GetActorLocation (Variables|/Game/Secpholand/Blueprints/ControllersYModes/baseClasses/ClientSide_Controller.ClientSide_Controller_C|GetClientSidePawnRef (Variables|Default|GetPlayerController))) (Transformation|GetWorldLocation (Variables|Default|GetGotoTop))) 2e+02)
    (CallFunction|TopElevatorEvent)
    (else
      (Variables|Default|Setactive true)))
  (Default|SpawnDecalatLocation _playercontroller _returnvalue)
  (Default|MovetoLocation _playercontroller _returnvalue))

(event Custom|BotElevatorEvent
  (params (serverSide :type Server%20Side%20Character%20Object%20Reference))
  (bind _playercontroller (Variables|Default|GetPlayerController))
  (bind _elevatorinsidetop (Variables|Default|GetElevatorInsideTOP))
  (bind _playercontroller_2 (Variables|Default|GetPlayerController))
  (bind _playercontroller_3 (Variables|Default|GetPlayerController))
  (bind _clientsidecontrollerref (Variables|/Game/Secpholand/Blueprints/ControllersYModes/baseClasses/ServerSide_Character.ServerSide_Character_C|GetclientSideControllerRef serverSide))
  (bind _camerasnapbot (Variables|Default|GetCameraSnapBOT))
  (bind _playercontroller_4 (Variables|Default|GetPlayerController))
  (bind _returnvalue (Transformation|GetWorldLocation _elevatorinsidetop))
  (bind _returnvalue_2 (Transformation|GetWorldLocation _camerasnapbot))
  (bind _clientsidepawnref (Variables|/Game/Secpholand/Blueprints/ControllersYModes/baseClasses/ClientSide_Controller.ClientSide_Controller_C|GetClientSidePawnRef _playercontroller_2))
  (bind _clientsidepawnref_2 (Variables|/Game/Secpholand/Blueprints/ControllersYModes/baseClasses/ClientSide_Controller.ClientSide_Controller_C|GetClientSidePawnRef _clientsidecontrollerref))
  (bind _clientsidepawnref_3 (Variables|/Game/Secpholand/Blueprints/ControllersYModes/baseClasses/ClientSide_Controller.ClientSide_Controller_C|GetClientSidePawnRef _playercontroller))
  (bind _camera (Variables|/Game/Secpholand/Blueprints/ControllersYModes/baseClasses/ClientSide_Pawn.ClientSide_Pawn_C|GetCamera _clientsidepawnref_2))
  (bind _returnvalue_3 (Transformation|GetWorldLocation _camera))
  (bind _returnvalue_4 (Math|Vector|Distance(Vector) _returnvalue_3 _returnvalue_2))
  (bind _returnvalue_5 (/ _returnvalue_4 1.5e+03))
  (bind _returnvalue_6 (Math|Float|Clamp(Float) _returnvalue_5))
  (Variables|Default|Setactive false)
  (bind _output_get (Variables|Default|SetairVol (Math|Float|Lerp 0.2 0.7 _returnvalue_6)))
  (Components|Timeline|SetPlayRate (Variables|Default|GetCameraTimeline) (Math|Float|Lerp 1.0 0.7 _returnvalue_6))
  (Audio|PlaySound2D "/Game/Secpholand/audio/transition.transition" _output_get 1.0 0.0 0 0)
  (CallFunction|ResetClick)
  (bind _output_get_2 (Variables|Default|Setcharacter serverSide))
  (Default|SetControllsConstraints (Variables|/Game/Secpholand/Blueprints/ControllersYModes/baseClasses/ServerSide_Character.ServerSide_Character_C|GetclientSideControllerRef _output_get_2) true false false false)
  (Default|StopOutliningActor (Variables|/Game/Secpholand/Blueprints/ControllersYModes/baseClasses/ServerSide_Character.ServerSide_Character_C|GetclientSideControllerRef _output_get_2) self)
  (Variables|Default|SetCameraSnap (Transformation|GetWorldTransform (Variables|Default|GetCameraSnapBOT)))
  (CallFunction|Abrir/cerrarPuertas)
  (CallFunction|CameraTraveling true)
  (Utilities|FlowControl|Delay 1.0)
  (Transformation|DetachFromComponent (Variables|/Game/Secpholand/Blueprints/ControllersYModes/baseClasses/ClientSide_Pawn.ClientSide_Pawn_C|GetCamera (Variables|/Game/Secpholand/Blueprints/ControllersYModes/baseClasses/ClientSide_Controller.ClientSide_Controller_C|GetClientSidePawnRef (Variables|Default|GetPlayerController))) "KeepWorld" "KeepWorld" "KeepWorld" false)
  (Default|ChangeSpeed:Server _playercontroller_4 2.5e+02)
  (Default|MovetoLocation _playercontroller_4 (Transformation|GetWorldLocation (Variables|Default|GetElevatorInsideBOT)))
  (Utilities|FlowControl|Delay 2.5)
  (Default|HideNamePlate (Variables|Default|GetCharacter) true)
  (CameraFades|StartCameraFade :self (Variables|/Script/Engine.PlayerController|GetPlayerCameraManager (Variables|Default|GetPlayerController)) :ToAlpha 1.0 :Duration 0.6 :bHoldWhenFinished true)
  (Utilities|FlowControl|Delay 0.6)
  (Default|TeleportPlayer:Client (Variables|Default|GetPlayerController) _returnvalue)
  (Transformation|SetActorLocation (Variables|/Game/Secpholand/Blueprints/ControllersYModes/baseClasses/ClientSide_Controller.ClientSide_Controller_C|GetClientSidePawnRef (Variables|Default|GetPlayerController)) _returnvalue false false)
  (Transformation|SetWorldRotation (Variables|/Game/Secpholand/Blueprints/ControllersYModes/baseClasses/ClientSide_Pawn.ClientSide_Pawn_C|GetSpringArm _clientsidepawnref_3) "40.000000,270.000000, 0" false false)
  (Default|ZoomEvent _clientsidepawnref_3 (Variables|/Game/Secpholand/Blueprints/ControllersYModes/baseClasses/ClientSide_Controller.ClientSide_Controller_C|Getzoom (Variables|Default|GetPlayerController)))
  (Transformation|SetWorldTransform (Variables|/Game/Secpholand/Blueprints/ControllersYModes/baseClasses/ClientSide_Pawn.ClientSide_Pawn_C|GetCamera _clientsidepawnref_3) (Transformation|GetWorldTransform (Variables|Default|GetCameraSnapTOP)) false false)
  (Utilities|FlowControl|Delay 1.0)
  (CameraFades|StartCameraFade :self (Variables|/Script/Engine.PlayerController|GetPlayerCameraManager (Variables|Default|GetPlayerController)) :FromAlpha 1.0 :Duration 0.6 :bHoldWhenFinished true)
  (Utilities|FlowControl|Delay 0.6)
  (CallFunction|Abrir/cerrarPuertas)
  (Utilities|FlowControl|Delay 1.0)
  (Default|MovetoLocation (Variables|Default|GetPlayerController) (Transformation|GetWorldLocation (Variables|Default|GetGotoTop)))
  (Variables|Default|SetCameraSnap (Transformation|GetWorldTransform (Variables|Default|GetCameraSnapTOP)))
  (Utilities|FlowControl|Delay 2.0)
  (Transformation|AttachComponentToComponent (Variables|/Game/Secpholand/Blueprints/ControllersYModes/baseClasses/ClientSide_Pawn.ClientSide_Pawn_C|GetCamera _clientsidepawnref) (Variables|/Game/Secpholand/Blueprints/ControllersYModes/baseClasses/ClientSide_Pawn.ClientSide_Pawn_C|GetSpringArm _clientsidepawnref) "None" "KeepWorld" "KeepWorld" "KeepWorld" true)
  (CallFunction|CameraTraveling false)
  (Utilities|FlowControl|Delay 1.0)
  (for _array_element (Variables|Default|GetmeshesToActivate)
    (Collision|SetActorEnableCollision _array_element true)
    (Collision|SetCollisionEnabled (Variables|/Script/Engine.StaticMeshActor|GetStaticMeshComponent _array_element) "QueryOnly"))
  (Default|SetControllsConstraints (Variables|Default|GetPlayerController) true true true true)
  (Variables|Default|SetonTop true)
  (Collision|SetCollisionEnabled (Variables|Default|GetColliderWalls) "QueryOnly")
  (Collision|SetCollisionEnabled (Variables|Default|GetColliderStructure) "NoCollision")
  (Variables|Default|SethoverTitle "Volver a la calle")
  (Variables|Default|SetHoverNormalHint "Haz click para bajar...")
  (UserInterface|Viewport|AddtoViewport (Variables|/Game/Secpholand/Blueprints/ControllersYModes/baseClasses/ClientSide_Controller.ClientSide_Controller_C|GetHUD _playercontroller_3) 0)
  (Default|CangeSpeed:Client _playercontroller_3 9.5e+02)
  (Default|HideNamePlate (Variables|Default|GetCharacter) false))

(event Custom|TopElevatorEvent
  (bind _playercontroller (Variables|Default|GetPlayerController))
  (bind _elevatorinsidebot (Variables|Default|GetElevatorInsideBOT))
  (bind _camerasnapbot (Variables|Default|GetCameraSnapBOT))
  (bind _playercontroller_2 (Variables|Default|GetPlayerController))
  (bind _playercontroller_3 (Variables|Default|GetPlayerController))
  (bind _playercontroller_4 (Variables|Default|GetPlayerController))
  (bind _playercontroller_5 (Variables|Default|GetPlayerController))
  (bind _returnvalue (Transformation|GetWorldLocation _elevatorinsidebot))
  (bind _returnvalue_2 (Transformation|GetWorldLocation _camerasnapbot))
  (bind _clientsidepawnref (Variables|/Game/Secpholand/Blueprints/ControllersYModes/baseClasses/ClientSide_Controller.ClientSide_Controller_C|GetClientSidePawnRef _playercontroller_3))
  (bind _clientsidepawnref_2 (Variables|/Game/Secpholand/Blueprints/ControllersYModes/baseClasses/ClientSide_Controller.ClientSide_Controller_C|GetClientSidePawnRef _playercontroller_2))
  (bind _clientsidepawnref_3 (Variables|/Game/Secpholand/Blueprints/ControllersYModes/baseClasses/ClientSide_Controller.ClientSide_Controller_C|GetClientSidePawnRef _playercontroller_5))
  (bind _camera (Variables|/Game/Secpholand/Blueprints/ControllersYModes/baseClasses/ClientSide_Pawn.ClientSide_Pawn_C|GetCamera _clientsidepawnref))
  (bind _returnvalue_3 (Transformation|GetWorldLocation _camera))
  (bind _returnvalue_4 (Math|Vector|Distance(Vector) _returnvalue_3 _returnvalue_2))
  (bind _returnvalue_5 (/ _returnvalue_4 1.5e+03))
  (bind _returnvalue_6 (Math|Float|Clamp(Float) _returnvalue_5))
  (Utilities|FlowControl|DoOnce false
    (:Completed
      (Variables|Default|Setactive false)
      (Variables|Default|SetairVol (Math|Float|Lerp 0.2 0.7 _returnvalue_6))
      (Components|Timeline|SetPlayRate (Variables|Default|GetCameraTimeline) (Math|Float|Lerp 1.0 0.7 _returnvalue_6))
      (Audio|PlaySound2D "/Game/Secpholand/audio/transition.transition" 1.0 1.0 0.0 0 0)
      (Default|SetControllsConstraints _playercontroller_4 true false false false)
      (Default|StopOutliningActor _playercontroller_4 self)
      (CallFunction|ResetClick)
      (Variables|Default|SetCameraSnap (Transformation|GetWorldTransform (Variables|Default|GetCameraSnapTOP)))
      (CallFunction|Abrir/cerrarPuertas)
      (CallFunction|CameraTraveling true)
      (Utilities|FlowControl|Delay 1.0)
      (Transformation|DetachFromComponent (Variables|/Game/Secpholand/Blueprints/ControllersYModes/baseClasses/ClientSide_Pawn.ClientSide_Pawn_C|GetCamera (Variables|/Game/Secpholand/Blueprints/ControllersYModes/baseClasses/ClientSide_Controller.ClientSide_Controller_C|GetClientSidePawnRef (Variables|Default|GetPlayerController))) "KeepWorld" "KeepWorld" "KeepWorld" false)
      (Default|ChangeSpeed:Server _playercontroller 2.5e+02)
      (Default|MovetoLocation _playercontroller (Transformation|GetWorldLocation (Variables|Default|GetElevatorInsideTOP)))
      (Utilities|FlowControl|Delay 2.5)
      (Default|HideNamePlate (Variables|Default|GetCharacter) true)
      (CameraFades|StartCameraFade :self (Variables|/Script/Engine.PlayerController|GetPlayerCameraManager (Variables|Default|GetPlayerController)) :ToAlpha 1.0 :Duration 0.6 :bHoldWhenFinished true)
      (Utilities|FlowControl|Delay 0.6)
      (Default|TeleportPlayer:Client (Variables|Default|GetPlayerController) _returnvalue)
      (Transformation|SetActorLocation (Variables|/Game/Secpholand/Blueprints/ControllersYModes/baseClasses/ClientSide_Controller.ClientSide_Controller_C|GetClientSidePawnRef (Variables|Default|GetPlayerController)) _returnvalue false false)
      (Transformation|SetWorldRotation (Variables|/Game/Secpholand/Blueprints/ControllersYModes/baseClasses/ClientSide_Pawn.ClientSide_Pawn_C|GetSpringArm _clientsidepawnref_2) "40.000000,90.000000, 0" false false)
      (Default|ZoomEvent _clientsidepawnref_2 (Variables|/Game/Secpholand/Blueprints/ControllersYModes/baseClasses/ClientSide_Controller.ClientSide_Controller_C|Getzoom (Variables|Default|GetPlayerController)))
      (Transformation|SetWorldTransform (Variables|/Game/Secpholand/Blueprints/ControllersYModes/baseClasses/ClientSide_Pawn.ClientSide_Pawn_C|GetCamera _clientsidepawnref_2) (Transformation|GetWorldTransform (Variables|Default|GetCameraSnapBOT)) false false)
      (Utilities|FlowControl|Delay 1.0)
      (CameraFades|StartCameraFade :self (Variables|/Script/Engine.PlayerController|GetPlayerCameraManager (Variables|Default|GetPlayerController)) :FromAlpha 1.0 :Duration 0.6 :bHoldWhenFinished true)
      (Utilities|FlowControl|Delay 0.6)
      (CallFunction|Abrir/cerrarPuertas)
      (Collision|SetCollisionEnabled (Variables|Default|GetColliderWalls) "NoCollision")
      (Utilities|FlowControl|Delay 1.0)
      (Default|MovetoLocation (Variables|Default|GetPlayerController) (Transformation|GetWorldLocation (Variables|Default|GetGotoBot)))
      (Variables|Default|SetCameraSnap (Transformation|GetWorldTransform (Variables|Default|GetCameraSnapBOT)))
      (Utilities|FlowControl|Delay 2.0)
      (Transformation|AttachComponentToComponent (Variables|/Game/Secpholand/Blueprints/ControllersYModes/baseClasses/ClientSide_Pawn.ClientSide_Pawn_C|GetCamera _clientsidepawnref_3) (Variables|/Game/Secpholand/Blueprints/ControllersYModes/baseClasses/ClientSide_Pawn.ClientSide_Pawn_C|GetSpringArm _clientsidepawnref_3) "None" "KeepWorld" "KeepWorld" "KeepWorld" true)
      (CallFunction|CameraTraveling false)
      (Utilities|FlowControl|Delay 1.0)
      (for _array_element (Variables|Default|GetmeshesToActivate)
        (Collision|SetActorEnableCollision _array_element false)
        (Collision|SetCollisionEnabled (Variables|/Script/Engine.StaticMeshActor|GetStaticMeshComponent _array_element) "NoCollision"))
      (Default|SetControllsConstraints (Variables|Default|GetPlayerController) true true true true)
      (Variables|Default|SetonTop false)
      (Collision|SetCollisionEnabled (Variables|Default|GetColliderStructure) "QueryOnly")
      (Variables|Default|SethoverTitle "Cafetería")
      (Variables|Default|SetHoverNormalHint "Haz click para subir...")
      (Default|CangeSpeed:Client (Variables|Default|GetPlayerController) 9.5e+02)
      (Default|HideNamePlate (Variables|Default|GetCharacter) false))))

(event EventBeginPlay
  (for _array_element (Variables|Default|GetmeshesToActivate)
    (Collision|SetActorEnableCollision _array_element false)
    (Collision|SetCollisionEnabled (Variables|/Script/Engine.StaticMeshActor|GetStaticMeshComponent _array_element) "NoCollision")
    (Collision|SetCollisionEnabled (Variables|Default|GetColliderWalls) "NoCollision")))

(event EventClick
  (params (controller :type Client%20Side%20Controller%20Object%20Reference))
  (bind _gotobot (Variables|Default|GetGotoBot))
  (bind _gotobot_2 (Variables|Default|GetGotoBot))
  (bind _returnvalue (Transformation|GetWorldLocation _gotobot))
  (bind _returnvalue_2 (Transformation|GetWorldLocation _gotobot_2))
  (if (Variables|Default|GetonTop)
    (bind _output_get (Variables|Default|SetPlayerController controller))
    (|CallParentFunction _output_get)
    (CallFunction|GotoTOPEvent)
    (else
      (bind _output_get_2 (Variables|Default|SetPlayerController controller))
      (|CallParentFunction _output_get_2)
      (if (Utilities|Array|Get(acopy) (.TutorialsDoneFlags (Utilities|Struct|BreakUserInfo_Private (Variables|/Game/Secpholand/Blueprints/ControllersYModes/baseClasses/ClientSide_Controller.ClientSide_Controller_C|GetuserInfo_Private controller))) 7)
        _
        (else
          (bind _returnvalue_3 (UserInterface|CreateWidget "/Game/Secpholand/UI/Widgets/Tutoriales/PrimeraVezEdificios/PrimeraVezEdificio.PrimeraVezEdificio_C" 0 "NewEnumerator7" self))
          (UserInterface|Viewport|AddtoViewport _returnvalue_3 0)))
      (if (Variables|Default|GetAllowedToUse)
        (if (Variables|/Game/Secpholand/Blueprints/ControllersYModes/baseClasses/ClientSide_Pawn.ClientSide_Pawn_C|Getb_VistaPajaro (Variables|/Game/Secpholand/Blueprints/ControllersYModes/baseClasses/ClientSide_Controller.ClientSide_Controller_C|GetClientSidePawnRef (Variables|Default|GetPlayerController)))
          (Transformation|SetWorldRotation (Variables|/Game/Secpholand/Blueprints/ControllersYModes/baseClasses/ClientSide_Pawn.ClientSide_Pawn_C|GetSpringArm (Variables|/Game/Secpholand/Blueprints/ControllersYModes/baseClasses/ClientSide_Controller.ClientSide_Controller_C|GetClientSidePawnRef (Variables|Default|GetPlayerController))) (Math|Rotator|MakeRotator 0.0 (.pitch (Transformation|GetWorldRotation (Variables|/Game/Secpholand/Blueprints/ControllersYModes/baseClasses/ClientSide_Pawn.ClientSide_Pawn_C|GetSpringArm (Variables|/Game/Secpholand/Blueprints/ControllersYModes/baseClasses/ClientSide_Controller.ClientSide_Controller_C|GetClientSidePawnRef (Variables|Default|GetPlayerController))))) (.yaw (Math|Rotator|FindLookatRotation (Transformation|GetActorLocation (Variables|/Game/Secpholand/Blueprints/ControllersYModes/baseClasses/ClientSide_Controller.ClientSide_Controller_C|GetClientSidePawnRef (Variables|Default|GetPlayerController))) _returnvalue))) false false)
          (bind _foundwidgets (Widget|GetAllWidgetsOfClass "/Game/Secpholand/UI/Widgets/HUDYChat/Minimapa/BotonVistaPajaro.BotonVistaPajaro_C" true))
          (Default|ClicarVistaCalle (Utilities|Array|Get(acopy) _foundwidgets))
          (Utilities|FlowControl|Delay (* (Math|Float|Clamp(Float) (- 1.0 (/ (Math|Vector|Distance(Vector) _returnvalue (Transformation|GetActorLocation (Variables|/Game/Secpholand/Blueprints/ControllersYModes/baseClasses/ClientSide_Controller.ClientSide_Controller_C|GetClientSidePawnRef (Variables|Default|GetPlayerController)))) (* (Class|MovementComponent|GetMaxSpeed (Variables|/Script/Engine.Character|GetCharacterMovement (Variables|/Game/Secpholand/Blueprints/ControllersYModes/baseClasses/ClientSide_Controller.ClientSide_Controller_C|GetServerSideCharacterRef (Variables|Default|GetPlayerController)))) 2.5)))) 2.5)))
        (if (<= (Math|Vector|Distance(Vector) (Transformation|GetActorLocation (Variables|/Game/Secpholand/Blueprints/ControllersYModes/baseClasses/ClientSide_Controller.ClientSide_Controller_C|GetClientSidePawnRef (Variables|Default|GetPlayerController))) (Transformation|GetWorldLocation (Variables|Default|GetGotoBot))) 2e+02)
          (CallFunction|BotElevatorEvent (Variables|/Game/Secpholand/Blueprints/ControllersYModes/baseClasses/ClientSide_Controller.ClientSide_Controller_C|GetServerSideCharacterRef (Variables|Default|GetPlayerController)))
          (else
            (Variables|Default|Setactive true)))
        (Default|SpawnDecalatLocation (Variables|Default|GetPlayerController) _returnvalue_2)
        (Default|MovetoLocation (Variables|Default|GetPlayerController) _returnvalue_2)))))

(event EventResetClick
  (bind _playercontroller (Variables|Default|GetPlayerController))
  (bind _elevatorinsidebot (Variables|Default|GetElevatorInsideBOT))
  (bind _camerasnapbot (Variables|Default|GetCameraSnapBOT))
  (bind _playercontroller_2 (Variables|Default|GetPlayerController))
  (bind _playercontroller_3 (Variables|Default|GetPlayerController))
  (bind _playercontroller_4 (Variables|Default|GetPlayerController))
  (bind _playercontroller_5 (Variables|Default|GetPlayerController))
  (bind _returnvalue (Transformation|GetWorldLocation _elevatorinsidebot))
  (bind _returnvalue_2 (Transformation|GetWorldLocation _camerasnapbot))
  (bind _clientsidepawnref (Variables|/Game/Secpholand/Blueprints/ControllersYModes/baseClasses/ClientSide_Controller.ClientSide_Controller_C|GetClientSidePawnRef _playercontroller_3))
  (bind _clientsidepawnref_2 (Variables|/Game/Secpholand/Blueprints/ControllersYModes/baseClasses/ClientSide_Controller.ClientSide_Controller_C|GetClientSidePawnRef _playercontroller_2))
  (bind _clientsidepawnref_3 (Variables|/Game/Secpholand/Blueprints/ControllersYModes/baseClasses/ClientSide_Controller.ClientSide_Controller_C|GetClientSidePawnRef _playercontroller_5))
  (bind _camera (Variables|/Game/Secpholand/Blueprints/ControllersYModes/baseClasses/ClientSide_Pawn.ClientSide_Pawn_C|GetCamera _clientsidepawnref))
  (bind _returnvalue_3 (Transformation|GetWorldLocation _camera))
  (bind _returnvalue_4 (Math|Vector|Distance(Vector) _returnvalue_3 _returnvalue_2))
  (bind _returnvalue_5 (/ _returnvalue_4 1.5e+03))
  (bind _returnvalue_6 (Math|Float|Clamp(Float) _returnvalue_5))
  (|CallParentFunction)
  (Variables|Default|Setactive false)
  (Utilities|FlowControl|DoOnce false) ; enters at Reset
)

(fn ConstructionScript
  (|CallParentFunction))