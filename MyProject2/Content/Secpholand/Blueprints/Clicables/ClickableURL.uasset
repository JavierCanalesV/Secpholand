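; ClickableURL is a clickable world actor that opens a web link when clicked.
; Its construction script applies the configurable Mesh to the StaticMesh component, so each instance can look different.
; The Click event passes the Url variable to LaunchURL, while the default BeginPlay, overlap and Tick events remain disabled.
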(event EventBeginPlay
  (|CallParentFunction) ; This node is disabled and will not be called.\nDrag off pins to build functionality.
)

(event Collision|EventActorBeginOverlap
  (params (OtherActor :type Actor%20Object%20Reference))
  (|CallParentFunction OtherActor) ; This node is disabled and will not be called.\nDrag off pins to build functionality.
)

(event EventTick
  (params (DeltaSeconds :type Float%20%28single-precision%29))
  (|CallParentFunction DeltaSeconds) ; This node is disabled and will not be called.\nDrag off pins to build functionality.
)

(event EventClick
  (params (controller :type Client%20Side%20Controller%20Object%20Reference))
  (Utilities|Platform|LaunchURL (Variables|Default|Geturl)))

(fn ConstructionScript
  (|CallParentFunction)
  (Components|StaticMesh|SetStaticMesh (Variables|Default|GetStaticMesh) (Variables|Default|GetMesh)))