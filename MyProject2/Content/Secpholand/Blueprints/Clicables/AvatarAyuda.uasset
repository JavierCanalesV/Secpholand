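; AvatarAyuda is a clickable help avatar that shows a name widget and, when clicked, a help speech bubble.
; BeginPlay writes Username into the NombreyEmpresa widget, then creates a BocadilloDeAyuda from TextosDeAyuda for WidgetAyuda, which updateTexts can also rebuild.
; Click calls the parent and ResetClick, disables actor collision, reveals the bubble and hides the name widget, with no path here to revert this.
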(event Custom|updateTexts
  (bind _returnvalue (UserInterface|CreateWidget "/Game/Secpholand/UI/Widgets/Tutoriales/BocadilloDeAyuda.BocadilloDeAyuda_C"))
  (Default|SetTexts _returnvalue (Variables|Default|GetTextosDeAyuda))
  (UserInterface|SetWidget (Variables|Default|GetwidgetAyuda) _returnvalue))

(event EventStopHover
  (|CallParentFunction))

(event EventClick
  (params (controller :type Client%20Side%20Controller%20Object%20Reference))
  (|CallParentFunction controller)
  (CallFunction|ResetClick)
  (Collision|SetActorEnableCollision false)
  (Development|SetHiddeninGame (Variables|Default|GetwidgetAyuda) false false)
  (Development|SetHiddeninGame (Variables|Default|GetNombreyEmpresa) true false))

(event EventHover
  (|CallParentFunction))

(event EventBeginPlay
  (bind _asnombre_player (Utilities|Casting|CastToNombrePlayer (UserInterface|GetUserWidgetObject (Variables|Default|GetNombreyEmpresa))))
  (Rendering|Components|TextRender|SetText (Variables|/Game/Secpholand/UI/Widgets/NombrePlayer.NombrePlayer_C|GetNombre _asnombre_player) (Utilities|Text|ToText(String) (Utilities|String|ToString(Name) (Variables|Default|GetUsername))))
  (bind _returnvalue (UserInterface|CreateWidget "/Game/Secpholand/UI/Widgets/Tutoriales/BocadilloDeAyuda.BocadilloDeAyuda_C"))
  (Default|SetTexts _returnvalue (Variables|Default|GetTextosDeAyuda))
  (UserInterface|SetWidget (Variables|Default|GetwidgetAyuda) _returnvalue))

(fn ConstructionScript
  (|CallParentFunction))