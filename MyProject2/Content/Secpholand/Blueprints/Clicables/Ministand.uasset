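; Ministand is an actor in the Clicables folder that builds a small stand from two Banner child actors.
; Its construction script resets both banner meshes to unit scale, giving the first the SM_Stand mesh and zeroing the second's relative rotation.
; The mesh swap for the second banner is disconnected, and the event graph holds no active logic.
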(event EventBeginPlay)

(fn ConstructionScript
  (bind _asbanner (Utilities|Casting|CastToBanner (Variables|/Script/Engine.ChildActorComponent|GetChildActor (Variables|Default|GetChildActor1))))
  (Transformation|SetRelativeScale3D (Variables|/Game/Secpholand/Blueprints/clasesBase/ClickableActor.ClickableActor_C|GetStaticMesh _asbanner) "1.000000,1.000000,1.000000")
  (Components|StaticMesh|SetStaticMesh (Variables|/Game/Secpholand/Blueprints/clasesBase/ClickableActor.ClickableActor_C|GetStaticMesh _asbanner) "/Game/Secpholand/Assets/meshes/Props_Actividades/SM_Stand.SM_Stand")
  (bind _asbanner_2 (Utilities|Casting|CastToBanner (Variables|/Script/Engine.ChildActorComponent|GetChildActor (Variables|Default|GetChildActor))))
  (Transformation|SetRelativeScale3D (Variables|/Game/Secpholand/Blueprints/clasesBase/ClickableActor.ClickableActor_C|GetStaticMesh _asbanner_2) "1.000000,1.000000,1.000000")
  (Transformation|SetRelativeRotation (Variables|/Game/Secpholand/Blueprints/clasesBase/ClickableActor.ClickableActor_C|GetStaticMesh _asbanner_2) "0, 0, 0" false false))