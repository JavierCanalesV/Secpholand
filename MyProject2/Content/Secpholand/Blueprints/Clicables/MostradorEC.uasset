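; Clickable company stand counter that lets players view the company profile or leave a personal card.
; Clicking opens a screen-clamped dropdown widget and disables the counter's collision.
; GotoEventmopstrador walks the player to GotoBox unless already overlapping; Arrived then resets the click and opens either FichaEmpresa, requesting company data through the controller, or DejarTargetaPersonal.
; The construction script picks the desk mesh from the stand index.
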(event Custom|GotoEventmopstrador
  (params (Verperfil :type Boolean))
  (bind _gotobox (Variables|Default|GetGotoBox))
  (bind _returnvalue (Transformation|GetWorldLocation _gotobox))
  (Variables|Default|SetVerPerfil Verperfil)
  (Variables|Default|Setactive true)
  (bind _asclient_side_controller (Utilities|Casting|CastToClientSide_Controller (Game|GetPlayerController 0)))
  (|CallParentFunction _asclient_side_controller)
  (if (Collision|IsOverlappingActor (Variables|Default|GetGotoBox) (Variables|/Game/Secpholand/Blueprints/ControllersYModes/baseClasses/ClientSide_Controller.ClientSide_Controller_C|GetClientSidePawnRef _asclient_side_controller) :!class /Script/Engine.PrimitiveComponent)
    (CallFunction|Arrived)
    (else
      (bind _asclient_side_controller_2 (Utilities|Casting|CastToClientSide_Controller (Game|GetPlayerController 0)))
      (Default|SpawnDecalatLocation _asclient_side_controller_2 _returnvalue)
      (Default|MovetoLocation _asclient_side_controller_2 _returnvalue))))

(event EventClick
  (params (controller :type Client%20Side%20Controller%20Object%20Reference))
  (Collision|SetActorEnableCollision false)
  (bind _returnvalue (UserInterface|CreateWidget "/Game/Secpholand/UI/Widgets/EC/DesplegableMostradorStand.DesplegableMostradorStand_C" 0 self (Utilities|String|StringToName (.NombreEmpresa (Utilities|Struct|BreakUserInfo_Public (Variables|/Game/Secpholand/Blueprints/ControllersYModes/baseClasses/ServerSide_Character.ServerSide_Character_C|GetUserInfo (Variables|/Game/Secpholand/Blueprints/ControllersYModes/baseClasses/ClientSide_Controller.ClientSide_Controller_C|GetServerSideCharacterRef (.AsClient%20Side%20Controller (Utilities|Casting|CastToClientSide_Controller controller)))))))))
  (bind (_x _y _hswaped _vswapped) (CallFunction|ClampWidgedPostoScreen 341.0 138.0))
  (Class|UserWidget|SetPositioninViewport _returnvalue (Math|Vector2D|MakeVector2D _x _y) false)
  (Class|Widget|SetRenderTransformPivot _returnvalue (Math|Vector2D|MakeVector2D (select _hswaped 1.0 0.0) (select _vswapped 1.0 0.0)))
  (UserInterface|Viewport|AddtoViewport _returnvalue 0))

(event EventArrived
  (bind _empresa (Variables|Default|Getempresa))
  (CallFunction|ResetClick)
  (if (Variables|Default|GetVerPerfil)
    (bind _returnvalue (UserInterface|CreateWidget "/Game/Secpholand/UI/Widgets/Perfiles/FichaEmpresa.FichaEmpresa_C" 0 (Utilities|String|ToString(Name) _empresa)))
    (UserInterface|Viewport|AddtoViewport _returnvalue 0)
    (bind _asclient_side_controller (Utilities|Casting|CastToClientSide_Controller (Game|GetPlayerController 0)))
    (Default|Client:RetrieveEmpresa _asclient_side_controller _empresa)
    (else
      (bind _returnvalue_2 (UserInterface|CreateWidget "/Game/Secpholand/UI/Widgets/EC/DejarTargetaPersonal.DejarTargetaPersonal_C" 0 _empresa self))
      (UserInterface|Viewport|AddtoViewport _returnvalue_2 0))))

(event EventResetClick
  (|CallParentFunction)
  (Collision|SetActorEnableCollision true)
  (bind _foundwidgets (Widget|GetAllWidgetsOfClass "/Game/Secpholand/UI/Widgets/EC/DesplegableMostradorStand.DesplegableMostradorStand_C" true))
  (if (> (Utilities|Array|Length _foundwidgets) 0)
    (Widget|RemovefromParent (Utilities|Array|Get(acopy) _foundwidgets))))

(fn ConstructionScript
  (|CallParentFunction)
  (Components|StaticMesh|SetStaticMesh (Variables|Default|GetStaticMesh) (Utilities|Select :Index (Variables|Default|GetindiceStand) :Option%200 "/Game/Secpholand/Assets/meshes/Event_Fair/Props/SM_Desktop_A.SM_Desktop_A" :Option%201 "/Game/Secpholand/Assets/meshes/Event_Fair/Props/SM_Desktop_B.SM_Desktop_B" :Option%202 0 :Option%203 0 :Option%204 0)))