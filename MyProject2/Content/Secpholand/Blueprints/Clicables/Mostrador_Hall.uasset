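; Clickable hall counter (Mostrador_Hall) that opens the Proyectos (projects) widget when clicked.
; Shortly after BeginPlay it calls RetrieveProjectsXenterpriseListServer on the MeetingCenterGameState to request the list of projects by enterprise.
; On click it runs the parent logic, adds the RefWB widget to the viewport, then fills it from ListProyectos after a short retriggerable delay.
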(event EventClick
  (params (controller :type Client%20Side%20Controller%20Object%20Reference))
  (bind _ref_wb (Variables|Default|GetRef_WB))
  (bind _asproyectos (Utilities|Casting|CastToProyectos _ref_wb))
  (|CallParentFunction controller)
  (UserInterface|Viewport|AddtoViewport _asproyectos 0)
  (Utilities|FlowControl|RetriggerableDelay 0.3)
  (Default|FillPlayers _asproyectos (Variables|Default|GetList%20Proyectos)))

(event Collision|EventActorBeginOverlap
  (params (OtherActor :type Actor%20Object%20Reference)))

(event EventTick
  (params (DeltaSeconds :type Float%20%28single-precision%29)))

(event EventBeginPlay
  (|CallParentFunction)
  (Utilities|FlowControl|Delay 1.0)
  (Default|RetrieveProjectsXenterpriseList:Server (.AsMeeting%20Center%20Game%20State (Utilities|Casting|CastToMeetingCenterGameState (Game|GetGameState)))))

(fn ConstructionScript
  (|CallParentFunction))