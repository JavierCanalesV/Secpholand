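; Clickable podcast zone Blueprint that fills a podcast container widget with titles and URLs when clicked.
; Click runs the parent's click logic, then casts RefWB to ContenedorDePodCast only on the branch where RefWB is invalid.
; The Rewritedates event passes Titulos and Urls to FillPods if the stored RefWBPods reference is valid.
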(event Custom|Rewrite%20dates
  (params (Titulos :type Array%20of%20Names) (Urls :type Array%20of%20Strings))
  (bind _ref_wb_pods (Variables|Default|GetRef_WB_Pods))
  (Utilities|IsValid _ref_wb_pods
    (:Is%20Valid
      (Default|FillPods _ref_wb_pods Titulos Urls))))

(event Collision|EventActorBeginOverlap
  (params (OtherActor :type Actor%20Object%20Reference)))

(event EventTick
  (params (DeltaSeconds :type Float%20%28single-precision%29)))

(event EventClick
  (params (controller :type Client%20Side%20Controller%20Object%20Reference))
  (bind _ref_wb (Variables|Default|GetRef_WB))
  (|CallParentFunction controller)
  (Utilities|IsValid _ref_wb
    (:Is%20Valid
      _)
    (:Is%20Not%20Valid
      (Variables|Default|SetRef_WB_Pods (.AsContenedor%20De%20Pod%20Cast (Utilities|Casting|CastToContenedorDePodCast _ref_wb)))))
  (CallFunction|RewriteDates (Variables|Default|GetTitulos) (Variables|Default|GetUrls)))

(event EventBeginPlay
  (|CallParentFunction))

(fn ConstructionScript
  (|CallParentFunction))