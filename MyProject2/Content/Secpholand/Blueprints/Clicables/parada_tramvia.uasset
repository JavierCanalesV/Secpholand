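; Clickable tram stop that lets the player ride a tram to another level.
; Clicking walks the controller to the stop and updates the hover widget; the local player's overlap then locks input and plays the tram's arrival timeline.
; When it finishes, remote clients get the MenuTramvia menu.
; Go hides the character, animates the tram away, fades the camera and opens the level passed in.
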(event OnComponentBeginOverlap(Box)
  (params (OverlappedComponent :type Primitive%20Component%20Object%20Reference) (OtherActor :type Actor%20Object%20Reference) (OtherComp :type Primitive%20Component%20Object%20Reference) (OtherBodyIndex :type Integer) (bFromSweep :type Boolean) (SweepResult :type Hit%20Result%20Structure%20%28by%20ref%29))
  (bind _tramvia (Variables|Default|Gettramvia))
  (bind _relativelocation (Variables|/Script/Engine.SceneComponent|GetRelativeLocation _tramvia))
  (if (Variables|Default|Getactive)
    (bind _asserver_side_character (Utilities|Casting|CastToServerSide_Character OtherActor))
    (Variables|Default|Setchar _asserver_side_character)
    (bind _asclient_side_controller (Utilities|Casting|CastToClientSide_Controller (Game|GetPlayerController 0)))
    (if (== OtherActor (Variables|/Game/Secpholand/Blueprints/ControllersYModes/ClientSide_Controller.ClientSide_Controller_C|GetServerSideCharacterRef _asclient_side_controller))
      (Variables|/Game/Secpholand/Blueprints/ControllersYModes/ClientSide_Controller.ClientSide_Controller_C|SetcanMove? _asclient_side_controller false)
      (Variables|/Game/Secpholand/Blueprints/ControllersYModes/ClientSide_Controller.ClientSide_Controller_C|SetcanRotate? _asclient_side_controller false)
      (Variables|/Game/Secpholand/Blueprints/ControllersYModes/ClientSide_Controller.ClientSide_Controller_C|SetcanClick? _asclient_side_controller false)
      (CallFunction|StopHover)
      (Development|SetHiddeninGame (Variables|Default|Gettramvia) false false)
      (Default|StopOutliningActor _asclient_side_controller self)
      (bind _newtrack_1 (Timeline|coming Play)
        (:Update
          (Transformation|SetRelativeLocation _tramvia (Math|Vector|MakeVector (.x _relativelocation) _newtrack_1 (.z _relativelocation)) false false))
        (:Finished
          (Networking|SwitchHasAuthority
            (:Remote
              (bind _returnvalue (UserInterface|CreateWidget "/Game/Secpholand/UI/Widgets/MenuTramvia.MenuTramvia_C" _asclient_side_controller self))
              (UserInterface|Viewport|AddtoViewport _returnvalue 0))))))))

(event Custom|Go
  (params (NewParam :type Name))
  (bind _tramvia (Variables|Default|Gettramvia))
  (bind _relativelocation (Variables|/Script/Engine.SceneComponent|GetRelativeLocation _tramvia))
  (Rendering|SetActorHiddenInGame (Variables|Default|Getchar) true)
  (Viewport|RemoveAllWidgets)
  (bind _newtrack_1 (Timeline|Timeline_0 Play)
    (:Update
      (Transformation|SetRelativeLocation _tramvia (Math|Vector|MakeVector (.x _relativelocation) _newtrack_1 (.z _relativelocation)) false false)
      (if (> _newtrack_1 6e+03)
        (Utilities|FlowControl|DoOnce false
          (:Completed
            (CameraFades|StartCameraFade :self (Variables|/Script/Engine.PlayerController|GetPlayerCameraManager (Variables|/Game/Secpholand/Blueprints/ControllersYModes/ServerSide_Character.ServerSide_Character_C|GetclientSideControllerRef (Variables|Default|Getchar))) :ToAlpha 1.0 :Duration 0.6 :bHoldWhenFinished true)
            (Utilities|FlowControl|Delay 0.6)
            (Game|OpenLevel(byName) NewParam)))))))

(event EventBeginPlay
  (|CallParentFunction))

(event Collision|EventActorBeginOverlap
  (params (OtherActor :type Actor%20Object%20Reference))
  (|CallParentFunction OtherActor) ; This node is disabled and will not be called.\nDrag off pins to build functionality.
)

(event EventTick
  (params (DeltaSeconds :type Float%20%28single-precision%29))
  (|CallParentFunction DeltaSeconds) ; This node is disabled and will not be called.\nDrag off pins to build functionality.
)

(event EventClick
  (params (hit :type Hit%20Result%20Structure) (controller :type Client%20Side%20Controller%20Object%20Reference))
  (Variables|Default|SetActive true)
  (Default|MovetoLocation controller (Transformation|GetWorldLocation (Variables|Default|GetgotoLocation)))
  (bind _asestacion_tramvia (Utilities|Casting|CastToEstacionTramvia (Variables|Default|GethoverUserWidget)))
  (Rendering|Components|TextRender|SetText (Variables|/Game/Secpholand/UI/Widgets/HoverWidgets/EstacionTramvia.EstacionTramvia_C|GetTextBlock _asestacion_tramvia) "Yendo")
  (Widget|SetRenderOpacity (Variables|/Game/Secpholand/UI/Widgets/HoverWidgets/EstacionTramvia.EstacionTramvia_C|GetCircularThrobber_249 _asestacion_tramvia) 1.0))

(fn ConstructionScript
  (|CallParentFunction))