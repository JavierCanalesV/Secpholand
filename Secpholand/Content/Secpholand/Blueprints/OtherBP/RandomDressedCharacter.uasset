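; Decorative character that dresses itself as a random avatar at BeginPlay and idles, sitting or standing, with actor collision disabled.
; It randomizes gender, hair, skin, beard, glasses and outfit into UserInfo, picking clothing colors from gender-specific material sets, then calls DressLocaly.
; It destroys the inherited nameplate and VOIP audio, then loops a slowed idle from a random start position to desynchronize copies.
; Spawned instances also zero the mesh's relative location.
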(event EventBeginPlay
  (bind _returnvalue (Math|Random|RandomInteger 6))
  (bind _mesh (Variables|Character|GetMesh))
  (bind _materiales (Variables|Default|GetMateriales))
  (bind (_0 _1 _2 _3 _4 _5 _6 _7 _8 _9 _10 _11 _12 _13 _14 _15 _16 _17 _18 _19) (Utilities|Struct|BreakCodigodeColorPorVestimenta _materiales))
  (bind _returnvalue_2 (Math|Conversions|ToByte(Integer) _returnvalue))
  (bind _returnvalue_3 (Utilities|Select :Index _returnvalue_2 :Option%200 _0 :Option%201 _1 :Option%202 _2 :Option%203 _3 :Option%204 _4 :Option%205 _5))
  (bind _returnvalue_4 (Utilities|Select :Index _returnvalue_2 :Option%200 _6 :Option%201 _7 :Option%202 _8 :Option%203 _9 :Option%204 _10 :Option%205 _11 :Option%206 _12 :Option%207 _13 :Option%208 _14 :Option%209 _15 :Option%2010 _16 :Option%2011 _17 :Option%2012 _18 :Option%2013 _19))
  (|CallParentFunction)
  (bind _output_get (Variables|Default|Setmale (Math|Random|RandomBool)))
  (Utilities|Struct|SetmembersinUserInfo_Public (Variables|Default|GetUserInfo) (Utilities|Struct|MakeAvatar _output_get (Math|Conversions|ToByte(Integer) (+ (Math|Random|RandomInteger 6) 1)) (Math|Conversions|ToByte(Integer) (Math|Random|RandomInteger 8)) (Math|Conversions|ToByte(Integer) (Math|Random|RandomInteger 3)) (Math|Conversions|ToByte(Integer) (Math|Random|RandomInteger 9)) (Math|Conversions|ToByte(Integer) (Math|Random|RandomInteger 6)) 0 0 _returnvalue_2 (select (Variables|Default|Getmale) (Utilities|Array|Get(acopy) _returnvalue_3) (Utilities|Array|Get(acopy) _returnvalue_4)) (select (Variables|Default|Getmale) (Utilities|Array|Get(acopy) _returnvalue_3 1) (Utilities|Array|Get(acopy) _returnvalue_4 1)) (select (Variables|Default|Getmale) (Utilities|Array|Get(acopy) _returnvalue_3 2) (Utilities|Array|Get(acopy) _returnvalue_4 2)) (select (Variables|Default|Getmale) (Utilities|Array|Get(acopy) _returnvalue_3 3) (Utilities|Array|Get(acopy) _returnvalue_4 3))))
  (CallFunction|DressLocaly)
  (Components|DestroyComponent (Variables|Default|GetnamePlate))
  (Components|Animation|PlayAnimation _mesh (select (Variables|Default|GetSit) "/Game/Secpholand/Assets/meshes/01Characters/04Animations/Sitting_Idle01.Sitting_Idle01" "/Game/Secpholand/Assets/meshes/01Characters/04Animations/Idle02.Idle02") true)
  (Components|Animation|SetPosition _mesh (Math|Random|RandomFloatinRange 0.0 3.0) true)
  (Components|Timeline|SetPlayRate _mesh 0.8)
  (if (Variables|Default|Getspawned)
    (Transformation|SetRelativeLocation (Variables|Character|GetMesh) "0, 0, 0" false false)))

(fn ConstructionScript
  (|CallParentFunction)
  (Collision|SetActorEnableCollision false))