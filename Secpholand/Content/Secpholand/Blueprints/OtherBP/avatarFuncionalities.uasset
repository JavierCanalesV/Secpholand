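; Avatar helper that dresses a customizable character from an AvatarInfo record and supplies accessory placement rules.
; DressAvatar picks male or female body, hair, glasses and accessory meshes from Meshes arrays, resets the beard for females, and tints skin, clothes and hair through dynamic material instances.
; Other functions map accessory indices to sockets, offset the beret (Boina) by hair mesh, and return an accessory's whole group for removal.
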(fn DressAvatar
  (params (AvatarInfo :type Avatar%20Structure) (BodyMesh :type Skinned%20Mesh%20Component%20Object%20Reference) (Gafas :type Static%20Mesh%20Component%20Object%20Reference) (Barba :type Static%20Mesh%20Component%20Object%20Reference) (Pelo :type Static%20Mesh%20Component%20Object%20Reference) (Complemento :type Static%20Mesh%20Component%20Object%20Reference) (Complemento2 :type Static%20Mesh%20Component%20Object%20Reference))
  (bind (_male_ _hairtype _haircolor _skincolor _beardtype _glasses _complemento _complemento2 _vestimenta _colorropa1 _colorropa2 _colorropa3 _colorropa4) (Utilities|Struct|BreakAvatar AvatarInfo))
  (bind _meshes (LocalVariables|Getmeshes))
  (bind (_peinado_f _peinado_m _barba _gafasm _gafasf _skeletal_m _skeletal_f _complement_f _complement_m _skincolors _haircolors _clothcolors) (Utilities|Struct|BreakAvatarCustomization _meshes))
  (bind _returnvalue (Math|Conversions|ToInteger(Byte) _glasses))
  (bind _returnvalue_2 (Math|Conversions|ToInteger(Byte) _complemento2))
  (bind _returnvalue_3 (Math|Conversions|ToInteger(Byte) _colorropa1))
  (bind _returnvalue_4 (Math|Conversions|ToInteger(Byte) _colorropa2))
  (bind _returnvalue_5 (Math|Conversions|ToInteger(Byte) _colorropa3))
  (bind _returnvalue_6 (Math|Conversions|ToInteger(Byte) _colorropa4))
  (bind _returnvalue_7 (Math|Conversions|ToInteger(Byte) _skincolor))
  (bind _returnvalue_8 (Math|Conversions|ToInteger(Byte) _haircolor))
  (bind _output (Utilities|Array|Get(acopy) _haircolors _returnvalue_8))
  (bind _output_2 (Utilities|Array|Get(acopy) _clothcolors _returnvalue_3))
  (bind _output_3 (Utilities|Array|Get(acopy) _clothcolors _returnvalue_4))
  (bind _output_4 (Utilities|Array|Get(acopy) _clothcolors _returnvalue_5))
  (bind _output_5 (Utilities|Array|Get(acopy) _clothcolors _returnvalue_6))
  (bind _output_6 (Utilities|Array|Get(acopy) _skincolors _returnvalue_7))
  (if _male_
    (Utilities|IsValid BodyMesh
      (:Is%20Valid
        (Class|SkinnedMeshComponent|SetSkeletalMesh BodyMesh (Utilities|Array|Get(acopy) _skeletal_m (Math|Conversions|ToInteger(Byte) _vestimenta)) true)
        (bind _returnvalue_9 (Rendering|Material|CreateDynamicMaterialInstance BodyMesh 0 "/Game/Secpholand/Assets/Materials/MaterialInstances/Characters/MI_Skin.MI_Skin" "None" :!class /Script/Engine.PrimitiveComponent))
        (Rendering|Material|SetVectorParameterValue _returnvalue_9 "SkinColor" _output_6 :!class /Script/Engine.MaterialInstanceDynamic)
        (bind _returnvalue_10 (Rendering|Material|CreateDynamicMaterialInstance BodyMesh 1 "/Game/Secpholand/Assets/Materials/MaterialInstances/Characters/MI_Cloth1.MI_Cloth1" "None" :!class /Script/Engine.PrimitiveComponent))
        (Rendering|Material|SetVectorParameterValue _returnvalue_10 "Color_A" _output_2 :!class /Script/Engine.MaterialInstanceDynamic)
        (Rendering|Material|SetVectorParameterValue _returnvalue_10 "Color_B" _output_3 :!class /Script/Engine.MaterialInstanceDynamic)
        (Rendering|Material|SetVectorParameterValue _returnvalue_10 "Color_C" _output_4 :!class /Script/Engine.MaterialInstanceDynamic)
        (Rendering|Material|SetVectorParameterValue _returnvalue_10 "Color_D" _output_5 :!class /Script/Engine.MaterialInstanceDynamic))
      (:Is%20Not%20Valid
        _))
    (Utilities|IsValid Gafas
      (:Is%20Valid
        ;[1 1 1] Gafas
        (Components|StaticMesh|SetStaticMesh Gafas (Utilities|Array|Get(acopy) _gafasm _returnvalue)))
      (:Is%20Not%20Valid
        _))
    (Utilities|IsValid Pelo
      (:Is%20Valid
        ;[1 1 1] Pelo
        (Components|StaticMesh|SetStaticMesh Pelo (Utilities|Array|Get(acopy) _peinado_m (Math|Conversions|ToInteger(Byte) _hairtype)))
        (bind _returnvalue_11 (Rendering|Material|CreateDynamicMaterialInstance Pelo 0 "/Game/Secpholand/Assets/Materials/MaterialInstances/Characters/MI_Hair.MI_Hair" "None" :!class /Script/Engine.PrimitiveComponent))
        (Rendering|Material|SetVectorParameterValue _returnvalue_11 "SkinColor" _output :!class /Script/Engine.MaterialInstanceDynamic))
      (:Is%20Not%20Valid
        _))
    (Utilities|IsValid Complemento
      (:Is%20Valid
        ;[1 1 1] Complemento
        (Components|StaticMesh|SetStaticMesh Complemento (Utilities|Array|Get(acopy) _complement_m (Math|Conversions|ToInteger(Byte) _complemento))))
      (:Is%20Not%20Valid
        _))
    (Utilities|IsValid Barba
      (:Is%20Valid
        (Components|StaticMesh|SetStaticMesh Barba (Utilities|Array|Get(acopy) _barba (Math|Conversions|ToInteger(Byte) _beardtype)))
        (bind _returnvalue_12 (Rendering|Material|CreateDynamicMaterialInstance Barba 0 "/Game/Secpholand/Assets/Materials/MaterialInstances/Characters/MI_Hair.MI_Hair" "None" :!class /Script/Engine.PrimitiveComponent))
        (Rendering|Material|SetVectorParameterValue _returnvalue_12 "SkinColor" _output :!class /Script/Engine.MaterialInstanceDynamic))
      (:Is%20Not%20Valid
        _))
    (Utilities|IsValid Complemento2
      (:Is%20Valid
        ;[1 1 1] Complemento 2
        (Components|StaticMesh|SetStaticMesh Complemento2 (Utilities|Array|Get(acopy) _complement_m _returnvalue_2))))
    (else
      (Utilities|IsValid Barba
        (:Is%20Valid
          (Components|StaticMesh|SetStaticMesh Barba (Utilities|Array|Get(acopy) _barba)))
        (:Is%20Not%20Valid
          _))
      (Utilities|IsValid BodyMesh
        (:Is%20Valid
          (Class|SkinnedMeshComponent|SetSkeletalMesh BodyMesh (Utilities|Array|Get(acopy) _skeletal_f (Math|Conversions|ToInteger(Byte) _vestimenta)) true)
          (bind _returnvalue_13 (Rendering|Material|CreateDynamicMaterialInstance BodyMesh 0 "/Game/Secpholand/Assets/Materials/MaterialInstances/Characters/MI_Skin.MI_Skin" "None" :!class /Script/Engine.PrimitiveComponent))
          (Rendering|Material|SetVectorParameterValue _returnvalue_13 "SkinColor" _output_6 :!class /Script/Engine.MaterialInstanceDynamic)
          (bind _returnvalue_14 (Rendering|Material|CreateDynamicMaterialInstance BodyMesh 1 "/Game/Secpholand/Assets/Materials/MaterialInstances/Characters/MI_Cloth1.MI_Cloth1" "None" :!class /Script/Engine.PrimitiveComponent))
          (Rendering|Material|SetVectorParameterValue _returnvalue_14 "Color_A" _output_2 :!class /Script/Engine.MaterialInstanceDynamic)
          (Rendering|Material|SetVectorParameterValue _returnvalue_14 "Color_B" _output_3 :!class /Script/Engine.MaterialInstanceDynamic)
          (Rendering|Material|SetVectorParameterValue _returnvalue_14 "Color_C" _output_4 :!class /Script/Engine.MaterialInstanceDynamic)
          (Rendering|Material|SetVectorParameterValue _returnvalue_14 "Color_D" _output_5 :!class /Script/Engine.MaterialInstanceDynamic))
        (:Is%20Not%20Valid
          _))
      (Utilities|IsValid Gafas
        (:Is%20Valid
          (Components|StaticMesh|SetStaticMesh Gafas (Utilities|Array|Get(acopy) _gafasf _returnvalue)))
        (:Is%20Not%20Valid
          _))
      (Utilities|IsValid Pelo
        (:Is%20Valid
          (Components|StaticMesh|SetStaticMesh Pelo (Utilities|Array|Get(acopy) _peinado_f (Math|Conversions|ToInteger(Byte) _hairtype)))
          (bind _returnvalue_15 (Rendering|Material|CreateDynamicMaterialInstance Pelo 0 "/Game/Secpholand/Assets/Materials/MaterialInstances/Characters/MI_Hair.MI_Hair" "None" :!class /Script/Engine.PrimitiveComponent))
          (Rendering|Material|SetVectorParameterValue _returnvalue_15 "SkinColor" _output :!class /Script/Engine.MaterialInstanceDynamic))
        (:Is%20Not%20Valid
          _))
      (Utilities|IsValid Complemento
        (:Is%20Valid
          ;[1 1 1] Complemento
          (Components|StaticMesh|SetStaticMesh Complemento (Utilities|Array|Get(acopy) _complement_f (Math|Conversions|ToInteger(Byte) _complemento))))
        (:Is%20Not%20Valid
          _))
      (Utilities|IsValid Complemento2
        (:Is%20Valid
          ;[1 1 1] Complemento 2
          (Components|StaticMesh|SetStaticMesh Complemento2 (Utilities|Array|Get(acopy) _complement_f _returnvalue_2)))))))

(fn GetSocketNameforComplIdx
  (params (Index :type Integer))
  (return (Utilities|Select :Index Index :Option%200 "None" :Option%201 "LeftHandSocket" :Option%202 "LeftHandSocket" :Option%203 "LeftHandSocket" :Option%204 "LeftHandSocket" :Option%205 "HeadSocket" :Option%206 "BackPack_Socket" :Option%207 "HeadSocket" :Option%208 "HeadSocket" :Option%209 "HeadSocket" :Option%2010 "LeftHandSocket" :Option%2011 "LeftHandSocket")))

(fn GetZOffsetforBoina
  (params (Mesh :type Static%20Mesh%20Object%20Reference%20%28by%20ref%29))
  (bind _zoffsetsformesh (LocalVariables|GetZOffsetsForMesh))
  (bind (_value _returnvalue) (Utilities|Map|Find _zoffsetsformesh Mesh))
  (if _returnvalue
    (return _value)
    (else
      (return 0.0))))

(fn GetZOffsetforComplemento
  (params (ComplementoMesh :type Static%20Mesh%20Object%20Reference%20%28by%20ref%29) (PeloMesh :type Static%20Mesh%20Object%20Reference))
  (if (== ComplementoMesh "/Game/Secpholand/Assets/meshes/01Characters/03Accesories/03Accesories/Boina.Boina")
    (bind _value (CallFunction|GetZOffsetforBoina PeloMesh))
    (return _value)
    (else
      (return 0.0))))

(fn GetComponentstoRemove
  (params (ComponentSelected :type Byte))
  (bind _accessorygroupsdata (LocalVariables|GetAccessoryGroupsData))
  (if (!= ComponentSelected 0)
    (for (_array_element _array_index) _accessorygroupsdata
      (for (_array_element_2 _array_index_2) (Utilities|Struct|BreakArrayOfBytes _array_element)
        (if (== _array_element_2 ComponentSelected)
          (bind _output_get (LocalVariables|SetFinalArray (Utilities|Struct|BreakArrayOfBytes (Utilities|Array|Get(acopy) _accessorygroupsdata _array_index))))
          (return (LocalVariables|GetFinalArray)))))
    (return (Utilities|Array|MakeArray ComponentSelected))
    (else
      (return (Utilities|Array|MakeArray)))))