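; MediaPlayerManager is a manager Blueprint that controls playback of three videos: GalaxyNote, WatchVideo and AICongress.
; On BeginPlay it opens each media source on its own Media Player and starts playback.
; The StopVideosToExit event pauses all three players, apparently ahead of an exit.
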(event Custom|StopVideosToExit
  (Sequencer|Player|Pause (Variables|Default|GetmediaPlayer))
  (Sequencer|Player|Pause (Variables|Default|GetmediaPlayer2))
  (Sequencer|Player|Pause (Variables|Default|GetmediaPlayer2_0)))

(event EventBeginPlay
  (bind _mediaplayer (Variables|Default|GetmediaPlayer))
  (bind _mediaplayer2 (Variables|Default|GetmediaPlayer2))
  (bind _mediaplayer2_0 (Variables|Default|GetmediaPlayer2_0))
  (Media|MediaPlayer|OpenSource _mediaplayer "/Game/Movies/GalaxyNote.GalaxyNote")
  (Media|MediaPlayer|Play _mediaplayer :!class /Script/MediaAssets.MediaPlayer)
  (Media|MediaPlayer|OpenSource _mediaplayer2 "/Game/Movies/watchVideo.watchVideo")
  (Media|MediaPlayer|Play _mediaplayer2 :!class /Script/MediaAssets.MediaPlayer)
  (Media|MediaPlayer|OpenSource _mediaplayer2_0 "/Game/Movies/AICongress.AICongress")
  (Media|MediaPlayer|Play _mediaplayer2_0 :!class /Script/MediaAssets.MediaPlayer))

(fn ConstructionScript)