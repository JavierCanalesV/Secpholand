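; Info screen actor that shows a rotating slideshow of event thumbnail images on three material slots of its mesh.
; On non-authority instances, it creates three dynamic materials and polls until the local controller's HUD has an event list.
; It downloads each thumbnail sequentially, retrying failures without limit, then starts the slideshow.
; A self-repeating timed event advances separate wrapping indices to set each material's texture.
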(event Custom|DisplayEventImages
  (if (> (Variables|Default|Geti) (Utilities|Array|LastIndex (Variables|Default|GeteventTextures)))
    (Variables|Default|Seti 0))
  (Rendering|Material|SetTextureParameterValue (Variables|Default|Getmat1) "Texture" (Utilities|Array|Get(acopy) (Variables|Default|GeteventTextures) (Variables|Default|Geti)))
  (if (> (Variables|Default|Geti2) (Utilities|Array|LastIndex (Variables|Default|GeteventTextures)))
    (Variables|Default|Seti2 0))
  (Rendering|Material|SetTextureParameterValue (Variables|Default|Getmat2) "Texture" (Utilities|Array|Get(acopy) (Variables|Default|GeteventTextures) (Variables|Default|Geti2)))
  (if (> (Variables|Default|Geti3) (Utilities|Array|LastIndex (Variables|Default|GeteventTextures)))
    (Variables|Default|Seti3 0))
  (Rendering|Material|SetTextureParameterValue (Variables|Default|GetMat3) "Texture" (Utilities|Array|Get(acopy) (Variables|Default|GeteventTextures) (Variables|Default|Geti3)))
  (Math|Integer|IncrementInt (Variables|Default|Geti)
    (:%20%20
      (Math|Integer|IncrementInt (Variables|Default|Geti2)
        (:%20%20
          (Math|Integer|IncrementInt (Variables|Default|Geti3)
            (:%20%20
              (Utilities|FlowControl|Delay 3.0)
              (CallFunction|DisplayEventImages))))))))

(event Custom|Initialize3Materials
  (bind _returnvalue (Rendering|Material|CreateDynamicMaterialInstance (Variables|Default|GetSM_InfoScreen_A) 0 "/Game/Secpholand/UI/Images/Slides/SlideTexture+Emisive_Inst.SlideTexture+Emisive_Inst" "None" :!class /Script/Engine.PrimitiveComponent))
  (Variables|Default|Setmat1 _returnvalue)
  (bind _returnvalue_2 (Rendering|Material|CreateDynamicMaterialInstance (Variables|Default|GetSM_InfoScreen_A) 1 "/Game/Secpholand/UI/Images/Slides/SlideTexture+Emisive_Inst.SlideTexture+Emisive_Inst" "None" :!class /Script/Engine.PrimitiveComponent))
  (Variables|Default|Setmat2 _returnvalue_2)
  (bind _returnvalue_3 (Rendering|Material|CreateDynamicMaterialInstance (Variables|Default|GetSM_InfoScreen_A) 2 "/Game/Secpholand/UI/Images/Slides/SlideTexture+Emisive_Inst.SlideTexture+Emisive_Inst" "None" :!class /Script/Engine.PrimitiveComponent))
  (Variables|Default|SetMat3 _returnvalue_3))

(event EventBeginPlay
  (bind _returnvalue (Game|GetPlayerController 0))
  (bind _asclient_side_controller (Utilities|Casting|CastToClientSide_Controller _returnvalue))
  (bind _hud (Variables|/Game/Secpholand/Blueprints/ControllersYModes/baseClasses/ClientSide_Controller.ClientSide_Controller_C|GetHUD _asclient_side_controller))
  (bind _listadeeventos (Variables|/Game/Secpholand/UI/Widgets/HUDYChat/HUD.HUD_C|GetListaDeEventos _hud))
  (bind _returnvalue_2 (Utilities|Array|Length _listadeeventos))
  (Networking|SwitchHasAuthority
    (:Remote
      (CallFunction|Initialize3Materials)
      (Utilities|FlowControl|Delay 2.0)
      (Utilities|IsValid _hud :!label _label
        (:Is%20Valid
          (if (> _returnvalue_2 0) :!label _label_2
            (if (< (Variables|Default|Geti) _returnvalue_2) :!label _label_3
              (bind _texture (|DownloadImage (.URLThumbnailImage (Utilities|Struct|BreakEventoEnSecpholand (Utilities|Array|Get(acopy) _listadeeventos (Variables|Default|Geti)))))
                (:OnSuccess
                  (Utilities|Array|Add (Variables|Default|GeteventTextures) _texture)
                  (Math|Integer|IncrementInt (Variables|Default|Geti)
                    (:%20%20
                      (goto _label_3))))
                (:OnFail
                  (goto _label_3)))
              (else
                (Variables|Default|Seti 0)
                (CallFunction|DisplayEventImages)))
            (else
              (Utilities|FlowControl|Delay 0.2)
              (goto _label_2))))
        (:Is%20Not%20Valid
          (Utilities|FlowControl|Delay 0.2)
          (goto _label))))))

(fn ConstructionScript)