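; Round-table auditorium armchairs actor whose mesh visibility and collision follow a replicated Visible flag.
; One second after BeginPlay it applies the flag to its hierarchical instanced mesh, static mesh and actor collision.
; The OnRep handler reapplies it to collision and the instanced mesh only, leaving the static mesh untouched.
; Click events pass straight through to the parent class.
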(event EventBeginPlay
  (Utilities|FlowControl|Delay 1.0)
  (Rendering|SetVisibility (Variables|Default|GetHierarchicalInstancedStaticMesh) (Variables|Default|GetVisible) false)
  (Collision|SetActorEnableCollision (Variables|Default|GetVisible)))

(event EventClick
  (params (controller :type Client%20Side%20Controller%20Object%20Reference))
  (|CallParentFunction controller))

(fn ConstructionScript)

(fn OnRepVisible?
  (Rendering|SetVisibility (Variables|Default|GetHierarchicalInstancedStaticMesh) (Variables|Default|GetVisible) false)
  (Collision|SetActorEnableCollision (Variables|Default|GetVisible)))