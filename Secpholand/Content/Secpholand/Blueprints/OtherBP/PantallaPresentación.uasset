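; Clickable in-world presentation screen that shows downloaded slide images and extends a parent zoom-in interaction.
; Downloads numbered JPGs one by one until a request fails, then applies a dynamic material whose texture follows the slide index.
; Clicking caches the view target transform for camera reset; finishing zoom-in reveals a presenter-only HUD element.
; Zoom-out re-enables collision on linked screens; the call disabling it is unconnected.
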(event Custom|BuildTexturesAndInitScreen
  (params (Presentacion :type Presentacion%20Structure))
  ;[1 1 1] Build textures for Role Presentator
  (Variables|Default|SetPresentacionCached Presentacion)
  (Variables|Default|SetCountHelper 0)
  (Utilities|Array|Clear (Variables|Default|GetTexturasPresentacion))
  (bind _texture (|DownloadImage (select (Utilities|String|Contains (.UrlPresentacion (Utilities|Struct|BreakPresentacion (Variables|Default|GetPresentacionCached))) "localhost") (select (and (>= (.TotalDiapos (Utilities|Struct|BreakPresentacion (Variables|Default|GetPresentacionCached))) 10) (< (+ (Variables|Default|GetCountHelper) 1) 10)) (Utilities|String|Append (.UrlPresentacion (Utilities|Struct|BreakPresentacion (Variables|Default|GetPresentacionCached))) (.Username (Utilities|Struct|BreakUserInfo_Public (.Presentador (Utilities|Struct|BreakPresentacion (Variables|Default|GetPresentacionCached))))) "-slide-" "0" (Utilities|String|ToString(Integer) (+ (Variables|Default|GetCountHelper) 1)) ".jpg") (Utilities|String|Append (.UrlPresentacion (Utilities|Struct|BreakPresentacion (Variables|Default|GetPresentacionCached))) (.Username (Utilities|Struct|BreakUserInfo_Public (.Presentador (Utilities|Struct|BreakPresentacion (Variables|Default|GetPresentacionCached))))) "-slide-" (Utilities|String|ToString(Integer) (+ (Variables|Default|GetCountHelper) 1)) ".jpg")) (Utilities|String|Append (.UrlPresentacion (Utilities|Struct|BreakPresentacion (Variables|Default|GetPresentacionCached))) (Utilities|String|ToString(Integer) (+ (Variables|Default|GetCountHelper) 1)) ".jpg")) :!label _label)
    (:OnSuccess
      (Math|Integer|IncrementInt (Variables|Default|GetCountHelper)
        (:%20%20
          (Utilities|Array|Add (Variables|Default|GetTexturasPresentacion) _texture)
          (goto _label))))
    (:OnFail
      (Development|PrintString "Error Downloading Textures" true true "(R=0.000000,G=0.660000,B=1.000000,A=1.000000)" 1e+01)
      (bind _returnvalue (Rendering|Material|CreateDynamicMaterialInstance (Variables|Default|GetStaticMesh) (Variables|Default|GetScreenMaterialIndex) "/Game/Secpholand/UI/Images/Slides/SlideTexture.SlideTexture" "None" :!class /Script/Engine.PrimitiveComponent))
      (Variables|Default|SetMaterialDynamic _returnvalue)
      (CallFunction|UpdateDiapositiva (.CurrentDiapo (Utilities|Struct|BreakPresentacion (Variables|Default|GetPresentacionCached)))))))

(event Custom|UpdateDiapositiva
  (params (Index :type Integer))
  ;[1 1 1] Build textures for Role Presentator
  (Rendering|Material|SetTextureParameterValue (Variables|Default|GetMaterialDynamic) "Texture" (Utilities|Array|Get(acopy) (Variables|Default|GetTexturasPresentacion) Index)))

(event Custom|resetCamera
  (bind _originaltransform (Variables|Default|GetoriginalTransform))
  (if (Class|KismetMathLibrary|NotEqualExactlyVectorVector (.Location (Math|Transform|BreakTransform _originaltransform)) "0, 0, 0")
    (Transformation|SetActorTransform (Pawn|GetViewTarget (Game|GetPlayerController 0)) _originaltransform)))

(event Custom|CacheTransform
  (Variables|Default|SetoriginalTransform (Transformation|GetActorTransform (Pawn|GetViewTarget (Game|GetPlayerController 0)))))

(event Custom|DesactivarPantalla
  ;[1 1 1] Build textures for Role Presentator
  (Rendering|Material|SetMaterial (Variables|Default|GetStaticMesh) (Variables|Default|GetScreenMaterialIndex) "/Game/Secpholand/Assets/Materials/MaterialInstances/Tileables/Screen.Screen")
  (Variables|Default|SetPresentacionCached ""))

(event Custom|ToggleScreens
  (params (TurnOnCollision? :type Boolean))
  ;[1 1 1] Zoom al pulsar y widgets de salida de sala
  (for _array_element (Variables|Default|GetScreensToInvalidate)
    (Utilities|IsValid _array_element
      (:Is%20Valid
        (Collision|SetActorEnableCollision _array_element TurnOnCollision?)
        (Collision|SetCollisionEnabled (Variables|/Game/Secpholand/Blueprints/clasesBase/ClickableActor.ClickableActor_C|GetStaticMesh _array_element) (select TurnOnCollision? "QueryAndPhysics" "NoCollision"))))))

(event EventFinishedZoomin
  ;[1 1 1] Zoom al pulsar y widgets de salida de sala
  (|CallParentFunction)
  (bind _asinterior_controller (Utilities|Casting|CastToInteriorController (Game|GetPlayerController 0)))
  (if (Variables|/Game/Secpholand/Blueprints/ControllersYModes/InteriorController.InteriorController_C|GetIsPresenter? _asinterior_controller)
    (Widget|SetVisibility (Variables|/Game/Secpholand/UI/Widgets/HUDYChat/HUD.HUD_C|GetHudArribaizquierda (Variables|/Game/Secpholand/Blueprints/ControllersYModes/baseClasses/ClientSide_Controller.ClientSide_Controller_C|GetHUD _asinterior_controller)) "SelfHitTestInvisible")))

(event EventFinishedZoomOut
  ;[1 1 1] Zoom al pulsar y widgets de salida de sala
  (|CallParentFunction)
  (CallFunction|ToggleScreens true)
  (Default|CallHasUnZoomed))

(event EventClick
  (params (controller :type Client%20Side%20Controller%20Object%20Reference))
  ;[1 1 1] Zoom al pulsar y widgets de salida de sala
  (|CallParentFunction controller)
  (Default|CallHasZoomed)
  (CallFunction|CacheTransform))

(fn ConstructionScript)