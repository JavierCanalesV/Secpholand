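; Outdoor company stand actor combining a counter, two banners with clickable URL actors, and a call zone as child actors.
; On BeginPlay, after a one-second delay, it passes InfoOutdoorStand's company name and URLs to counter and banners, then hides the clickables.
; The call zone's room ID is 70 plus the level's total ZonaDeLlamada count.
; HoverMode skips this setup; the construction script instead applies a holographic material and disables collision.
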(event Custom|SetZonaLlamadaID
  (bind _aszona_de_llamada (Utilities|Casting|CastToZonaDeLlamada (Variables|/Script/Engine.ChildActorComponent|GetChildActor (Variables|Default|GetZonaLlamada))))
  (bind _outactors (Actor|GetAllActorsOfClass "/Game/Secpholand/Blueprints/OtherBP/ZonaDeLlamada.ZonaDeLlamada_C"))
  (bind _output_get (Variables|/Game/Secpholand/Blueprints/OtherBP/ZonaDeLlamada.ZonaDeLlamada_C|SetIDRoom _aszona_de_llamada (+ 70 (Utilities|Array|Length _outactors))))
  (Development|PrintString (Utilities|String|Append "ID: " (Utilities|String|ToString(Integer) _output_get))))

(event EventBeginPlay
  (bind _infooutdoorstand (Variables|Default|GetInfoOutdoorStand))
  (bind _infooutdoorstand_2 (Variables|Default|GetInfoOutdoorStand))
  (bind (_nombreempresa _urlvideopantalla1 _urlvideopantalla2 _urlclickpantalla1 _urlclickpantalla2) (Utilities|Struct|BreakInfoOutdoorStand _infooutdoorstand_2))
  (bind (_nombreempresa_2 _urlvideopantalla1_2 _urlvideopantalla2_2 _urlclickpantalla1_2) (Utilities|Struct|BreakInfoOutdoorStand _infooutdoorstand))
  (Networking|SwitchHasAuthority
    (:Authority
      _)
    (:Remote
      _))
  (if (not (Variables|Default|GetHoverMode))
    (Development|PrintString "updating remote")
    (Utilities|FlowControl|Delay 1.0)
    (bind _asmostrador_outdoor_stand (Utilities|Casting|CastToMostradorOutdoorStand (Variables|/Script/Engine.ChildActorComponent|GetChildActor (Variables|Default|GetMostrador))))
    (Default|Init _asmostrador_outdoor_stand (.NombreEmpresa (Utilities|Struct|BreakInfoOutdoorStand (Variables|Default|GetInfoOutdoorStand))))
    (bind _asbanner_outdoor_stand (Utilities|Casting|CastToBanner_OutdoorStand (Variables|/Script/Engine.ChildActorComponent|GetChildActor (Variables|Default|GetBanner))))
    (Default|Init _asbanner_outdoor_stand _nombreempresa_2 _urlvideopantalla1_2 _urlclickpantalla1_2)
    (bind _asclickable_url (Utilities|Casting|CastToClickableURL (Variables|/Script/Engine.ChildActorComponent|GetChildActor (Variables|Default|GetClickable))))
    (Utilities|Array|Add (Variables|/Game/Secpholand/Blueprints/clasesBase/ZoomClickable.ZoomClickable_C|Getclicables _asbanner_outdoor_stand) _asclickable_url)
    (Default|UnshowClicables _asbanner_outdoor_stand)
    (bind _asbanner_outdoor_stand_2 (Utilities|Casting|CastToBanner_OutdoorStand (Variables|/Script/Engine.ChildActorComponent|GetChildActor (Variables|Default|GetBanner1))))
    (Default|Init _asbanner_outdoor_stand_2 _nombreempresa _urlvideopantalla2 _urlclickpantalla2)
    (bind _asclickable_url_2 (Utilities|Casting|CastToClickableURL (Variables|/Script/Engine.ChildActorComponent|GetChildActor (Variables|Default|GetClickable1))))
    (Utilities|Array|Add (Variables|/Game/Secpholand/Blueprints/clasesBase/ZoomClickable.ZoomClickable_C|Getclicables _asbanner_outdoor_stand_2) _asclickable_url_2)
    (Default|UnshowClicables _asbanner_outdoor_stand_2)
    (CallFunction|SetZonaLlamadaID)))

(fn ConstructionScript
  (if (Variables|Default|GethoverMode)
    (Rendering|Material|SetMaterial (Variables|Default|GetStaticMesh) 0 "/Game/Secpholand/Assets/Materials/HOLOGRAFIC.HOLOGRAFIC")
    (Collision|SetActorEnableCollision false)
    (for _array_element (Actor|GetAllChildActors true)
      (Collision|SetActorEnableCollision _array_element false))))