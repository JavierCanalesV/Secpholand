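; Spline-based ambient traffic actor that runs two vehicles in opposite directions along the Camino spline, offset sideways into separate lanes.
; ActivateTrafic toggles tick and starts the vehicles, each getting a random mesh (two cars or a bus) and a random body color through a dynamic material.
; Tick advances each vehicle's spline alpha by DeltaSeconds over Divider, then relaunches it after a random delay at the end.
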(event Custom|startVehicleWithDelay
  ;[1 1 1] StartVehicles
  (Utilities|FlowControl|Delay (Math|Random|RandomFloatinRange 2.0 12.0))
  (Variables|Default|SetrandomInt (Math|Random|RandomInteger 3))
  (Components|StaticMesh|SetStaticMesh (Variables|Default|GetCar_01) (Utilities|Select :Index (Variables|Default|GetrandomInt) :Option%200 "/Game/Secpholand/Assets/meshes/Secpholand_Island/Props/SM_Car1.SM_Car1" :Option%201 "/Game/Secpholand/Assets/meshes/Secpholand_Island/Props/SM_Bus.SM_Bus" :Option%202 "/Game/Secpholand/Assets/meshes/Secpholand_Island/Props/SM_Car2.SM_Car2"))
  (Variables|Default|Setgo1 true)
  (Variables|Default|Setalfa 0.0)
  (Transformation|SetRelativeScale3D (Variables|Default|GetCar_01) (Math|Vector|MakeVector (Utilities|Select :Index (Variables|Default|GetrandomInt) :Option%200 -1.0 :Option%201 1.0 :Option%202 -1.0) 1.0 1.0))
  (bind _returnvalue (Rendering|Material|CreateDynamicMaterialInstance (Variables|Default|GetCar_01) 0 "/Game/Secpholand/Assets/Materials/MaterialInstances/Cars/MI_Car_White.MI_Car_White" "None" :!class /Script/Engine.PrimitiveComponent))
  (Rendering|Material|SetVectorParameterValue _returnvalue "BC_A" (Utilities|Select :Index (Math|Random|RandomInteger 5) :Option%200 "(R=0.598958,G=0.081838,B=0.068631,A=1.000000)" :Option%201 "(R=0.063639,G=0.119821,B=0.718750,A=1.000000)" :Option%202 "(R=0.037992,G=0.140625,B=0.025635,A=1.000000)" :Option%203 "(R=0.859375,G=0.859375,B=0.859375,A=1.000000)" :Option%204 "(R=0.145833,G=0.145833,B=0.145833,A=1.000000)") :!class /Script/Engine.MaterialInstanceDynamic)
  (Development|SetHiddeninGame (Variables|Default|Getcar_01) false false))

(event Custom|SetPosAlfa2
  (params (alfa :type Float%20%28single-precision%29))
  (bind _returnvalue (- 1.0 alfa))
  (bind _car_02 (Variables|Default|Getcar_02))
  (bind _camino (Variables|Default|Getcamino))
  ;[1 1 1] Tick
  (Transformation|SetWorldLocation _car_02 (+ (Spline|GetLocationatTime _camino _returnvalue "World" false) (* (Math|Vector|GetRightVector _car_02) -300)) false false)
  (Transformation|SetRelativeRotation _car_02 (Class|SplineComponent|GetRotationatTime _camino _returnvalue "Local" false) false false))

(event Custom|setPosAlfa
  (params (alfa :type Float%20%28single-precision%29))
  (bind _camino (Variables|Default|Getcamino))
  (bind _car_01 (Variables|Default|GetCar_01))
  (bind _returnvalue (Class|SplineComponent|GetRotationatTime _camino alfa "Local" false))
  ;[1 1 1] Tick
  (Transformation|SetWorldLocation _car_01 (+ (Spline|GetLocationatTime _camino alfa "World" false) (* (Math|Vector|GetRightVector (Variables|Default|Getcar_01)) 300)) false false)
  (Transformation|SetRelativeRotation _car_01 (Math|Rotator|MakeRotator (.roll _returnvalue) (.pitch _returnvalue) (.yaw _returnvalue)) false false))

(event Custom|startVehicle2WithDelay
  ;[1 1 1] StartVehicles
  (Utilities|FlowControl|Delay (Math|Random|RandomFloatinRange 2.0 5.0))
  (Variables|Default|SetrandomInt (Math|Random|RandomInteger 3))
  (Components|StaticMesh|SetStaticMesh (Variables|Default|Getcar_02) (Utilities|Select :Index (Variables|Default|GetrandomInt) :Option%200 "/Game/Secpholand/Assets/meshes/Secpholand_Island/Props/SM_Car1.SM_Car1" :Option%201 "/Game/Secpholand/Assets/meshes/Secpholand_Island/Props/SM_Bus.SM_Bus" :Option%202 "/Game/Secpholand/Assets/meshes/Secpholand_Island/Props/SM_Car2.SM_Car2"))
  (Variables|Default|Setgo2 true)
  (Variables|Default|Setalfa2 0.0)
  (Transformation|SetRelativeScale3D (Variables|Default|Getcar_02) (Math|Vector|MakeVector (Utilities|Select :Index (Variables|Default|GetrandomInt) :Option%200 1.0 :Option%201 -1.0 :Option%202 1.0) 1.0 1.0))
  (bind _returnvalue (Rendering|Material|CreateDynamicMaterialInstance (Variables|Default|Getcar_02) 0 "/Game/Secpholand/Assets/Materials/MaterialInstances/Cars/MI_Car_White.MI_Car_White" "None" :!class /Script/Engine.PrimitiveComponent))
  (Rendering|Material|SetVectorParameterValue _returnvalue "BC_A" (Utilities|Select :Index (Math|Random|RandomInteger 5) :Option%200 "(R=0.598958,G=0.081838,B=0.068631,A=1.000000)" :Option%201 "(R=0.063639,G=0.119821,B=0.718750,A=1.000000)" :Option%202 "(R=0.037992,G=0.140625,B=0.025635,A=1.000000)" :Option%203 "(R=0.859375,G=0.859375,B=0.859375,A=1.000000)" :Option%204 "(R=0.145833,G=0.145833,B=0.145833,A=1.000000)") :!class /Script/Engine.MaterialInstanceDynamic)
  (Development|SetHiddeninGame (Variables|Default|Getcar_02) false false))

(event Custom|ActivateTrafic
  (params (activate :type Boolean))
  ;[1 1 1] ActivateTrafic
  (Actor|Tick|SetActorTickEnabled activate)
  (if activate
    (CallFunction|StartVehicles)
    (else
      (Development|SetHiddeninGame (Variables|Default|Getcar_01) false false)
      (Variables|Default|Setgo1 false)
      (Variables|Default|Setgo2 false))))

(event Custom|StartVehicles
  (bind _returnvalue (Math|Random|RandomInteger 2))
  (bind _returnvalue_2 (== _returnvalue 1))
  ;[1 1 1] StartVehicles
  (Utilities|FlowControl|Sequence
    (:then_0
      (Utilities|FlowControl|Delay (select _returnvalue_2 0.0 (Math|Random|RandomFloatinRange 2.0 5.0)))
      (Variables|Default|SetrandomInt (Math|Random|RandomInteger 3))
      (Components|StaticMesh|SetStaticMesh (Variables|Default|GetCar_01) (Utilities|Select :Index (Variables|Default|GetrandomInt) :Option%200 "/Game/Secpholand/Assets/meshes/Secpholand_Island/Props/SM_Car1.SM_Car1" :Option%201 "/Game/Secpholand/Assets/meshes/Secpholand_Island/Props/SM_Bus.SM_Bus" :Option%202 "/Game/Secpholand/Assets/meshes/Secpholand_Island/Props/SM_Car2.SM_Car2"))
      (Variables|Default|Setgo1 true)
      (Variables|Default|Setalfa 0.0)
      (Transformation|SetRelativeScale3D (Variables|Default|GetCar_01) (Math|Vector|MakeVector (Utilities|Select :Index (Variables|Default|GetrandomInt) :Option%200 -1.0 :Option%201 1.0 :Option%202 -1.0) 1.0 1.0))
      (bind _returnvalue_3 (Rendering|Material|CreateDynamicMaterialInstance (Variables|Default|GetCar_01) 0 "/Game/Secpholand/Assets/Materials/MaterialInstances/Cars/MI_Car_White.MI_Car_White" "None" :!class /Script/Engine.PrimitiveComponent))
      (Rendering|Material|SetVectorParameterValue _returnvalue_3 "BC_A" (Utilities|Select :Index (Math|Random|RandomInteger 5) :Option%200 "(R=0.598958,G=0.081838,B=0.068631,A=1.000000)" :Option%201 "(R=0.063639,G=0.119821,B=0.718750,A=1.000000)" :Option%202 "(R=0.037992,G=0.140625,B=0.025635,A=1.000000)" :Option%203 "(R=0.859375,G=0.859375,B=0.859375,A=1.000000)" :Option%204 "(R=0.145833,G=0.145833,B=0.145833,A=1.000000)") :!class /Script/Engine.MaterialInstanceDynamic)
      (Development|SetHiddeninGame (Variables|Default|Getcar_01) false false))
    (:then_1
      (Utilities|FlowControl|Delay (select _returnvalue_2 (Math|Random|RandomFloatinRange 2.0 5.0) 0.0))
      (Variables|Default|SetrandomInt (Math|Random|RandomInteger 3))
      (Components|StaticMesh|SetStaticMesh (Variables|Default|Getcar_02) (Utilities|Select :Index (Variables|Default|GetrandomInt) :Option%200 "/Game/Secpholand/Assets/meshes/Secpholand_Island/Props/SM_Car1.SM_Car1" :Option%201 "/Game/Secpholand/Assets/meshes/Secpholand_Island/Props/SM_Bus.SM_Bus" :Option%202 "/Game/Secpholand/Assets/meshes/Secpholand_Island/Props/SM_Car2.SM_Car2"))
      (Variables|Default|Setgo2 true)
      (Variables|Default|Setalfa2 0.0)
      (Transformation|SetRelativeScale3D (Variables|Default|Getcar_02) (Math|Vector|MakeVector (Utilities|Select :Index (Variables|Default|GetrandomInt) :Option%200 1.0 :Option%201 -1.0 :Option%202 1.0) 1.0 1.0))
      (bind _returnvalue_4 (Rendering|Material|CreateDynamicMaterialInstance (Variables|Default|Getcar_02) 0 "/Game/Secpholand/Assets/Materials/MaterialInstances/Cars/MI_Car_White.MI_Car_White" "None" :!class /Script/Engine.PrimitiveComponent))
      (Rendering|Material|SetVectorParameterValue _returnvalue_4 "BC_A" (Utilities|Select :Index (Math|Random|RandomInteger 5) :Option%200 "(R=0.598958,G=0.081838,B=0.068631,A=1.000000)" :Option%201 "(R=0.063639,G=0.119821,B=0.718750,A=1.000000)" :Option%202 "(R=0.037992,G=0.140625,B=0.025635,A=1.000000)" :Option%203 "(R=0.859375,G=0.859375,B=0.859375,A=1.000000)" :Option%204 "(R=0.145833,G=0.145833,B=0.145833,A=1.000000)") :!class /Script/Engine.MaterialInstanceDynamic)
      (Development|SetHiddeninGame (Variables|Default|Getcar_02) false false))))

(event EventBeginPlay
  (CallFunction|ActivateTrafic (Variables|Default|GetStartActivated)))

(event EventTick
  (params (DeltaSeconds :type Float%20%28single-precision%29))
  ;[1 1 1] Tick
  (Utilities|FlowControl|Sequence
    (:then_0
      (if (Variables|Default|Getgo1)
        (if (< (Variables|Default|Getalfa) 1.0)
          (bind _output_get (Variables|Default|Setalfa (+ (Variables|Default|Getalfa) (/ DeltaSeconds (Variables|Default|Getdivider)))))
          (CallFunction|SetPosAlfa _output_get)
          (else
            (Development|SetHiddeninGame (Variables|Default|Getcar_01) false false)
            (CallFunction|StartVehiclewithDelay)
            (Variables|Default|Setgo1 false)))))
    (:then_1
      (if (Variables|Default|Getgo2)
        (if (< (Variables|Default|Getalfa2) 1.0)
          (bind _output_get_2 (Variables|Default|Setalfa2 (+ (Variables|Default|Getalfa2) (/ DeltaSeconds (Variables|Default|Getdivider)))))
          (CallFunction|SetPosAlfa2 _output_get_2)
          (else
            (Development|SetHiddeninGame (Variables|Default|Getcar_02) true false)
            (CallFunction|StartVehicle2withDelay)
            (Variables|Default|Setgo2 false)))))))

(fn ConstructionScript)

(fn GetXLength
  (params (Mesured%20mesh :type Static%20Mesh%20Object%20Reference))
  (return (* (.X (Math|Vector|BreakVector (.Max (Utilities|Struct|BreakBox (StaticMesh|GetBoundingBox Mesured%20mesh))))) 2.0)))