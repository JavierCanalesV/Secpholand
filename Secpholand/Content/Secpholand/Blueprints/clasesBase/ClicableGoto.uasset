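; Base clickable that sends the player's client-side pawn to its GotoBox and fires an empty Arrived event on arrival.
; A permitted click calls Arrived if already overlapping; otherwise it arms the object, spawns a decal and starts the move.
; From bird's-eye view, it first turns the spring arm toward the box, triggers street view and waits longer the closer the target is.
; Client-side box overlap by the local pawn stops movement while armed.
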(event OnComponentBeginOverlap(GotoBox)
  (params (OverlappedComponent :type Primitive%20Component%20Object%20Reference) (OtherActor :type Actor%20Object%20Reference) (OtherComp :type Primitive%20Component%20Object%20Reference) (OtherBodyIndex :type Integer) (bFromSweep :type Boolean) (SweepResult :type Hit%20Result%20Structure%20%28by%20ref%29))
  (Networking|SwitchHasAuthority
    (:Remote
      (if (Variables|Default|Getactive)
        (bind _asclient_side_pawn (Utilities|Casting|CastToClientSide_Pawn OtherActor))
        (bind _asclient_side_controller (Utilities|Casting|CastToClientSide_Controller (Game|GetPlayerController 0)))
        (if (== (Variables|/Game/Secpholand/Blueprints/ControllersYModes/baseClasses/ClientSide_Controller.ClientSide_Controller_C|GetClientSidePawnRef _asclient_side_controller) _asclient_side_pawn)
          (Default|StopMovement:Client _asclient_side_controller)
          (CallFunction|Arrived)
          (Development|PrintString "Hello"))))))

(event Custom|Arrived)

(event EventClick
  (params (controller :type Client%20Side%20Controller%20Object%20Reference))
  (bind _clientsidepawnref (Variables|/Game/Secpholand/Blueprints/ControllersYModes/baseClasses/ClientSide_Controller.ClientSide_Controller_C|GetClientSidePawnRef controller))
  (bind _gotobox (Variables|Default|GetGotoBox))
  (bind _gotobox_2 (Variables|Default|GetGotoBox))
  (bind _clientsidepawnref_2 (Variables|/Game/Secpholand/Blueprints/ControllersYModes/baseClasses/ClientSide_Controller.ClientSide_Controller_C|GetClientSidePawnRef controller))
  (bind _returnvalue (Transformation|GetWorldLocation _gotobox))
  (bind _returnvalue_2 (Transformation|GetActorLocation _clientsidepawnref_2))
  (bind _returnvalue_3 (Transformation|GetWorldLocation _gotobox_2))
  (bind _springarm (Variables|/Game/Secpholand/Blueprints/ControllersYModes/baseClasses/ClientSide_Pawn.ClientSide_Pawn_C|GetSpringArm _clientsidepawnref_2))
  (|CallParentFunction controller)
  (if (Variables|Default|GetAllowedToUse)
    (if (Variables|/Game/Secpholand/Blueprints/ControllersYModes/baseClasses/ClientSide_Pawn.ClientSide_Pawn_C|Getb_VistaPajaro _clientsidepawnref)
      (Transformation|SetWorldRotation _springarm (Math|Rotator|MakeRotator 0.0 (.pitch (Transformation|GetWorldRotation _springarm)) (.yaw (Math|Rotator|FindLookatRotation _returnvalue_2 _returnvalue))) false false)
      (for _array_element (Class|PanelWidget|GetAllChildren (Variables|/Game/Secpholand/UI/Widgets/HUDYChat/HUD.HUD_C|GetHudArribaizquierda (Variables|/Game/Secpholand/Blueprints/ControllersYModes/baseClasses/ClientSide_Controller.ClientSide_Controller_C|GetHUD controller)))
        (bind _asboton_vista_pajaro (Utilities|Casting|CastToBotonVistaPajaro _array_element))
        (Default|ClicarVistaCalle _asboton_vista_pajaro)
        (Utilities|FlowControl|Delay (* (Math|Float|Clamp(Float) (- 1.0 (/ (Math|Vector|Distance(Vector) _returnvalue _returnvalue_2) (* (Class|MovementComponent|GetMaxSpeed (Variables|/Script/Engine.Character|GetCharacterMovement (Variables|/Game/Secpholand/Blueprints/ControllersYModes/baseClasses/ClientSide_Controller.ClientSide_Controller_C|GetServerSideCharacterRef controller))) 2.5)))) 2.5))
        (if (Collision|IsOverlappingActor (Variables|Default|GetGotoBox) _clientsidepawnref :!class /Script/Engine.PrimitiveComponent)
          (CallFunction|Arrived)
          (else
            (Variables|Default|Setactive true)
            (Default|SpawnDecalatLocation controller _returnvalue_3)
            (Default|MovetoLocation controller _returnvalue_3))))
      (else
        (if (Collision|IsOverlappingActor (Variables|Default|GetGotoBox) _clientsidepawnref :!class /Script/Engine.PrimitiveComponent)
          (CallFunction|Arrived)
          (else
            (Variables|Default|Setactive true)
            (Default|SpawnDecalatLocation controller _returnvalue_3)
            (Default|MovetoLocation controller _returnvalue_3)))))))

(event EventResetClick
  (|CallParentFunction)
  (Variables|Default|Setactive false))

(fn ConstructionScript
  (|CallParentFunction))