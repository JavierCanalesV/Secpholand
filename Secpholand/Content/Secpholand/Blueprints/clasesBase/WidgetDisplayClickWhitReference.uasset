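; Base clickable Blueprint that displays a widget on screen when clicked, extending its parent's click and hover behavior.
; Click creates a new WidgetClass instance each time, stores it in RefWB, adds it to the viewport and calls ResetClick.
; Hover skips the parent response once when JustClicked is set, clearing the flag.
; Disconnected nodes hold an unused validity check that would reuse the stored widget.
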(event EventHover
  (if (Variables|Default|GetjustClicked)
    (Variables|Default|SetjustClicked false)
    (else
      (|CallParentFunction))))

(event EventBeginPlay
  (|CallParentFunction))

(event EventClick
  (params (controller :type Client%20Side%20Controller%20Object%20Reference))
  (|CallParentFunction controller)
  (bind _returnvalue (UserInterface|CreateWidget (Variables|Default|GetwidgetClass)))
  (bind _output_get (Variables|Default|SetRef_WB _returnvalue))
  (UserInterface|Viewport|AddtoViewport _output_get 0)
  (CallFunction|ResetClick))

(fn ConstructionScript)