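; AscensorB2B is a clickable elevator actor that teleports the local player behind a screen fade.
; A click from a MenuLobbyController triggers Arrived immediately, while other controllers get the parent click behavior.
; Arrived fades to black, moves and rotates the player to LocationTeleport relative to the actor, resets spring-arm yaw and zoom, then fades back in.
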(event EventArrived
  (bind _returnvalue (Transformation|GetActorTransform))
  (bind _locationteleport (Variables|Default|GetlocationTeleport))
  (bind (_location _rotation) (Math|Transform|BreakTransform _locationteleport))
  (bind _asclient_side_controller (Utilities|Casting|CastToClientSide_Controller (Game|GetPlayerController 0)))
  (CameraFades|StartCameraFade :self (Variables|/Script/Engine.PlayerController|GetPlayerCameraManager _asclient_side_controller) :ToAlpha 1.0 :Duration 0.6 :bHoldWhenFinished true)
  (Utilities|FlowControl|Delay 0.6)
  (Default|TeleportPlayer:Client _asclient_side_controller (Math|Transform|TransformLocation _returnvalue _location))
  (Default|RotatePlayer:Client _asclient_side_controller (Math|Transform|TransformRotation _returnvalue _rotation))
  (Transformation|SetWorldRotation (Variables|/Game/Secpholand/Blueprints/ControllersYModes/baseClasses/ClientSide_Pawn.ClientSide_Pawn_C|GetSpringArm (Variables|/Game/Secpholand/Blueprints/ControllersYModes/baseClasses/ClientSide_Controller.ClientSide_Controller_C|GetClientSidePawnRef _asclient_side_controller)) (Math|Rotator|MakeRotator (.roll (Transformation|GetWorldRotation (Variables|/Game/Secpholand/Blueprints/ControllersYModes/baseClasses/ClientSide_Pawn.ClientSide_Pawn_C|GetSpringArm (Variables|/Game/Secpholand/Blueprints/ControllersYModes/baseClasses/ClientSide_Controller.ClientSide_Controller_C|GetClientSidePawnRef _asclient_side_controller)))) (.pitch (Transformation|GetWorldRotation (Variables|/Game/Secpholand/Blueprints/ControllersYModes/baseClasses/ClientSide_Pawn.ClientSide_Pawn_C|GetSpringArm (Variables|/Game/Secpholand/Blueprints/ControllersYModes/baseClasses/ClientSide_Controller.ClientSide_Controller_C|GetClientSidePawnRef _asclient_side_controller)))) 9e+01) false false)
  (bind _output_get (Variables|/Game/Secpholand/Blueprints/ControllersYModes/baseClasses/ClientSide_Controller.ClientSide_Controller_C|Setzoom _asclient_side_controller 0.1))
  (bind _output_get_2 (Variables|/Game/Secpholand/Blueprints/ControllersYModes/baseClasses/ClientSide_Controller.ClientSide_Controller_C|SetzoomTarget _asclient_side_controller _output_get))
  (Default|ZoomEvent (Variables|/Game/Secpholand/Blueprints/ControllersYModes/baseClasses/ClientSide_Controller.ClientSide_Controller_C|GetClientSidePawnRef _asclient_side_controller) _output_get_2)
  (Utilities|FlowControl|Delay 0.4)
  (CameraFades|StartCameraFade :self (Variables|/Script/Engine.PlayerController|GetPlayerCameraManager _asclient_side_controller) :FromAlpha 1.0 :Duration 0.6 :bHoldWhenFinished true))

(event EventClick
  (params (controller :type Client%20Side%20Controller%20Object%20Reference))
  (Utilities|Casting|CastToMenuLobbyController controller
    (:then
      (CallFunction|Arrived))
    (:CastFailed
      (|CallParentFunction controller))))

(fn ConstructionScript
  (|CallParentFunction))