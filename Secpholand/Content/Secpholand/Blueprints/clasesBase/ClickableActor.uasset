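; Base class for clickable world actors that show a hover tooltip and gate interaction by the player's level.
; Hover creates or re-adds a title and hint widget, clamped on screen.
; Click compares the controller's user level with MinLvl, then either plays a sound and shows the active hint or clears the tooltip, or marks it blocked with a Spanish level-required or unavailable message.
; ResetClick removes the widget and clears the controller's clicked reference.
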(event Custom|Click
  (params (controller :type Client%20Side%20Controller%20Object%20Reference))
  (bind _userinfo_private (Variables|/Game/Secpholand/Blueprints/ControllersYModes/baseClasses/ClientSide_Controller.ClientSide_Controller_C|GetuserInfo_Private controller))
  (bind _minlvl (Variables|Default|GetminLvl))
  (bind _level (Utilities|Struct|BreakUserInfo_Private _userinfo_private))
  (bind _returnvalue (>= _minlvl 0))
  (if (and (>= _level _minlvl) _returnvalue)
    (Audio|PlaySound2D "/Game/Secpholand/audio/UISounds/UIBright.UIBright" 1.0 1.0 0.0 0 0)
    (if (> (Utilities|String|Len (Utilities|String|ToString(Text) (Variables|Default|GethoverActiveHint))) 0)
      (Utilities|IsValid (Variables|Default|GethoverUserWidget)
        (:Is%20Valid
          (Default|ChangeState (Variables|Default|GethoverUserWidget) (Utilities|Text|ToText(String) (Utilities|String|ToString(Text) (Variables|Default|GethoverActiveHint))) true)))
      (elif (> (Utilities|String|Len (Utilities|String|ToString(Text) (Variables|Default|GethoverTitle))) 0)
        (Utilities|IsValid (Variables|Default|GethoverUserWidget)
          (:Is%20Valid
            (Widget|RemovefromParent (Variables|Default|GethoverUserWidget))
            (Variables|Default|SethoverUserWidget 0)
            (Default|StopOutliningActor controller self)))))
    (else
      (Variables|Default|SetAllowedToUse false)
      (Default|FillHoverInfo (Variables|Default|GethoverUserWidget) (select _returnvalue (Utilities|Text|ToText(String) (Utilities|String|Append (Utilities|String|ToString(Text) (Utilities|Text|MakeLiteralText "Requiere nivel ")) (Utilities|String|ToString(Integer) (Variables|Default|GetminLvl)))) "No disponible") (select _returnvalue (Utilities|Text|ToText(String) (Utilities|String|Append (Utilities|String|ToString(Text) (Utilities|Text|MakeLiteralText "Eres nivel ")) (Utilities|String|ToString(Integer) _level))) "Te avisaremos cuando lo esté"))
      (Default|Blocked (Variables|Default|GethoverUserWidget)))))

(event Custom|ResetClick
  (Utilities|IsValid (Variables|Default|GethoverUserWidget)
    (:Is%20Valid
      (Widget|RemovefromParent (Variables|Default|GethoverUserWidget))
      (Variables|Default|SethoverUserWidget 0))
    (:Is%20Not%20Valid
      _))
  (bind _asclient_side_controller (Utilities|Casting|CastToClientSide_Controller (Game|GetPlayerController 0)))
  (Variables|/Game/Secpholand/Blueprints/ControllersYModes/baseClasses/ClientSide_Controller.ClientSide_Controller_C|SetClickableClicked _asclient_side_controller 0))

(event Custom|Hover
  (if (> (Utilities|String|Len (Utilities|String|ToString(Text) (Variables|Default|GethoverTitle))) 0)
    (Utilities|IsValid (Variables|Default|GethoverUserWidget)
      (:Is%20Valid
        (if (UserInterface|Viewport|IsinViewport (Variables|Default|GethoverUserWidget))
          _
          (else
            (UserInterface|Viewport|AddtoViewport (Variables|Default|GethoverUserWidget) 1))))
      (:Is%20Not%20Valid
        (bind _returnvalue (UserInterface|CreateWidget "/Game/Secpholand/UI/Widgets/HoverWidgets/HoverWidMaster.HoverWidMaster_C"))
        (bind _output_get (Variables|Default|SethoverUserWidget _returnvalue))
        (Default|FillHoverInfo _output_get (Utilities|Text|ToText(String) (Utilities|String|ToString(Text) (Variables|Default|GethoverTitle))) (Utilities|Text|ToText(String) (Utilities|String|ToString(Text) (Variables|Default|GetHoverNormalHint))))
        (UserInterface|Viewport|AddtoViewport _output_get 0)))
    (Utilities|Casting|CastToClientSide_Controller (Game|GetPlayerController 0))
    (bind (_x _y) (CallFunction|ClampWidgedPostoScreenMiddle (.x (Class|Widget|GetDesiredSize (Variables|Default|GethoverUserWidget))) (.y (Class|Widget|GetDesiredSize (Variables|Default|GethoverUserWidget)))))
    (Class|UserWidget|SetPositioninViewport (Variables|Default|GethoverUserWidget) (Math|Vector2D|MakeVector2D _x (+ _y -1e+01)) false)))

(event Custom|StopHover
  (bind _hoveruserwidget (Variables|Default|GethoverUserWidget))
  (Utilities|IsValid _hoveruserwidget
    (:Is%20Valid
      (Widget|RemovefromParent _hoveruserwidget))))

(fn ConstructionScript)