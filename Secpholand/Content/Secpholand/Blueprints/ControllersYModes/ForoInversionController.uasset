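; Player controller for the investment forum map, handling entry into three meeting rooms and a pitch room.
; Entering a room starts a group call with its HUD widget and chat, checks for an existing presentation, and notifies ForoInversionGameState through server events.
; Tagged camera actors cached at spawn give each meeting room default, left and right views with eased blends.
; Meeting room entry also resets the floating camera-switch actors' visibility and collision.
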(event Custom|GoToLeftView
  ;[1 1 1] Cam Views
  (Game|Player|SetViewTargetwithBlend (Utilities|Select :Index (- (Variables|Default|GetIDSala) 1) :Option%200 (Variables|Default|GetReunion1Left) :Option%201 (Variables|Default|GetReunion2Left) :Option%202 (Variables|Default|GetReunion3Left)) (Variables|Default|GetTiempoTransicion) "VTBlend_EaseInOut" (Variables|Default|GetExponenteTransicion) false))

(event Custom|ReturnToOriginalView
  ;[1 1 1] Cam Views
  (Game|Player|SetViewTargetwithBlend (Utilities|Select :Index (- (Variables|Default|GetIDSala) 1) :Option%200 (Variables|Default|GetReunion1Default) :Option%201 (Variables|Default|GetReunion2Default) :Option%202 (Variables|Default|GetReunion3Default)) (Variables|Default|GetTiempoTransicion) "VTBlend_EaseInOut" (Variables|Default|GetExponenteTransicion) false))

(event Custom|HasEnteredSalaPitches:Client
  ;[1 1 1] Handle Has Entered Sala Pitches
  (CallFunction|StartCallwithEveryone 20)
  (CallFunction|ComprobarSiExistePresentacion:Client)
  (CallFunction|HasEnteredSalaPitches:Server)
  (bind (_widget _found) (CallFunction|GetWidgetLlamada))
  (if _found
    (Default|AñadirChat _widget)))

(event Custom|GetCamerasReferences
  ;[1 1 1] Get Cameras References
  (bind _cameraactor (CallFunction|GetCameraActorwithTag "Sala de reuniones1"))
  (Variables|Default|SetReunion1Default _cameraactor)
  (bind _cameraactor_2 (CallFunction|GetCameraActorwithTag "Sala de reuniones1_left"))
  (Variables|Default|SetReunion1Left _cameraactor_2)
  (bind _cameraactor_3 (CallFunction|GetCameraActorwithTag "Sala de reuniones1_right"))
  (Variables|Default|SetReunion1Right _cameraactor_3)
  (bind _cameraactor_4 (CallFunction|GetCameraActorwithTag "Sala de reuniones2"))
  (Variables|Default|SetReunion2Default _cameraactor_4)
  (bind _cameraactor_5 (CallFunction|GetCameraActorwithTag "Sala de reuniones2_left"))
  (Variables|Default|SetReunion2Left _cameraactor_5)
  (bind _cameraactor_6 (CallFunction|GetCameraActorwithTag "Sala de reuniones2_right"))
  (Variables|Default|SetReunion2Right _cameraactor_6)
  (bind _cameraactor_7 (CallFunction|GetCameraActorwithTag "Sala de reuniones3"))
  (Variables|Default|SetReunion3Default _cameraactor_7)
  (bind _cameraactor_8 (CallFunction|GetCameraActorwithTag "Sala de reuniones3_left"))
  (Variables|Default|SetReunion3Left _cameraactor_8)
  (bind _cameraactor_9 (CallFunction|GetCameraActorwithTag "Sala de reuniones3_right"))
  (Variables|Default|SetReunion3Right _cameraactor_9))

(event Custom|HasEnteredSalaReunion:Client
  (params (IDSala :type Integer))
  ;[1 1 1] Has Entered Sala de Reunión
  (CallFunction|StartCallwithEveryone IDSala)
  (CallFunction|ComprobarSiExistePresentacion:Client)
  (CallFunction|HasEnteredSalaReunion:Server IDSala)
  (bind (_widget _found) (CallFunction|GetWidgetLlamada))
  (if _found
    (Default|AñadirChat _widget)
    (CallFunction|ResetWidgetCambiarCamara)))

(event Custom|GoToRightView
  ;[1 1 1] Cam Views
  (Game|Player|SetViewTargetwithBlend (Utilities|Select :Index (- (Variables|Default|GetIDSala) 1) :Option%200 (Variables|Default|GetReunion1Right) :Option%201 (Variables|Default|GetReunion2Right) :Option%202 (Variables|Default|GetReunion3Right)) (Variables|Default|GetTiempoTransicion) "VTBlend_EaseInOut" (Variables|Default|GetExponenteTransicion) false))

(event Custom|HasEnteredSalaReunion:Server
  (params (IdxSala :type Integer))
  ;[1 1 1] Has Entered Sala de Reunión
  (bind _asforo_inversion_game_state (Utilities|Casting|CastToForoInversionGameState (Game|GetGameState)))
  (Default|AvatarHasEnteredSala _asforo_inversion_game_state IdxSala self))

(event Custom|ResetWidgetCambiarCamara
  ;[1 1 1] Reset Widget Camara Flotante
  (bind _outactors (Actor|GetAllActorsOfClass "/Game/Secpholand/Blueprints/clasesBase/CambiarCamaraForoInversion.CambiarCamaraForoInversion_C"))
  (for _array_element _outactors
    (switch int (Variables|/Game/Secpholand/Blueprints/clasesBase/CambiarCamaraForoInversion.CambiarCamaraForoInversion_C|Getaction _array_element)
      (:0
        (Rendering|SetActorHiddenInGame _array_element false :!label _label)
        (Collision|SetActorEnableCollision _array_element true))
      (:1
        (goto _label))
      (:2
        (Rendering|SetActorHiddenInGame _array_element true)
        (Collision|SetActorEnableCollision _array_element false)))))

(event Custom|HasEnteredSalaPitches:Server
  ;[1 1 1] Handle Has Entered Sala Pitches
  (bind _asforo_inversion_game_state (Utilities|Casting|CastToForoInversionGameState (Game|GetGameState)))
  (Default|AvatarHasEnteredSala _asforo_inversion_game_state 0 self))

(event Custom|StartCallWithEveryone
  (params (TalkRoomID :type Integer))
  ;[1 1 1] Start Call & Create Widgets
  (Utilities|FlowControl|Sequence
    (:then_0
      (CallFunction|EntrarEnLlamada TalkRoomID)
      (bind _returnvalue (UserInterface|CreateWidget "/Game/Secpholand/UI/Widgets/Llamada.Llamada_C"))
      (bind _output_get (Variables|Default|SetLlamada _returnvalue))
      (Class|VerticalBox|AddChildtoVerticalBox (Variables|/Game/Secpholand/UI/Widgets/HUDYChat/HUD.HUD_C|GetHudArribaizquierda (Variables|Default|GetHUD)) _output_get)
      (CallFunction|ModifyWidgetLlamadaBasedonLocation))
    (:then_1
      (Utilities|FlowControl|Delay 3.0)
      (CallFunction|UpdateUsuariosLLamada))))

(event EventPlayerHasBeenSpawn:Client
  (|CallParentFunction)
  (Variables|Default|SetPlayerOriginalViewTarget (Pawn|GetViewTarget (Game|GetPlayerController 0)))
  (CallFunction|GetCamerasReferences))

(fn ConstructionScript
  (|CallParentFunction))

(fn GetCameraActorwithTag
  (params (Tag :type Name))
  (bind _outactors (Actor|GetAllActorsOfClasswithTag "/Script/Engine.CameraActor" Tag))
  (bind _ascamera_actor (Utilities|Casting|CastToCameraActor (Utilities|Array|Get(acopy) _outactors)))
  (return _ascamera_actor))