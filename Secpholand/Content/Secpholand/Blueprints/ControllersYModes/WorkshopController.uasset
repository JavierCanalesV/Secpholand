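; Player controller for the Secpholand workshop room, handling each participant's call, camera views and attendance.
; On client spawn it polls until the HUD is valid, then joins the group call, adds its widget and shows first-visit tutorial or controls help.
; Tagged CameraActors provide left and right views, blended to and from the original view target.
; Server spawn registers the avatar with WorkshopGameState; travel or disconnect requests its removal.
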(event Custom|GoToLeftView
  ;[1 1 1] Cam Views
  (Game|Player|SetViewTargetwithBlend (Variables|Default|GetCameraLeft) (Variables|Default|GetTiempoTransicion) "VTBlend_EaseInOut" (Variables|Default|GetExponenteTransicion) false)
  (Variables|Default|SetCurrentView 0))

(event Custom|ReturnToOriginalView
  ;[1 1 1] Cam Views
  (Game|Player|SetViewTargetwithBlend (Variables|Default|GetPlayerOriginalViewTarget) (Variables|Default|GetTiempoTransicion) "VTBlend_EaseInOut" (Variables|Default|GetExponenteTransicion) false)
  (Variables|Default|SetCurrentView 1))

(event Custom|HandlePlayerLeaving
  ;[1 1 1] Handle Player Leave or Disconnect
  (bind _asworkshop_game_state (Utilities|Casting|CastToWorkshopGameState (Game|GetGameState)))
  (Default|RemoveAvatar _asworkshop_game_state (Variables|/Game/Secpholand/Blueprints/ControllersYModes/baseClasses/ServerSide_Character.ServerSide_Character_C|GetUserInfo (Variables|Default|GetServerSideCharacterRef))))

(event Custom|GoToRightView
  ;[1 1 1] Cam Views
  (Game|Player|SetViewTargetwithBlend (Variables|Default|GetCameraRight) (Variables|Default|GetTiempoTransicion) "VTBlend_EaseInOut" (Variables|Default|GetExponenteTransicion) false)
  (Variables|Default|SetCurrentView 2))

(event Custom|GetCamerasReferences
  ;[1 1 1] Initialization
  (bind _cameraactor (CallFunction|GetCameraActorwithTag "StartCam"))
  (Variables|Default|SetCamaraPosInicial _cameraactor)
  (bind _cameraactor_2 (CallFunction|GetCameraActorwithTag "LeftLocation"))
  (Variables|Default|SetCameraLeft _cameraactor_2)
  (bind _cameraactor_3 (CallFunction|GetCameraActorwithTag "RightLocation"))
  (Variables|Default|SetCameraRight _cameraactor_3))

(event Custom|StartCallWithEveryone
  ;[1 1 1] Start Call & Create Widgets
  (Utilities|FlowControl|Sequence
    (:then_0
      (CallFunction|EntrarEnLlamada)
      (bind _returnvalue (UserInterface|CreateWidget "/Game/Secpholand/UI/Widgets/Llamada.Llamada_C"))
      (bind _output_get (Variables|Default|SetLlamada _returnvalue))
      (Class|VerticalBox|AddChildtoVerticalBox (Variables|/Game/Secpholand/UI/Widgets/HUDYChat/HUD.HUD_C|GetHudArribaizquierda (Variables|Default|GetHUD)) _output_get)
      (Default|AñadirPedirTurno _output_get)
      (CallFunction|ModifyWidgetLlamadaBasedonLocation))
    (:then_1
      (Utilities|FlowControl|Delay 3.0)
      (CallFunction|UpdateUsuariosLLamada))))

(event EventClient:travel
  (params (map :type ServerMaps%20Enum :default "NewEnumerator0") (newLocation :type InGameLocation%20Enum :default "NewEnumerator12"))
  ;[1 1 1] Handle Player Leave or Disconnect
  (|CallParentFunction map newLocation)
  (CallFunction|HandlePlayerLeaving))

(event EventAyudasPorMapas
  (bind _returnvalue (Game|GetPlayerController 0))
  (bind _serversidecharacterref (Variables|Default|GetServerSideCharacterRef))
  (bind _asclient_side_controller (Utilities|Casting|CastToClientSide_Controller _returnvalue))
  (bind _userinfo (Variables|/Game/Secpholand/Blueprints/ControllersYModes/baseClasses/ServerSide_Character.ServerSide_Character_C|GetUserInfo _serversidecharacterref))
  (bind _ingamelocation (Utilities|Struct|BreakUserInfo_Public _userinfo))
  (bind _userinfo_private (Variables|/Game/Secpholand/Blueprints/ControllersYModes/baseClasses/ClientSide_Controller.ClientSide_Controller_C|GetuserInfo_Private _asclient_side_controller))
  (bind (_level _tutorialsdoneflags) (Utilities|Struct|BreakUserInfo_Private _userinfo_private))
  (bind _returnvalue_2 (|locationToprimeraveztuto_2 _ingamelocation))
  (Utilities|IsValid (Variables|Default|GetLlamada)
    (:Is%20Valid
      (if (Utilities|Array|Get(acopy) _tutorialsdoneflags (Math|Conversions|ToInteger(Byte) _returnvalue_2))
        _
        (else
          (bind _returnvalue_3 (UserInterface|CreateWidget "/Game/Secpholand/UI/Widgets/Tutoriales/PrimeraVezEdificios/PrimeraVezEdificio.PrimeraVezEdificio_C" 0 _returnvalue_2 0))
          (UserInterface|Viewport|AddtoViewport _returnvalue_3 1)))
      (bind _servermapret (CallFunction|IngameLoctoServerMap _ingamelocation))
      (if (Math|Boolean|ANDBoolean (CallFunction|IsNavegableMap? _servermapret) (< _level 4) (not (Variables|/Game/Secpholand/Blueprints/ControllersYModes/baseClasses/NetworkGameInstance.NetworkGameInstance_C|GetControllsHelpClosed (.AsNetwork%20Game%20Instance (Utilities|Casting|CastToNetworkGameInstance (Game|GetGameInstance))))))
        (bind _returnvalue_4 (UserInterface|CreateWidget "/Game/Secpholand/UI/Widgets/Tutoriales/AyudaControles.AyudaControles_C"))
        (Widget|Panel|AddChild (Variables|/Game/Secpholand/UI/Widgets/HUDYChat/HUD.HUD_C|GetHudArribaizquierda (Variables|Default|GetHUD)) _returnvalue_4)))))

(event EventPlayerHasBeenSpawn:Client
  ;[1 1 1] Initialization
  (|CallParentFunction)
  (Utilities|IsValid (Variables|Default|GetHUD) :!label _label
    (:Is%20Valid
      (CallFunction|StartCallwithEveryone)
      (CallFunction|CompleteObjective 1)
      (Variables|Default|SetPlayerOriginalViewTarget (Pawn|GetViewTarget (Game|GetPlayerController 0)))
      (CallFunction|GetCamerasReferences)
      (CallFunction|ComprobarSiExistePresentacion:Client)
      (CallFunction|AyudasPorMapas))
    (:Is%20Not%20Valid
      (Utilities|FlowControl|Delay 0.2)
      (goto _label))))

(event EventDisconnect:Server
  (params (MapChange? :type Boolean) (securityToken :type String))
  ;[1 1 1] Handle Player Leave or Disconnect
  (CallFunction|HandlePlayerLeaving)
  (|CallParentFunction MapChange? securityToken))

(event EventSetLocationBypassed
  (Utilities|Struct|SetmembersinUserInfo_Public (Variables|/Game/Secpholand/Blueprints/ControllersYModes/baseClasses/ServerSide_Character.ServerSide_Character_C|GetUserInfo (Variables|Default|GetServerSideCharacterRef)) "NewEnumerator23"))

(event EventServerSpawnPlayer
  (params (playerStartIndex :type Player%20Start%20Object%20Reference) (UserInfo :type User%20Info%20Public%20Structure))
  ;[1 1 1] Initialization
  (|CallParentFunction playerStartIndex UserInfo)
  (bind _asworkshop_game_state (Utilities|Casting|CastToWorkshopGameState (Game|GetGameState)))
  (Default|AvatarHasEntered _asworkshop_game_state self))

(fn ConstructionScript
  (|CallParentFunction))

(fn GetCameraActorwithTag
  (params (Tag :type Name))
  (bind _outactors (Actor|GetAllActorsOfClasswithTag "/Script/Engine.CameraActor" Tag))
  (bind _asactor_de_la_cámara (Utilities|Casting|CastToCameraActor (Utilities|Array|Get(acopy) _outactors)))
  (return _asactor_de_la_cámara))