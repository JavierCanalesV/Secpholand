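; Player controller for the menu lobby, which fades in, shows the login widget and handles guest account creation and account recovery.
; Account requests pass through a server event to MenuLobbyGameState, and results return through client events to the open guest-login or recovery widget.
; After spawn it updates friend state and user location and, with automatic graphics quality on, spawns a PerformanceController.
; It overrides RetrievePersonalInfo with an empty event.
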(event Custom|EmailDeInvitadoYaEnUso:Client
  ;[1 1 1] Create invited Account
  (bind _foundwidgets (Widget|GetAllWidgetsOfClass "/Game/Secpholand/UI/Widgets/Loggin/LogginInputInvitado.LogginInputInvitado_C" true))
  (if (> (Utilities|Array|Length _foundwidgets) 0)
    (Default|EmailYaEnUso (Utilities|Array|Get(acopy) _foundwidgets))
    (else
      (bind _foundwidgets_2 (Widget|GetAllWidgetsOfClass "/Game/Secpholand/UI/Widgets/Loggin/RecoveryInputUser.RecoveryInputUser_C" true))
      (if (> (Utilities|Array|Length _foundwidgets_2) 0)
        (Default|UsuarioNoExiste (Utilities|Array|Get(acopy) _foundwidgets_2))))))

(event Custom|EmailDeInvitadoYaEnUso:Server
  ;[1 1 1] Create invited Account
  (CallFunction|EmailDeInvitadoYaEnUso:Client))

(event Custom|InvitedAccSentSuccesfully:Server
  (params (Succesfull :type Boolean))
  ;[1 1 1] Create invited Account
  (CallFunction|InvitedAccCreatedSuccewfullyClient Succesfull))

(event Custom|CreateInvited/RecoverAccountClient
  (params (Nombre :type String) (Empresa :type String) (Mail :type String) (RecuperarCuenta? :type Boolean))
  ;[1 1 1] Create invited Account
  (CallFunction|CreateInvited/RecoverAccountServer Nombre Empresa Mail RecuperarCuenta?))

(event Custom|CreateInvited/RecoverAccountServer
  (params (Nombre :type String) (Empreesa :type String) (Mail :type String) (RecuperarCuenta? :type Boolean))
  ;[1 1 1] Create invited Account
  (Default|CreateInvitedAccount/RecoverAccount (.AsMenu%20Lobby%20Game%20State (Utilities|Casting|CastToMenuLobbyGameState (Game|GetGameState))) Nombre Empreesa Mail self RecuperarCuenta?))

(event Custom|InvitedAccCreatedSuccewfullyClient
  (params (Succesfull :type Boolean))
  ;[1 1 1] Create invited Account
  (bind _foundwidgets (Widget|GetAllWidgetsOfClass "/Game/Secpholand/UI/Widgets/Loggin/LogginInputInvitado.LogginInputInvitado_C" true))
  (if (> (Utilities|Array|Length _foundwidgets) 0)
    (Default|CuentaCreada? (Utilities|Array|Get(acopy) _foundwidgets) Succesfull)
    (else
      (bind _foundwidgets_2 (Widget|GetAllWidgetsOfClass "/Game/Secpholand/UI/Widgets/Loggin/RecoveryInputUser.RecoveryInputUser_C" true))
      (if (> (Utilities|Array|Length _foundwidgets_2) 0)
        (Default|PeticiónAceptada (Utilities|Array|Get(acopy) _foundwidgets_2) Succesfull)))))

(event EventPlayerHasBeenSpawn:Client
  (CallFunction|Client:UpdateStatetoFriends "NewEnumerator0")
  (CallFunction|Server:UpdateUserLocation "NewEnumerator20" (Variables|/Game/Secpholand/Blueprints/ControllersYModes/baseClasses/NetworkGameInstance.NetworkGameInstance_C|GetsecurityToken (.AsNetwork%20Game%20Instance (Utilities|Casting|CastToNetworkGameInstance (Game|GetGameInstance)))))
  (if (.AutomaticGraphicQuality? (Utilities|Struct|BreakSettingValues (Variables|/Game/Secpholand/Blueprints/ControllersYModes/baseClasses/NetworkGameInstance.NetworkGameInstance_C|Getsettings (.AsNetwork%20Game%20Instance (Utilities|Casting|CastToNetworkGameInstance (Game|GetGameInstance))))))
    (Utilities|FlowControl|Delay 3.0)
    (Game|SpawnActorfromClass "/Game/Secpholand/Blueprints/OtherBP/PerformanceController.PerformanceController_C" (Math|Transform|MakeTransform "0, 0, 0") "Undefined" 0 0)))

(event EventClient:Init
  (bind _returnvalue (Game|GetPlayerCameraManager 0))
  (CallFunction|SetControllsConstraints false false false false)
  (CameraFades|StartCameraFade :self _returnvalue :FromAlpha 1.0 :ToAlpha 1.0 :Duration 1.0)
  (Utilities|FlowControl|Delay 1.0)
  (CameraFades|StartCameraFade :self _returnvalue :FromAlpha 1.0 :Duration 0.6)
  (Utilities|FlowControl|Delay 0.6)
  (Variables|Default|SetbShowMouseCursor true)
  (Input|SetInputModeGameandUI self 0 "DoNotLock" false)
  (bind _returnvalue_2 (UserInterface|CreateWidget "/Game/Secpholand/UI/Widgets/Loggin/Loggin.Loggin_C"))
  (bind _output_get (Variables|Default|SetlogginScreen _returnvalue_2))
  (UserInterface|Viewport|AddtoViewport _output_get 0)
  (CallFunction|ServerInitPlayer))

(event EventServer:RetrievePersonalInfo
  (params (username :type String) (securityToken :type String))
  ;[1 1 1] para que no lo haga
)

(event EventSetControllsConstraints
  (params (CanMove? :type Boolean) (CanRotate? :type Boolean) (CanZoom? :type Boolean) (CanClick? :type Boolean))
  (Variables|Default|SetcanClick? (and CanClick? (Variables|Default|GetcanChangeClick?))))

(fn ConstructionScript
  (|CallParentFunction))