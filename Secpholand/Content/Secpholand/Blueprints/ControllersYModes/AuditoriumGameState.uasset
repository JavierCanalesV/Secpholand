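; Auditorium game state that seats a set of users at a round table (mesa redonda) and later removes them.
; A server event stores the user names, resolves each to its AuditoriumController and sends it an enter or leave call, using the list index as seat ID.
; DoOnce gates toggle the round-table armchair actor's visibility once per pass, hiding it after a short delay on exit.
; Removal acts on the stored list, then clears it.
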(event Custom|MesaRedondaAuditorio:Server
  (params (usersToSit :type Array%20of%20Strings) (Add? :type Boolean))
  (if Add?
    (bind _output_get (Variables|Default|SetMesaRedondaUsers usersToSit))
    (for (_array_element _array_index) _output_get
      (bind (_found_ _user) (CallFunction|GetUser "NewEnumerator1" 0 _array_element))
      (if _found_
        (bind _asauditorium_controller (Utilities|Casting|CastToAuditoriumController (.PlayerController (Utilities|Struct|BreakUser _user))))
        (Default|ReceiveIrAMesaRedonda:Server _asauditorium_controller _array_index true)
        (Utilities|FlowControl|DoOnce false
          (:Completed
            (bind _outactors (Actor|GetAllActorsOfClass "/Game/Secpholand/Blueprints/OtherBP/SillonesMesaRedondaAudi.SillonesMesaRedondaAudi_C"))
            (Variables|/Game/Secpholand/Blueprints/OtherBP/SillonesMesaRedondaAudi.SillonesMesaRedondaAudi_C|SetVisible (Utilities|Array|Get(acopy) _outactors) true)))))
    (Utilities|FlowControl|DoOnce false) ; enters at Reset
    (else
      (for (_array_element_2 _array_index_2) (Variables|Default|GetMesaRedondaUsers)
        (bind (_found__2 _user_2) (CallFunction|GetUser "NewEnumerator1" 0 _array_element_2))
        (if _found__2
          (bind _asauditorium_controller_2 (Utilities|Casting|CastToAuditoriumController (.PlayerController (Utilities|Struct|BreakUser _user_2))))
          (Default|ReceiveIrAMesaRedonda:Server _asauditorium_controller_2 _array_index_2 false)
          (Utilities|FlowControl|DoOnce false
            (:Completed
              (Utilities|FlowControl|Delay 2.0)
              (bind _outactors_2 (Actor|GetAllActorsOfClass "/Game/Secpholand/Blueprints/OtherBP/SillonesMesaRedondaAudi.SillonesMesaRedondaAudi_C"))
              (Variables|/Game/Secpholand/Blueprints/OtherBP/SillonesMesaRedondaAudi.SillonesMesaRedondaAudi_C|SetVisible (Utilities|Array|Get(acopy) _outactors_2) false)))))
      (Utilities|Array|Clear (Variables|Default|GetMesaRedondaUsers))
      (Utilities|FlowControl|DoOnce false) ; enters at Reset
    )))

(fn ConstructionScript
  (|CallParentFunction))