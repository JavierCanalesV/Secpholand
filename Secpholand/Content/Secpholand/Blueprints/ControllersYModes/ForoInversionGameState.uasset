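; Game state for the investment forum (ForoInversion) that tracks avatar seats and their occupants across meeting rooms in ReunionesMapa.
; An init event gathers each room's ClicableAvatar actors by "AvatarSala" index tag and sizes matching state and user arrays.
; Helpers pick a random free seat or locate a user's room and seat by username.
; After a presenter is removed, users still in the standing-presenter room re-enter it through AvatarHasEnteredSala.
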(event EventBeginPlay
  (|CallParentFunction) ; This node is disabled and will not be called.\nDrag off pins to build functionality.
)

(event EventInitAvataresReuniones
  (bind _reunionesmapa (Variables|Default|GetReunionesMapa))
  (for (_ _array_index) _reunionesmapa
    (bind _outactors (Actor|GetAllActorsOfClasswithTag "/Game/Secpholand/Blueprints/Clicables/Avatares/ClicableAvatar.ClicableAvatar_C" (Utilities|String|StringToName (Utilities|String|Append "AvatarSala" (Utilities|String|ToString(Integer) _array_index)))))
    (for _array_element _outactors
      (bind _asclicable_avatar (Utilities|Casting|CastToClicableAvatar _array_element))
      (Utilities|Array|Add (.Avatars (Utilities|Struct|BreakReunionMapa (Utilities|Array|Get(acopy) _reunionesmapa _array_index))) _asclicable_avatar))
    (Utilities|Array|Resize (.AvatarStates (Utilities|Struct|BreakReunionMapa (Utilities|Array|Get(acopy) _reunionesmapa _array_index))) (Utilities|Array|Length _outactors))
    (Utilities|Array|Resize (.UserInfos (Utilities|Struct|BreakReunionMapa (Utilities|Array|Get(acopy) _reunionesmapa _array_index))) (Utilities|Array|Length _outactors))))

(event EventGestionarPostQuitarPresentador
  (params (UserName :type String))
  (bind _salapresentadordepie (Variables|Default|GetSalaPresentadorDePie))
  (bind _indexsala (CallFunction|FindAsientoandSalaIdxbyUsername UserName (Variables|Default|GetReunionesMapa)))
  (if (== _indexsala (Variables|Default|GetSalaPresentadorDePie))
    (bind (_found_ _user) (CallFunction|GetUser "NewEnumerator1" 0 UserName))
    (if _found_
      (bind _asinterior_controller (Utilities|Casting|CastToInteriorController (.PlayerController (Utilities|Struct|BreakUser _user))))
      (if (== (Variables|/Game/Secpholand/Blueprints/ControllersYModes/InteriorController.InteriorController_C|GetIDSala _asinterior_controller) _salapresentadordepie)
        (CallFunction|AvatarHasEnteredSala _salapresentadordepie (.AsForo%20Inversion%20Controller (Utilities|Casting|CastToForoInversionController (.PlayerController (Utilities|Struct|BreakUser _user)))))))))

(fn ConstructionScript
  (|CallParentFunction)
  (Networking|SwitchHasAuthority))

(fn CheckifAllSeatsAreFull
  (params (AvatarState :type Array%20of%20Booleans))
  (for _array_element AvatarState
    (if (not _array_element)
      (return false)))
  (return true))

(fn GetFirstIndexAvailable0
  (params (AvatarState :type Array%20of%20Booleans))
  (bind _allfull_ (CallFunction|CheckifAllSeatsAreFull AvatarState))
  (if _allfull_
    (return -1)
    (else
      (LocalVariables|SetMaxIdx (- (Utilities|Array|Length AvatarState) 1))
      (LocalVariables|SetCurrIndx (Math|Random|RandomIntegerinRange 0 (LocalVariables|GetMaxIdx)))
      (while (Utilities|Array|Get(acopy) AvatarState (LocalVariables|GetCurrIndx))
        (LocalVariables|SetCurrIndx (Math|Random|RandomIntegerinRange 0 (LocalVariables|GetMaxIdx))))
      (return (LocalVariables|GetCurrIndx)))))

(fn FindAsientoandSalaIndexbyUserInfo
  (params (UserInfo :type User%20Info%20Public%20Structure) (Reuniones :type Array%20of%20Reunion%20Mapa%20Structures))
  (for (_array_element _array_index) Reuniones
    (for (_array_element_2 _array_index_2) (.UserInfos (Utilities|Struct|BreakReunionMapa _array_element))
      (if (Utilities|Enum|Equal(Enum) (.Username (Utilities|Struct|BreakUserInfo_Public _array_element_2)) (.Username (Utilities|Struct|BreakUserInfo_Public UserInfo)))
        (return _array_index_2 _array_index))))
  (return -1 -1))