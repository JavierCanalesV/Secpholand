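; Lobby menu GameState that handles guest account creation and recovery for Secpholand.
; Requests go through NetworkGameMode as a byte-packed TCP message with a random string, while the requesting controller is queued by email.
; The reply handler finds that controller, reports an email already in use or emails credentials over TLS and reports the send result, then dequeues it.
; A flagged partner-company match also emails a registration report to a hard-coded address.
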(event Custom|ReturnCrearCuentaInvitado
  (params (Message :type Array%20of%20Bytes))
  ;[1 1 1] Crear cuenta de Invitado
  (bind _returnvalue (Class|TcpSocketConnection|MessageReadByte Message))
  (bind _returnvalue_2 (Class|TcpSocketConnection|MessageReadByte Message))
  (bind _returnvalue_3 (Class|TcpSocketConnection|MessageReadInt Message))
  (bind _returnvalue_4 (Class|TcpSocketConnection|MessageReadString Message _returnvalue_3))
  (bind _returnvalue_5 (Class|TcpSocketConnection|MessageReadInt Message))
  (bind _returnvalue_6 (Class|TcpSocketConnection|MessageReadString Message _returnvalue_5))
  (bind _returnvalue_7 (Class|TcpSocketConnection|MessageReadInt Message))
  (bind _returnvalue_8 (Class|TcpSocketConnection|MessageReadString Message _returnvalue_7))
  (bind _returnvalue_9 (Class|TcpSocketConnection|MessageReadInt Message))
  (bind _returnvalue_10 (Class|TcpSocketConnection|MessageReadString Message _returnvalue_9))
  (bind _returnvalue_11 (Class|TcpSocketConnection|MessageReadInt Message))
  (bind _returnvalue_12 (Class|TcpSocketConnection|MessageReadString Message _returnvalue_11))
  (bind (_found_ _user) (CallFunction|GetInvitedUser _returnvalue_4))
  (if _found_
    (if (Math|Conversions|ToBoolean(Integer) (Math|Conversions|ToInteger(Byte) _returnvalue))
      (Default|EmailDeInvitadoYaEnUso:Server (.AsMenu%20Lobby%20Controller (Utilities|Casting|CastToMenuLobbyController _user)))
      (else
        (bind _outresult (Class|EmailFL|SendEmailV2 (Class|EmailFL|MakeEmailDetailsfromAsset "Secpholand" "/Game/Secpholand/Blueprints/OtherBP/emailSecpho.emailSecpho" (select (Utilities|Enum|Equal(Enum) _returnvalue_8 "") _returnvalue_4 _returnvalue_8) 0 0 (select (Utilities|Enum|Equal(Enum) _returnvalue_8 "") "Cuenta Creada de Secpholand" "Recuperar credenciales de Secpholand") (select (Utilities|Enum|Equal(Enum) _returnvalue_8 "") (Utilities|String|Append "Bienvenido a Secpholand! Ya puedes acceder al entorno virtual con los siguientes credenciales 
 
Nombre de usuario: 
" _returnvalue_4 " 
Contraseña: 
" _returnvalue_6 " 
 
Una vez realices la primera entrada deberás asignar un nombre de usuario y contraseña escogidos por ti.  
 
Si tienes cualquier problema contacta con: 
SecpholandSupport@secpho.org") (Utilities|String|Append "Hemos recuperado tu cuenta Para acceder utiliza la siguiente contraseña que te hemos generado: 
" " 
Contraseña: 
" _returnvalue_6 " 
 
Una vez realices la primera entrada deberás asignar un nombre de usuario y contraseña escogidos por ti.  
Recuerda que puedes iniciar sesión tanto con tu nombre de usuario como tu email 
 
Si tienes cualquier problema contacta con: 
SecpholandSupport@secpho.org")) (Utilities|Array|MakeArray)) "UTF8" "TLS"))
        (Default|InvitedAccSentSuccesfully:Server (.AsMenu%20Lobby%20Controller (Utilities|Casting|CastToMenuLobbyController _user)) (Utilities|Enum|Equal(Enum) _outresult "Success"))))
    (CallFunction|RemoveInvitedUser _returnvalue_4)
    (if (Math|Conversions|ToBoolean(Integer) (Math|Conversions|ToInteger(Byte) _returnvalue_2))
      (Class|EmailFL|SendEmailV2 (Class|EmailFL|MakeEmailDetailsfromAsset "Secpholand" "/Game/Secpholand/Blueprints/OtherBP/emailSecpho.emailSecpho" "ischoent_d20l@fuluj.com" 0 0 "Registro de usuario en empresa socia del cluster" (Utilities|String|Append "Se ha detectado el registro de un usuario en el sistema,  en una empresa socia del cluster. 
----------------------------------------------- 
   Informe 
----------------------------------------------- 
Nombre de usuario: 
" _returnvalue_4 " 
Nombre: 
" _returnvalue_10 " 
Empresa: 
" _returnvalue_12) (Utilities|Array|MakeArray)) "UTF8" "TLS"))))

(event Custom|CreateInvitedAccount/RecoverAccount
  (params (Nombre :type String) (Empresa :type String) (Mail :type String) (controller :type Client%20Side%20Controller%20Object%20Reference) (RecuperarCuenta? :type Boolean))
  (bind _returnvalue (Class|TcpSocketConnection|ToBytes(String) Mail))
  (bind _returnvalue_2 (Class|TcpSocketConnection|ToBytes(String) Nombre))
  (bind _returnvalue_3 (Class|TcpSocketConnection|ToBytes(String) Empresa))
  (bind _randomstring1 (CallFunction|MakeRandomString 12))
  (bind _returnvalue_4 (Class|TcpSocketConnection|ToBytes(String) _randomstring1))
  ;[1 1 1] Crear cuenta de Invitado
  (Utilities|Array|Add (Variables|Default|GetCreatingInvited/RecoverUsers) (Utilities|Struct|MakeUser 0 Mail "" controller))
  (Default|SendMessage (.AsNetwork%20Game%20Mode (Utilities|Casting|CastToNetworkGameMode (Game|GetGameMode))) (Class|TcpSocketConnection|ConcatBytesBytes (Class|TcpSocketConnection|ToBytes(Byte) (Utilities|Enum|LiteralenumTCPProtocol "NewEnumerator73")) (Class|TcpSocketConnection|ToBytes(Integer) (Utilities|Array|Length _returnvalue_2)) _returnvalue_2 (Class|TcpSocketConnection|ToBytes(Integer) (Utilities|Array|Length _returnvalue_3)) _returnvalue_3 (Class|TcpSocketConnection|ToBytes(Integer) (Utilities|Array|Length _returnvalue)) _returnvalue (Class|TcpSocketConnection|ToBytes(Integer) (Utilities|Array|Length _returnvalue_4)) _returnvalue_4 (Class|TcpSocketConnection|ToBytes(Byte) (Math|Conversions|ToByte(Integer) RecuperarCuenta?)))))

(fn ConstructionScript
  (|CallParentFunction))

(fn GetInvitedUser
  (params (Mail :type String))
  (for _array_element (Variables|Default|GetCreatingInvited/RecoverUsers)
    (if (Utilities|Enum|Equal(Enum) Mail (.UserName (Utilities|Struct|BreakUser _array_element)))
      (return true (.PlayerController (Utilities|Struct|BreakUser _array_element)))))
  (return false 0))

(fn RemoveInvitedUser
  (params (Mail :type String))
  (for (_array_element _array_index) (Variables|Default|GetCreatingInvited/RecoverUsers)
    (if (Utilities|Enum|Equal(Enum) Mail (.UserName (Utilities|Struct|BreakUser _array_element)))
      (Utilities|Array|RemoveIndex (Variables|Default|GetCreatingInvited/RecoverUsers) _array_index)
      (return))))