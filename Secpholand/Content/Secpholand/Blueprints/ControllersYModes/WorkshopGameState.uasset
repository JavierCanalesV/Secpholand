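; Game state for the workshop that assigns entering players to tagged seat avatars and manages their nameplates.
; On authority, construction gathers the avatars and sizes parallel occupancy and username arrays; entry claims a random free seat by retrying random indices.
; Removal frees the seat by username, drops the user from the first call list and, after a delay, refreshes workshop controllers.
; Gaining the presenter role frees the seat; losing it reseats the user after a delay.
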(event Custom|InitAvatars
  (Utilities|Array|Clear (Variables|Default|GetAvatars))
  (bind _outactors (Actor|GetAllActorsOfClasswithTag "/Game/Secpholand/Blueprints/Clicables/Avatares/ClicableAvatar.ClicableAvatar_C" "AvatarsWorkshop"))
  (for _array_element _outactors
    (bind _asclicable_avatar (Utilities|Casting|CastToClicableAvatar _array_element))
    (Utilities|Array|Add (Variables|Default|GetAvatars) _asclicable_avatar))
  (Utilities|Array|Resize (Variables|Default|GetAvatarState) (Utilities|Array|Length _outactors))
  (Utilities|Array|Resize (Variables|Default|GetUsernames) (Utilities|Array|Length _outactors)))

(event Custom|UpdateNamePlateInWorkshop
  (params (AvatarSlotReference :type Clicable%20Avatar%20Object%20Reference%20%28by%20ref%29) (UserInfo :type User%20Info%20Public%20Structure) (Hide? :type Boolean))
  (bind _asclicable_avatar_workshop (Utilities|Casting|CastToClicableAvatar_Workshop AvatarSlotReference))
  (Default|UpdateNamePlate _asclicable_avatar_workshop Hide? UserInfo))

(event Custom|AvatarHasEntered
  (params (coontroller :type Interior%20Controller%20Object%20Reference))
  (bind _serversidecharacterref (Variables|/Game/Secpholand/Blueprints/ControllersYModes/baseClasses/ClientSide_Controller.ClientSide_Controller_C|GetServerSideCharacterRef coontroller))
  (bind _userinfo (Variables|/Game/Secpholand/Blueprints/ControllersYModes/baseClasses/ServerSide_Character.ServerSide_Character_C|GetUserInfo _serversidecharacterref))
  (bind _index (CallFunction|GetFirstIndexAvailable0))
  (if (!= _index -1)
    (Default|SetRepresentativeAvatar coontroller (Utilities|Array|Get(acopy) (Variables|Default|GetAvatars) _index) false)
    (CallFunction|UpdateNamePlateinWorkshop (Utilities|Array|Get(acopy) (Variables|Default|GetAvatars) _index) _userinfo false)
    (Utilities|Array|SetArrayElem (Variables|Default|GetAvatarState) _index true)
    (Utilities|Array|SetArrayElem (Variables|Default|GetUsernames) _index (.Username (Utilities|Struct|BreakUserInfo_Public _userinfo)))))

(event Custom|RemoveAvatar
  (params (UserInfo :type User%20Info%20Public%20Structure))
  (bind _usuarios_por_llamadas (Variables|Default|GetUsuarios%20por%20Llamadas))
  (bind _output (Utilities|Array|Get(acopy) _usuarios_por_llamadas))
  (bind _usuarioenllamada (Utilities|Struct|BreakUsuarioPorLlamada _output))
  (bind _index (CallFunction|FindIndexbyUserInfo UserInfo))
  (if (!= _index -1)
    (CallFunction|RemoveAvataratIndexW _index)
    (bind (_array_element _array_index) (Utilities|Array|ForEachLoopwithBreak _usuarioenllamada :!label _label)
      (:LoopBody
        (if (Utilities|Enum|Equal(Enum) (Utilities|Struct|BreakUsuarioEncontrado _array_element) (.Username (Utilities|Struct|BreakUserInfo_Public UserInfo)))
          (Utilities|Array|RemoveIndex _usuarioenllamada _array_index)
          (Utilities|FlowControl|Delay 0.8)
          (for _array_element_2 (Variables|Default|GetUserArray)
            (bind _asworkshop_controller (Utilities|Casting|CastToWorkshopController (Utilities|Struct|BreakUserInfocpp _array_element_2)))
            (Default|Server:UpdateUsuarioLLamada _asworkshop_controller))
          (goto _label Break))))))

(event Custom|RemoveAvatarAtIndexW
  (params (Index :type Integer))
  (CallFunction|UpdateNamePlateinWorkshop :AvatarSlotReference (Utilities|Array|Get(acopy) (Variables|Default|GetAvatars) Index) :Hide? true)
  (Utilities|Array|SetArrayElem (Variables|Default|GetAvatarState) Index false)
  (Utilities|Array|SetArrayElem (Variables|Default|GetUsernames) Index ""))

(event EventGestionarPostQuitarPresentador
  (params (UserName :type String))
  ;[1 1 1] Update Avatars when Presentador Changes
  (bind (_found_ _user) (CallFunction|GetUser "NewEnumerator1" 0 UserName))
  (if _found_
    (Utilities|FlowControl|Delay 2.5)
    (CallFunction|AvatarHasEntered (.AsWorkshop%20Controller (Utilities|Casting|CastToWorkshopController (.PlayerController (Utilities|Struct|BreakUser _user)))))))

(event EventEventPostDarRolPresentador
  (params (UserName :type String))
  ;[1 1 1] Update Avatars when Presentador Changes
  (bind (_found_ _user) (CallFunction|GetUser "NewEnumerator1" 0 UserName))
  (if _found_
    (bind _index (CallFunction|FindIndexbyUserInfo (Variables|/Game/Secpholand/Blueprints/ControllersYModes/baseClasses/ServerSide_Character.ServerSide_Character_C|GetUserInfo (Variables|/Game/Secpholand/Blueprints/ControllersYModes/baseClasses/ClientSide_Controller.ClientSide_Controller_C|GetServerSideCharacterRef (.PlayerController (Utilities|Struct|BreakUser _user))))))
    (if (!= _index -1)
      (CallFunction|RemoveAvataratIndexW _index))))

(fn ConstructionScript
  (|CallParentFunction)
  (Networking|SwitchHasAuthority
    (:Authority
      (CallFunction|InitAvatars))))

(fn GetFirstIndexAvailable0
  (bind _allfull_ (CallFunction|CheckifAllSeatsAreFull))
  (if _allfull_
    (return -1)
    (else
      (LocalVariables|SetMaxIdx (- (Utilities|Array|Length (Variables|Default|GetAvatarState)) 1))
      (LocalVariables|SetCurrIndx (Math|Random|RandomIntegerinRange 0 (LocalVariables|GetMaxIdx)))
      (while (Utilities|Array|Get(acopy) (Variables|Default|GetAvatarState) (LocalVariables|GetCurrIndx))
        (LocalVariables|SetCurrIndx (Math|Random|RandomIntegerinRange 0 (LocalVariables|GetMaxIdx))))
      (return (LocalVariables|GetCurrIndx)))))

(fn FindIndexbyUserInfo
  (params (UserInfo :type User%20Info%20Public%20Structure))
  (for (_array_element _array_index) (Variables|Default|GetUsernames)
    (if (Utilities|Enum|Equal(Enum) _array_element (.Username (Utilities|Struct|BreakUserInfo_Public UserInfo)))
      (return _array_index)))
  (return -1))

(fn CheckifAllSeatsAreFull
  (for _array_element (Variables|Default|GetAvatarState)
    (if (not _array_element)
      (return false)))
  (return true))