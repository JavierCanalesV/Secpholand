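; B2B player controller that runs client-side setup once the player has spawned.
; It polls until the pawn reference is valid, then adds the HUD, attaches a player-collision actor, removes the loading screen, starts voice capture and enables controls.
; It also points map-change elevator actors at the GameInstance's post-tutorial map and syncs settings from the GameInstance, spawning a PerformanceController when automatic graphics quality is on.
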(event Custom|SetAscensoresMapa
  (bind _outactors (Actor|GetAllActorsOfClass "/Game/Secpholand/Blueprints/Clicables/cambiosDeMapa/EdificioGotoCambioMapa.EdificioGotoCambioMapa_C"))
  (for _array_element _outactors
    (Variables|/Game/Secpholand/Blueprints/Clicables/cambiosDeMapa/EdificioGotoCambioMapa.EdificioGotoCambioMapa_C|SetMapa _array_element (Variables|/Game/Secpholand/Blueprints/ControllersYModes/baseClasses/NetworkGameInstance.NetworkGameInstance_C|GetmapaDespuesDeTutorial (.AsNetwork%20Game%20Instance (Utilities|Casting|CastToNetworkGameInstance (Game|GetGameInstance)))))))

(event EventPlayerHasBeenSpawn:Client
  (bind _returnvalue (Game|GetGameInstance))
  (bind _asnetwork_game_instance (Utilities|Casting|CastToNetworkGameInstance _returnvalue))
  (Utilities|FlowControl|Delay 1.0)
  (bind _foundwidgets (Widget|GetAllWidgetsOfClass "/Game/Secpholand/UI/Widgets/LoadingScreen.LoadingScreen_C" true))
  (Progress|SetPercent (Variables|/Game/Secpholand/UI/Widgets/LoadingScreen.LoadingScreen_C|GetProgressBar_111 (Utilities|Array|Get(acopy) _foundwidgets)) 1.0)
  (Utilities|IsValid (Variables|Default|GetClientSidePawnRef) :!label _label
    (:Is%20Valid
      (bind _returnvalue_2 (UserInterface|CreateWidget "/Game/Secpholand/UI/Widgets/HUDYChat/HUD.HUD_C" self))
      (bind _output_get (Variables|Default|SetHUD _returnvalue_2))
      (UserInterface|Viewport|AddtoViewport _output_get 1)
      (bind _returnvalue_3 (Game|SpawnActorfromClass "/Game/Secpholand/Blueprints/ControllersYModes/CollisionWithOtherPlayers.CollisionWithOtherPlayers_C" (Math|Transform|MakeTransform "0, 0, 0") "Undefined" self 0))
      (Transformation|AttachActorToActor _returnvalue_3 (Variables|Default|GetClientSidePawnRef) "None" "SnapToTarget" "SnapToTarget" "SnapToTarget" true)
      (Variables|Default|SetcolisionWithPlayers _returnvalue_3)
      (CallFunction|SetAscensoresMapa)
      (CallFunction|AyudasPorMapas)
      (bind _foundwidgets_2 (Widget|GetAllWidgetsOfClass "/Game/Secpholand/UI/Widgets/LoadingScreen.LoadingScreen_C" true))
      (Widget|RemovefromParent (Utilities|Array|Get(acopy) _foundwidgets_2))
      (CallFunction|InitVoiceCapture)
      (CallFunction|SetControllsConstraints true true true true)
      (if (Math|Boolean|ANDBoolean (== (.sfxvolume (Variables|Default|Getsettings)) (.sfxvolume (Variables|/Game/Secpholand/Blueprints/ControllersYModes/baseClasses/NetworkGameInstance.NetworkGameInstance_C|Getsettings _asnetwork_game_instance))) (== (.musicvolume (Variables|Default|Getsettings)) (.musicvolume (Variables|/Game/Secpholand/Blueprints/ControllersYModes/baseClasses/NetworkGameInstance.NetworkGameInstance_C|Getsettings _asnetwork_game_instance))) (== (.othersvoicevolume (Variables|Default|Getsettings)) (.othersvoicevolume (Variables|/Game/Secpholand/Blueprints/ControllersYModes/baseClasses/NetworkGameInstance.NetworkGameInstance_C|Getsettings _asnetwork_game_instance))) (== (.mastervolume (Variables|Default|Getsettings)) (.mastervolume (Variables|/Game/Secpholand/Blueprints/ControllersYModes/baseClasses/NetworkGameInstance.NetworkGameInstance_C|Getsettings _asnetwork_game_instance))) (== (.graphicquality (Variables|Default|Getsettings)) 0) (Math|Boolean|Equal(Boolean) (.automaticgraphicquality? (Variables|Default|Getsettings)) (.automaticgraphicquality? (Variables|/Game/Secpholand/Blueprints/ControllersYModes/baseClasses/NetworkGameInstance.NetworkGameInstance_C|Getsettings _asnetwork_game_instance))))
        _
        (else
          (Variables|Default|Setsettings (Variables|/Game/Secpholand/Blueprints/ControllersYModes/baseClasses/NetworkGameInstance.NetworkGameInstance_C|Getsettings _asnetwork_game_instance))))
      (if (.AutomaticGraphicQuality? (Utilities|Struct|BreakSettingValues (Variables|Default|Getsettings)))
        (Utilities|FlowControl|Delay 3.0)
        (Game|SpawnActorfromClass "/Game/Secpholand/Blueprints/OtherBP/PerformanceController.PerformanceController_C" (Math|Transform|MakeTransform "0, 0, 0") "Undefined" 0 0)))
    (:Is%20Not%20Valid
      (Utilities|FlowControl|Delay 0.2)
      (goto _label))))

(fn ConstructionScript
  (|CallParentFunction))