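; Meeting Center game state managing challenges (retos), meeting-room seating, private-meeting attendees, event access and project lists.
; It sends byte-packed TCP requests through NetworkGameMode, parses replies into arrays, controllers or hall counters, and returns leftover bytes to PendingMessages.
; Tagged avatar actors become room seats, assigned by random free-slot search and released by username.
; The room-full check always returns false, so that search cannot terminate normally when every seat is taken.
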(event Custom|RetrieveRetoInfo
  (params (RetoID :type Integer))
  ;[1 1 1] Reto Info
  (Default|SendMessage (.AsNetwork%20Game%20Mode (Utilities|Casting|CastToNetworkGameMode (Game|GetGameMode))) (Class|TcpSocketConnection|ConcatBytesBytes (Class|TcpSocketConnection|ToBytes(Byte) (Utilities|Enum|LiteralenumTCPProtocol "NewEnumerator26")) (Class|TcpSocketConnection|ToBytes(Integer) RetoID))))

(event Custom|ReceiveRetoInfo
  (params (bytes :type Array%20of%20Bytes))
  (bind _retoinfos (Variables|Default|GetRetoInfos))
  ;[1 1 1] Reto Info
  (bind (_reto _pendingbytes) (CallFunction|MakeRetoInfo bytes))
  (bind (_found _index) (CallFunction|GetRetoInfo (.SalaDeRetoID (Utilities|Struct|BreakRetoInfo _reto))))
  (if _found
    (Utilities|Array|SetArrayElem _retoinfos _index _reto)
    (else
      (Utilities|Array|Add _retoinfos _reto)))
  (bind _asnetwork_game_mode (Utilities|Casting|CastToNetworkGameMode (Game|GetGameMode)))
  (Default|PendingMessages _asnetwork_game_mode _pendingbytes))

(event Custom|SuperUser:RemoveUsuarioReunion
  (params (NumReunion :type Integer) (UsernameToRemove :type String%20%28by%20ref%29) (Token :type String) (PlayerController :type Client%20Side%20Controller%20Object%20Reference))
  (bind _usernamesenreuniones (Variables|Default|GetUsernamesEnReuniones))
  (bind _output (Utilities|Array|Get(acopy) _usernamesenreuniones NumReunion))
  (bind (_nombrereunion _asistentesusernames) (Utilities|Struct|BreakreunionMC _output))
  ;[1 1 1] SuperUser:SalasReunion
  (bind _returnvalue (Utilities|Array|RemoveItem _asistentesusernames UsernameToRemove))
  (if _returnvalue
    (CallFunction|AñadirRemoverNovedadPersonal NumReunion PlayerController Token UsernameToRemove _nombrereunion false "Reunion" 255)))

(event Custom|ReceiveAccessToEvent:Server
  (params (Data :type Array%20of%20Bytes))
  ;[1 1 1] Solicitar Acceder al Evento
  (bind _returnvalue (Class|TcpSocketConnection|MessageReadInt Data))
  (bind _returnvalue_2 (Class|TcpSocketConnection|MessageReadString Data _returnvalue)) ; Username
  (bind (_found_ _user) (CallFunction|GetUser "NewEnumerator1" 0 _returnvalue_2))
  (bind _returnvalue_3 (Class|TcpSocketConnection|MessageReadInt Data))
  (bind _returnvalue_4 (Class|TcpSocketConnection|MessageReadString Data _returnvalue_3)) ; Event Name
  (bind _returnvalue_5 (Class|TcpSocketConnection|MessageReadByte Data)) ; Event Found?
  (bind _returnvalue_6 (Class|TcpSocketConnection|MessageReadByte Data)) ; Is In List?
  (bind _returnvalue_7 (Class|TcpSocketConnection|MessageReadByte Data)) ; Starts in More than 1hr?
  (bind _returnvalue_8 (Class|TcpSocketConnection|MessageReadByte Data)) ; Location
  (if _found_
    (Default|ReceiveAccesstoEvent:Server (.AsInterior%20Controller (Utilities|Casting|CastToInteriorController (.playercontroller _user))) (Math|Conversions|ToBoolean(Integer) (Math|Conversions|ToInteger(Byte) _returnvalue_5)) (Math|Conversions|ToBoolean(Integer) (Math|Conversions|ToInteger(Byte) _returnvalue_6)) _returnvalue_4 (Utilities|Enum|ByteToEnumServerMaps _returnvalue_8) (Math|Conversions|ToBoolean(Integer) (Math|Conversions|ToInteger(Byte) _returnvalue_7))))
  (Default|PendingMessages (.AsNetwork%20Game%20Mode (Utilities|Casting|CastToNetworkGameMode (Game|GetGameMode))) Data))

(event Custom|SuperUsuario:ResetSalaReunión
  (params (SalaReunion :type Integer))
  ;[1 1 1] SuperUser:SalasReunion
  (Utilities|Struct|SetmembersinreunionMC (Utilities|Array|Get(acopy) (Variables|Default|GetUsernamesEnReuniones) SalaReunion) "" (Utilities|Array|MakeArray)))

(event Custom|SuperUser:AddUsuarioToReunión
  (params (NumReunion :type Integer) (UsernameToAdd :type String%20%28by%20ref%29) (NombreReunion :type String) (PlayerController :type Client%20Side%20Controller%20Object%20Reference) (Token :type String))
  (bind _usernamesenreuniones (Variables|Default|GetUsernamesEnReuniones))
  (bind _output (Utilities|Array|Get(acopy) _usernamesenreuniones NumReunion))
  ;[1 1 1] SuperUser:SalasReunion
  (if (Utilities|Enum|Equal(Enum) NombreReunion "")
    _
    (else
      (Utilities|Struct|SetmembersinreunionMC _output NombreReunion)))
  (Utilities|Array|Add (.AsistentesUsernames (Utilities|Struct|BreakreunionMC _output)) UsernameToAdd)
  (CallFunction|AñadirRemoverNovedadPersonal NumReunion PlayerController Token UsernameToAdd NombreReunion true "Reunión privada" 255))

(event Custom|SetRepresentativeAvatar
  (params (UserName :type String) (Repr.Avatar :type Clicable%20Avatar%20Object%20Reference%20%28by%20ref%29) (StandUp? :type Boolean))
  ;[1 1 1] Set Representative Avatar
  (bind (_found_ _user) (CallFunction|GetUser "NewEnumerator1" 0 UserName))
  (if _found_
    (bind _asinterior_controller (Utilities|Casting|CastToInteriorController (.PlayerController (Utilities|Struct|BreakUser _user))))
    (Default|SetRepresentativeAvatar _asinterior_controller Repr.Avatar StandUp?)))

(event Custom|RemoveAvatarFromSala
  (params (UserName :type String))
  (bind _usuarios_por_llamadas (Variables|Default|GetUsuarios%20por%20Llamadas))
  (bind _output (Utilities|Array|Get(acopy) _usuarios_por_llamadas))
  (bind _usuarioenllamada (Utilities|Struct|BreakUsuarioPorLlamada _output))
  ;[1 1 1] Enter / Exit Sala Reuniones Update Avatars
  (bind (_indexasiento _indexsala) (CallFunction|FindAsientoandSalaIdxbyUsername UserName (Variables|Default|GetReunionesMapa)))
  (if (!= _indexasiento -1)
    (CallFunction|RemoveAvataratIndex _indexasiento _indexsala)
    (bind (_array_element _array_index) (Utilities|Array|ForEachLoopwithBreak _usuarioenllamada :!label _label)
      (:LoopBody
        (if (Utilities|Enum|Equal(Enum) (Utilities|Struct|BreakUsuarioEncontrado _array_element) UserName)
          (Utilities|Array|RemoveIndex _usuarioenllamada _array_index)
          (Utilities|FlowControl|Delay 0.8)
          (for _array_element_2 (Variables|Default|GetUserArray)
            (bind _asclient_side_controller (Utilities|Casting|CastToClientSide_Controller (Utilities|Struct|BreakUserInfocpp _array_element_2)))
            (Default|Server:UpdateUsuarioLLamada _asclient_side_controller))
          (goto _label Break))))))

(event Custom|AvatarHasEnteredSala
  (params (SalaIdx :type Integer) (controllerInt :type Interior%20Controller%20Object%20Reference))
  (bind _reunionesmapa (Variables|Default|GetReunionesMapa))
  (bind _output (Utilities|Array|Get(acopy) _reunionesmapa SalaIdx))
  (bind (_avatarstates _avatars _userinfos) (Utilities|Struct|BreakReunionMapa _output))
  ;[1 1 1] Enter / Exit Sala Reuniones Update Avatars
  (bind _index (CallFunction|GetFirstIndexAvailable _avatarstates))
  (if (!= _index -1)
    (Default|SetRepresentativeAvatar controllerInt (Utilities|Array|Get(acopy) _avatars _index) false)
    (Utilities|Array|SetArrayElem _avatarstates _index true)
    (Utilities|Array|SetArrayElem _userinfos _index (Variables|/Game/Secpholand/Blueprints/ControllersYModes/baseClasses/ServerSide_Character.ServerSide_Character_C|GetUserInfo (Variables|/Game/Secpholand/Blueprints/ControllersYModes/baseClasses/ClientSide_Controller.ClientSide_Controller_C|GetServerSideCharacterRef controllerInt)))))

(event Custom|VerReto
  (params (RetoID :type Integer) (User :type Client%20Side%20Controller%20Object%20Reference) (token :type String))
  (bind _returnvalue (Class|TcpSocketConnection|ToBytes(String) token))
  ;[1 1 1] Ver Reto / Enviar Propuesta
  (bind (_found_ _user) (CallFunction|GetUser "NewEnumerator2" 0 "" "" User))
  (if _found_
    (bind _asnetwork_game_mode (Utilities|Casting|CastToNetworkGameMode (Game|GetGameMode)))
    (Default|SendMessage _asnetwork_game_mode (Class|TcpSocketConnection|ConcatBytesBytes (Class|TcpSocketConnection|ToBytes(Byte) (Utilities|Enum|LiteralenumTCPProtocol "NewEnumerator29")) (Class|TcpSocketConnection|ToBytes(Integer) (Utilities|Array|Length (Class|TcpSocketConnection|ToBytes(String) (.username _user)))) (Class|TcpSocketConnection|ToBytes(String) (.username _user)) (Class|TcpSocketConnection|ToBytes(Integer) RetoID) (Class|TcpSocketConnection|ToBytes(Integer) (Utilities|Array|Length _returnvalue)) _returnvalue))))

(event Custom|ADD_REMOVE_Proyecto_MC_SuperUser:Server
  (params (Titulo :type Name) (Empresa :type Name) (Url%20Proyecto :type String) (Participantes :type Array%20of%20Strings) (Token :type String) (PlayerController :type Client%20Side%20Controller%20Object%20Reference) (add :type Boolean))
  (bind _returnvalue (Class|TcpSocketConnection|ToBytes(String) Url%20Proyecto))
  (bind _returnvalue_2 (Class|TcpSocketConnection|ToBytes(String) Token))
  (bind _returnvalue_3 (Utilities|String|ToString(Name) Titulo))
  (bind _returnvalue_4 (Utilities|String|ToString(Name) Empresa))
  (bind _returnvalue_5 (Class|TcpSocketConnection|ToBytes(String) _returnvalue_3))
  (bind _returnvalue_6 (Class|TcpSocketConnection|ToBytes(String) _returnvalue_4))
  ;[1 1 1] Projects List
  (bind (_found_ _user) (CallFunction|GetUser "NewEnumerator2" 0 "" "" PlayerController))
  (if _found_
    (bind _asnetwork_game_mode (Utilities|Casting|CastToNetworkGameMode (Game|GetGameMode)))
    (bind _bytes (CallFunction|StringListtoBytesList Participantes))
    (Default|SendMessage _asnetwork_game_mode (Class|TcpSocketConnection|ConcatBytesBytes (Class|TcpSocketConnection|ToBytes(Byte) (Utilities|Enum|LiteralenumTCPProtocol "NewEnumerator83")) (Class|TcpSocketConnection|ToBytes(Integer) (Utilities|Array|Length (Class|TcpSocketConnection|ToBytes(String) (.username _user)))) (Class|TcpSocketConnection|ToBytes(String) (.username _user)) (Class|TcpSocketConnection|ToBytes(Integer) (Utilities|Array|Length _returnvalue_2)) _returnvalue_2 (Class|TcpSocketConnection|ToBytes(Integer) (Utilities|Array|Length _returnvalue_5)) _returnvalue_5 (Class|TcpSocketConnection|ToBytes(Integer) (Utilities|Array|Length _returnvalue_6)) _returnvalue_6 (Class|TcpSocketConnection|ToBytes(Integer) (Utilities|Array|Length _returnvalue)) _returnvalue _bytes (Class|TcpSocketConnection|ToBytes(Byte) (Math|Conversions|ToByte(Integer) add))))))

(event Custom|RetrieveAvatarsToSit
  (params (ID :type Integer))
  ;[1 1 1] Avatars To Sit
  (bind _asnetwork_game_mode (Utilities|Casting|CastToNetworkGameMode (Game|GetGameMode)))
  (Default|SendMessage _asnetwork_game_mode (Class|TcpSocketConnection|ConcatBytesBytes (Class|TcpSocketConnection|ToBytes(Byte) (Utilities|Enum|LiteralenumTCPProtocol "NewEnumerator28")) (Class|TcpSocketConnection|ToBytes(Integer) ID))))

(event Custom|Aceptar/cancelarPropuestaReto
  (params (user :type Client%20Side%20Controller%20Object%20Reference) (token :type String) (usernameAActualizar :type String) (retoID :type Integer) (aceptar :type Boolean))
  (bind _returnvalue (Class|NetShieldBPLibrary|StringtoBytes usernameAActualizar))
  (bind (_found_ _user) (CallFunction|GetUser "NewEnumerator2" 0 "" "" user))
  (if _found_
    (bind _asnetwork_game_mode (Utilities|Casting|CastToNetworkGameMode (Game|GetGameMode)))
    (Default|SendMessage _asnetwork_game_mode (Class|TcpSocketConnection|ConcatBytesBytes (Class|TcpSocketConnection|ToBytes(Byte) (Utilities|Enum|LiteralenumTCPProtocol "NewEnumerator88")) (Class|TcpSocketConnection|ToBytes(Integer) (Utilities|Array|Length (Class|NetShieldBPLibrary|StringtoBytes (.UserName (Utilities|Struct|BreakUser _user))))) (Class|NetShieldBPLibrary|StringtoBytes (.UserName (Utilities|Struct|BreakUser _user))) (Class|TcpSocketConnection|ToBytes(Integer) (Utilities|Array|Length (Class|NetShieldBPLibrary|StringtoBytes token))) (Class|TcpSocketConnection|ToBytes(Integer) (Utilities|Array|Length _returnvalue)) _returnvalue (Class|TcpSocketConnection|ToBytes(Integer) retoID) (Class|TcpSocketConnection|ToBytes(Byte) (Math|Conversions|ToByte(Integer) aceptar))))))

(event Custom|InitAvataresReuniones
  (bind _reunionesmapa (Variables|Default|GetReunionesMapa))
  ;[1 1 1] Init Avatares Reuniones
  (for (_ _array_index) _reunionesmapa
    (bind _outactors (Actor|GetAllActorsOfClasswithTag "/Game/Secpholand/Blueprints/Clicables/Avatares/ClicableAvatar.ClicableAvatar_C" (Utilities|String|StringToName (Utilities|String|Append "AvatarSala" (Utilities|String|ToString(Integer) (+ _array_index 1))))))
    (for _array_element _outactors
      (bind _asclicable_avatar (Utilities|Casting|CastToClicableAvatar _array_element))
      (Utilities|Array|Add (.Avatars (Utilities|Struct|BreakReunionMapa (Utilities|Array|Get(acopy) _reunionesmapa _array_index))) _asclicable_avatar))
    (Utilities|Array|Resize (.AvatarStates (Utilities|Struct|BreakReunionMapa (Utilities|Array|Get(acopy) _reunionesmapa _array_index))) (Utilities|Array|Length _outactors))
    (Utilities|Array|Resize (.UserInfos (Utilities|Struct|BreakReunionMapa (Utilities|Array|Get(acopy) _reunionesmapa _array_index))) (Utilities|Array|Length _outactors))))

(event Custom|ReceiveAvatarsToSit
  (params (bytes :type Array%20of%20Bytes))
  (bind _retoavatars (Variables|Default|GetRetoAvatars))
  ;[1 1 1] Avatars To Sit
  (bind (_retoavatars_2 _pendingbytes) (CallFunction|MakeAvatarstoSit bytes))
  (bind (_found _index) (CallFunction|GetRetoAvatars))
  (if _found
    (Utilities|Array|SetArrayElem _retoavatars _index _retoavatars_2)
    (else
      (Utilities|Array|Add _retoavatars _retoavatars_2)))
  (bind _asnetwork_game_mode (Utilities|Casting|CastToNetworkGameMode (Game|GetGameMode)))
  (Default|PendingMessages _asnetwork_game_mode _pendingbytes))

(event Custom|ToggleB2BAccess
  ;[1 1 1] toggle B2B Access
  (Variables|Default|SetAccesoSalaMultiusos (not (Variables|Default|GetAccesoSalaMultiusos))))

(event Custom|EnviarPropuesta
  (params (RetoID :type Integer) (User :type Client%20Side%20Controller%20Object%20Reference) (token :type String))
  (bind _returnvalue (Class|TcpSocketConnection|ToBytes(String) token))
  ;[1 1 1] Ver Reto / Enviar Propuesta
  (bind (_found_ _user) (CallFunction|GetUser "NewEnumerator2" 0 "" "" User))
  (if _found_
    (bind _asnetwork_game_mode (Utilities|Casting|CastToNetworkGameMode (Game|GetGameMode)))
    (Default|SendMessage _asnetwork_game_mode (Class|TcpSocketConnection|ConcatBytesBytes (Class|TcpSocketConnection|ToBytes(Byte) (Utilities|Enum|LiteralenumTCPProtocol "NewEnumerator30")) (Class|TcpSocketConnection|ToBytes(Integer) (Utilities|Array|Length (Class|TcpSocketConnection|ToBytes(String) (.username _user)))) (Class|TcpSocketConnection|ToBytes(String) (.username _user)) (Class|TcpSocketConnection|ToBytes(Integer) RetoID) (Class|TcpSocketConnection|ToBytes(Integer) (Utilities|Array|Length _returnvalue)) _returnvalue))))

(event Custom|RetrieveAllRetos
  ;[1 1 1] Init Reto Infos
  (bind _asnetwork_game_mode (Utilities|Casting|CastToNetworkGameMode (Game|GetGameMode)))
  (Default|SendMessage _asnetwork_game_mode (Class|TcpSocketConnection|ToBytes(Byte) (Utilities|Enum|LiteralenumTCPProtocol "NewEnumerator31"))))

(event Custom|ReceiveAllRetos
  (params (bytes :type Array%20of%20Bytes))
  ;[1 1 1] Init Reto Infos
  (bind _pendingbytes (CallFunction|FillAllRetos bytes))
  (bind _asnetwork_game_mode (Utilities|Casting|CastToNetworkGameMode (Game|GetGameMode)))
  (Default|PendingMessages _asnetwork_game_mode _pendingbytes))

(event Custom|RetrieveProjectsXenterpriseList:Server
  ;[1 1 1] Projects List
  (bind _asnetwork_game_mode (Utilities|Casting|CastToNetworkGameMode (Game|GetGameMode)))
  (Default|SendMessage _asnetwork_game_mode (Class|TcpSocketConnection|ToBytes(Byte) (Utilities|Enum|LiteralenumTCPProtocol "NewEnumerator41"))))

(event Custom|ReceiveProjectsXenterprise
  (params (Array :type Array%20of%20Bytes))
  ;[1 1 1] Projects List
  (bind (_list _arrayrs) (CallFunction|MakeProjectsList Array))
  (bind _outactors (Actor|GetAllActorsOfClass "/Game/Secpholand/Blueprints/Clicables/Mostrador_Hall.Mostrador_Hall_C"))
  (for _array_element _outactors
    (Variables|/Game/Secpholand/Blueprints/Clicables/Mostrador_Hall.Mostrador_Hall_C|SetList%20Proyectos _array_element _list))
  (Default|PendingMessages (.AsNetwork%20Game%20Mode (Utilities|Casting|CastToNetworkGameMode (Game|GetGameMode))) _arrayrs))

(event Custom|RequestAccessToEvent:Server
  (params (Event%20Name :type String) (Username :type String) (Token :type String) (Location :type ServerMaps%20Enum :default "NewEnumerator0"))
  (bind _returnvalue (Class|TcpSocketConnection|ToBytes(String) Event%20Name))
  (bind _returnvalue_2 (Class|TcpSocketConnection|ToBytes(String) Token))
  ;[1 1 1] Solicitar Acceder al Evento
  (bind (_found_ _user) (CallFunction|GetUser "NewEnumerator1" 0 Username))
  (if _found_
    (if (and (Variables|Default|GetUsingBypasses) (not (Variables|Default|GetUsingByPassesDani)))
      (Utilities|FlowControl|Delay 0.3)
      (Default|ReceiveAccesstoEvent:Server (.AsInterior%20Controller (Utilities|Casting|CastToInteriorController (.playercontroller _user))) true true Event%20Name Location false)
      (else
        (Default|SendMessage (.AsNetwork%20Game%20Mode (Utilities|Casting|CastToNetworkGameMode (Game|GetGameMode))) (Class|TcpSocketConnection|ConcatBytesBytes (Class|TcpSocketConnection|ToBytes(Byte) (Utilities|Enum|LiteralenumTCPProtocol "NewEnumerator82")) (Class|TcpSocketConnection|ToBytes(Integer) (Utilities|Array|Length (Class|TcpSocketConnection|ToBytes(String) (.username _user)))) (Class|TcpSocketConnection|ToBytes(String) (.username _user)) (Class|TcpSocketConnection|ToBytes(Integer) (Utilities|Array|Length _returnvalue_2)) _returnvalue_2 (Class|TcpSocketConnection|ToBytes(Integer) (Utilities|Array|Length _returnvalue)) _returnvalue (Class|TcpSocketConnection|ToBytes(Byte) Location)))))))

(event Custom|RemoveAvatarAtIndex
  (params (IndexAsiento :type Integer) (IndexSala :type Integer))
  (bind _reunionesmapa (Variables|Default|GetReunionesMapa))
  (bind _output (Utilities|Array|Get(acopy) _reunionesmapa IndexSala))
  (bind (_avatarstates _userinfos) (Utilities|Struct|BreakReunionMapa _output))
  ;[1 1 1] Enter / Exit Sala Reuniones Update Avatars
  (Utilities|Array|SetArrayElem _avatarstates IndexAsiento false)
  (Utilities|Array|SetArrayElem _userinfos IndexAsiento (Utilities|Struct|MakeUserInfo_Public)))

(event EventBeginPlay
  (CallFunction|InitAvataresReuniones))

(event EventOnServerConnected
  ;[1 1 1] Initialize Info
  (|CallParentFunction)
  (Utilities|FlowControl|Delay 1.0)
  (CallFunction|RetrieveAllRetos))

(fn ConstructionScript
  (|CallParentFunction))

(fn MakeRetoInfo
  (params (bytes :type Array%20of%20Bytes))
  (bind _returnvalue (Class|TcpSocketConnection|MessageReadInt bytes))
  (bind _returnvalue_2 (Class|TcpSocketConnection|MessageReadInt bytes))
  (bind _returnvalue_3 (Class|TcpSocketConnection|MessageReadString bytes _returnvalue_2))
  (bind _returnvalue_4 (Class|TcpSocketConnection|MessageReadInt bytes))
  (bind _returnvalue_5 (Class|TcpSocketConnection|MessageReadString bytes _returnvalue_4))
  (bind _returnvalue_6 (Class|TcpSocketConnection|MessageReadInt bytes))
  (bind (_stringlist _namelist _pendingbytes) (CallFunction|MakeStringList bytes _returnvalue_6))
  (LocalVariables|SetpendingBytesAux _pendingbytes)
  (Utilities|FlowControl|Sequence
    (:then_0
      (for _index (range 0 (- _returnvalue_6 1))
        (bind _returnvalue_7 (Class|TcpSocketConnection|MessageReadInt (LocalVariables|GetpendingBytesAux)))
        (bind (_stringlist_2 _namelist_2 _pendingbytes_2) (CallFunction|MakeStringList (LocalVariables|GetpendingBytesAux) _returnvalue_7))
        (LocalVariables|SetpendingBytesAux _pendingbytes_2)
        (Utilities|Array|Add (LocalVariables|GetEspectadoresXEmpresaAux) (Utilities|Struct|MakestringArray _stringlist_2))))
    (:then_1
      (for _index_2 (range 0 (- _returnvalue_6 1))
        (bind _returnvalue_8 (Class|TcpSocketConnection|MessageReadInt (LocalVariables|GetpendingBytesAux)))
        (bind (_stringlist_3 _namelist_3 _pendingbytes_3) (CallFunction|MakeStringList (LocalVariables|GetpendingBytesAux) _returnvalue_8))
        (LocalVariables|SetpendingBytesAux _pendingbytes_3)
        (Utilities|Array|Add (LocalVariables|GetParticipantesSinValidarXEmpresaAux) (Utilities|Struct|MakestringArray _stringlist_3))))
    (:then_2
      (for _index_3 (range 0 (- _returnvalue_6 1))
        (bind _returnvalue_9 (Class|TcpSocketConnection|MessageReadInt (LocalVariables|GetpendingBytesAux)))
        (bind (_stringlist_4 _namelist_4 _pendingbytes_4) (CallFunction|MakeStringList (LocalVariables|GetpendingBytesAux) _returnvalue_9))
        (LocalVariables|SetpendingBytesAux _pendingbytes_4)
        (Utilities|Array|Add (LocalVariables|GetParticipantesValidadosXEmpresaAux) (Utilities|Struct|MakestringArray _stringlist_4))))
    (:then_3
      (bind _returnvalue_10 (Class|TcpSocketConnection|MessageReadInt (LocalVariables|GetpendingBytesAux)))
      (for _index_4 (range 0 (- _returnvalue_10 1))
        (bind _returnvalue_11 (Class|TcpSocketConnection|MessageReadInt (LocalVariables|GetpendingBytesAux)))
        (bind (_stringlist_5 _namelist_5 _pendingbytes_5) (CallFunction|MakeStringList (LocalVariables|GetpendingBytesAux) _returnvalue_11))
        (bind _output_get (LocalVariables|SetpendingBytesAux _pendingbytes_5))
        (bind (_intlist _pendingbytes_6) (CallFunction|MakeIntList _output_get _returnvalue_11))
        (LocalVariables|SetpendingBytesAux _pendingbytes_6)
        (Utilities|Array|Add (LocalVariables|GetPorcentajesDeRequerimientosAux) (Utilities|Struct|MakeRequerimientoReto _namelist_5 _intlist "Req test"))))
    (:then_4
      (LocalVariables|SetAuxReto (Utilities|Struct|MakeRetoInfo (+ _returnvalue 1) _returnvalue_3 _returnvalue_5 "" _stringlist (LocalVariables|GetEspectadoresXEmpresaAux) (LocalVariables|GetParticipantesSinValidarXEmpresaAux) (LocalVariables|GetParticipantesValidadosXEmpresaAux) (LocalVariables|GetPorcentajesDeRequerimientosAux)))
      (return (LocalVariables|GetAuxReto) (LocalVariables|GetpendingBytesAux)))))

(fn MakeAvatarstoSit
  (params (bytes :type Array%20of%20Bytes))
  (bind _output_get (LocalVariables|SetPendingBytesAux bytes))
  (bind _returnvalue (Class|TcpSocketConnection|MessageReadInt _output_get))
  (bind _returnvalue_2 (Class|TcpSocketConnection|MessageReadInt _output_get))
  (Utilities|FlowControl|Sequence
    (:then_0
      (for _index (range 0 (- _returnvalue_2 1))
        (bind _returnvalue_3 (Class|TcpSocketConnection|MessageReadByte (LocalVariables|GetPendingBytesAux)))
        (bind _returnvalue_4 (Class|TcpSocketConnection|MessageReadByte (LocalVariables|GetPendingBytesAux)))
        (bind _returnvalue_5 (Class|TcpSocketConnection|MessageReadByte (LocalVariables|GetPendingBytesAux)))
        (bind _returnvalue_6 (Class|TcpSocketConnection|MessageReadByte (LocalVariables|GetPendingBytesAux)))
        (bind _returnvalue_7 (Class|TcpSocketConnection|MessageReadByte (LocalVariables|GetPendingBytesAux)))
        (bind _returnvalue_8 (Class|TcpSocketConnection|MessageReadByte (LocalVariables|GetPendingBytesAux)))
        (bind _returnvalue_9 (Class|TcpSocketConnection|MessageReadByte (LocalVariables|GetPendingBytesAux)))
        (bind _returnvalue_10 (Class|TcpSocketConnection|MessageReadByte (LocalVariables|GetPendingBytesAux)))
        (Utilities|Array|Add (LocalVariables|GetAvatarsToSitAux) (Utilities|Struct|MakeAvatar (Math|Conversions|ToBoolean(Integer) (Math|Conversions|ToInteger(Byte) _returnvalue_3)) _returnvalue_4 _returnvalue_5 _returnvalue_6 _returnvalue_8 _returnvalue_9 _returnvalue_10))))
    (:then_1
      (bind (_stringlist _namelist _pendingbytes) (CallFunction|MakeStringList (LocalVariables|GetPendingBytesAux) (- _returnvalue_2 1)))
      (LocalVariables|SetPendingBytesAux _pendingbytes)
      (for _array_element _stringlist
        (Utilities|FlowControl|FlipFlop
          (:A
            (Utilities|Array|Add (LocalVariables|GetnameListAux) _array_element))
          (:B
            (Utilities|Array|Add (LocalVariables|GetusernameListAux) _array_element)))))
    (:then_2
      (LocalVariables|SetRetoAvatarsAux (Utilities|Struct|MakeRetoAvatars _returnvalue (LocalVariables|GetAvatarsToSitAux) (LocalVariables|GetusernameListAux) (LocalVariables|GetnameListAux)))
      (return (LocalVariables|GetRetoAvatarsAux) (LocalVariables|GetPendingBytesAux)))))

(fn GetRetoInfo
  (params (RetoID :type Integer))
  (bind (_array_element _array_index) (Utilities|Array|ForEachLoopwithBreak (Variables|Default|GetRetoInfos))
    (:LoopBody
      (if (== (.SalaDeRetoID (Utilities|Struct|BreakRetoInfo _array_element)) RetoID)
        (LocalVariables|SetauxFound true)
        (LocalVariables|SetauxReto _array_element)))
    (:Completed
      (return (LocalVariables|GetauxFound) (LocalVariables|GetauxIndex) (LocalVariables|GetauxReto)))))

(fn GetRetoAvatars
  (params (RetoID :type Integer))
  (bind (_array_element _array_index) (Utilities|Array|ForEachLoopwithBreak (Variables|Default|GetRetoAvatars) :!label _label)
    (:LoopBody
      (if (== (.RetoID (Utilities|Struct|BreakRetoAvatars _array_element)) RetoID)
        (LocalVariables|SetfoundAux true)
        (LocalVariables|SetindexAux _array_index)
        (LocalVariables|SetRetoAvatarAux _array_element)
        (goto _label Break)))
    (:Completed
      (return (LocalVariables|GetfoundAux) (LocalVariables|GetindexAux) (LocalVariables|GetRetoAvatarAux)))))

(fn FillAllRetos
  (params (bytes :type Array%20of%20Bytes))
  (bind _output_get (LocalVariables|SetauxBytes bytes))
  (bind _returnvalue (Class|TcpSocketConnection|MessageReadInt _output_get))
  (for _index (range 0 (- _returnvalue 1))
    (bind (_reto _pendingbytes) (CallFunction|MakeRetoInfo (LocalVariables|GetauxBytes)))
    (LocalVariables|SetauxBytes _pendingbytes)
    (Utilities|Array|SetArrayElem (Variables|Default|GetRetoInfos) (- (Utilities|Struct|BreakRetoInfo _reto) 1) _reto true))
  (return (LocalVariables|GetauxBytes)))

(fn ReadBytetoString
  (params (Message :type Array%20of%20Bytes))
  (bind _returnvalue (Class|TcpSocketConnection|MessageReadInt Message))
  (bind _returnvalue_2 (Class|TcpSocketConnection|MessageReadString Message _returnvalue))
  (return _returnvalue_2))

(fn CheckifAsientosSalaAreFull
  (params (AsientosArr :type Array%20of%20Booleans))
  (for _array_element AsientosArr
    (if (not _array_element)
      (return false)))
  (return false))

(fn GetFirstIndexAvailable
  (params (AsientosArr :type Array%20of%20Booleans))
  (bind _salallena_ (CallFunction|CheckifAsientosSalaAreFull AsientosArr))
  (if _salallena_
    (return -1)
    (else
      (LocalVariables|SetMaxIdx (- (Utilities|Array|Length AsientosArr) 1))
      (LocalVariables|SetCurrIndx (Math|Random|RandomIntegerinRange 0 (LocalVariables|GetMaxIdx)))
      (while (Utilities|Array|Get(acopy) AsientosArr (LocalVariables|GetCurrIndx))
        (LocalVariables|SetCurrIndx (Math|Random|RandomIntegerinRange 0 (LocalVariables|GetMaxIdx))))
      (return (LocalVariables|GetCurrIndx)))))

(fn FindAsientoandSalaIdxbyUsername
  (params (Username :type String) (Reuniones :type Array%20of%20Reunion%20Mapa%20Structures))
  (for (_array_element _array_index) Reuniones
    (for (_array_element_2 _array_index_2) (Utilities|Struct|BreakReunionMapa _array_element)
      (if (Utilities|Enum|Equal(Enum) (.Username (Utilities|Struct|BreakUserInfo_Public _array_element_2)) Username)
        (return _array_index_2 _array_index))))
  (return -1 -1))