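; Clickable market actor in Secpholand that opens a marketplace screen of listings (Anuncios).
; One second after BeginPlay it calls RetrieveOfertasMarketsServer on the SecpholandCentralGameState to request market offers.
; On click it runs the parent logic, resets the click and adds a new Marketplace2 widget to the viewport.
; After a short retriggerable delay, it fills that widget from its Anuncios data.
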(event Collision|EventActorBeginOverlap
  (params (OtherActor :type Actor%20Object%20Reference)))

(event EventTick
  (params (DeltaSeconds :type Float%20%28single-precision%29)))

(event EventClick
  (params (controller :type Client%20Side%20Controller%20Object%20Reference))
  (|CallParentFunction controller)
  (CallFunction|ResetClick)
  (bind _returnvalue (UserInterface|CreateWidget "/Game/Secpholand/UI/Widgets/OficinaInfo/Marketplace2.Marketplace2_C"))
  (UserInterface|Viewport|AddtoViewport _returnvalue 0)
  (Utilities|FlowControl|RetriggerableDelay 0.3)
  (Default|FillAnuncios _returnvalue (Variables|Default|GetAnuncios)))

(event EventBeginPlay
  (|CallParentFunction)
  (Utilities|FlowControl|Delay 1.0)
  (Default|RetrieveOfertasMarkets:Server (.AsSecpholand%20Central%20Game%20State (Utilities|Casting|CastToSecpholandCentralGameState (Game|GetGameState)))))

(fn ConstructionScript
  (|CallParentFunction))