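; Clickable auditorium elevator that controls player access to a destination room.
; On click it clears its outline, then has the InteriorController either grant access directly when always open or request event access while the hover widget shows a loading throbber.
; A blocked response shows an access-denied title and error message on the hover widget, while an allowed response resets the click.
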(event Custom|ReceiveElevatorBlocked
  (params (MensajeError :type String))
  (bind _hoveruserwidget (Variables|Default|GethoverUserWidget))
  (bind _hoveruserwidget_2 (Variables|Default|GethoverUserWidget))
  (Utilities|IsValid _hoveruserwidget_2
    (:Is%20Valid
      (Default|ChangeState _hoveruserwidget_2 "" false)
      (Default|FillHoverInfo _hoveruserwidget "Acceso no permitido" (Utilities|Text|ToText(String) MensajeError))
      (Default|Blocked _hoveruserwidget))))

(event Custom|ReceiveCanEnterElevator
  (CallFunction|ResetClick))

(event EventBeginPlay
  (|CallParentFunction))

(event EventClick
  (params (controller :type Client%20Side%20Controller%20Object%20Reference))
  (bind _hoveruserwidget (Variables|Default|GethoverUserWidget))
  (Default|StopOutliningActor controller self)
  (bind _asinterior_controller (Utilities|Casting|CastToInteriorController controller))
  (if (Variables|Default|GetSiempreAbierto)
    (Default|ElevatorAccessAllowed:Client _asinterior_controller (Variables|Default|GetIDSalaDestinacion))
    (else
      (Default|AccesstoEvent:Client _asinterior_controller "NewEnumerator6")
      (Utilities|IsValid _hoveruserwidget
        (:Is%20Valid
          (Default|ChangeState _hoveruserwidget (Utilities|Text|ToText(String) (Utilities|String|ToString(Text) (Variables|Default|GethoverActiveHint))) true))))))

(fn ConstructionScript
  (|CallParentFunction))