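; Hall counter clickable in Secpholand that feeds a list of projects to a Proyectos widget when clicked.
; One second after BeginPlay it calls the MeetingCenterGameState server request for the projects-per-enterprise list.
; A click runs the parent clickable logic, waits on a short retriggerable delay, passes ListProyectos to the widget's FillPlayers if that widget is valid, then resets the click.
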(event EventClick
  (params (controller :type Client%20Side%20Controller%20Object%20Reference))
  (bind _ref_wb (Variables|Default|GetRef_WB))
  (|CallParentFunction controller)
  (Utilities|FlowControl|RetriggerableDelay 0.2)
  (Utilities|IsValid _ref_wb
    (:Is%20Valid
      (Default|FillPlayers (.AsProyectos (Utilities|Casting|CastToProyectos _ref_wb)) (Variables|Default|GetList%20Proyectos)))
    (:Is%20Not%20Valid
      _))
  (CallFunction|ResetClick))

(event Collision|EventActorBeginOverlap
  (params (OtherActor :type Actor%20Object%20Reference)))

(event EventTick
  (params (DeltaSeconds :type Float%20%28single-precision%29)))

(event EventBeginPlay
  (|CallParentFunction)
  (Utilities|FlowControl|Delay 1.0)
  (Default|RetrieveProjectsXenterpriseList:Server (.AsMeeting%20Center%20Game%20State (Utilities|Casting|CastToMeetingCenterGameState (Game|GetGameState)))))

(fn ConstructionScript
  (|CallParentFunction))