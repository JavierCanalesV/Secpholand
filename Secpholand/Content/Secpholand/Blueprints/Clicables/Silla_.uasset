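; Clickable chair that sends the local player's character to walk over and sit, unless it is occupied (Ocupada).
; A click from bird's-eye view first turns the camera toward the chair, switches to street view and waits a distance-scaled delay.
; If out of range, it moves the player to Box, whose overlap triggers SitPlayerClient with the chair's yaw.
; Box1 overlaps track occupancy and disable mesh collision while taken.
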(event OnComponentEndOverlap(Box1)
  (params (OverlappedComponent :type Primitive%20Component%20Object%20Reference) (OtherActor :type Actor%20Object%20Reference) (OtherComp :type Primitive%20Component%20Object%20Reference) (OtherBodyIndex :type Integer))
  (Utilities|Casting|CastToServerSide_Character OtherActor)
  (Utilities|FlowControl|Delay 0.2)
  (if (> (Utilities|Array|Length (Collision|GetOverlappingActors (Variables|Default|GetBox1) "/Game/Secpholand/Blueprints/ControllersYModes/baseClasses/ServerSide_Character.ServerSide_Character_C" :!class /Script/Engine.PrimitiveComponent)) 0)
    (Collision|SetCollisionEnabled (Variables|Default|GetStaticMesh) "NoCollision")
    (Variables|Default|Setocupada true)
    (else
      (Collision|SetCollisionEnabled (Variables|Default|GetStaticMesh) "QueryOnly")
      (Variables|Default|Setocupada false))))

(event OnComponentBeginOverlap(Box)
  (params (OverlappedComponent :type Primitive%20Component%20Object%20Reference) (OtherActor :type Actor%20Object%20Reference) (OtherComp :type Primitive%20Component%20Object%20Reference) (OtherBodyIndex :type Integer) (bFromSweep :type Boolean) (SweepResult :type Hit%20Result%20Structure%20%28by%20ref%29))
  (if (Variables|Default|Getactive)
    (if (== "/Script/Engine.CapsuleComponent" (Utilities|GetClass OtherComp))
      (bind _asserver_side_character (Utilities|Casting|CastToServerSide_Character OtherActor))
      (bind _asclient_side_controller (Utilities|Casting|CastToClientSide_Controller (Game|GetPlayerController 0)))
      (if (== _asserver_side_character (Variables|/Game/Secpholand/Blueprints/ControllersYModes/baseClasses/ClientSide_Controller.ClientSide_Controller_C|GetServerSideCharacterRef _asclient_side_controller))
        (if (not (Variables|Default|Getocupada))
          (Utilities|FlowControl|Delay 0.5)
          (Default|SitPlayer:Client _asclient_side_controller (Variables|Default|Getrotation)))))))

(event OnComponentBeginOverlap(Box1)
  (params (OverlappedComponent :type Primitive%20Component%20Object%20Reference) (OtherActor :type Actor%20Object%20Reference) (OtherComp :type Primitive%20Component%20Object%20Reference) (OtherBodyIndex :type Integer) (bFromSweep :type Boolean) (SweepResult :type Hit%20Result%20Structure%20%28by%20ref%29))
  (Utilities|Casting|CastToServerSide_Character OtherActor)
  (Collision|SetCollisionEnabled (Variables|Default|GetStaticMesh) "NoCollision")
  (Variables|Default|Setocupada true))

(event EventBeginPlay
  (Variables|Default|Setrotation (.yaw (Transformation|GetWorldRotation (Variables|Default|GetStaticMesh)))))

(event EventClick
  (params (controller :type Client%20Side%20Controller%20Object%20Reference))
  (bind _clientsidepawnref (Variables|/Game/Secpholand/Blueprints/ControllersYModes/baseClasses/ClientSide_Controller.ClientSide_Controller_C|GetClientSidePawnRef controller))
  (bind _box (Variables|Components|GetBox))
  (bind _box_2 (Variables|Components|GetBox))
  (bind _clientsidepawnref_2 (Variables|/Game/Secpholand/Blueprints/ControllersYModes/baseClasses/ClientSide_Controller.ClientSide_Controller_C|GetClientSidePawnRef controller))
  (bind _returnvalue (Transformation|GetWorldLocation _box))
  (bind _returnvalue_2 (Transformation|GetActorLocation _clientsidepawnref_2))
  (bind _returnvalue_3 (Transformation|GetWorldLocation _box_2))
  (bind _springarm (Variables|/Game/Secpholand/Blueprints/ControllersYModes/baseClasses/ClientSide_Pawn.ClientSide_Pawn_C|GetSpringArm _clientsidepawnref_2))
  (if (not (Variables|Default|Getocupada))
    (|CallParentFunction controller)
    (if (Variables|/Game/Secpholand/Blueprints/ControllersYModes/baseClasses/ClientSide_Pawn.ClientSide_Pawn_C|Getb_VistaPajaro _clientsidepawnref)
      (Transformation|SetWorldRotation _springarm (Math|Rotator|MakeRotator 0.0 (.pitch (Transformation|GetWorldRotation _springarm)) (.yaw (Math|Rotator|FindLookatRotation _returnvalue_2 _returnvalue))) false false)
      (bind _foundwidgets (Widget|GetAllWidgetsOfClass "/Game/Secpholand/UI/Widgets/HUDYChat/Minimapa/BotonVistaPajaro.BotonVistaPajaro_C" true))
      (Default|ClicarVistaCalle (Utilities|Array|Get(acopy) _foundwidgets))
      (Utilities|FlowControl|Delay (* (Math|Float|Clamp(Float) (- 1.0 (/ (Math|Vector|Distance(Vector) _returnvalue _returnvalue_2) (* (Class|MovementComponent|GetMaxSpeed (Variables|/Script/Engine.Character|GetCharacterMovement (Variables|/Game/Secpholand/Blueprints/ControllersYModes/baseClasses/ClientSide_Controller.ClientSide_Controller_C|GetServerSideCharacterRef controller))) 2.5)))) 2.5)))
    (if (not (<= (Math|Vector|Distance(Vector) (Transformation|GetActorLocation _clientsidepawnref) (Transformation|GetWorldLocation (Variables|Components|GetBox))) (+ (.x (Variables|Default|GetBoxOverlapExtent)) 8e+01)))
      (Variables|Default|Setactive true)
      (Default|SpawnDecalatLocation controller _returnvalue_3)
      (Default|MovetoLocation controller _returnvalue_3))))

(event EventResetClick
  (|CallParentFunction)
  (Variables|Default|Setactive false))

(fn ConstructionScript
  (bind _gotopoint (Variables|Default|GetGotoPoint))
  (Transformation|SetRelativeLocation (Variables|Components|GetBox) (Math|Vector|MakeVector (.x _gotopoint) (.y _gotopoint) (.z _gotopoint)) false false)
  (Components|Box|SetBoxExtent (Variables|Components|GetBox) (Variables|Default|GetBoxOverlapExtent) true)
  (|CallParentFunction))