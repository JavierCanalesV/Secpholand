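; Clickable counter for an outdoor exhibitor stand in Secpholand, shown with the outdoor stand table mesh.
; Init receives a company name, stores it as Empresa and builds the hover title "Mostrador de" plus that name, then resets the click state.
; The construction script assigns the table mesh, and BeginPlay only calls the parent.
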(event Custom|Init
  (params (NombreEmpresa :type String))
  (bind _output_get (Variables|Default|Setempresa (Utilities|String|StringToName NombreEmpresa)))
  (Variables|Default|SethoverTitle (Utilities|Text|ToText(String) (Utilities|String|Append "Mostrador de " (Utilities|String|ToString(Name) _output_get))))
  (CallFunction|ResetClick))

(event EventBeginPlay
  (|CallParentFunction))

(fn ConstructionScript
  (Components|StaticMesh|SetStaticMesh (Variables|Default|GetStaticMesh) "/Game/Secpholand/Assets/meshes/Secpholand_Island/SM_OutdoorStandTable.SM_OutdoorStandTable"))