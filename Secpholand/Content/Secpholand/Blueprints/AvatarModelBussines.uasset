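; Business avatar model actor that animates a face zoom and a return to its profile pose.
; The ZoomCara timeline offsets the actor's relative location from its captured start and blends the Scene component's yaw toward a close-up angle.
; Zooming out reverses that timeline, blending from the current yaw back to zero.
; The profile-return event, when zoomed, stops the timeline and resets rotation, leaving location untouched.
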(event Custom|ZoomearCara
  (Variables|Default|SetZoomed true)
  (Variables|Default|SetOriginalLoc (Transformation|GetActorLocation))
  (Variables|Default|SetoriginalRot (.yaw (Variables|/Script/Engine.SceneComponent|GetRelativeRotation (Variables|Default|GetScene))))
  (Variables|Default|SetZoomedRot 3.4e+02)
  (bind (_direction _newtrack_0 _rot) (Timeline|ZoomCara PlayFromStart)
    (:Update
      (Transformation|SetActorRelativeLocation (Math|Vector|Lerp(Vector) (Variables|Default|GetOriginalLoc) (+ (Variables|Default|GetOriginalLoc) "-60.000000,65.000000,135.000000") _newtrack_0))
      (Transformation|SetRelativeRotation (Variables|Default|GetScene) (Math|Rotator|MakeRotator 0.0 0.0 (+ (* _rot (- (Variables|Default|GetZoomedRot) (Variables|Default|GetoriginalRot))) (Variables|Default|GetoriginalRot))) false false))))

(event Custom|ZoomOutCara
  (bind _originalloc (Variables|Default|GetOriginalLoc))
  (Variables|Default|SetoriginalRot 0.0)
  (Variables|Default|SetZoomedRot (.yaw (Variables|/Script/Engine.SceneComponent|GetRelativeRotation (Variables|Default|GetScene))))
  (bind (_direction _newtrack_0 _rot) (Timeline|ZoomCara ReverseFromEnd)
    (:Update
      (Transformation|SetActorRelativeLocation (Math|Vector|Lerp(Vector) _originalloc (+ _originalloc "-60.000000,65.000000,135.000000") _newtrack_0))
      (Transformation|SetRelativeRotation (Variables|Default|GetScene) (Math|Rotator|MakeRotator 0.0 0.0 (+ (* _rot (- (Variables|Default|GetZoomedRot) (Variables|Default|GetoriginalRot))) (Variables|Default|GetoriginalRot))) false false))))

(event Custom|ReturnToP^rofilePos
  (if (Variables|Default|GetZoomed)
    (CallFunction|StopRotation)
    (Variables|Default|SetZoomed false)
    (Transformation|SetRelativeRotation (Variables|Default|GetScene) (Math|Rotator|MakeRotator 0.0 0.0 0.0) false false)
    (Variables|Default|SetoriginalRot 0.0)
    (Variables|Default|SetZoomedRot 3.4e+02)))

(event Custom|StopRotation
  (bind _originalloc (Variables|Default|GetOriginalLoc))
  (bind _originalrot (Variables|Default|GetoriginalRot))
  (bind (_direction _newtrack_0 _rot) (Timeline|ZoomCara Stop)
    (:Update
      (Transformation|SetActorRelativeLocation (Math|Vector|Lerp(Vector) _originalloc (+ _originalloc "-60.000000,65.000000,135.000000") _newtrack_0))
      (Transformation|SetRelativeRotation (Variables|Default|GetScene) (Math|Rotator|MakeRotator 0.0 0.0 (+ (* _rot (- (Variables|Default|GetZoomedRot) _originalrot)) _originalrot)) false false))))

(fn ConstructionScript)